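; Actor wrapper around a Hierarchical Instanced Static Mesh component, with a utility to split its instances into individual static mesh actors.
; The construction script rolls a non-zero RandomSeed when unset and assigns it as the component's instancing random seed.
; SplitInstances spawns a StaticMeshActor at each instance's world transform, copying the mesh and materials, and leaves the original instances in place.
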(event Custom|SplitInstances
  (bind _hierarchicalinstancedstaticmesh (Variables|Default|GetHierarchicalInstancedStaticMesh))
  (for _index (range 0 (- (Components|InstancedStaticMesh|GetInstanceCount _hierarchicalinstancedstaticmesh) 1))
    (bind _returnvalue (Game|SpawnActorfromClass "/Script/Engine.StaticMeshActor" (.OutInstanceTransform (Components|InstancedStaticMesh|GetInstanceTransform _hierarchicalinstancedstaticmesh _index true)) "Undefined" 0 0))
    (Components|StaticMesh|SetStaticMesh (Variables|/Script/Engine.StaticMeshActor|GetStaticMeshComponent _returnvalue) (Variables|/Script/Engine.StaticMeshComponent|GetStaticMesh _hierarchicalinstancedstaticmesh))
    (for _index_2 (range 0 (- (Rendering|Material|GetNumMaterials _hierarchicalinstancedstaticmesh) 1))
      (Rendering|Material|SetMaterial (Variables|/Script/Engine.StaticMeshActor|GetStaticMeshComponent _returnvalue) _index_2 (Rendering|Material|GetMaterial _hierarchicalinstancedstaticmesh _index_2)))))

(event EventBeginPlay)

(event Collision|EventActorBeginOverlap
  (params (OtherActor :type Actor%20Object%20Reference)))

(event EventTick
  (params (DeltaSeconds :type Float%20%28single-precision%29)))

(fn ConstructionScript
  (while (== (Variables|Default|GetRandomSeed) 0)
    (Variables|Default|SetRandomSeed (Math|Random|RandomInteger 1562067968)))
  (Variables|/Script/Engine.InstancedStaticMeshComponent|SetInstancingRandomSeed (Variables|Default|GetHierarchicalInstancedStaticMesh) (Variables|Default|GetRandomSeed)))