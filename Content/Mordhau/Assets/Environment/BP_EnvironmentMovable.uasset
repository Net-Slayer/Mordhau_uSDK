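; Environment actor base that sways its SwayHolder component in rotation, configured per axis for roll, pitch and yaw.
; On BeginPlay it packs the frequency, magnitude and speed variables into three vectors and passes them with SwayHolder to InitializeMovable.
; The graph holds no motion logic of its own, and the construction script is empty.
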(event EventBeginPlay
  (Class|EnvironmentMovable|InitializeMovable (Variables|Default|GetSwayHolder) (Math|Vector|MakeVector (Variables|Sway|GetRoll%20Frequency) (Variables|Sway|GetPitch%20Frequency) (Variables|Sway|GetJaw%20Frequency)) (Math|Vector|MakeVector (Variables|Sway|GetRoll%20Magnitude) (Variables|Sway|GetPitch%20Magnitude) (Variables|Sway|GetJaw%20Magnitude)) (Math|Vector|MakeVector (Variables|ConstantRotation|GetRoll%20Speed) (Variables|ConstantRotation|GetPitch%20Speed) (Variables|ConstantRotation|GetJaw%20Speed))))

(fn ConstructionScript)