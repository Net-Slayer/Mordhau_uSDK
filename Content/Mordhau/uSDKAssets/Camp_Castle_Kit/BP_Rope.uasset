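; BP_Rope is a construction-script rope actor from the castle camp kit, shaped along an editable spline.
; A RopeType choice of short, medium or long selects the rope mesh.
; The script adds one collision-enabled spline mesh per pair of adjacent points, bending each with the points' local positions and tangents and storing it in Segments.
; The event graph has no active logic.
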(event EventBeginPlay
  (|CallParentFunction) ; This node is disabled and will not be called.\nDrag off pins to build functionality.
)

(event Collision|EventActorBeginOverlap
  (params (OtherActor :type Actor%20Object%20Reference)))

(event EventTick
  (params (DeltaSeconds :type Float%20%28single-precision%29))
  (|CallParentFunction DeltaSeconds) ; This node is disabled and will not be called.\nDrag off pins to build functionality.
)

(fn ConstructionScript
  (bind _spline (Variables|Default|GetSpline))
  (|CallParentFunction)
  (Spline|SetSplinePointType (Variables|Default|GetSpline) 0 "Curve" true)
  (Variables|Default|SetSegments (Utilities|Array|MakeArray 0))
  (switch Utilities|FlowControl|Switch|SwitchonERopes (Variables|Default|GetRopeType)
    (:NewEnumerator0
      (Variables|Default|SetStaticmesh "/Game/Mordhau/uSDKAssets/Camp_Castle_Kit/Rope_S4.Rope_S4"))
    (:NewEnumerator1
      (Variables|Default|SetStaticmesh "/Game/Mordhau/uSDKAssets/Camp_Castle_Kit/Rope_M4.Rope_M4"))
    (:NewEnumerator2
      (Variables|Default|SetStaticmesh "/Game/Mordhau/uSDKAssets/Camp_Castle_Kit/Rope_L4.Rope_L4")))
  (for _index (range 0 (- (Spline|GetNumberOfSplinePoints (Variables|Default|GetSpline)) 2))
    (bind _returnvalue (AddComponent|AddSplineMeshComponent false))
    (Components|StaticMesh|SetStaticMesh _returnvalue (Variables|Default|Getstaticmesh))
    (SplineMesh|SetForwardAxis _returnvalue (Variables|Default|GetForwardAxis) true)
    (Utilities|Array|AddUnique (Variables|Default|GetSegments) _returnvalue)
    (Transformation|AttachComponentToComponent _returnvalue 0 "None" "KeepRelative" "KeepRelative" "KeepRelative" true)
    (SplineMesh|SetStartandEnd _returnvalue (Spline|GetLocationatSplinePoint _spline _index "Local") (Spline|GetTangentatSplinePoint _spline _index "Local") (Spline|GetLocationatSplinePoint _spline (+ _index 1) "Local") (Spline|GetTangentatSplinePoint _spline (+ _index 1) "Local") true :!class /Script/Engine.SplineMeshComponent)
    (Collision|SetCollisionEnabled _returnvalue "QueryAndPhysics")))