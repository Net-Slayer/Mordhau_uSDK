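; Configurable castle tower from the camp castle kit, with selectable tower body, topper and optional mortar.
; The construction script adds the body mesh for TowerType, plus a TopperType mesh that matches the round or square shape.
; On BeginPlay, square toppers spawn an 8m ladder at LadderSpawnPoint.
; With Mortar enabled, round and square towers spawn a mortar spawner at MortarSpawnPoint, raised for square variants.
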(event EventBeginPlay
  (bind _mortarspawnpoint (Variables|Default|GetMortarSpawnPoint))
  (bind _returnvalue (Transformation|GetWorldTransform _mortarspawnpoint))
  (bind (_location _rotation _scale) (Math|Transform|BreakTransform _returnvalue))
  (switch Utilities|FlowControl|Switch|SwitchonETowerToppers (Variables|Default|GetTopper%20Type)
    (:NewEnumerator0
      _)
    (:NewEnumerator1
      _)
    (:NewEnumerator2
      _)
    (:NewEnumerator3
      (Game|SpawnActorfromClass "/Game/Mordhau/Blueprints/Interactables/SiegeEngines/BP_Ladder_8m.BP_Ladder_8m_C" (Transformation|GetWorldTransform (Variables|Default|GetLadderSpawnPoint)) "Undefined" 0 0 :!label _label))
    (:NewEnumerator4
      (goto _label)))
  (if (Variables|Default|GetMortar?)
    (switch Utilities|FlowControl|Switch|SwitchonETowers (Variables|Default|GetTower%20Type)
      (:NewEnumerator1
        (Game|SpawnActorfromClass "/Game/Mordhau/Blueprints/Interactables/SiegeEngines/BP_MortarSpawner.BP_MortarSpawner_C" _returnvalue "Undefined" 0 0))
      (:NewEnumerator2
        (Game|SpawnActorfromClass "/Game/Mordhau/Blueprints/Interactables/SiegeEngines/BP_MortarSpawner.BP_MortarSpawner_C" (Math|Transform|MakeTransform (+ _location "0,0.000000,150.000000") _rotation _scale) "Undefined" 0 0 :!label _label_2))
      (:NewEnumerator3
        (goto _label_2)))))

(fn ConstructionScript
  (bind _topper_type (Variables|Default|GetTopper%20Type))
  (switch Utilities|FlowControl|Switch|SwitchonETowers (Variables|Default|GetTower%20Type)
    (:NewEnumerator0
      (AddComponent|AddStaticMeshComponent false))
    (:NewEnumerator1
      (AddComponent|AddStaticMeshComponent false)
      (switch Utilities|FlowControl|Switch|SwitchonETowerToppers _topper_type
        (:NewEnumerator1
          (AddComponent|AddStaticMeshComponent false))
        (:NewEnumerator2
          (AddComponent|AddStaticMeshComponent false))))
    (:NewEnumerator2
      (AddComponent|AddStaticMeshComponent false)
      (switch Utilities|FlowControl|Switch|SwitchonETowerToppers _topper_type :!label _label
        (:NewEnumerator3
          (AddComponent|AddStaticMeshComponent false))
        (:NewEnumerator4
          (AddComponent|AddStaticMeshComponent false))))
    (:NewEnumerator3
      (AddComponent|AddStaticMeshComponent false)
      (goto _label))))