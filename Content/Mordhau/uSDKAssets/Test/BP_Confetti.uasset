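; BP_Confetti is an interactable confetti trigger with an animated lever.
; Interaction calls ServerConfetti, which passes to MCConfetti, named as a server-to-multicast relay.
; MCConfetti fires every emitter in ConfettiEmitters, plays explosion and party horn sounds in 2D, and animates the lever.
; Interaction is disabled during a short delay, then the lever animation replays at negative rate and interaction is re-enabled.
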(event Custom|MCConfetti
  (bind _skeletalmesh (Variables|Default|GetSkeletalMesh))
  (bind _skeletalmesh_2 (Variables|Default|GetSkeletalMesh))
  (for _array_element (Variables|Default|GetConfettiEmitters)
    (Default|SpawnConfetti _array_element))
  (Audio|PlaySound2D "/Game/Mordhau/Audio/Raw/Projectiles/Catapult/Explosion.Explosion" 1.0 1.0 0.0 0 0)
  (Audio|PlaySound2D "/Game/Mordhau/uSDKAssets/Test/party-horn-sound-effect.party-horn-sound-effect" 1.0 1.0 0.0 0 0)
  (Components|Timeline|SetPlayRate _skeletalmesh_2 1.0)
  (Components|Animation|PlayAnimation _skeletalmesh_2 "/Game/Mordhau/Assets/Interactables/Mesh/AlternateCranks/LeverAnimation.LeverAnimation" false)
  (Variables|Default|SetbIsInteractable false)
  (Utilities|FlowControl|Delay 3.0)
  (Components|Timeline|SetPlayRate _skeletalmesh -1.0)
  (Components|Animation|PlayAnimation _skeletalmesh "/Game/Mordhau/Assets/Interactables/Mesh/AlternateCranks/LeverAnimation.LeverAnimation" false)
  (Variables|Default|SetbIsInteractable true))

(event Custom|ServerConfetti
  (CallFunction|MCConfetti))

(event EventBeginPlay
  (|CallParentFunction) ; This node is disabled and will not be called.\nDrag off pins to build functionality.
)

(event Collision|EventActorBeginOverlap
  (params (OtherActor :type Actor%20Object%20Reference))
  (|CallParentFunction OtherActor) ; This node is disabled and will not be called.\nDrag off pins to build functionality.
)

(event EventTick
  (params (DeltaSeconds :type Float%20%28single-precision%29))
  (|CallParentFunction DeltaSeconds) ; This node is disabled and will not be called.\nDrag off pins to build functionality.
)

(event EventOnInteractionStart
  (params (Character :type Mordhau%20Character%20Object%20Reference))
  (CallFunction|ServerConfetti))

(fn ConstructionScript
  (|CallParentFunction))