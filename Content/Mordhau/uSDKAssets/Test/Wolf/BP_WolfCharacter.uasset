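; Test wolf character for Mordhau that roams the navmesh and can be toggled to follow a player.
; It moves to random nearby points with random pauses, looping on success or failure until following starts.
; Interaction flip-flops between following and roaming through WolfController.
; It also handles movement, look and jump input, and on death ragdolls, plays a sound at world origin and disables capsule collision.
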(event Custom|MoveToRandom
  ;[1 1 1] Roam
  (if (not (Variables|Default|GetFollowing))
    (AI|AIMoveTo self (.RandomLocation (Class|NavigationSystemV1|GetRandomPointinNavigableRadius (Transformation|GetActorLocation) 9.5e+02 0 0)) 0 5.0 false
      (:OnSuccess
        _)
      (:OnFail
        _))
    (Utilities|FlowControl|Delay (Math|Random|RandomFloatinRange 0.5 6.0))
    (CallFunction|MovetoRandom)))

(event EventBeginPlay
  (CallFunction|MovetoRandom))

(event EventOnKilled
  (params (EventInstigator :type Controller%20Object%20Reference))
  (Class|AdvancedCharacter|StartRagdoll)
  (Audio|PlaySoundatLocation "/Game/Mordhau/uSDKAssets/Test/Wolf/wolf5.wolf5" "0, 0, 0" "0, 0, 0" 1.0 1.0 0.0 0 0 0)
  (Collision|SetCollisionEnabled (Variables|Default|GetCapsule) "NoCollision"))

(event EventOnInteractionStart
  (params (Character :type Advanced%20Character%20Object%20Reference))
  (bind _returnvalue (Pawn|GetController))
  (Utilities|FlowControl|FlipFlop
    (:A
      (bind _aswolf_controller (Utilities|Casting|CastToWolfController _returnvalue))
      (bind _asbp_mordhau_character (Utilities|Casting|CastToBP_MordhauCharacter Character))
      (Default|Follow _aswolf_controller _asbp_mordhau_character)
      (Variables|Default|SetFollowing true))
    (:B
      (bind _aswolf_controller_2 (Utilities|Casting|CastToWolfController _returnvalue))
      (Default|StopFollowing _aswolf_controller_2)
      (Variables|Default|SetFollowing false)
      (Utilities|FlowControl|Delay (Math|Random|RandomFloatinRange 0.5 6.0))
      (CallFunction|MovetoRandom))))

(event Input|AxisEvents|InputAxisTurn
  (params (AxisValue :type Float%20%28single-precision%29))
  ;[1 1 1] Placeheld By TheMattman
  (Pawn|Input|AddControllerYawInput (Pawn|GetControlledPawn (Pawn|GetController)) AxisValue))

(event Input|AxisEvents|InputAxisMoveRight
  (params (AxisValue :type Float%20%28single-precision%29))
  (bind _returnvalue (Pawn|GetControlRotation :!class /Script/Engine.Pawn))
  (bind (_roll _pitch _yaw) (Math|Rotator|BreakRotator _returnvalue))
  ;[1 1 1] Placeheld By TheMattman
  (Pawn|Input|AddMovementInput (Math|Vector|GetRightVector (Math|Rotator|MakeRotator 0.0 _pitch _yaw)) AxisValue false))

(event Input|AxisEvents|InputAxisMoveForward
  (params (AxisValue :type Float%20%28single-precision%29))
  (bind _returnvalue (Pawn|GetControlRotation :!class /Script/Engine.Pawn))
  (bind (_roll _pitch _yaw) (Math|Rotator|BreakRotator _returnvalue))
  ;[1 1 1] Placeheld By TheMattman
  (Pawn|Input|AddMovementInput (Math|Vector|GetForwardVector (Math|Rotator|MakeRotator 0.0 _pitch _yaw)) AxisValue false))

(event Input|AxisEvents|InputAxisLookUp
  (params (AxisValue :type Float%20%28single-precision%29))
  ;[1 1 1] Placeheld By TheMattman
  (Pawn|Input|AddControllerPitchInput (Pawn|GetControlledPawn (Pawn|GetController)) AxisValue))

(event Input|KeyboardEvents|SpaceBar
  (params (Key :type Key%20Structure))
  ;[1 1 1] Placeheld By TheMattman
  (:Pressed
    (Character|Jump)))

(fn ConstructionScript
  (|CallParentFunction))