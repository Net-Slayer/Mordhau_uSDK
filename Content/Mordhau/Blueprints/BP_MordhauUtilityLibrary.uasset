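; Blueprint function library of shared helpers for Mordhau's UI and gameplay code.
; UI helpers cover combo boxes, dialog and context popup creation, unlock tooltips, rank and MMR lookups, team colors and key prompt icons that follow controller use.
; Others validate profile names, map a combined default/custom profile index to loadouts, resolve player states through vehicles and open Steam profiles.
; ComputeRagdollForce derives impulses from weapon, kick, projectile or actor agents and damage type.
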(fn GetLastComboBoxOption
  (params (ComboBox :type Combo%20Box%20Text%20Object%20Reference))
  (if (> (stale _returnvalue) 0)
    (return (stale _returnvalue))
    (else
      (return (Class|KismetTextLibrary|GetEmptyText)))))

(fn SelectLastComboBoxOption
  (params (ComboBox :type Combo%20Box%20Text%20Object%20Reference))
  (if (> (stale _returnvalue) 0)
    (bind _returnvalue (Class|ComboBoxText|GetOptionatIndex ComboBox (- (stale _returnvalue) 1)))
    (Class|ComboBoxText|SetSelectedOption ComboBox _returnvalue)))

(fn IsFirstOptionSelected
  (params (ComboBox :type Combo%20Box%20Text%20Object%20Reference))
  (return (== (stale _returnvalue) 0)))

(fn IsProfileNameValid
  (params (ProfiletName :type Text))
  (bind _array_element (Utilities|Array|ForEachLoopwithBreak (Variables|/Script/Mordhau.MordhauSingleton|GetCharacterProfiles (Class|MordhauUtilityLibrary|GetMordhauSingleton)))
    (:LoopBody
      (if (Utilities|Enum|Equal(Enum) (.Name (Utilities|Struct|BreakCharacterProfile _array_element)) ProfiletName)
        (return false)))
    (:Completed
      (return (not (Utilities|Text|TextIsEmpty ProfiletName))))))

(fn SelectFirstComboBoxOption
  (params (ComboBox :type Combo%20Box%20Text%20Object%20Reference))
  (bind _returnvalue (Class|ComboBoxText|GetOptionatIndex ComboBox))
  (Class|ComboBoxText|SetSelectedOption ComboBox _returnvalue))

(fn GetSelectedIndex
  (params (ComboBox :type Combo%20Box%20Text%20Object%20Reference))
  (return (stale _returnvalue)))

(fn ComputeRagdollForce
  (params (Agent :type Actor%20Object%20Reference) (DamageType :type Byte) (DamageSubType :type Byte) (RandomByte :type Byte) (Receiver :type Actor%20Object%20Reference))
  (bind _returnvalue (Transformation|GetActorLocation Agent))
  (bind _returnvalue_2 (Transformation|GetActorLocation Receiver))
  (bind _returnvalue_3 (Utilities|Enum|LiteralenumEMordhauDamageType "Melee"))
  (bind _returnvalue_4 (Math|Vector|GetUnitDirection(Vector) _returnvalue _returnvalue_2))
  (bind _returnvalue_5 (== DamageType _returnvalue_3))
  (Utilities|IsValid Agent
    (:Is%20Valid
      (Utilities|IsValid Receiver
        (:Is%20Valid
          (bind _asmordhau_weapon (Utilities|Casting|CastToMordhauWeapon Agent)
            (:then
              (bind _askick_weapon (Utilities|Casting|CastToKickWeapon _asmordhau_weapon)
                (:then
                  (bind _output_get (LocalVariables|SetForceDir (- (Transformation|GetSocketLocation (Variables|/Script/Engine.Character|GetMesh (Class|MordhauEquipment|GetParentCharacter _askick_weapon)) "KickTracerEnd") (Transformation|GetSocketLocation (Variables|/Script/Engine.Character|GetMesh (Class|MordhauEquipment|GetParentCharacter _askick_weapon)) "KickTracerStart"))))
                  (LocalVariables|SetForceDir (Math|Vector|Normalize (Math|Vector|MakeVector (.X (Math|Vector|BreakVector _output_get)) (.Y (Math|Vector|BreakVector _output_get)) (* (.Z (Math|Vector|BreakVector _output_get)) 0.5)))))
                (:CastFailed
                  (LocalVariables|SetForceDir (Variables|/Script/Mordhau.MordhauWeapon|GetLastObservedTraceDirection _asmordhau_weapon))))
              (if (== DamageType (Utilities|Enum|LiteralenumEMordhauDamageType "Generic"))
                (return "0, 0, 0")
                (else
                  (return (* (LocalVariables|GetForceDir) (* (Math|Float|Min(Float) (* 1e+04 (Variables|/Script/Mordhau.MordhauWeapon|GetRagdollForceMultiplier _asmordhau_weapon) (Math|Float|MapRangeClamped (Math|Conversions|ToFloat(Byte) RandomByte) 0.0 255.0 0.2 1.0)) (* (- 1.0 (* 0.25 (Math|Conversions|ToFloat(Boolean) (and (or (== DamageSubType (Utilities|Enum|LiteralenumEAttackMove "Stab")) (== DamageSubType (Utilities|Enum|LiteralenumEAttackMove "AltStab"))) _returnvalue_5)))) 3e+04)) (+ (* (Math|Conversions|ToFloat(Boolean) (and (== DamageSubType (Utilities|Enum|LiteralenumEAttackMove "Couch")) _returnvalue_5)) 2.0) 1.0)))))))
            (:CastFailed
              (bind _asmordhau_projectile (Utilities|Casting|CastToMordhauProjectile Agent)
                (:then
                  (if (== DamageType (Utilities|Enum|LiteralenumEMordhauDamageType "Ranged"))
                    (return (* (Transformation|GetActorForwardVector _asmordhau_projectile) (* (Variables|/Script/Mordhau.MordhauProjectile|GetRagdollForceMultiplier _asmordhau_projectile) 5e+03)))
                    (else
                      (return (* _returnvalue_4 (* (Variables|/Script/Mordhau.MordhauProjectile|GetRagdollForceMultiplier _asmordhau_projectile) 5e+03))))))
                (:CastFailed
                  (bind _asadvanced_character (Utilities|Casting|CastToAdvancedCharacter Agent)
                    (:then
                      (return (* _returnvalue_4 (* (Variables|/Script/Mordhau.AdvancedCharacter|GetRagdollForceMultIfDmgAgent _asadvanced_character) 5e+03))))
                    (:CastFailed
                      (bind _asmordhau_actor (Utilities|Casting|CastToMordhauActor Agent)
                        (:then
                          (return (* _returnvalue_4 (* (Variables|/Script/Mordhau.MordhauActor|GetRagdollForceMultiplier _asmordhau_actor) 5e+03))))
                        (:CastFailed
                          (return "0, 0, 0"))))))))))
        (:Is%20Not%20Valid
          _)))
    (:Is%20Not%20Valid
      _))
  (return "0, 0, 0"))

(fn CreateTextInputDialog
  (params (OwningPlayer :type Player%20Controller%20Object%20Reference) (TitleText :type Text) (HintText :type Text) (LeftButtonText :type Text) (RightButtonText :type Text) (bIsPassword :type Boolean))
  (bind _returnvalue (UserInterface|CreateWidget "/Game/Mordhau/UI/BP_TextInputDialog.BP_TextInputDialog_C" OwningPlayer))
  (Variables|/Game/Mordhau/UI/BP_TextInputDialog.BP_TextInputDialog_C|SetbIsPassword _returnvalue bIsPassword)
  (Default|SetRightButtonText _returnvalue RightButtonText)
  (Default|SetLeftButtonText _returnvalue LeftButtonText)
  (Variables|/Game/Mordhau/UI/BP_TextInputDialog.BP_TextInputDialog_C|SetHintText _returnvalue HintText)
  (Default|SetTitleText _returnvalue TitleText)
  (return _returnvalue))

(fn CreateChoiceDialog
  (params (OwningPlayer :type Player%20Controller%20Object%20Reference) (TitleText :type Text) (ChoiceText :type Text) (LeftButtonText :type Text) (RightButtonText :type Text))
  (bind _returnvalue (UserInterface|CreateWidget "/Game/Mordhau/UI/BP_ChoiceDialog.BP_ChoiceDialog_C" OwningPlayer))
  (Default|SetRightButtonText _returnvalue RightButtonText)
  (Default|SetLeftButtonText _returnvalue LeftButtonText)
  (Variables|/Game/Mordhau/UI/BP_ChoiceDialog.BP_ChoiceDialog_C|SetChoiceText _returnvalue ChoiceText)
  (Default|SetTitleText _returnvalue TitleText)
  (return _returnvalue))

(fn CreateInformationDialog
  (params (OwningPlayer :type Player%20Controller%20Object%20Reference) (TitleText :type Text) (InformationText :type Text) (ButtonText :type Text))
  (bind _returnvalue (UserInterface|CreateWidget "/Game/Mordhau/UI/BP_InformationDialog.BP_InformationDialog_C" OwningPlayer))
  (Default|SetButtonText _returnvalue ButtonText)
  (Variables|/Game/Mordhau/UI/BP_InformationDialog.BP_InformationDialog_C|SetInfoText _returnvalue InformationText)
  (Default|SetTitleText _returnvalue TitleText)
  (return _returnvalue))

(fn GetUnlockTooltipText
  (params (ItemDefIDs :type Array%20of%20Integers))
  (LocalVariables|SetGoldRequirement 0)
  (LocalVariables|SetXPRequirement 0)
  (for _array_element ItemDefIDs
    (bind _recipe (Class|MordhauInventory|GetUnlockRecipe (Class|MordhauUtilityLibrary|GetMordhauInventory) _array_element)
      (:Success
        (LocalVariables|SetGoldRequirement (+ (LocalVariables|GetGoldRequirement) (.requiredgold _recipe)))
        (LocalVariables|SetXPRequirement (+ (LocalVariables|GetXPRequirement) (.requiredxp _recipe))))))
  (if (== (LocalVariables|GetGoldRequirement) 0)
    (if (<= (Class|MordhauUtilityLibrary|GetRankfromXP (LocalVariables|GetXPRequirement)) 1)
      (return "")
      (else
        (return (Utilities|Text|FormatText "Level: {r}" (Class|MordhauUtilityLibrary|GetRankfromXP (LocalVariables|GetXPRequirement))))))
    (elif (<= (Class|MordhauUtilityLibrary|GetRankfromXP (LocalVariables|GetXPRequirement)) 1)
      (return (Utilities|Text|FormatText "Gold: {g}" (LocalVariables|GetGoldRequirement)))
      (else
        (return (Utilities|Text|FormatText "{a} 
{b}" (Utilities|Text|FormatText "Level: {r}" (Class|MordhauUtilityLibrary|GetRankfromXP (LocalVariables|GetXPRequirement))) (Utilities|Text|FormatText "Gold: {g}" (LocalVariables|GetGoldRequirement))))))))

(fn GetGoldandRankUnlockRequirement
  (params (ItemDefIDs :type Array%20of%20Integers))
  (LocalVariables|SetGoldRequirement 0)
  (LocalVariables|SetXPRequirement 0)
  (for _array_element ItemDefIDs
    (bind _recipe (Class|MordhauInventory|GetUnlockRecipe (Class|MordhauUtilityLibrary|GetMordhauInventory) _array_element)
      (:Success
        (LocalVariables|SetGoldRequirement (+ (LocalVariables|GetGoldRequirement) (.requiredgold _recipe)))
        (LocalVariables|SetXPRequirement (+ (LocalVariables|GetXPRequirement) (.requiredxp _recipe))))))
  (return (LocalVariables|GetGoldRequirement) (Class|MordhauUtilityLibrary|GetRankfromXP (LocalVariables|GetXPRequirement))))

(fn CreateContextPopup
  (params (Option%20Map :type Map%20of%20Strings%20to%20Texts))
  (bind _asbp_mordhau_hud (Utilities|Casting|CastToBP_MordhauHUD (Class|MordhauUtilityLibrary|GetMordhauHUD)))
  (bind _wrapper (Default|ConstructContextMenu (Variables|/Game/Mordhau/Blueprints/BP_MordhauHUD.BP_MordhauHUD_C|GetContextPopupWrapper _asbp_mordhau_hud) Option%20Map))
  (return _wrapper))

(fn Get1v1MMRfromStats
  (bind _returnvalue (Class|MordhauUtilityLibrary|GetMordhauStats))
  (bind _value (Class|MordhauStats|GetValue _returnvalue (Variables|/Script/Mordhau.MordhauStats|GetDuelRankLeaderboard _returnvalue))
    (:Success
      (return _value))
    (:Failure
      (return 0))))

(fn GetRank
  (bind _returnvalue (Class|MordhauUtilityLibrary|GetMordhauStats))
  (switch Utilities|FlowControl|Switch|SwitchonE_RankDisplayType (Utilities|Enum|ByteToEnumE_RankDisplayType (Variables|/Script/Mordhau.MordhauSingleton|GetSelectedLevelDisplayType (Class|MordhauUtilityLibrary|GetMordhauSingleton)))
    (:NewEnumerator0
      (return (Class|MordhauUtilityLibrary|GetRankfromXP (Class|MordhauInventory|GetXP (Class|MordhauUtilityLibrary|GetMordhauInventory)))))
    (:NewEnumerator1
      (bind _value (Class|MordhauStats|GetValue _returnvalue (Variables|/Script/Mordhau.MordhauStats|GetDuelRankLeaderboard _returnvalue))
        (:Success
          (return _value))
        (:Failure
          _)))
    (:NewEnumerator2
      (bind _value_2 (Class|MordhauStats|GetValue _returnvalue (Variables|/Script/Mordhau.MordhauStats|GetTeamfightRankLeaderboard _returnvalue))
        (:Success
          (return _value_2))
        (:Failure
          _))))
  (return 0))

(fn GetKeyInfofromActionName
  (params (Action%20Name :type Name))
  (bind _returnvalue (Class|MordhauUtilityLibrary|GetMordhauInput))
  (bind _returnvalue_2 (Class|MordhauInput|GetPrimaryActionKeyBinding _returnvalue Action%20Name))
  (bind _returnvalue_3 (Class|MordhauInput|GetSecondaryActionKeyBinding _returnvalue Action%20Name))
  (bind _returnvalue_4 (Class|MordhauInput|GetActionKey _returnvalue_2))
  (bind _returnvalue_5 (Class|MordhauInput|GetActionKey _returnvalue_3))
  (if (Class|KismetInputLibrary|KeyIsValid _returnvalue_4)
    _
    (elif (Class|KismetInputLibrary|KeyIsValid _returnvalue_5)
      _
      (else
        (return 0 "" "None"))))
  (bind _returnvalue_6 (Class|VirtualCursorFunctionLibrary|GetIsUsingController))
  (bind _asbp_mordhau_singleton (Utilities|Casting|CastToBP_MordhauSingleton (Class|MordhauUtilityLibrary|GetMordhauSingleton))
    (:then
      (if (.ReturnValue (Utilities|Map|Find (Variables|/Game/Mordhau/Blueprints/BP_MordhauSingleton.BP_MordhauSingleton_C|GetButtonPromptImageMap _asbp_mordhau_singleton) (select _returnvalue_6 _returnvalue_5 _returnvalue_4)))
        (return (.Value (Utilities|Map|Find (Variables|/Game/Mordhau/Blueprints/BP_MordhauSingleton.BP_MordhauSingleton_C|GetButtonPromptImageMap _asbp_mordhau_singleton) (select _returnvalue_6 _returnvalue_5 _returnvalue_4))) (select _returnvalue_6 _returnvalue_5 _returnvalue_4) (select _returnvalue_6 (Class|KismetInputLibrary|KeyGetDisplayName _returnvalue_5) (Class|KismetInputLibrary|KeyGetDisplayName _returnvalue_4)))
        (else
          _)))
    (:CastFailed
      _))
  (return 0 (select _returnvalue_6 _returnvalue_5 _returnvalue_4) (select _returnvalue_6 (Class|KismetInputLibrary|KeyGetDisplayName _returnvalue_5) (Class|KismetInputLibrary|KeyGetDisplayName _returnvalue_4))))

(fn GetKeyInfofromKey
  (params (Key%20 :type Key%20Structure))
  (bind _returnvalue (Class|KismetInputLibrary|KeyGetDisplayName Key%20))
  (if (Class|KismetInputLibrary|KeyIsValid Key%20)
    (bind _asbp_mordhau_singleton (Utilities|Casting|CastToBP_MordhauSingleton (Class|MordhauUtilityLibrary|GetMordhauSingleton))
      (:then
        (if (.ReturnValue (Utilities|Map|Find (Variables|/Game/Mordhau/Blueprints/BP_MordhauSingleton.BP_MordhauSingleton_C|GetButtonPromptImageMap _asbp_mordhau_singleton) Key%20))
          (return (.Value (Utilities|Map|Find (Variables|/Game/Mordhau/Blueprints/BP_MordhauSingleton.BP_MordhauSingleton_C|GetButtonPromptImageMap _asbp_mordhau_singleton) Key%20)) Key%20 _returnvalue)
          (else
            _)))
      (:CastFailed
        _))
    (return 0 Key%20 _returnvalue)
    (else
      (return 0 "" "None"))))

(fn GetPlayerStatefromActor
  (params (Actor :type Actor%20Object%20Reference))
  (Utilities|FlowControl|Sequence
    (:then_0
      (bind _asmordhau_vehicle (Utilities|Casting|CastToMordhauVehicle Actor)
        (:then
          (LocalVariables|SetFoundState (Variables|/Script/Engine.Pawn|GetPlayerState _asmordhau_vehicle)))
        (:CastFailed
          (bind _asmordhau_character (Utilities|Casting|CastToMordhauCharacter Actor))
          (Utilities|IsValid (Variables|/Script/Mordhau.MordhauCharacter|GetCurrentVehicle _asmordhau_character)
            (:Is%20Valid
              (LocalVariables|SetFoundState (Variables|/Script/Engine.Pawn|GetPlayerState (Variables|/Script/Mordhau.MordhauCharacter|GetCurrentVehicle _asmordhau_character))))
            (:Is%20Not%20Valid
              (LocalVariables|SetFoundState (Variables|/Script/Engine.Pawn|GetPlayerState _asmordhau_character)))))))
    (:then_1
      (bind _asmordhau_player_state (Utilities|Casting|CastToMordhauPlayerState (LocalVariables|GetFoundState))
        (:then
          (return _asmordhau_player_state))
        (:CastFailed
          (return 0))))))

(fn OpenSteamProfile
  (params (SteamID :type String%20%28by%20ref%29))
  (Class|MordhauUtilityLibrary|OpenURL (Utilities|String|ToString(Text) (Utilities|Text|FormatText "http://steamcommunity.com/profiles/{steamID}" (Utilities|Text|ToText(String) SteamID))))
  (return))

(fn Get3v3MMRfromStats
  (bind _returnvalue (Class|MordhauUtilityLibrary|GetMordhauStats))
  (bind _value (Class|MordhauStats|GetValue _returnvalue (Variables|/Script/Mordhau.MordhauStats|GetTeamfightRankLeaderboard _returnvalue))
    (:Success
      (return _value))
    (:Failure
      (return 0))))

(fn GetTeamColor
  (params (Team :type Integer))
  (bind _asbp_mordhau_game_state (Utilities|Casting|CastToBP_MordhauGameState (Game|GetGameState (LocalVariables|Get__WorldContext))))
  (if (Utilities|Array|IsValidIndex (Variables|/Script/Mordhau.MordhauGameState|GetTeamColors _asbp_mordhau_game_state) Team)
    (return (Utilities|Array|Get(acopy) (Variables|/Script/Mordhau.MordhauGameState|GetTeamColors _asbp_mordhau_game_state) Team) (Utilities|Struct|MakeSlateColor (Utilities|Array|Get(acopy) (Variables|/Script/Mordhau.MordhauGameState|GetTeamColors _asbp_mordhau_game_state) Team)))
    (else
      (return "(R=0.000000,G=0.000000,B=0.000000,A=0.000000)" ""))))

(fn GetLoadoutfromSingleton
  (params (Id :type Integer))
  (bind _returnvalue (Class|MordhauUtilityLibrary|GetMordhauSingleton))
  (bind _defaultprofiles (Variables|/Script/Mordhau.MordhauSingleton|GetDefaultProfiles _returnvalue))
  (bind _returnvalue_2 (Utilities|Array|Length _defaultprofiles))
  (bind _returnvalue_3 (< Id _returnvalue_2))
  (return (select _returnvalue_3 (Utilities|Array|Get(acopy) _defaultprofiles Id) (Utilities|Array|Get(acopy) (Variables|/Script/Mordhau.MordhauSingleton|GetCharacterProfiles _returnvalue) (- Id _returnvalue_2))) _returnvalue_3))

(fn SetSpawnLoadout
  (params (Player%20Controller :type Player%20Controller%20Object%20Reference) (Id :type Integer))
  (bind _returnvalue (Class|MordhauUtilityLibrary|GetMordhauSingleton))
  (bind _defaultprofiles (Variables|/Script/Mordhau.MordhauSingleton|GetDefaultProfiles _returnvalue))
  (bind _returnvalue_2 (Utilities|Array|Length _defaultprofiles))
  (bind _returnvalue_3 (- Id _returnvalue_2))
  (bind _asmordhau_player_controller (Utilities|Casting|CastToMordhauPlayerController Player%20Controller))
  (if (>= Id _returnvalue_2) ; Is custom profile?
    (if (Utilities|Array|IsValidIndex (Variables|/Script/Mordhau.MordhauSingleton|GetCharacterProfiles _returnvalue) _returnvalue_3) ; Is a valid index?
      (Variables|/Script/Mordhau.MordhauPlayerController|SetSelectedCharacterProfile _asmordhau_player_controller _returnvalue_3)
      (Variables|/Script/Mordhau.MordhauPlayerController|SetSelectedDefaultProfile _asmordhau_player_controller -1))
    (else
      (Variables|/Script/Mordhau.MordhauPlayerController|SetSelectedDefaultProfile _asmordhau_player_controller Id)
      (Variables|/Script/Mordhau.MordhauPlayerController|SetSelectedCharacterProfile _asmordhau_player_controller -1))))

(fn CreateContextPopupString
  (params (Option%20Map :type Map%20of%20Strings%20to%20Texts))
  (bind _asbp_mordhau_hud (Utilities|Casting|CastToBP_MordhauHUD (Class|MordhauUtilityLibrary|GetMordhauHUD)))
  (bind _wrapper (Default|ConstructContextMenu (Variables|/Game/Mordhau/Blueprints/BP_MordhauHUD.BP_MordhauHUD_C|GetContextPopupWrapperString _asbp_mordhau_hud) Option%20Map))
  (return _wrapper))