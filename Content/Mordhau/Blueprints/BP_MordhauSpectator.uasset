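; Spectator pawn for Mordhau with a cine camera that has hotkey-driven movement and focus controls.
; The mouse wheel changes flying speed, while line traces set manual focus distance or toggle tracking focus on a hit actor, and other keys nudge focus.
; Further keys save and restore a camera position and rotation, or open the demo UI during replay playback.
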(event EventBeginPlay)

(event Collision|EventActorBeginOverlap
  (params (OtherActor :type Actor%20Object%20Reference)))

(event Input|MouseEvents|MouseWheelUp
  (params (Key :type Key%20Structure :default "None"))
  (:Pressed
    (if (== (Pawn|GetViewTarget (Pawn|GetController)) self)
      (bind _asfloating_pawn_movement (Utilities|Casting|CastToFloatingPawnMovement (Variables|Default|GetMovementComponent)))
      (Variables|/Script/Engine.FloatingPawnMovement|SetMaxSpeed _asfloating_pawn_movement (Math|Float|Max(Float) (+ (Variables|/Script/Engine.FloatingPawnMovement|GetMaxSpeed _asfloating_pawn_movement) (Variables|Default|GetSpeedChangeDelta)) 0.0)))))

(event Input|MouseEvents|MouseWheelDown
  (params (Key :type Key%20Structure :default "None"))
  (:Pressed
    (if (== (Pawn|GetViewTarget (Pawn|GetController)) self)
      (bind _asfloating_pawn_movement (Utilities|Casting|CastToFloatingPawnMovement (Variables|Default|GetMovementComponent)))
      (Variables|/Script/Engine.FloatingPawnMovement|SetMaxSpeed _asfloating_pawn_movement (Math|Float|Max(Float) (- (Variables|/Script/Engine.FloatingPawnMovement|GetMaxSpeed _asfloating_pawn_movement) (Variables|Default|GetSpeedChangeDelta)) 0.0)))))

(event Input|KeyboardEvents|H
  (params (Key :type Key%20Structure :default "None"))
  (:Pressed
    (bind _output_get (Variables|Default|SetCameraFocus (Math|Float|Clamp(Float) (+ (Variables|Default|GetCameraFocus) (Variables|Default|GetFocusChangeDelta)) 0.0 5e+04)))
    (Variables|/Script/CinematicCamera.CineCameraComponent|SetFocusSettings (Variables|Default|GetCineCamera) (Utilities|Struct|MakeCameraFocusSettings "Manual" _output_get))))

(event Input|KeyboardEvents|O
  (params (Key :type Key%20Structure :default "None"))
  (bind _returnvalue (Transformation|GetActorLocation))
  (:Pressed
    (Utilities|FlowControl|FlipFlop
      (:A
        (if (== (Pawn|GetViewTarget (Pawn|GetController)) self)
          (bind _outhit (Collision|LineTraceForObjects _returnvalue (+ _returnvalue (* (Math|Vector|GetForwardVector (Transformation|GetActorRotation)) 1e+05)) (Variables|Default|GetFocusOnObjectTypes) true 0 "None"))
          (Variables|/Script/CinematicCamera.CineCameraComponent|SetFocusSettings (Variables|Default|GetCineCamera) (Utilities|Struct|MakeCameraFocusSettings "Tracking" 1e+05 (Utilities|Struct|MakeCameraTrackingFocusSettings (Utilities|ResolveSoftReference (.hitactor _outhit)) "0.000000,0.000000,0.000000" false) false 0.0))))
      (:B
        (Variables|/Script/CinematicCamera.CineCameraComponent|SetFocusSettings (Variables|Default|GetCineCamera) (Utilities|Struct|MakeCameraFocusSettings "Tracking" 1e+05 "(ActorToTrack=None,RelativeOffset=(X=0.000000,Y=0.000000,Z=0.000000))" false 0.0))))))

(event Input|KeyboardEvents|I
  (params (Key :type Key%20Structure :default "None"))
  (bind _returnvalue (Game|GetPlayerController 0))
  (:Pressed
    (if (Class|MordhauUtilityLibrary|IsDemoPlayback (Class|MordhauUtilityLibrary|GetWorldOf self))
      (bind _returnvalue_2 (UserInterface|CreateWidget "/Game/Mordhau/UI/BP_DemoUI.BP_DemoUI_C"))
      (UserInterface|Viewport|AddtoViewport _returnvalue_2 0)
      (Input|SetInputModeUIOnly _returnvalue _returnvalue_2 "DoNotLock")
      (Variables|/Script/Engine.PlayerController|SetbShowMouseCursor _returnvalue true)
      (Widget|SetKeyboardFocus _returnvalue_2))))

(event Input|KeyboardEvents|F
  (params (Key :type Key%20Structure :default "None"))
  (bind _returnvalue (Transformation|GetActorLocation))
  (:Pressed
    (if (== (Pawn|GetViewTarget (Pawn|GetController)) self)
      (bind _outhit (Collision|LineTraceForObjects _returnvalue (+ _returnvalue (* (Math|Vector|GetForwardVector (Transformation|GetActorRotation)) 1e+05)) (Variables|Default|GetFocusOnObjectTypes) true 0 "None"))
      (if (.bBlockingHit (Collision|BreakHitResult _outhit))
        (bind _output_get (Variables|Default|SetCameraFocus (.Distance (Collision|BreakHitResult _outhit))))
        (Variables|/Script/CinematicCamera.CineCameraComponent|SetFocusSettings (Variables|Default|GetCineCamera) (Utilities|Struct|MakeCameraFocusSettings "Manual" _output_get))))))

(event Input|KeyboardEvents|R
  (params (Key :type Key%20Structure :default "None"))
  (:Pressed
    (if (or (Class|MordhauUtilityLibrary|IsDemoPlayback (Class|MordhauUtilityLibrary|GetWorldOf self)) (== (Pawn|GetViewTarget (Pawn|GetController)) self))
      (Pawn|SetControlRotation (Pawn|GetController) (Variables|Default|GetCameraRotation))
      (Transformation|SetActorLocation (Variables|Default|GetCameraLocation) false false))))

(event Input|KeyboardEvents|G
  (params (Key :type Key%20Structure :default "None"))
  (:Pressed
    (bind _output_get (Variables|Default|SetCameraFocus (Math|Float|Clamp(Float) (- (Variables|Default|GetCameraFocus) (Variables|Default|GetFocusChangeDelta)) 0.0 5e+04)))
    (Variables|/Script/CinematicCamera.CineCameraComponent|SetFocusSettings (Variables|Default|GetCineCamera) (Utilities|Struct|MakeCameraFocusSettings "Manual" _output_get))))

(event Input|KeyboardEvents|T
  (params (Key :type Key%20Structure :default "None"))
  (:Pressed
    (if (or (Class|MordhauUtilityLibrary|IsDemoPlayback (Class|MordhauUtilityLibrary|GetWorldOf self)) (== (Pawn|GetViewTarget (Pawn|GetController)) self))
      (Variables|Default|SetCameraRotation (Pawn|GetControlRotation (Pawn|GetController) :!class /Script/Engine.Controller))
      (Variables|Default|SetCameraLocation (Transformation|GetWorldLocation (Variables|Default|GetCineCamera))))))

(fn ConstructionScript)