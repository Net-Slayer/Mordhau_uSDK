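; Base Blueprint for a sub-field, a piece of a field effect with a box area and a particle system.
; The construction script assigns the box as the area, and both deactivation events switch off the particles alongside the parent logic.
; Hiding scales the particle system to zero and showing restores unit scale, acting only when the hidden state changes.
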(event EventBeginPlay)

(event Collision|EventActorBeginOverlap
  (params (OtherActor :type Actor%20Object%20Reference)))

(event EventSetSubFieldHidden
  (params (bValue :type Boolean))
  (bind _particlesystem (Variables|Default|GetParticleSystem))
  (if (Math|Boolean|NotEqual(Boolean) bValue (Variables|Default|GetbIsSubFieldHidden))
    (bind _output_get (Variables|Default|SetbIsSubFieldHidden bValue))
    (if _output_get
      (Transformation|SetWorldScale3D _particlesystem "0, 0, 0")
      (else
        (Transformation|SetWorldScale3D _particlesystem "1.000000,1.000000,1.000000")))))

(event EventTick
  (params (DeltaSeconds :type Float%20%28single-precision%29)))

(event EventDeactivateSubField
  (Components|Activation|Deactivate (Variables|Default|GetParticleSystem))
  (|CallParentFunction))

(event EventBeginSubFieldDeactivation
  (|CallParentFunction)
  (Components|Activation|Deactivate (Variables|Default|GetParticleSystem)))

(fn ConstructionScript
  (|CallParentFunction)
  (Variables|Default|SetArea (Variables|Default|GetBox)))