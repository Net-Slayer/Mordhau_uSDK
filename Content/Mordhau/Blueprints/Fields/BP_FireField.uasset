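; BP_FireField is a fire area, credited to BP_FireBomb, that burns actors inside it after a warmup.
; Each tick it sets tracked characters on fire; the authority burns those deep enough, with damage and tick rate from curves over presence time.
; Other Mordhau actors take periodic damage, with destroyables measured by closest collision point, and newly overlapped sub-fields of same-age or older fire fields are deactivated.
; Audio fades out when the field deactivates.
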(event EventBeginPlay)

(event Collision|EventActorBeginOverlap
  (params (OtherActor :type Actor%20Object%20Reference)))

(event EventTick
  (params (DeltaSeconds :type Float%20%28single-precision%29))
  (bind _actorpresencetickcount (Variables|Default|GetActorPresenceTickCount))
  (if (<= (+ (Variables|Default|GetCreatedTime) (Variables|Default|GetWarmupTime)) (Utilities|Time|GetTimeSeconds))
    (|CallParentFunction DeltaSeconds)
    (Utilities|IsValid self
      (:Is%20Valid
        (bind _keys (Utilities|Map|Keys _actorpresencetickcount))
        (for _array_element _keys
          (Utilities|FlowControl|Sequence
            (:then_0
              (bind _asadvanced_character (Utilities|Casting|CastToAdvancedCharacter _array_element))
              (Class|AdvancedCharacter|SetonFire _asadvanced_character self))
            (:then_1
              (Networking|SwitchHasAuthority
                (:Authority
                  (bind _asadvanced_character_2 (Utilities|Casting|CastToAdvancedCharacter _array_element)
                    (:then
                      (bind _returnvalue (Class|MasterField|ComputeDistanceIntoField (Transformation|GetActorLocation _asadvanced_character_2)))
                      (if (>= _returnvalue 2e+02)
                        (Class|AdvancedCharacter|StartBurning _asadvanced_character_2 0.5 (Math|Curves|GetFloatValue (Variables|Default|GetCharFireDmgByTime) (* (Class|Actor|GetActorTickInterval) (Math|Conversions|ToFloat(Integer) (.Value (Utilities|Map|Find _actorpresencetickcount _array_element))))) (Math|Curves|GetFloatValue (Variables|Default|GetCharFireTickByTime) (* (Class|Actor|GetActorTickInterval) (Math|Conversions|ToFloat(Integer) (.Value (Utilities|Map|Find _actorpresencetickcount _array_element))))) (CallFunction|GetAgent) (Variables|Default|GetInstigatorController))
                        (else
                          (Utilities|Map|Remove _actorpresencetickcount _asadvanced_character_2))))
                    (:CastFailed
                      (bind _asmordhau_actor (Utilities|Casting|CastToMordhauActor _array_element)
                        (:then
                          (if (== (Math|Integer|%(Integer) (.Value (Utilities|Map|Find _actorpresencetickcount _array_element)) 2) 0)
                            (bind _asbp_destroyable_actor (Utilities|Casting|CastToBP_DestroyableActor _asmordhau_actor)
                              (:then
                                (bind _returnvalue_2 (Class|MasterField|ComputeDistanceIntoField (.OutPointOnBody (Collision|GetClosestPointonCollision (Variables|/Game/Mordhau/Blueprints/Interactables/Environment/BP_DestroyableActor.BP_DestroyableActor_C|GetStaticMesh _asbp_destroyable_actor) (Class|MasterField|GetFieldBoundsCenter) "None"))))
                                (if (>= _returnvalue_2 2.5e+02)
                                  (Game|Damage|ApplyDamage _asmordhau_actor (Variables|Default|GetOtherDamage) (Variables|Default|GetInstigatorController) (CallFunction|GetAgent) :!label _label)))
                              (:CastFailed
                                (bind _returnvalue_3 (Class|MasterField|ComputeDistanceIntoField (Transformation|GetActorLocation _asmordhau_actor)))
                                (if (>= _returnvalue_3 2.5e+02)
                                  (goto _label))))))
                        (:CastFailed
                          (if (== (.Value (Utilities|Map|Find _actorpresencetickcount _array_element)) 1)
                            (bind _asbp_fire_sub_field (Utilities|Casting|CastToBP_FireSubField _array_element))
                            (bind _returnvalue_4 (Class|MasterField|ComputeDistanceIntoField (Transformation|GetActorLocation _asbp_fire_sub_field)))
                            (if (and (<= (Variables|/Script/Mordhau.MasterField|GetCreatedTime (Class|SubField|GetMaster _asbp_fire_sub_field)) (Variables|Default|GetCreatedTime)) (>= _returnvalue_4 225.0))
                              (Class|SubField|DeactivateSubField _asbp_fire_sub_field))))))))))))))))

(event EventBeginFieldDeactivation
  (|CallParentFunction)
  (Audio|Components|Audio|FadeOut (Variables|Default|GetAudio) 1.5 0.0 :!class /Script/Engine.AudioComponent))

(fn ConstructionScript
  (|CallParentFunction))

(fn GetAgent
  (return (Class|MordhauUtilityLibrary|GetDefaultActor "/Game/Mordhau/Blueprints/Equipment/Thrown/BP_FireBomb.BP_FireBomb_C")))