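; Smoke field that marks characters inside as in smoke, douses their fire when deep enough and fades its audio on deactivation.
; Starting a second after creation, Tick walks the presence map, checking non-character overlaps only on first contact to save performance.
; Deep overlap with fire deactivates both fields, while overlapping smoke subfields from same-age or older fields are deactivated.
; Subfield effects hide when the local view-target character has full smoke overlay.
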(event EventBeginPlay)

(event Collision|EventActorBeginOverlap
  (params (OtherActor :type Actor%20Object%20Reference)))

(event EventBeginFieldDeactivation
  (|CallParentFunction)
  (Audio|Components|Audio|FadeOut (Variables|Default|GetAudio) 4.0 0.0 :!class /Script/Engine.AudioComponent))

(event EventTick
  (params (DeltaSeconds :type Float%20%28single-precision%29))
  (bind _actorpresencetickcount (Variables|Default|GetActorPresenceTickCount))
  (if (<= (+ (Variables|Default|GetCreatedTime) 1.0) (Utilities|Time|GetTimeSeconds))
    (|CallParentFunction DeltaSeconds)
    (Utilities|IsValid self
      (:Is%20Valid
        (Variables|Default|SetShouldHideEffects false)
        (bind _keys (Utilities|Map|Keys _actorpresencetickcount))
        (for _array_element _keys
          (bind _asadvanced_character (Utilities|Casting|CastToAdvancedCharacter _array_element)
            (:then
              (Utilities|FlowControl|Sequence
                (:then_0
                  (Class|AdvancedCharacter|SetonSmoke _asadvanced_character self)
                  (if (>= (Variables|/Script/Mordhau.AdvancedCharacter|GetDistanceIntoSmokeField _asadvanced_character) 3.5e+02)
                    (Class|AdvancedCharacter|DouseFire _asadvanced_character)))
                (:then_1
                  (bind _returnvalue (Class|MordhauUtilityLibrary|GetViewTargetCharacter 0 false))
                  (if (== _returnvalue _asadvanced_character)
                    (bind _asbp_mordhau_player_controller (Utilities|Casting|CastToBP_MordhauPlayerController (Game|GetPlayerController 0)))
                    (if (and (Pawn|IsLocalPlayerController _asbp_mordhau_player_controller) (== (Variables|/Game/Mordhau/Blueprints/BP_MordhauPlayerController.BP_MordhauPlayerController_C|GetSmokeOverlay _asbp_mordhau_player_controller) 1.0))
                      (Variables|Default|SetShouldHideEffects true))))))
            (:CastFailed
              (if (== (.Value (Utilities|Map|Find _actorpresencetickcount _array_element)) 1)
                (bind _asbp_fire_sub_field (Utilities|Casting|CastToBP_FireSubField _array_element)
                  (:then
                    (bind _returnvalue_2 (Class|MasterField|ComputeDistanceIntoField (Transformation|GetActorLocation _asbp_fire_sub_field)))
                    (if (>= _returnvalue_2 3.5e+02)
                      (Class|MasterField|BeginFieldDeactivation (Class|SubField|GetMaster _asbp_fire_sub_field))
                      (Class|MasterField|BeginFieldDeactivation)))
                  (:CastFailed
                    (bind _asbp_smoke_sub_field (Utilities|Casting|CastToBP_SmokeSubField _array_element))
                    (bind _returnvalue_3 (Class|MasterField|ComputeDistanceIntoField (Transformation|GetActorLocation _asbp_smoke_sub_field)))
                    (if (>= _returnvalue_3 4e+02)
                      (if (<= (Variables|/Script/Mordhau.MasterField|GetCreatedTime (Class|SubField|GetMaster _asbp_smoke_sub_field)) (Variables|Default|GetCreatedTime))
                        (Class|SubField|DeactivateSubField _asbp_smoke_sub_field)))))))))
        (Class|MasterField|SetSubFieldsHidden (Variables|Default|GetShouldHideEffects))))))

(fn ConstructionScript
  (|CallParentFunction))