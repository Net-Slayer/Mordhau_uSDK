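; BP_EnvFireField is an environmental fire field that ignites characters and damages other Mordhau actors inside it.
; Each tick, it calls the parent tick, then loops over tracked presence counts, calling SetOnFire on characters.
; On authority, characters deep enough inside start burning after more than one count, while shallower ones are untracked.
; Other Mordhau actors deep enough inside take damage when their count is even.
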(event EventBeginPlay)

(event Collision|EventActorBeginOverlap
  (params (OtherActor :type Actor%20Object%20Reference)))

(event EventTick
  (params (DeltaSeconds :type Float%20%28single-precision%29))
  (bind _actorpresencetickcount (Variables|Default|GetActorPresenceTickCount))
  (|CallParentFunction DeltaSeconds)
  (Utilities|IsValid self
    (:Is%20Valid
      (bind _keys (Utilities|Map|Keys _actorpresencetickcount))
      (for _array_element _keys
        (Utilities|FlowControl|Sequence
          (:then_0
            (bind _asadvanced_character (Utilities|Casting|CastToAdvancedCharacter _array_element))
            (Class|AdvancedCharacter|SetonFire _asadvanced_character self))
          (:then_1
            (Networking|SwitchHasAuthority
              (:Authority
                (bind _asadvanced_character_2 (Utilities|Casting|CastToAdvancedCharacter _array_element)
                  (:then
                    (bind _returnvalue (Class|MasterField|ComputeDistanceIntoField (Transformation|GetActorLocation _asadvanced_character_2)))
                    (if (>= _returnvalue 2e+02)
                      (if (> (.Value (Utilities|Map|Find _actorpresencetickcount _array_element)) 1)
                        (Class|AdvancedCharacter|StartBurning _asadvanced_character_2 1.5 (Variables|Default|GetCharacterDamage) 0.0 0 (Variables|Default|GetInstigatorController)))
                      (else
                        (Utilities|Map|Remove _actorpresencetickcount _asadvanced_character_2))))
                  (:CastFailed
                    (bind _asmordhau_actor (Utilities|Casting|CastToMordhauActor _array_element))
                    (if (== (Math|Integer|%(Integer) (.Value (Utilities|Map|Find _actorpresencetickcount _array_element)) 2) 0)
                      (bind _returnvalue_2 (Class|MasterField|ComputeDistanceIntoField (Transformation|GetActorLocation _asmordhau_actor)))
                      (if (>= _returnvalue_2 2e+02)
                        (Game|Damage|ApplyDamage _asmordhau_actor (Variables|Default|GetOtherDamage) (Variables|Default|GetInstigatorController) 0)))))))))))))

(fn ConstructionScript
  (|CallParentFunction))