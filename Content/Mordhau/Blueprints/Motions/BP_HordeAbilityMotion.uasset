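; Motion that drives a Horde mode character's special abilities: Hookshot, Shockwave, Taunt, Divine Favor, Immortality and Vanish.
; The net motion's MotionParam0 selects which ability's Begin function runs on the BP_HordeCharacter when the motion starts.
; A tick countdown then fires that ability's Stage2 function once, leaving the ability logic to the character.
; An interrupted motion destroys its Projectile if one is valid.
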(event EventOnBegin
  (|CallParentFunction)
  (bind _asbp_horde_character (Utilities|Casting|CastToBP_HordeCharacter (Class|MordhauMotion|GetOwnerMordhauCharacter)))
  (switch int (Math|Conversions|ToInteger(Byte) (.MotionParam0 (Utilities|Struct|BreakNetMotion (Class|MordhauCharacter|GetCurrentNetMotion _asbp_horde_character))))
    (:0
      (Default|BeginHookshot _asbp_horde_character))
    (:1
      (Default|BeginShockwave _asbp_horde_character))
    (:2
      (Default|BeginTaunt _asbp_horde_character))
    (:3
      (Default|BeginDivineFavor _asbp_horde_character))
    (:4
      (Default|BeginImmortality _asbp_horde_character))
    (:5
      (Default|BeginVanish _asbp_horde_character))))

(event EventOnTick
  (params (DeltaTime :type Float%20%28single-precision%29))
  (|CallParentFunction DeltaTime)
  (if (== (Variables|Default|GetCurrentStage) 0)
    (bind _output_get (Variables|Default|SetStage2Time (- (Variables|Default|GetStage2Time) DeltaTime)))
    (if (<= _output_get 0.0)
      (Variables|Default|SetCurrentStage 1)
      (bind _asbp_horde_character (Utilities|Casting|CastToBP_HordeCharacter (Class|MordhauMotion|GetOwnerMordhauCharacter)))
      (switch int (Math|Conversions|ToInteger(Byte) (.MotionParam0 (Utilities|Struct|BreakNetMotion (Class|MordhauCharacter|GetCurrentNetMotion _asbp_horde_character))))
        (:0
          (Default|Stage2Hookshot _asbp_horde_character))
        (:1
          (Default|Stage2Shockwave _asbp_horde_character))
        (:2
          (Default|Stage2Taunt _asbp_horde_character))
        (:3
          (Default|Stage2DivineFavor _asbp_horde_character))
        (:4
          (Default|Stage2Immortality _asbp_horde_character))
        (:5
          (Default|Stage2Vanish _asbp_horde_character))))))

(event EventOnLeave
  (params (Interrupted :type Boolean))
  (bind _projectile (Variables|Default|GetProjectile))
  (|CallParentFunction Interrupted)
  (if Interrupted
    (Utilities|IsValid _projectile
      (:Is%20Valid
        (Actor|DestroyActor _projectile)))))