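; BP_BloodSplash is a short-lived blood particle effect actor that leaves blood splat decals where its particles collide.
; On each particle collision it spawns a decal aligned to the surface normal, with a timed fade and small fade screen size.
; A dynamic material instance randomizes Row and Column parameters to vary the splat shape from an atlas.
; The actor destroys itself when the particle system finishes.
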(event OnParticleCollide(ParticleSystem)
  (params (EventName :type Name :default "None") (EmitterTime :type Float%20%28single-precision%29) (ParticleTime :type Integer) (Location :type Vector :default "0, 0, 0") (Velocity :type Vector :default "0, 0, 0") (Direction :type Vector :default "0, 0, 0") (Normal :type Vector :default "0, 0, 0") (BoneName :type Name :default "None") (PhysMat :type Physical%20Material%20Object%20Reference))
  (bind _returnvalue (Class|MordhauUtilityLibrary|SpawnBloodDecalatLocation 0 "/Game/Mordhau/Assets/Environment/DecalMaterials/INST_DM_Bloodsplash.INST_DM_Bloodsplash" "50.000000,50.000000,50.000000" Location (Math|Rotator|MakeRotfromX (* Normal -1.0)) 9e+01))
  (Utilities|IsValid _returnvalue
    (:Is%20Valid
      (Rendering|Components|Decal|SetFadeOut _returnvalue 9e+01 0.2 false)
      (Class|MordhauUtilityLibrary|SetDecalFadeScreenSize _returnvalue 0.05)
      (Class|DecalComponent|SetSortOrder _returnvalue 1)
      (bind _returnvalue_2 (Rendering|Material|CreateDynamicMaterialInstance _returnvalue :!class /Script/Engine.DecalComponent))
      (Rendering|Material|SetScalarParameterValue _returnvalue_2 "Row" (Math|Conversions|ToFloat(Integer) (Math|Random|RandomIntegerinRange 0 7)) :!class /Script/Engine.MaterialInstanceDynamic)
      (Rendering|Material|SetScalarParameterValue _returnvalue_2 "Column" (Math|Conversions|ToFloat(Integer) (Math|Random|RandomIntegerinRange 0 7)) :!class /Script/Engine.MaterialInstanceDynamic))))

(event OnSystemFinished(ParticleSystem)
  (params (PSystem :type Particle%20System%20Component%20Object%20Reference))
  (Components|DestroyComponent (Variables|Default|GetParticleSystem))
  (Actor|DestroyActor))

(fn ConstructionScript)