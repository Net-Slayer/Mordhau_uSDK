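; Music player actor that plays a track from a start offset on BeginPlay and repeats defined loop regions within it.
; A chained timer drives LoopLogic, which either repeats the current region or, when ShouldLoop is false, re-arms looping and lets playback continue to the next region.
; RepeatCurrent crossfades between two players sharing the track.
; Real-time timestamps measure timer drift to correct delays, fades and seek positions.
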(event Custom|LoopLogic
  (bind _loops (Variables|Default|GetLoops))
  (Development|PrintString "LoopLogic")
  (Variables|Default|SetTimerOffTargetDelta (- (Utilities|Time|GetRealTimeSeconds) (Variables|Default|GetTimerTargetTime)))
  (if (Variables|Default|GetShouldLoop)
    (CallFunction|RepeatCurrent)
    (Variables|Default|SetTimerTargetTime (+ (Utilities|Time|GetRealTimeSeconds) (- (- (.Y (Math|Vector2D|BreakVector2D (.LoopRegion (Utilities|Struct|BreakBP_MusicTrackData (Utilities|Array|Get(acopy) (Variables|Default|GetLoops) (Variables|Default|GetCurrentLoopIndex)))))) (.X (Math|Vector2D|BreakVector2D (.LoopRegion (Utilities|Struct|BreakBP_MusicTrackData (Utilities|Array|Get(acopy) (Variables|Default|GetLoops) (Variables|Default|GetCurrentLoopIndex))))))) (Variables|Default|GetTimerOffTargetDelta))))
    (Utilities|Time|SetTimerbyEvent (delegate Custom|LoopLogic) (- (- (.Y (Math|Vector2D|BreakVector2D (.LoopRegion (Utilities|Struct|BreakBP_MusicTrackData (Utilities|Array|Get(acopy) (Variables|Default|GetLoops) (Variables|Default|GetCurrentLoopIndex)))))) (.X (Math|Vector2D|BreakVector2D (.LoopRegion (Utilities|Struct|BreakBP_MusicTrackData (Utilities|Array|Get(acopy) (Variables|Default|GetLoops) (Variables|Default|GetCurrentLoopIndex))))))) (Variables|Default|GetTimerOffTargetDelta)))
    (else
      (Variables|Default|SetShouldLoop true)
      (if (Utilities|Array|IsValidIndex (Variables|Default|GetLoops) (+ (Variables|Default|GetCurrentLoopIndex) 1))
        (bind _output_get (Variables|Default|SetCurrentLoopIndex (+ (Variables|Default|GetCurrentLoopIndex) 1)))
        (Variables|Default|SetTimerTargetTime (+ (Utilities|Time|GetRealTimeSeconds) (- (- (- (.X (Math|Vector2D|BreakVector2D (.LoopRegion (Utilities|Struct|BreakBP_MusicTrackData (Utilities|Array|Get(acopy) _loops _output_get))))) (- (.Y (Math|Vector2D|BreakVector2D (.LoopRegion (Utilities|Struct|BreakBP_MusicTrackData (Utilities|Array|Get(acopy) _loops (- _output_get 1)))))) (.Crossfade (Utilities|Struct|BreakBP_MusicTrackData (Utilities|Array|Get(acopy) _loops (- _output_get 1)))))) (.Crossfade (Utilities|Struct|BreakBP_MusicTrackData (Utilities|Array|Get(acopy) _loops _output_get)))) (Variables|Default|GetTimerOffTargetDelta))))
        (Utilities|Time|SetTimerbyEvent (delegate Custom|LoopLogic) (- (- (- (.X (Math|Vector2D|BreakVector2D (.LoopRegion (Utilities|Struct|BreakBP_MusicTrackData (Utilities|Array|Get(acopy) _loops _output_get))))) (- (.Y (Math|Vector2D|BreakVector2D (.LoopRegion (Utilities|Struct|BreakBP_MusicTrackData (Utilities|Array|Get(acopy) _loops (- _output_get 1)))))) (.Crossfade (Utilities|Struct|BreakBP_MusicTrackData (Utilities|Array|Get(acopy) _loops (- _output_get 1)))))) (.Crossfade (Utilities|Struct|BreakBP_MusicTrackData (Utilities|Array|Get(acopy) _loops _output_get)))) (Variables|Default|GetTimerOffTargetDelta)))))))

(event Custom|StartMusic
  (bind _firstplayer (Variables|Default|GetFirstPlayer))
  (bind _startoffset (Variables|Default|GetStartOffset))
  (bind _track (Variables|Default|GetTrack))
  (bind _secondplayer (Variables|Default|GetSecondPlayer))
  (bind _loops (Variables|Default|GetLoops))
  (bind _output (Utilities|Array|Get(acopy) _loops))
  (bind (_loopregion _crossfade) (Utilities|Struct|BreakBP_MusicTrackData _output))
  (bind _y (Math|Vector2D|BreakVector2D _loopregion))
  (bind _returnvalue (- _y _startoffset))
  (bind _returnvalue_2 (- _returnvalue _crossfade))
  (Variables|Default|SetShouldLoop true)
  (Variables|Default|SetCurrentLoopIndex 0)
  (Audio|Components|Audio|Stop _firstplayer)
  (Audio|Components|Audio|Stop _secondplayer)
  (Audio|Components|Audio|SetSound _firstplayer _track)
  (Audio|Components|Audio|SetSound _secondplayer _track)
  (Audio|Components|Audio|Play _firstplayer (Variables|Default|GetStartOffset))
  (if (> (Utilities|Array|Length _loops) 0)
    (Variables|Default|SetTimerTargetTime (+ (Utilities|Time|GetRealTimeSeconds) _returnvalue_2))
    (Utilities|Time|SetTimerbyEvent (delegate Custom|LoopLogic) _returnvalue_2)))

(event EventBeginPlay
  (CallFunction|StartMusic))

(event Collision|EventActorBeginOverlap
  (params (OtherActor :type Actor%20Object%20Reference)))

(event EventTick
  (params (DeltaSeconds :type Float%20%28single-precision%29)))

(fn ConstructionScript)

(fn RepeatCurrent
  (bind _timerofftargetdelta (Variables|Default|GetTimerOffTargetDelta))
  (bind _loops (Variables|Default|GetLoops))
  (bind _currentloopindex (Variables|Default|GetCurrentLoopIndex))
  (bind _secondplayer (Variables|Default|GetSecondPlayer))
  (bind _firstplayer (Variables|Default|GetFirstPlayer))
  (bind _output (Utilities|Array|Get(acopy) _loops _currentloopindex))
  (bind (_loopregion _crossfade) (Utilities|Struct|BreakBP_MusicTrackData _output))
  (bind _x (Math|Vector2D|BreakVector2D _loopregion))
  (bind _returnvalue (- _crossfade _timerofftargetdelta))
  (bind _returnvalue_2 (+ _x _timerofftargetdelta))
  (if (Variables|Default|GetCurrentPlayerIsSecond)
    (Audio|Components|Audio|FadeOut _secondplayer _returnvalue 0.0 :!class /Script/Engine.AudioComponent)
    (Audio|Components|Audio|FadeIn _firstplayer _returnvalue 1.0 _returnvalue_2 :!class /Script/Engine.AudioComponent)
    (Variables|Default|SetCurrentPlayerIsSecond false)
    (else
      (Audio|Components|Audio|FadeOut _firstplayer _returnvalue 0.0 :!class /Script/Engine.AudioComponent)
      (Audio|Components|Audio|FadeIn _secondplayer _returnvalue 1.0 _returnvalue_2 :!class /Script/Engine.AudioComponent)
      (Variables|Default|SetCurrentPlayerIsSecond true))))