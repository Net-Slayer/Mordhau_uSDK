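; Spectator crowd manager that replaces BP_CrowdSystemActor placeholders with its own cosmetic skeletal meshes and drives their animation and sound.
; A timer switches between idle, cheering and bored states using average character health drops and match or round stage.
; Finished animations restart from the current state's set at random play rates, while audio components change sound one at a time to stagger transitions.
; The effects quality setting hides crowd members.
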(event Custom|CheckForInterestingEvents
  (bind _returnvalue (Class|MordhauUtilityLibrary|GetMordhauGameUserSettings))
  (bind _returnvalue_2 (Utilities|Time|GetTimeSeconds))
  (bind _lastinterestingeventtime (Variables|Default|GetLastInterestingEventTime))
  (bind _returnvalue_3 (Settings|GetVisualEffectQuality _returnvalue))
  (bind _returnvalue_4 (- _returnvalue_2 _lastinterestingeventtime))
  (Utilities|FlowControl|Sequence
    (:then_0
      (if (!= _returnvalue_3 (Variables|Default|GetLastObservedEffectsSetting))
        (Variables|Default|SetLastObservedEffectsSetting _returnvalue_3)
        (CallFunction|UpdateEffectsHiding)))
    (:then_1
      (CallFunction|CheckInterestingEventsFunction)
      (switch int (Variables|Default|GetTargetCrowdState)
        (:0
          (if (> _returnvalue_4 15.0)
            (Variables|Default|SetTargetCrowdState 2)
            (else
              (if (< _returnvalue_4 1.0) :!label _label
                (Variables|Default|SetTargetCrowdState 1)))))
        (:1
          (if (> _returnvalue_4 5.0)
            (Variables|Default|SetTargetCrowdState 0)))
        (:2
          (goto _label))))))

(event Custom|UpdateCrowdSoundState
  (if (!= (Variables|Default|GetCurrentCrowdSoundState) (Variables|Default|GetTargetCrowdState))
    (CallFunction|TransitionCrowdSoundState 1)))

(event EventBeginPlay
  (Utilities|FlowControl|Sequence
    (:then_0
      (Networking|CanExecuteCosmeticEvents
        (:True
          (Utilities|FlowControl|Sequence
            (:then_0
              (bind _outactors (Actor|GetAllActorsOfClass "/Game/Mordhau/Blueprints/Misc/BP_CrowdSystemActor.BP_CrowdSystemActor_C"))
              (Utilities|Array|Shuffle _outactors)
              (for _array_element _outactors
                (bind _returnvalue (AddComponent|AddSkeletalMeshComponent false (Transformation|GetWorldTransform (Variables|/Game/Mordhau/Blueprints/Misc/BP_CrowdSystemActor.BP_CrowdSystemActor_C|GetSkeletalMesh _array_element))))
                (Transformation|SetAbsolute _returnvalue true true true)
                (Utilities|Array|Add (Variables|Default|GetEntities) (Utilities|Struct|MakeSTRUCT_CrowdSystemEntity _returnvalue (Variables|/Game/Mordhau/Blueprints/Misc/BP_CrowdSystemActor.BP_CrowdSystemActor_C|GetIdleAnimations _array_element) (Variables|/Game/Mordhau/Blueprints/Misc/BP_CrowdSystemActor.BP_CrowdSystemActor_C|GetCheeringAnimations _array_element) (Variables|/Game/Mordhau/Blueprints/Misc/BP_CrowdSystemActor.BP_CrowdSystemActor_C|GetBoredAnimations _array_element) 0.0 -1 (Variables|/Game/Mordhau/Blueprints/Misc/BP_CrowdSystemActor.BP_CrowdSystemActor_C|GetMinEffectsLevelToShow _array_element)))
                (Class|SkinnedMeshComponent|SetSkeletalMesh _returnvalue (Variables|/Script/Engine.SkinnedMeshComponent|GetSkeletalMesh (Variables|/Game/Mordhau/Blueprints/Misc/BP_CrowdSystemActor.BP_CrowdSystemActor_C|GetSkeletalMesh _array_element)) true)
                (for (_array_element_2 _array_index) (Rendering|Material|GetMaterials (Variables|/Game/Mordhau/Blueprints/Misc/BP_CrowdSystemActor.BP_CrowdSystemActor_C|GetSkeletalMesh _array_element))
                  (Rendering|Material|SetMaterial _returnvalue _array_index _array_element_2))))
            (:then_1
              (Variables|Default|SetTargetCrowdState 0)
              (CallFunction|UpdateCrowdAnims)
              (CallFunction|TransitionCrowdSoundState 999))
            (:then_2
              (Utilities|Time|SetTimerbyEvent (delegate Custom|CheckForInterestingEvents) 1.0 true)
              (Utilities|Time|SetTimerbyEvent (delegate Custom|UpdateCrowdSoundState) 0.5 true))))))
    (:then_1
      (bind _outactors_2 (Actor|GetAllActorsOfClass "/Game/Mordhau/Blueprints/Misc/BP_CrowdSystemActor.BP_CrowdSystemActor_C"))
      (for _array_element_3 _outactors_2
        (Default|DestroyDisplay _array_element_3)))))

(event Collision|EventActorBeginOverlap
  (params (OtherActor :type Actor%20Object%20Reference)))

(event EventTick
  (params (DeltaSeconds :type Float%20%28single-precision%29))
  (CallFunction|UpdateCrowdAnims))

(fn ConstructionScript)

(fn CheckInterestingEventsFunction
  (Utilities|FlowControl|Sequence
    (:then_0
      (bind _outactors (Actor|GetAllActorsOfClass "/Script/Mordhau.MordhauCharacter"))
      (for _array_element _outactors
        (if (not (Math|Boolean|Equal(Boolean) (Variables|/Script/Engine.Actor|GetbCanBeDamaged _array_element) false))
          (LocalVariables|SetNewAverageHealth (+ (LocalVariables|GetNewAverageHealth) (Math|Conversions|ToFloat(Byte) (Variables|/Script/Mordhau.AdvancedCharacter|GetHealth _array_element))))
          (LocalVariables|SetTotalChars (+ (LocalVariables|GetTotalChars) 1))))
      (if (> (LocalVariables|GetTotalChars) 0)
        (bind _output_get (LocalVariables|SetDivisor (Math|Conversions|ToFloat(Integer) (LocalVariables|GetTotalChars))))
        (LocalVariables|SetNewAverageHealth (/ (LocalVariables|GetNewAverageHealth) _output_get))))
    (:then_1
      (if (> (- (Variables|Default|GetAveragePlayerHealth) (LocalVariables|GetNewAverageHealth)) (/ (Variables|Default|GetInterestingEventHealthThreshold) (LocalVariables|GetDivisor)))
        (Variables|Default|SetLastInterestingEventTime (Utilities|Time|GetTimeSeconds) :!label _label)
        (elif (Class|GameStateBase|HasMatchStarted (Game|GetGameState))
          (bind _asbp_duel_player_controller (Utilities|Casting|CastToBP_DuelPlayerController (Game|GetPlayerController 0))
            (:then
              (if (Pawn|IsLocalPlayerController _asbp_duel_player_controller)
                (if (Utilities|Enum|NotEqual(Enum) (.Stage (Utilities|Struct|BreakSTRUCT_DuelRoundInfo (.RoundInfo (Utilities|Struct|BreakST_DuelRoomGame (Variables|/Game/Mordhau/Blueprints/GameModes/Duel/BP_DuelPlayerController.BP_DuelPlayerController_C|GetReplicatedRoomGame _asbp_duel_player_controller))))) "NewEnumerator2")
                  (goto _label))))
            (:CastFailed
              (bind _asbp_skirmish_game_state (Utilities|Casting|CastToBP_SkirmishGameState (Game|GetGameState)))
              (if (Utilities|Enum|NotEqual(Enum) (.Stage (Utilities|Struct|BreakSTRUCT_SkirmishRoundInfo (Variables|/Game/Mordhau/Blueprints/GameModes/Skirmish/BP_SkirmishGameState.BP_SkirmishGameState_C|GetRoundInfo _asbp_skirmish_game_state))) "NewEnumerator2")
                (goto _label))))
          (else
            (goto _label)))))
    (:then_2
      (Variables|Default|SetAveragePlayerHealth (LocalVariables|GetNewAverageHealth)))))

(fn UpdateCrowdAnims
  (bind _entities (Variables|Default|GetEntities))
  (LocalVariables|SetTimeNow (Utilities|Time|GetTimeSeconds))
  (Utilities|FlowControl|Sequence
    (:then_0
      (bind (_array_element _array_index) (Utilities|Array|ForEachLoopwithBreak _entities)
        (:LoopBody
          (if (not (or (Audio|Components|Audio|IsPlaying (.MeshComponent (Utilities|Struct|BreakSTRUCT_CrowdSystemEntity _array_element))) (Variables|/Script/Engine.SceneComponent|GetbHiddenInGame (.MeshComponent (Utilities|Struct|BreakSTRUCT_CrowdSystemEntity _array_element)))))
            (Utilities|FlowControl|Sequence
              (:then_0
                (switch int (Variables|Default|GetTargetCrowdState)
                  (:0
                    (LocalVariables|SetRandomAnimSeq (Utilities|Array|Get(acopy) (.IdleAnimations (Utilities|Struct|BreakSTRUCT_CrowdSystemEntity _array_element)) (Math|Random|RandomIntegerinRange 0 (- (Utilities|Array|Length (.IdleAnimations (Utilities|Struct|BreakSTRUCT_CrowdSystemEntity _array_element))) 1)))))
                  (:1
                    (LocalVariables|SetRandomAnimSeq (Utilities|Array|Get(acopy) (.CheeringAnimations (Utilities|Struct|BreakSTRUCT_CrowdSystemEntity _array_element)) (Math|Random|RandomIntegerinRange 0 (- (Utilities|Array|Length (.CheeringAnimations (Utilities|Struct|BreakSTRUCT_CrowdSystemEntity _array_element))) 1)))))
                  (:2
                    (LocalVariables|SetRandomAnimSeq (Utilities|Array|Get(acopy) (.BoredAnimations (Utilities|Struct|BreakSTRUCT_CrowdSystemEntity _array_element)) (Math|Random|RandomIntegerinRange 0 (- (Utilities|Array|Length (.BoredAnimations (Utilities|Struct|BreakSTRUCT_CrowdSystemEntity _array_element))) 1)))))))
              (:then_1
                (bind _output_get (LocalVariables|SetPlayRate (Math|Random|RandomFloatinRange 0.8 1.2)))
                (Components|Animation|PlayAnimation (.MeshComponent (Utilities|Struct|BreakSTRUCT_CrowdSystemEntity _array_element)) (LocalVariables|GetRandomAnimSeq) false)
                (Components|Timeline|SetPlayRate (.MeshComponent (Utilities|Struct|BreakSTRUCT_CrowdSystemEntity _array_element)) _output_get))
              (:then_2
                (Utilities|Array|SetArrayElem _entities _array_index (Utilities|Struct|MakeSTRUCT_CrowdSystemEntity (.MeshComponent (Utilities|Struct|BreakSTRUCT_CrowdSystemEntity _array_element)) (.IdleAnimations (Utilities|Struct|BreakSTRUCT_CrowdSystemEntity _array_element)) (.CheeringAnimations (Utilities|Struct|BreakSTRUCT_CrowdSystemEntity _array_element)) (.BoredAnimations (Utilities|Struct|BreakSTRUCT_CrowdSystemEntity _array_element)) (+ (LocalVariables|GetTimeNow) (* (Variables|/Script/Engine.AnimSequenceBase|GetSequenceLength (LocalVariables|GetRandomAnimSeq)) (/ 1.0 (LocalVariables|GetPlayRate)))) (Variables|Default|GetTargetCrowdState) (.QualityLevel (Utilities|Struct|BreakSTRUCT_CrowdSystemEntity _array_element))))))))))))

(fn TransitionCrowdSoundState
  (params (MaxTransitions :type Integer))
  (bind _targetcrowdstate (Variables|Default|GetTargetCrowdState))
  (bind _idlesound (Variables|Default|GetIdleSound))
  (bind _boredsound (Variables|Default|GetBoredSound))
  (bind _cheeringsound (Variables|Default|GetCheeringSound))
  (bind _returnvalue (Utilities|Select :Index _targetcrowdstate :Option%200 _idlesound :Option%201 _cheeringsound :Option%202 _boredsound))
  (Utilities|FlowControl|Sequence
    (:then_0
      (bind _array_element (Utilities|Array|ForEachLoopwithBreak (Variables|Default|GetCrowdAudioComponents) :!label _label)
        (:LoopBody
          (if (not (== (Variables|/Script/Engine.AudioComponent|GetSound (Variables|/Script/Engine.AmbientSound|GetAudioComponent _array_element)) _returnvalue))
            (Audio|Components|Audio|SetSound (Variables|/Script/Engine.AmbientSound|GetAudioComponent _array_element) _returnvalue)
            (Audio|Components|Audio|Play (Variables|/Script/Engine.AmbientSound|GetAudioComponent _array_element) 0.0)
            (bind _result (Math|Integer|IncrementInt (LocalVariables|GetTransitions))
              (:%20%20
                (if (>= _result MaxTransitions)
                  (goto _label Break))))))))
    (:then_1
      ;[1 1 1] No updates done, means we must be in the target state.
      (if (== (LocalVariables|GetTransitions) 0)
        (Variables|Default|SetCurrentCrowdSoundState (Variables|Default|GetTargetCrowdState))))))

(fn UpdateEffectsHiding
  (bind _array_element (Utilities|Array|ForEachLoopwithBreak (Variables|Default|GetEntities))
    (:LoopBody
      (if (Math|Boolean|NotEqual(Boolean) (> (.QualityLevel (Utilities|Struct|BreakSTRUCT_CrowdSystemEntity _array_element)) (Variables|Default|GetLastObservedEffectsSetting)) (Variables|/Script/Engine.SceneComponent|GetbHiddenInGame (.MeshComponent (Utilities|Struct|BreakSTRUCT_CrowdSystemEntity _array_element))))
        (Development|SetHiddeninGame (.MeshComponent (Utilities|Struct|BreakSTRUCT_CrowdSystemEntity _array_element)) (not (Variables|/Script/Engine.SceneComponent|GetbHiddenInGame (.MeshComponent (Utilities|Struct|BreakSTRUCT_CrowdSystemEntity _array_element)))) false)))))