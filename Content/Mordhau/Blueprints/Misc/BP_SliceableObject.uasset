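; BP_SliceableObject is an actor that gets cut in two when struck by a weapon.
; On BeginPlay it copies its static mesh into a procedural mesh with collision, then destroys the static mesh.
; Cosmetic hits from Mordhau weapons using right or left strikes slice the procedural mesh at the impact point, using the weapon's forward vector as plane normal.
; The new half gets a cap and simulates physics.
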(event EventBeginPlay
  (bind _staticmesh (Variables|Default|GetStaticMesh))
  (Class|KismetProceduralMeshLibrary|CopyProceduralMeshfromStaticMeshComponent _staticmesh 0 (Variables|Default|GetProceduralMesh) true)
  (Components|DestroyComponent _staticmesh))

(event Collision|EventActorBeginOverlap
  (params (OtherActor :type Actor%20Object%20Reference)))

(event EventOnReceiveCosmeticHit
  (params (Source :type Actor%20Object%20Reference) (Agent :type Actor%20Object%20Reference) (Move :type EAttackMove%20Enum :default "RightStrike") (Hit :type Hit%20Result%20Structure%20%28by%20ref%29))
  (bind _asmordhau_weapon (Utilities|Casting|CastToMordhauWeapon Agent))
  (if (or (Utilities|Enum|Equal(Enum) Move "RightStrike") (Utilities|Enum|Equal(Enum) Move "LeftStrike"))
    (bind _outotherhalfprocmesh (Class|KismetProceduralMeshLibrary|SliceProceduralMesh (Variables|Default|GetProceduralMesh) (.ImpactPoint (Collision|BreakHitResult Hit)) (Transformation|GetActorForwardVector _asmordhau_weapon) true "CreateNewSectionForCap"))
    (Physics|SetSimulatePhysics _outotherhalfprocmesh true)))

(fn ConstructionScript)