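; BP_Ummmmm is an actor with a character mesh in helmet and pants that drifts steadily upward, with no clear gameplay purpose.
; The construction script slaves both clothing meshes to UMAMaster's pose via master pose.
; BeginPlay calls a looping PlayAnimation on UMAMaster, though no animation asset is specified.
; Tick lerps toward a world-Z offset transform using DeltaSeconds as alpha, producing a constant rise without sweeping.
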(event EventBeginPlay
  (Components|Animation|PlayAnimation (Variables|Default|GetUMA_Master) 0 true))

(event Collision|EventActorBeginOverlap
  (params (OtherActor :type Actor%20Object%20Reference)))

(event EventTick
  (params (DeltaSeconds :type Float%20%28single-precision%29))
  (bind _self self)
  (bind _returnvalue (Transformation|GetActorTransform _self))
  (Transformation|SetActorTransform _self (Math|Transform|Lerp(Transform) _returnvalue (Math|Transform|ComposeTransforms _returnvalue (Math|Transform|MakeTransform "0, 0,20.000000")) DeltaSeconds)))

(fn ConstructionScript
  (Class|SkinnedMeshComponent|SetMasterPoseComponent (Variables|Default|GetNice_helmet) (Variables|Default|GetUMA_Master) false))