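; Camera component for Mordhau characters that overrides the computed camera POV according to the owning character's CameraStyle.
; Most styles pass the parent class's POV through unchanged.
; The third style (index 2) places the camera at a fixed world-space offset from the mesh's "Position" socket, with a constant rotation and the parent's FOV, so it follows the character without turning with it.
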(fn ComputeCameraPOV
  (bind _returnvalue (|CallParentFunction))
  (bind _asmordhau_character (Utilities|Casting|CastToMordhauCharacter (Components|GetOwner)))
  (switch int (Math|Conversions|ToInteger(Byte) (Variables|/Script/Mordhau.MordhauCharacter|GetCameraStyle _asmordhau_character))
    (:Default
      _)
    (:0
      _)
    (:1
      _)
    (:2
      (return (Utilities|Struct|MakePOV (+ (Transformation|GetSocketLocation (Variables|/Script/Engine.Character|GetMesh _asmordhau_character) "Position") "240.000000,0.000000,150.000000") "0,180.000000, 0" (.FOV (Utilities|Struct|BreakPOV _returnvalue))))))
  (return _returnvalue))