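; Base-style Mordhau projectile Blueprint that can set characters it damages on fire.
; It extends the parent's damaged-character event, then, on the server only, checks that the hit is non-lethal and that fire damage is above zero.
; It then starts burning on the victim using the fire duration, damage and tick variables, crediting the projectile's owning controller as instigator.
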(event EventOnProjectileDamagedCharacter
  (params (Character :type Advanced%20Character%20Object%20Reference) (bWillKill :type Boolean) (WorldLocation :type Vector%20%28by%20ref%29 :default "0, 0, 0") (bone :type Name%20%28by%20ref%29 :default "None"))
  (|CallParentFunction Character bWillKill WorldLocation bone)
  (Networking|SwitchHasAuthority
    (:Authority
      (if (not bWillKill)
        (if (> (Variables|Default|GetFireDamage) 0.0)
          (bind _returnvalue (Class|MordhauProjectile|GetProjectileOwningController))
          (Class|AdvancedCharacter|StartBurning Character (Variables|Default|GetFireDuration) (Variables|Default|GetFireDamage) (Variables|Default|GetFireTick) 0 _returnvalue))))))

(event EventBeginPlay)

(event EventActorBeginOverlap
  (params (OtherActor :type Actor%20Object%20Reference)))

(event EventTick
  (params (DeltaSeconds :type Float%20%28single-precision%29)))

(fn ConstructionScript)