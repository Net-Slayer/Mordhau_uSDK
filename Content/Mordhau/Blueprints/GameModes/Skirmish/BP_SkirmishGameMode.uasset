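; Skirmish game mode: round-based team elimination with an optional capture point and coins for enemy kills.
; Tick drives waiting, start, play and end stages stored in the game state, closing spawns late and barring dead players from respawning.
; Rounds end by wipe, timeout or capture points, which are mirrored to the game state.
; Round start stores gear, resets the world and respawns players, with an optional halftime swap of teams, scores and economy.
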(event EventOnKilled
  (params (Killer :type Controller%20Object%20Reference) (KilledPlayer :type Controller%20Object%20Reference) (KilledPawn :type Pawn%20Object%20Reference) (Type :type EMordhauDamageType%20Enum :default "Generic") (SubType :type Byte :default 0) (DamageSource :type Actor%20Object%20Reference) (DamageAgent :type Actor%20Object%20Reference))
  (Utilities|FlowControl|Sequence
    (:then_0
      (bind _asbp_skirmish_game_state (Utilities|Casting|CastToBP_SkirmishGameState (Game|GetGameState)))
      (if (not (Utilities|Enum|Equal(Enum) (.Stage (Utilities|Struct|BreakSTRUCT_SkirmishRoundInfo (Variables|/Game/Mordhau/Blueprints/GameModes/Skirmish/BP_SkirmishGameState.BP_SkirmishGameState_C|GetRoundInfo _asbp_skirmish_game_state))) "NewEnumerator0"))
        (if (Class|GameMode|IsMatchinProgress)
          (Utilities|Array|Add (Variables|Default|GetAlreadyDiedArray) KilledPlayer)
          (Utilities|IsValid Killer
            (:Is%20Valid
              (Utilities|IsValid KilledPlayer
                (:Is%20Valid
                  (bind _asmordhau_game_state (Utilities|Casting|CastToMordhauGameState (Game|GetGameState)))
                  (bind _returnvalue (Class|MordhauGameState|IsFriendly _asmordhau_game_state Killer KilledPlayer))
                  (if (not _returnvalue)
                    (bind _asbp_economy_player_state (Utilities|Casting|CastToBP_EconomyPlayerState (Variables|/Script/Engine.Controller|GetPlayerState Killer)))
                    (Default|GiveCoins _asbp_economy_player_state (Variables|Default|GetCoinsPerKill))))))))))
    (:then_1
      (|CallParentFunction Killer KilledPlayer KilledPawn Type SubType DamageSource DamageAgent))))

(event EventBeginPlay
  (|CallParentFunction)
  (bind _outactors (Actor|GetAllActorsOfClass "/Game/Mordhau/Blueprints/GameModes/Skirmish/BP_SkirmishCapturePoint.BP_SkirmishCapturePoint_C"))
  (if (> (Utilities|Array|Length _outactors) 0)
    (bind _output_get (Variables|Default|SetCapturePoint (Utilities|Array|Get(acopy) _outactors)))
    (bind _asbp_skirmish_game_state (Utilities|Casting|CastToBP_SkirmishGameState (Game|GetGameState)))
    (Variables|/Game/Mordhau/Blueprints/GameModes/Skirmish/BP_SkirmishGameState.BP_SkirmishGameState_C|SetCapturePoint _asbp_skirmish_game_state _output_get)))

(event EventTick
  (params (DeltaSeconds :type Float%20%28single-precision%29))
  (bind _capturepoint (Variables|Default|GetCapturePoint))
  (bind _roundpointsperteam (Variables|Default|GetRoundPointsPerTeam))
  (bind _owningteam (Variables|/Script/Mordhau.ControlPoint|GetOwningTeam _capturepoint))
  (bind _returnvalue (Math|Conversions|ToInteger(Byte) _owningteam))
  (bind _output (Utilities|Array|Get(acopy) _roundpointsperteam _returnvalue))
  (if (Class|GameMode|IsMatchinProgress)
    (bind _asbp_skirmish_game_state (Utilities|Casting|CastToBP_SkirmishGameState (Game|GetGameState)))
    (switch Utilities|FlowControl|Switch|SwitchonE_SkirmishRoundStage (.Stage (Utilities|Struct|BreakSTRUCT_SkirmishRoundInfo (Variables|/Game/Mordhau/Blueprints/GameModes/Skirmish/BP_SkirmishGameState.BP_SkirmishGameState_C|GetRoundInfo _asbp_skirmish_game_state)))
      (:NewEnumerator0
        (Utilities|Array|Clear (Variables|Default|GetAlreadyDiedArray))
        (bind _return (CallFunction|CanStartRound))
        (if _return
          (CallFunction|StartRoundStart)))
      (:NewEnumerator1
        (if (>= (GameState|GetServerWorldTimeSeconds _asbp_skirmish_game_state) (+ (.StartTime (Utilities|Struct|BreakSTRUCT_SkirmishRoundInfo (Variables|/Game/Mordhau/Blueprints/GameModes/Skirmish/BP_SkirmishGameState.BP_SkirmishGameState_C|GetRoundInfo _asbp_skirmish_game_state))) (Variables|/Game/Mordhau/Blueprints/GameModes/Skirmish/BP_SkirmishGameState.BP_SkirmishGameState_C|GetRoundStartDuration _asbp_skirmish_game_state)))
          (bind _return_2 (CallFunction|CanStartRound))
          (if _return_2
            (CallFunction|StartRound)
            (else
              (CallFunction|StartWaitingforPlayers)))))
      (:NewEnumerator2
        (if (>= (GameState|GetServerWorldTimeSeconds _asbp_skirmish_game_state) (+ (.StartTime (Utilities|Struct|BreakSTRUCT_SkirmishRoundInfo (Variables|/Game/Mordhau/Blueprints/GameModes/Skirmish/BP_SkirmishGameState.BP_SkirmishGameState_C|GetRoundInfo _asbp_skirmish_game_state))) (Variables|/Game/Mordhau/Blueprints/GameModes/Skirmish/BP_SkirmishGameState.BP_SkirmishGameState_C|GetRoundDuration _asbp_skirmish_game_state)))
          (CallFunction|EndRound false :!label _label)
          (else
            (Utilities|FlowControl|Sequence
              (:then_0
                (if (>= (GameState|GetServerWorldTimeSeconds _asbp_skirmish_game_state) (+ (.StartTime (Utilities|Struct|BreakSTRUCT_SkirmishRoundInfo (Variables|/Game/Mordhau/Blueprints/GameModes/Skirmish/BP_SkirmishGameState.BP_SkirmishGameState_C|GetRoundInfo _asbp_skirmish_game_state))) (Variables|/Game/Mordhau/Blueprints/GameModes/Skirmish/BP_SkirmishGameState.BP_SkirmishGameState_C|GetLateRoundSpawnDuration _asbp_skirmish_game_state)))
                  (Variables|/Script/Mordhau.MordhauGameState|SetbAllowSpawning _asbp_skirmish_game_state false)))
              (:then_1
                (bind _return_3 (CallFunction|MoreThanOneTeamAlive))
                (if _return_3
                  (Utilities|IsValid _capturepoint
                    (:Is%20Valid
                      (if (!= _owningteam 255)
                        (Utilities|Array|SetArrayElem _roundpointsperteam _returnvalue (+ _output 1.0))
                        (CallFunction|UpdateStateReplicatedPoints)
                        (if (>= _output (Variables|Default|GetCapturePointTimeToWin))
                          (goto _label)))))
                  (else
                    (CallFunction|EndRound true))))))))
      (:NewEnumerator3
        (bind _return_4 (CallFunction|CanStartRound))
        (if _return_4
          (if (>= (GameState|GetServerWorldTimeSeconds _asbp_skirmish_game_state) (+ (.StartTime (Utilities|Struct|BreakSTRUCT_SkirmishRoundInfo (Variables|/Game/Mordhau/Blueprints/GameModes/Skirmish/BP_SkirmishGameState.BP_SkirmishGameState_C|GetRoundInfo _asbp_skirmish_game_state))) (Variables|/Game/Mordhau/Blueprints/GameModes/Skirmish/BP_SkirmishGameState.BP_SkirmishGameState_C|GetRoundEndDuration _asbp_skirmish_game_state)))
            (CallFunction|StartRoundStart))
          (else
            (CallFunction|StartWaitingforPlayers)))))))

(fn ConstructionScript
  (|CallParentFunction))

(fn StartRoundStart
  (bind _capturepoint (Variables|Default|GetCapturePoint))
  (bind _roundpointsperteam (Variables|Default|GetRoundPointsPerTeam))
  (Variables|Default|SetbIsScoringDisabled true)
  (bind _asbp_skirmish_game_state (Utilities|Casting|CastToBP_SkirmishGameState (Game|GetGameState)))
  (Utilities|FlowControl|Sequence
    (:then_0
      (bind _outactors (Actor|GetAllActorsOfClass "/Script/Engine.Controller"))
      (for _array_element _outactors
        (Utilities|FlowControl|Sequence
          (:then_0
            (LocalVariables|SetEcoCharacter 0)
            (bind _asbp_economy_character (Utilities|Casting|CastToBP_EconomyCharacter (Pawn|GetControlledPawn _array_element))
              (:then
                (LocalVariables|SetEcoCharacter _asbp_economy_character))
              (:CastFailed
                (bind _asmordhau_vehicle (Utilities|Casting|CastToMordhauVehicle (Pawn|GetControlledPawn _array_element)))
                (bind _asbp_economy_character_2 (Utilities|Casting|CastToBP_EconomyCharacter (Variables|/Script/Mordhau.MordhauVehicle|GetDriver _asmordhau_vehicle)))
                (LocalVariables|SetEcoCharacter _asbp_economy_character_2))))
          (:then_1
            (Utilities|IsValid (LocalVariables|GetEcoCharacter)
              (:Is%20Valid
                (Default|StoreGear (LocalVariables|GetEcoCharacter))))))))
    (:then_1
      (if (and (Variables|/Game/Mordhau/Blueprints/GameModes/Skirmish/BP_SkirmishGameState.BP_SkirmishGameState_C|GetTeamSwapAtHalftime _asbp_skirmish_game_state) (not (Variables|Default|GetHasSwappedTeams)))
        (if (== (+ (Utilities|Array|Get(acopy) (Variables|/Script/Mordhau.MordhauGameState|GetTeamScores _asbp_skirmish_game_state)) (Utilities|Array|Get(acopy) (Variables|/Script/Mordhau.MordhauGameState|GetTeamScores _asbp_skirmish_game_state) 1)) 6.0)
          (CallFunction|SwapTeams))))
    (:then_2
      (bind _outactors_2 (Actor|GetAllActorsOfClass "/Script/Mordhau.MordhauActor"))
      (for _array_element_2 _outactors_2
        (Utilities|IsValid _array_element_2
          (:Is%20Valid
            (bind _asmordhau_equipment (Utilities|Casting|CastToMordhauEquipment _array_element_2)
              (:then
                (if (Variables|/Script/Mordhau.MordhauEquipment|GetbAllowCleanup _asmordhau_equipment)
                  (Utilities|Casting|CastToBP_CharacterDoll (Class|MordhauEquipment|GetParentCharacter _asmordhau_equipment)
                    (:CastFailed
                      (Actor|DestroyActor _asmordhau_equipment)))))
              (:CastFailed
                (Utilities|Casting|CastToMordhauProjectile _array_element_2
                  (:then
                    (Actor|DestroyActor _array_element_2 :!label _label))
                  (:CastFailed
                    (Utilities|Casting|CastToBP_DestroyableDeployCover _array_element_2
                      (:then
                        (goto _label))
                      (:CastFailed
                        (Utilities|Casting|CastToBP_DestroyableDeploySpikeWall _array_element_2
                          (:then
                            (goto _label))
                          (:CastFailed
                            (bind _asbp_destroyable_actor (Utilities|Casting|CastToBP_DestroyableActor _array_element_2))
                            (if (Variables|/Game/Mordhau/Blueprints/Interactables/Environment/BP_DestroyableActor.BP_DestroyableActor_C|GetRepairable _asbp_destroyable_actor)
                              (Default|SetHealth _asbp_destroyable_actor (Variables|/Game/Mordhau/Blueprints/Interactables/Environment/BP_DestroyableActor.BP_DestroyableActor_C|GetSpawnHealth _asbp_destroyable_actor))
                              (bind _asbp_door (Utilities|Casting|CastToBP_Door _asbp_destroyable_actor))
                              (if (!= (Default|ConvertStartingStatetoDoorState _asbp_door (Variables|/Game/Mordhau/Blueprints/Interactables/Environment/BP_Door.BP_Door_C|GetStartingState _asbp_door)) (Variables|/Game/Mordhau/Blueprints/Interactables/Environment/BP_Door.BP_Door_C|GetDoorState _asbp_door))
                                (Variables|/Game/Mordhau/Blueprints/Interactables/Environment/BP_Door.BP_Door_C|SetDoorState _asbp_door (Default|ConvertStartingStatetoDoorState _asbp_door (Variables|/Game/Mordhau/Blueprints/Interactables/Environment/BP_Door.BP_Door_C|GetStartingState _asbp_door))))))))))))))))
      (bind _outactors_3 (Actor|GetAllActorsOfClass "/Game/Mordhau/Blueprints/Interactables/SiegeEngines/BP_DeployableBallista.BP_DeployableBallista_C"))
      (for _array_element_3 _outactors_3
        (Actor|DestroyActor _array_element_3)))
    (:then_3
      (for _index (range 0 (- (Utilities|Array|Length _roundpointsperteam) 1))
        (Utilities|Array|SetArrayElem _roundpointsperteam _index 0.0))
      (CallFunction|UpdateStateReplicatedPoints))
    (:then_4
      (Utilities|IsValid _capturepoint
        (:Is%20Valid
          (Default|RoundStarted _capturepoint))))
    (:then_5
      (Utilities|Array|Clear (Variables|Default|GetAlreadyDiedArray))
      (Variables|/Game/Mordhau/Blueprints/GameModes/Skirmish/BP_SkirmishGameState.BP_SkirmishGameState_C|SetRoundInfo _asbp_skirmish_game_state (Utilities|Struct|MakeSTRUCT_SkirmishRoundInfo "NewEnumerator1" 0 (GameState|GetServerWorldTimeSeconds (Game|GetGameState))))
      (Variables|/Script/Mordhau.MordhauGameState|SetbAllowSpawning _asbp_skirmish_game_state true)
      (bind _outactors_4 (Actor|GetAllActorsOfClass "/Script/Engine.Controller"))
      (for _array_element_4 _outactors_4
        (bind _asmordhau_player_state (Utilities|Casting|CastToMordhauPlayerState (Variables|/Script/Engine.Controller|GetPlayerState _array_element_4)))
        (if (>= (Variables|/Script/Mordhau.MordhauPlayerState|GetTeam _asmordhau_player_state) 0)
          (CallFunction|UnpossessandDestroyPawn _array_element_4 true))))))

(fn EndRound
  (params (IsWipe :type Boolean))
  (Utilities|FlowControl|Sequence
    (:then_0
      (bind _asbp_skirmish_game_state (Utilities|Casting|CastToBP_SkirmishGameState (Game|GetGameState)))
      (if IsWipe
        (bind _returnvalue (Class|MordhauGameState|GetPlayerCountsPerTeam _asbp_skirmish_game_state true false :!label _label))
        (if (.bFoundDraw (Class|MordhauUtilityLibrary|GetMaxIndexwithDraw _returnvalue))
          (LocalVariables|SetWinner 255)
          (Variables|/Game/Mordhau/Blueprints/GameModes/Skirmish/BP_SkirmishGameState.BP_SkirmishGameState_C|SetRoundInfo _asbp_skirmish_game_state (Utilities|Struct|MakeSTRUCT_SkirmishRoundInfo "NewEnumerator3" (LocalVariables|GetWinner) (GameState|GetServerWorldTimeSeconds (Game|GetGameState))) :!label _label_2)
          (Variables|/Script/Mordhau.MordhauGameState|SetbAllowSpawning _asbp_skirmish_game_state false)
          (else
            (LocalVariables|SetWinner (Math|Conversions|ToByte(Integer) (.ReturnValue (Class|MordhauUtilityLibrary|GetMaxIndexwithDraw _returnvalue))))
            (Class|MordhauGameMode|AddTeamScore (Math|Conversions|ToInteger(Byte) (LocalVariables|GetWinner)) 1.0 :!label _label_3)
            (if (>= (Utilities|Array|Get(acopy) (Variables|/Script/Mordhau.MordhauGameState|GetTeamScores _asbp_skirmish_game_state) (Math|Conversions|ToInteger(Byte) (LocalVariables|GetWinner))) (Math|Conversions|ToFloat(Integer) (Variables|/Game/Mordhau/Blueprints/GameModes/Skirmish/BP_SkirmishGameState.BP_SkirmishGameState_C|GetWinConditionRounds _asbp_skirmish_game_state)))
              (Class|GameMode|EndMatch)
              (Variables|/Game/Mordhau/Blueprints/GameModes/BP_MordhauGameState.BP_MordhauGameState_C|SetMatchEndInfo _asbp_skirmish_game_state (Utilities|Struct|MakeSTRUCT_MatchEndInfo 0 (Math|Conversions|ToInteger(Byte) (LocalVariables|GetWinner)) (Utilities|Array|Get(acopy) (Variables|/Script/Mordhau.MordhauGameState|GetTeamScores _asbp_skirmish_game_state) (Math|Conversions|ToInteger(Byte) (LocalVariables|GetWinner)))))
              (elif (Variables|/Game/Mordhau/Blueprints/GameModes/Skirmish/BP_SkirmishGameState.BP_SkirmishGameState_C|GetTeamSwapAtHalftime _asbp_skirmish_game_state)
                (if (>= (+ (Utilities|Array|Get(acopy) (Variables|/Script/Mordhau.MordhauGameState|GetTeamScores _asbp_skirmish_game_state)) (Utilities|Array|Get(acopy) (Variables|/Script/Mordhau.MordhauGameState|GetTeamScores _asbp_skirmish_game_state) 1)) (* (- (Math|Conversions|ToFloat(Integer) (Variables|/Game/Mordhau/Blueprints/GameModes/Skirmish/BP_SkirmishGameState.BP_SkirmishGameState_C|GetWinConditionRounds _asbp_skirmish_game_state)) 1.0) 2.0))
                  (Class|GameMode|EndMatch)
                  (Variables|/Game/Mordhau/Blueprints/GameModes/BP_MordhauGameState.BP_MordhauGameState_C|SetMatchEndInfo _asbp_skirmish_game_state (Utilities|Struct|MakeSTRUCT_MatchEndInfo 0 0 0.0 0.0 true))
                  (else
                    (goto _label_2)))
                (else
                  (goto _label_2))))))
        (elif (== (Utilities|Array|Get(acopy) (Variables|/Game/Mordhau/Blueprints/GameModes/Skirmish/BP_SkirmishGameState.BP_SkirmishGameState_C|GetRoundPointsPerTeam _asbp_skirmish_game_state)) (Utilities|Array|Get(acopy) (Variables|/Game/Mordhau/Blueprints/GameModes/Skirmish/BP_SkirmishGameState.BP_SkirmishGameState_C|GetRoundPointsPerTeam _asbp_skirmish_game_state) 1))
          (goto _label)
          (elif (> (Utilities|Array|Get(acopy) (Variables|/Game/Mordhau/Blueprints/GameModes/Skirmish/BP_SkirmishGameState.BP_SkirmishGameState_C|GetRoundPointsPerTeam _asbp_skirmish_game_state)) (Utilities|Array|Get(acopy) (Variables|/Game/Mordhau/Blueprints/GameModes/Skirmish/BP_SkirmishGameState.BP_SkirmishGameState_C|GetRoundPointsPerTeam _asbp_skirmish_game_state) 1))
            (LocalVariables|SetWinner 0)
            (goto _label_3)
            (else
              (LocalVariables|SetWinner 1)
              (goto _label_3))))))
    (:then_1
      (Variables|Default|SetbIsScoringDisabled true))))

(fn MoreThanOneTeamAlive
  (bind _asbp_skirmish_game_state (Utilities|Casting|CastToBP_SkirmishGameState (Game|GetGameState)))
  (if (Variables|/Script/Mordhau.MordhauGameState|GetbAllowSpawning _asbp_skirmish_game_state)
    (return true)
    (else
      (bind _returnvalue (Class|MordhauGameState|GetPlayerCountsPerTeam _asbp_skirmish_game_state true false))
      (for _array_element _returnvalue
        (if (> _array_element 0)
          (if (LocalVariables|GetFoundLivingTeam)
            (return true)
            (else
              (LocalVariables|SetFoundLivingTeam true)))))
      (return false))))

(fn ControllerCanRestart
  (params (Controller :type Controller%20Object%20Reference))
  (bind _returnvalue (|CallParentFunction Controller))
  (return (and _returnvalue (not (Utilities|Array|ContainsItem (Variables|Default|GetAlreadyDiedArray) Controller)))))

(fn StartWaitingforPlayers
  (Variables|Default|SetbIsScoringDisabled true)
  (bind _asbp_skirmish_game_state (Utilities|Casting|CastToBP_SkirmishGameState (Game|GetGameState)))
  (Utilities|Array|Clear (Variables|Default|GetAlreadyDiedArray))
  (Variables|/Game/Mordhau/Blueprints/GameModes/Skirmish/BP_SkirmishGameState.BP_SkirmishGameState_C|SetRoundInfo _asbp_skirmish_game_state (Utilities|Struct|MakeSTRUCT_SkirmishRoundInfo "NewEnumerator0" 0 (Utilities|Time|GetTimeSeconds)))
  (Variables|/Script/Mordhau.MordhauGameState|SetbAllowSpawning _asbp_skirmish_game_state true))

(fn CanStartRound
  (bind _asbp_skirmish_game_state (Utilities|Casting|CastToBP_SkirmishGameState (Game|GetGameState)))
  (bind _returnvalue (Class|MordhauGameState|GetPlayerCountsPerTeam _asbp_skirmish_game_state false true))
  (for _array_element _returnvalue
    (if (> _array_element 0)
      (if (LocalVariables|GetFoundFirstTeam)
        (return true)
        (else
          (LocalVariables|SetFoundFirstTeam true)))))
  (return false))

(fn StartRound
  (Variables|Default|SetbIsScoringDisabled false)
  (bind _asbp_skirmish_game_state (Utilities|Casting|CastToBP_SkirmishGameState (Game|GetGameState)))
  (Utilities|Array|Clear (Variables|Default|GetAlreadyDiedArray))
  (Variables|/Game/Mordhau/Blueprints/GameModes/Skirmish/BP_SkirmishGameState.BP_SkirmishGameState_C|SetRoundInfo _asbp_skirmish_game_state (Utilities|Struct|MakeSTRUCT_SkirmishRoundInfo "NewEnumerator2" 0 (GameState|GetServerWorldTimeSeconds (Game|GetGameState)))))

(fn UpdateStateReplicatedPoints
  (bind _roundpointsperteam (Variables|Default|GetRoundPointsPerTeam))
  (bind _asbp_skirmish_game_state (Utilities|Casting|CastToBP_SkirmishGameState (Game|GetGameState)))
  (Utilities|Array|Clear (Variables|/Game/Mordhau/Blueprints/GameModes/Skirmish/BP_SkirmishGameState.BP_SkirmishGameState_C|GetRoundPointsPerTeam _asbp_skirmish_game_state))
  (for _index (range 0 (- (Utilities|Array|Length _roundpointsperteam) 1))
    (Utilities|Array|Add (Variables|/Game/Mordhau/Blueprints/GameModes/Skirmish/BP_SkirmishGameState.BP_SkirmishGameState_C|GetRoundPointsPerTeam _asbp_skirmish_game_state) (Math|Conversions|ToByte(Integer) (Math|Float|Floor (Utilities|Array|Get(acopy) _roundpointsperteam _index))))))

(fn SwapTeams
  (Variables|Default|SetHasSwappedTeams true)
  (bind _outactors (Actor|GetAllActorsOfClass "/Script/Engine.Controller"))
  (for _array_element _outactors
    (bind _asmordhau_player_state (Utilities|Casting|CastToMordhauPlayerState (Variables|/Script/Engine.Controller|GetPlayerState _array_element)))
    (Utilities|FlowControl|Sequence
      (:then_0
        (if (>= (Variables|/Script/Mordhau.MordhauPlayerState|GetTeam _asmordhau_player_state) 0)
          (Class|MordhauPlayerState|SetTeam _asmordhau_player_state (Utilities|Select :Index (Variables|/Script/Mordhau.MordhauPlayerState|GetTeam _asmordhau_player_state) :Option%200 1 :Option%201 0))))
      (:then_1
        (bind _asbp_economy_player_controller (Utilities|Casting|CastToBP_EconomyPlayerController _array_element))
        (Default|ResetEconomy _asbp_economy_player_controller))))
  (bind _asbp_skirmish_game_state (Utilities|Casting|CastToBP_SkirmishGameState (Game|GetGameState)))
  (bind _output_get (LocalVariables|SetOldTeamScores (Variables|/Script/Mordhau.MordhauGameState|GetTeamScores _asbp_skirmish_game_state)))
  (Utilities|Array|SetArrayElem (Variables|/Script/Mordhau.MordhauGameState|GetTeamScores _asbp_skirmish_game_state) 0 (Utilities|Array|Get(acopy) _output_get 1))
  (Utilities|Array|SetArrayElem (Variables|/Script/Mordhau.MordhauGameState|GetTeamScores _asbp_skirmish_game_state) 1 (Utilities|Array|Get(acopy) _output_get))
  (Variables|/Game/Mordhau/Blueprints/GameModes/Skirmish/BP_SkirmishGameState.BP_SkirmishGameState_C|SetLastWinner _asbp_skirmish_game_state 255)
  (Variables|/Game/Mordhau/Blueprints/GameModes/Skirmish/BP_SkirmishGameState.BP_SkirmishGameState_C|SetLossStreak _asbp_skirmish_game_state 0))