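; Player controller for Skirmish mode that ties shop availability and countdown to the round state in BP_SkirmishGameState.
; IsShopAvailable returns false in two round stages or without a Skirmish game state, otherwise deferring to the parent.
; GetShopTimeLeft derives a non-negative countdown from round start time, shop duration and server time.
; The shop window spans two stages, with round-start duration deducted in the second; elsewhere it reports zero.
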(event EventBeginPlay
  (|CallParentFunction) ; This node is disabled and will not be called.\nDrag off pins to build functionality.
)

(event EventTick
  (params (DeltaSeconds :type Float%20%28single-precision%29))
  (|CallParentFunction DeltaSeconds) ; This node is disabled and will not be called.\nDrag off pins to build functionality.
)

(fn ConstructionScript
  (|CallParentFunction))

(fn IsShopAvailable
  (bind _asbp_skirmish_game_state (Utilities|Casting|CastToBP_SkirmishGameState (Game|GetGameState))
    (:then
      (if (or (Utilities|Enum|Equal(Enum) (.Stage (Utilities|Struct|BreakSTRUCT_SkirmishRoundInfo (Variables|/Game/Mordhau/Blueprints/GameModes/Skirmish/BP_SkirmishGameState.BP_SkirmishGameState_C|GetRoundInfo _asbp_skirmish_game_state))) "NewEnumerator0") (Utilities|Enum|Equal(Enum) (.Stage (Utilities|Struct|BreakSTRUCT_SkirmishRoundInfo (Variables|/Game/Mordhau/Blueprints/GameModes/Skirmish/BP_SkirmishGameState.BP_SkirmishGameState_C|GetRoundInfo _asbp_skirmish_game_state))) "NewEnumerator3"))
        _
        (else
          (bind _available (|CallParentFunction))
          (return _available))))
    (:CastFailed
      _))
  (return false))

(fn GetShopTimeLeft
  (bind _asbp_skirmish_game_state (Utilities|Casting|CastToBP_SkirmishGameState (Game|GetGameState))
    (:then
      (if (Utilities|Enum|Equal(Enum) (.Stage (Utilities|Struct|BreakSTRUCT_SkirmishRoundInfo (Variables|/Game/Mordhau/Blueprints/GameModes/Skirmish/BP_SkirmishGameState.BP_SkirmishGameState_C|GetRoundInfo _asbp_skirmish_game_state))) "NewEnumerator1")
        (return (Math|Float|Max(Float) (- (+ (.StartTime (Utilities|Struct|BreakSTRUCT_SkirmishRoundInfo (Variables|/Game/Mordhau/Blueprints/GameModes/Skirmish/BP_SkirmishGameState.BP_SkirmishGameState_C|GetRoundInfo _asbp_skirmish_game_state))) (Variables|Default|GetShopDuration)) (GameState|GetServerWorldTimeSeconds _asbp_skirmish_game_state)) 0.0))
        (elif (Utilities|Enum|Equal(Enum) (.Stage (Utilities|Struct|BreakSTRUCT_SkirmishRoundInfo (Variables|/Game/Mordhau/Blueprints/GameModes/Skirmish/BP_SkirmishGameState.BP_SkirmishGameState_C|GetRoundInfo _asbp_skirmish_game_state))) "NewEnumerator2")
          (return (Math|Float|Max(Float) (- (- (+ (.StartTime (Utilities|Struct|BreakSTRUCT_SkirmishRoundInfo (Variables|/Game/Mordhau/Blueprints/GameModes/Skirmish/BP_SkirmishGameState.BP_SkirmishGameState_C|GetRoundInfo _asbp_skirmish_game_state))) (Variables|Default|GetShopDuration)) (Variables|/Game/Mordhau/Blueprints/GameModes/Skirmish/BP_SkirmishGameState.BP_SkirmishGameState_C|GetRoundStartDuration _asbp_skirmish_game_state)) (GameState|GetServerWorldTimeSeconds _asbp_skirmish_game_state)) 0.0))
          (else
            _))))
    (:CastFailed
      _))
  (return 0.0))