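; Skirmish-mode capture point that resets and locks at round start, then unlocks after a delay.
; The replicated Locked flag drives capturability and the lock or gear icon on the floating widget, and refreshes the Skirmish HUD.
; Capturing and owning team changes trigger announcements relative to the local player's team, some with sounds and HUD animations.
; Team colors tint the top-bar and floater widgets, which also pulse while the point flashes.
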(event Custom|Pulse
  (bind _topbar_cap_point_widget (Variables|Default|GetTopBar%20Cap%20Point%20Widget))
  (bind _floaterwidget (Variables|Default|GetFloaterWidget))
  (UserInterface|Animation|PlayAnimation _topbar_cap_point_widget (Variables|/Game/Mordhau/Blueprints/GameModes/Battle/BP_CapPointWidget.BP_CapPointWidget_C|GetPulseAnim _topbar_cap_point_widget) 0.0 0 "Forward" 0.2)
  (Appearance|SetColorandOpacity (Variables|/Game/Mordhau/Blueprints/GameModes/Battle/BP_CapPointWidget.BP_CapPointWidget_C|GetPulse _topbar_cap_point_widget) "(R=1.000000,G=1.000000,B=1.000000,A=1.000000)" :!class /Script/UMG.Image)
  (Utilities|IsValid _floaterwidget
    (:Is%20Valid
      (UserInterface|Animation|PlayAnimation _floaterwidget (Variables|/Game/Mordhau/Blueprints/GameModes/Battle/BP_FloatingCapPointWidget.BP_FloatingCapPointWidget_C|GetPulseAnim _floaterwidget) 0.0 0 "Forward" 0.2)
      (Appearance|SetColorandOpacity (Variables|/Game/Mordhau/Blueprints/GameModes/Battle/BP_FloatingCapPointWidget.BP_FloatingCapPointWidget_C|GetPulse _floaterwidget) "(R=1.000000,G=1.000000,B=1.000000,A=1.000000)" :!class /Script/UMG.Image))))

(event Custom|RoundStarted
  (Class|ControlPoint|SetCaptureProgress 0.0 255 false)
  (Variables|Default|SetLocked true)
  (Utilities|FlowControl|RetriggerableDelay (Variables|Default|GetTimeToUnlock))
  (Variables|Default|SetLocked false))

(event EventBeginPlay
  (|CallParentFunction)
  (CallFunction|UpdateWidgetIcon))

(event EventOnCapturingTeamChanged
  (bind _capturingteam (Variables|Default|GetCapturingTeam))
  (|CallParentFunction)
  (Networking|CanExecuteCosmeticEvents
    (:True
      (if (and (> (Utilities|Time|GetTimeSeconds) 3.0) (Variables|Default|GetShowAnnouncements))
        (if (!= _capturingteam 255)
          (bind _relevance (CallFunction|GetTeamRelevance _capturingteam))
          (bind _asbp_mordhau_hud (Utilities|Casting|CastToBP_MordhauHUD (Class|MordhauUtilityLibrary|GetMordhauHUD)))
          (switch int _relevance
            (:0
              (Default|ShowAnnouncement _asbp_mordhau_hud (Utilities|Text|FormatText "We are capturing the point!") "" 4.0 "NewEnumerator0"))
            (:1
              (Default|ShowAnnouncement _asbp_mordhau_hud (Utilities|Text|FormatText "Enemy is capturing the point!") "" 4.0 "NewEnumerator0")
              (Audio|PlaySound2D 0 2.0 1.0 0.0 0 0))))))))

(event EventOnOwningTeamChanged
  (bind _topbar_cap_point_widget (Variables|Default|GetTopBar%20Cap%20Point%20Widget))
  (bind _owningteam (Variables|Default|GetOwningTeam))
  (|CallParentFunction)
  (Networking|CanExecuteCosmeticEvents
    (:True
      (Utilities|FlowControl|Sequence
        (:then_0
          (if (and (> (Utilities|Time|GetTimeSeconds) 3.0) (Variables|Default|GetShowAnnouncements))
            (if (!= _owningteam 255)
              (bind _relevance (CallFunction|GetTeamRelevance _owningteam))
              (bind _asbp_frontline_hud (Utilities|Casting|CastToBP_FrontlineHUD (Class|MordhauUtilityLibrary|GetMordhauHUD)))
              (Utilities|FlowControl|Sequence
                (:then_0
                  (switch int _relevance
                    (:0
                      (Utilities|FlowControl|Sequence
                        (:then_0
                          (Default|ShowAnnouncement _asbp_frontline_hud (Utilities|Text|FormatText "We have taken the point!") "" 4.0 "NewEnumerator0"))
                        (:then_1
                          (Audio|PlaySound2D 0 2.0 1.0 0.0 0 0)
                          (Utilities|IsValid _topbar_cap_point_widget :!label _label
                            (:Is%20Valid
                              (UserInterface|Animation|PlayAnimation _topbar_cap_point_widget (Variables|/Game/Mordhau/Blueprints/GameModes/Battle/BP_CapPointWidget.BP_CapPointWidget_C|GetCapAnim _topbar_cap_point_widget) 0.0 1 "Forward" 0.8)
                              (Utilities|IsValid (Variables|/Game/Mordhau/Blueprints/GameModes/Battle/BP_FrontlineHUD.BP_FrontlineHUD_C|GetFrontlineHUDWidget _asbp_frontline_hud)
                                (:Is%20Valid
                                  (UserInterface|Animation|PlayAnimation (Variables|/Game/Mordhau/Blueprints/GameModes/Battle/BP_FrontlineHUDWidget.BP_FrontlineHUDWidget_C|GetBP_CapPointInfoPanelWidget (Variables|/Game/Mordhau/Blueprints/GameModes/Battle/BP_FrontlineHUD.BP_FrontlineHUD_C|GetFrontlineHUDWidget _asbp_frontline_hud)) (Variables|/Game/Mordhau/Blueprints/GameModes/Battle/BP_CapPointInfoPanelWidget.BP_CapPointInfoPanelWidget_C|GetFlashAnim (Variables|/Game/Mordhau/Blueprints/GameModes/Battle/BP_FrontlineHUDWidget.BP_FrontlineHUDWidget_C|GetBP_CapPointInfoPanelWidget (Variables|/Game/Mordhau/Blueprints/GameModes/Battle/BP_FrontlineHUD.BP_FrontlineHUD_C|GetFrontlineHUDWidget _asbp_frontline_hud))) 0.0 1 "Forward" 1.0))))))))
                    (:1
                      (Utilities|FlowControl|Sequence
                        (:then_0
                          (Default|ShowAnnouncement _asbp_frontline_hud (Utilities|Text|FormatText "Enemy has taken the point!") "" 4.0 "NewEnumerator0"))
                        (:then_1
                          (Audio|PlaySound2D 0 2.0 1.0 0.0 0 0)
                          (goto _label))))))))))))))

(event EventUpdateUIWidgets
  (bind _owningteam (Variables|Default|GetOwningTeam))
  (bind _capturingteam (Variables|Default|GetCapturingTeam))
  (bind _returnvalue (Math|Conversions|ToInteger(Byte) _owningteam))
  (bind _returnvalue_2 (Math|Conversions|ToInteger(Byte) _capturingteam))
  (Utilities|FlowControl|Sequence
    (:then_0
      (bind _asmordhau_game_state (Utilities|Casting|CastToMordhauGameState (Game|GetGameState)))
      (if (!= (Variables|Default|GetOwningTeam) 255)
        (if (Utilities|Array|IsValidIndex (Variables|/Script/Mordhau.MordhauGameState|GetTeamColors _asmordhau_game_state) _returnvalue)
          (CallFunction|SetCapPointWidgetColors (Utilities|Array|Get(acopy) (Variables|/Script/Mordhau.MordhauGameState|GetTeamColors _asmordhau_game_state) _returnvalue) (Utilities|Struct|MakeLinearColor (* (.R (Utilities|Struct|BreakLinearColor (Utilities|Array|Get(acopy) (Variables|/Script/Mordhau.MordhauGameState|GetTeamColors _asmordhau_game_state) _returnvalue))) 4.0) (* (.G (Utilities|Struct|BreakLinearColor (Utilities|Array|Get(acopy) (Variables|/Script/Mordhau.MordhauGameState|GetTeamColors _asmordhau_game_state) _returnvalue))) 4.0) (* (.B (Utilities|Struct|BreakLinearColor (Utilities|Array|Get(acopy) (Variables|/Script/Mordhau.MordhauGameState|GetTeamColors _asmordhau_game_state) _returnvalue))) 4.0) (.A (Utilities|Struct|BreakLinearColor (Utilities|Array|Get(acopy) (Variables|/Script/Mordhau.MordhauGameState|GetTeamColors _asmordhau_game_state) _returnvalue))))))
        (elif (Utilities|Array|IsValidIndex (Variables|/Script/Mordhau.MordhauGameState|GetTeamColors _asmordhau_game_state) _returnvalue_2)
          (CallFunction|SetCapPointWidgetColors "(R=0.000000,G=0.000000,B=0.000000,A=0.750000)" (Utilities|Struct|MakeLinearColor (* (.R (Utilities|Struct|BreakLinearColor (Utilities|Array|Get(acopy) (Variables|/Script/Mordhau.MordhauGameState|GetTeamColors _asmordhau_game_state) _returnvalue_2))) 4.0) (* (.G (Utilities|Struct|BreakLinearColor (Utilities|Array|Get(acopy) (Variables|/Script/Mordhau.MordhauGameState|GetTeamColors _asmordhau_game_state) _returnvalue_2))) 4.0) (* (.B (Utilities|Struct|BreakLinearColor (Utilities|Array|Get(acopy) (Variables|/Script/Mordhau.MordhauGameState|GetTeamColors _asmordhau_game_state) _returnvalue_2))) 4.0) (.A (Utilities|Struct|BreakLinearColor (Utilities|Array|Get(acopy) (Variables|/Script/Mordhau.MordhauGameState|GetTeamColors _asmordhau_game_state) _returnvalue_2)))))
          (else
            (CallFunction|SetCapPointWidgetColors "(R=0.000000,G=0.000000,B=0.000000,A=0.750000)" "(R=1.000000,G=1.000000,B=1.000000,A=1.000000)")))))))

(event EventOnStartedFlashing
  (bind _topbar_cap_point_widget (Variables|Default|GetTopBar%20Cap%20Point%20Widget))
  (bind _capwarninganim (Variables|/Game/Mordhau/Blueprints/GameModes/Battle/BP_CapPointWidget.BP_CapPointWidget_C|GetCapWarningAnim _topbar_cap_point_widget))
  (Utilities|Casting|CastToMordhauGameState (Game|GetGameState))
  (Utilities|IsValid _topbar_cap_point_widget
    (:Is%20Valid
      (Class|MordhauUtilityLibrary|GetViewTargetCharacter 0 true)
      (if (Variables|Default|GetFlashShouldOnlyPulse)
        (CallFunction|Pulse)
        (else
          (UserInterface|Animation|PlayAnimation _topbar_cap_point_widget _capwarninganim 0.0 1 "Forward" 1.0) ; Play alert anim first
          (EventDispatchers|AssignOnAnimationFinished _capwarninganim (delegate Custom|Pulse)) ; Then start pulsing when it's done
        )))))

(event EventOnStoppedFlashing
  (bind _topbar_cap_point_widget (Variables|Default|GetTopBar%20Cap%20Point%20Widget))
  (bind _floaterwidget (Variables|Default|GetFloaterWidget))
  (bind _captureprogress (Variables|Default|GetCaptureProgress))
  (bind _returnvalue (== _captureprogress 0.0))
  (bind _pulseanim (Variables|/Game/Mordhau/Blueprints/GameModes/Battle/BP_FloatingCapPointWidget.BP_FloatingCapPointWidget_C|GetPulseAnim _floaterwidget))
  (bind _pulseanim_2 (Variables|/Game/Mordhau/Blueprints/GameModes/Battle/BP_CapPointWidget.BP_CapPointWidget_C|GetPulseAnim _topbar_cap_point_widget))
  (bind _capwarninganim (Variables|/Game/Mordhau/Blueprints/GameModes/Battle/BP_CapPointWidget.BP_CapPointWidget_C|GetCapWarningAnim _topbar_cap_point_widget))
  (Utilities|IsValid _topbar_cap_point_widget
    (:Is%20Valid
      (EventDispatchers|UnbindEventfromOnAnimationFinished _capwarninganim (delegate Custom|Pulse))
      (Utilities|FlowControl|Sequence
        (:then_0
          (if _returnvalue
            (if (Class|UserWidget|IsAnimationPlaying _topbar_cap_point_widget _capwarninganim)
              (Utilities|FlowControl|Delay (- (Class|WidgetAnimation|GetEndTime _capwarninganim) (Class|UserWidget|GetAnimationCurrentTime _topbar_cap_point_widget _capwarninganim))))
            (Class|UserWidget|StopAnimation _topbar_cap_point_widget _pulseanim_2)
            (else
              (UserInterface|Animation|PlayAnimation _topbar_cap_point_widget _pulseanim_2 0.0 1 "Forward" 0.2))))
        (:then_1
          (Utilities|IsValid _floaterwidget
            (:Is%20Valid
              (if _returnvalue
                (Class|UserWidget|StopAnimation _floaterwidget _pulseanim)
                (else
                  (UserInterface|Animation|PlayAnimation _floaterwidget _pulseanim 0.0 1 "Forward" 0.2))))))))))

(fn ConstructionScript
  (Variables|Default|SetCaptureArea (Variables|Components|GetCaptureAreaCollision))
  (Variables|Default|SetWidgetComponent (Variables|Components|GetMordhauWidget)))

(fn GetTeamRelevance
  (params (Team :type Byte))
  (bind _returnvalue (Game|GetPlayerController 0))
  (Utilities|IsValid _returnvalue
    (:Is%20Valid
      (bind _asmordhau_player_state (Utilities|Casting|CastToMordhauPlayerState (Variables|/Script/Engine.Controller|GetPlayerState _returnvalue))
        (:then
          (if (or (== (Variables|/Script/Mordhau.MordhauPlayerState|GetTeam _asmordhau_player_state) 0) (== (Variables|/Script/Mordhau.MordhauPlayerState|GetTeam _asmordhau_player_state) 1))
            (return (Math|Conversions|ToInteger(Boolean) (!= (Math|Conversions|ToInteger(Byte) Team) (Variables|/Script/Mordhau.MordhauPlayerState|GetTeam _asmordhau_player_state))))
            (else
              _)))
        (:CastFailed
          _)))
    (:Is%20Not%20Valid
      _))
  (return 2))

(fn SetCapPointWidgetColors
  (params (Fill%20Color :type Linear%20Color%20Structure) (Progress%20Bar%20Color :type Linear%20Color%20Structure))
  (bind _topbar_cap_point_widget (Variables|Default|GetTopBar%20Cap%20Point%20Widget))
  (bind _floaterwidget (Variables|Default|GetFloaterWidget))
  (Utilities|FlowControl|Sequence
    (:then_0
      (Utilities|IsValid _topbar_cap_point_widget
        (:Is%20Valid
          (Appearance|SetColorandOpacity (Variables|/Game/Mordhau/Blueprints/GameModes/Battle/BP_CapPointWidget.BP_CapPointWidget_C|GetFill _topbar_cap_point_widget) Fill%20Color :!class /Script/UMG.Image)
          (Appearance|SetColorandOpacity (Variables|/Game/Mordhau/Blueprints/GameModes/Battle/BP_CapPointWidget.BP_CapPointWidget_C|GetCapProgressBar _topbar_cap_point_widget) Progress%20Bar%20Color :!class /Script/UMG.Image))))
    (:then_1
      (Utilities|IsValid _floaterwidget
        (:Is%20Valid
          (Appearance|SetColorandOpacity (Variables|/Game/Mordhau/Blueprints/GameModes/Battle/BP_FloatingCapPointWidget.BP_FloatingCapPointWidget_C|GetCap _floaterwidget) Progress%20Bar%20Color :!class /Script/UMG.Image))))))

(fn OnRepActive)

(fn OnRepLocked
  (Variables|Default|SetbIsCapturable (not (Variables|Default|GetLocked)))
  (CallFunction|UpdateWidgetIcon))

(fn UpdateWidgetIcon
  (Networking|CanExecuteCosmeticEvents
    (:True
      (Utilities|FlowControl|Sequence
        (:then_0
          (bind _asbp_floating_cap_point_widget (Utilities|Casting|CastToBP_FloatingCapPointWidget (UserInterface|GetUserWidgetObject (Variables|Components|GetMordhauWidget))))
          (Variables|Default|SetFloaterWidget _asbp_floating_cap_point_widget)
          (Variables|/Game/Mordhau/Blueprints/GameModes/Battle/BP_FloatingCapPointWidget.BP_FloatingCapPointWidget_C|SetBrush _asbp_floating_cap_point_widget (Class|WidgetBlueprintLibrary|MakeBrushfromMaterial (Variables|Default|GetUIMaterialInstance) 48 48))
          (Appearance|SetBrushfromTexture (Variables|/Game/Mordhau/Blueprints/GameModes/Battle/BP_FloatingCapPointWidget.BP_FloatingCapPointWidget_C|GetIcon _asbp_floating_cap_point_widget) (select (Variables|Default|GetLocked) "/Game/Mordhau/UI/UIAssets/Textures/ic_lock.ic_lock" "/Game/Mordhau/UI/UIAssets/Textures/IC_gear.IC_gear") false))
        (:then_1
          (bind _asbp_skirmish_hud (Utilities|Casting|CastToBP_SkirmishHUD (Class|MordhauUtilityLibrary|GetMordhauHUD)))
          (Default|UpdateCapPointWidget _asbp_skirmish_hud))))))