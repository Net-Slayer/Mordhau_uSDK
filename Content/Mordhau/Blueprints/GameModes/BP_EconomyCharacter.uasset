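; Economy game mode character that carries a player's gear between lives by recording it on BP_EconomyPlayerController.
; Armor changes are saved to the controller on authority as each slot replicates.
; On death, WipeGearOnDeath decides between clearing all saved gear and storing equipment classes with ammo, with fists and invalid slots saved as empty entries.
; When that flag is set, possession also applies the pending character profile to the customization replication actor.
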(event EventBeginPlay
  (|CallParentFunction))

(event Collision|EventActorBeginOverlap
  (params (OtherActor :type Actor%20Object%20Reference))
  (|CallParentFunction OtherActor) ; This node is disabled and will not be called.\nDrag off pins to build functionality.
)

(event EventTick
  (params (DeltaSeconds :type Float%20%28single-precision%29))
  (|CallParentFunction DeltaSeconds) ; This node is disabled and will not be called.\nDrag off pins to build functionality.
)

(event EventPossessed
  (params (NewController :type Controller%20Object%20Reference))
  (Utilities|FlowControl|Sequence
    (:then_0
      (bind _asbp_economy_player_controller (Utilities|Casting|CastToBP_EconomyPlayerController NewController))
      (if (Variables|/Game/Mordhau/Blueprints/GameModes/BP_EconomyPlayerController.BP_EconomyPlayerController_C|GetWipeGearOnDeath _asbp_economy_player_controller)
        (Utilities|IsValid (Variables|/Script/Mordhau.MordhauPlayerController|GetCustomizationReplicationActor _asbp_economy_player_controller)
          (:Is%20Valid
            (Class|CustomizationReplicationActor|AssignDatafromProfile (Variables|/Script/Mordhau.MordhauPlayerController|GetCustomizationReplicationActor _asbp_economy_player_controller) (Variables|/Script/Mordhau.MordhauPlayerController|GetPendingCharacterProfile _asbp_economy_player_controller))))))
    (:then_1
      (|CallParentFunction NewController))))

(event EventOnArmorReplicated
  (params (Slot :type EWearableSlot%20Enum :default "Head"))
  (|CallParentFunction Slot)
  (bind _asbp_economy_player_controller (Utilities|Casting|CastToBP_EconomyPlayerController (Pawn|GetController)))
  (if (Ability|HasAuthority _asbp_economy_player_controller)
    (switch Utilities|FlowControl|Switch|SwitchonEWearableSlot Slot
      (:Head
        (Variables|/Game/Mordhau/Blueprints/GameModes/BP_EconomyPlayerController.BP_EconomyPlayerController_C|SetLastHeadArmor _asbp_economy_player_controller (Variables|Default|GetHeadArmor)))
      (:UpperChest
        (Variables|/Game/Mordhau/Blueprints/GameModes/BP_EconomyPlayerController.BP_EconomyPlayerController_C|SetLastChestArmor _asbp_economy_player_controller (Variables|Default|GetChestArmor)))
      (:Legs
        (Variables|/Game/Mordhau/Blueprints/GameModes/BP_EconomyPlayerController.BP_EconomyPlayerController_C|SetLastLegArmor _asbp_economy_player_controller (Variables|Default|GetLegArmor))))))

(event EventOnKilled
  (params (EventInstigator :type Controller%20Object%20Reference))
  (Utilities|FlowControl|Sequence
    (:then_0
      (bind _asbp_economy_player_controller (Utilities|Casting|CastToBP_EconomyPlayerController (Class|AdvancedCharacter|GetControllerIncludingVehicle)))
      (if (Variables|/Game/Mordhau/Blueprints/GameModes/BP_EconomyPlayerController.BP_EconomyPlayerController_C|GetWipeGearOnDeath _asbp_economy_player_controller)
        (CallFunction|WipeGear)
        (else
          (CallFunction|StoreGear))))
    (:then_1
      (|CallParentFunction EventInstigator))))

(fn ConstructionScript
  (|CallParentFunction))

(fn StoreGear
  (bind _asbp_economy_player_controller (Utilities|Casting|CastToBP_EconomyPlayerController (Class|AdvancedCharacter|GetControllerIncludingVehicle)))
  (Utilities|Array|Clear (Variables|/Game/Mordhau/Blueprints/GameModes/BP_EconomyPlayerController.BP_EconomyPlayerController_C|GetLastEquipment _asbp_economy_player_controller))
  (Utilities|Array|Clear (Variables|/Game/Mordhau/Blueprints/GameModes/BP_EconomyPlayerController.BP_EconomyPlayerController_C|GetLastEquipmentAmmo _asbp_economy_player_controller))
  (for _array_element (Variables|Default|GetEquipment)
    (Utilities|IsValid _array_element
      (:Is%20Valid
        (Utilities|Casting|CastToFistsWeapon _array_element
          (:then
            (Utilities|Array|Add (Variables|/Game/Mordhau/Blueprints/GameModes/BP_EconomyPlayerController.BP_EconomyPlayerController_C|GetLastEquipment _asbp_economy_player_controller) 0 :!label _label)
            (Utilities|Array|Add (Variables|/Game/Mordhau/Blueprints/GameModes/BP_EconomyPlayerController.BP_EconomyPlayerController_C|GetLastEquipmentAmmo _asbp_economy_player_controller) 0))
          (:CastFailed
            (Utilities|Array|Add (Variables|/Game/Mordhau/Blueprints/GameModes/BP_EconomyPlayerController.BP_EconomyPlayerController_C|GetLastEquipment _asbp_economy_player_controller) (Utilities|GetClass _array_element))
            (Utilities|Array|Add (Variables|/Game/Mordhau/Blueprints/GameModes/BP_EconomyPlayerController.BP_EconomyPlayerController_C|GetLastEquipmentAmmo _asbp_economy_player_controller) (Class|MordhauEquipment|GetAmmo _array_element)))))
      (:Is%20Not%20Valid
        (goto _label)))))

(fn WipeGear
  (bind _asbp_economy_player_controller (Utilities|Casting|CastToBP_EconomyPlayerController (Class|AdvancedCharacter|GetControllerIncludingVehicle)))
  (Utilities|Array|Clear (Variables|/Game/Mordhau/Blueprints/GameModes/BP_EconomyPlayerController.BP_EconomyPlayerController_C|GetLastEquipment _asbp_economy_player_controller))
  (Utilities|Array|Clear (Variables|/Game/Mordhau/Blueprints/GameModes/BP_EconomyPlayerController.BP_EconomyPlayerController_C|GetLastEquipmentAmmo _asbp_economy_player_controller))
  (Variables|/Game/Mordhau/Blueprints/GameModes/BP_EconomyPlayerController.BP_EconomyPlayerController_C|SetLastChestArmor _asbp_economy_player_controller 0)
  (Variables|/Game/Mordhau/Blueprints/GameModes/BP_EconomyPlayerController.BP_EconomyPlayerController_C|SetLastLegArmor _asbp_economy_player_controller 0)
  (Variables|/Game/Mordhau/Blueprints/GameModes/BP_EconomyPlayerController.BP_EconomyPlayerController_C|SetLastHeadArmor _asbp_economy_player_controller 0))