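; Team Deathmatch game state for Mordhau that displays the match result on the local player's HUD.
; Its match-end handler runs the parent logic, then compares the first player controller's team with the winning team in MatchEndInfo to show victory or defeat.
; Draws show a draw message flagged as non-victory, while players on team -1 always see victory unless the match is drawn.
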(event EventHandleMatchEndInfo
  (bind _matchendinfo (Variables|Default|GetMatchEndInfo))
  (bind (_winner _winnerteam _winnerscore _otherscore _draw) (Utilities|Struct|BreakSTRUCT_MatchEndInfo _matchendinfo))
  (|CallParentFunction)
  (bind _asbp_mordhau_hud (Utilities|Casting|CastToBP_MordhauHUD (Class|MordhauUtilityLibrary|GetMordhauHUD)))
  (bind _asmordhau_player_state (Utilities|Casting|CastToMordhauPlayerState (Variables|/Script/Engine.Controller|GetPlayerState (Game|GetPlayerController 0))))
  (if _draw
    (Default|ShowMatchResult _asbp_mordhau_hud false "draw")
    (elif (or (== (Variables|/Script/Mordhau.MordhauPlayerState|GetTeam _asmordhau_player_state) _winnerteam) (== (Variables|/Script/Mordhau.MordhauPlayerState|GetTeam _asmordhau_player_state) -1))
      (Default|ShowMatchResult _asbp_mordhau_hud true "victory")
      (else
        (Default|ShowMatchResult _asbp_mordhau_hud false "defeat")))))

(event EventTick
  (params (DeltaSeconds :type Float%20%28single-precision%29)))

(fn ConstructionScript
  (|CallParentFunction))