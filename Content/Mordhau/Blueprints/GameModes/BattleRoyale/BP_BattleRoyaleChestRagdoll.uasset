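; Battle Royale chest ragdoll actor that dissolves visually at the end of its lifespan.
; On its first Tick, a DoOnce creates a dynamic instance of the tier 1 chest material on the skeletal mesh's first slot.
; During the final second of life, each Tick feeds the remaining lifespan into that material's Dissolve parameter.
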(event EventBeginPlay)

(event Collision|EventActorBeginOverlap
  (params (OtherActor :type Actor%20Object%20Reference)))

(event EventTick
  (params (DeltaSeconds :type Float%20%28single-precision%29))
  (bind _returnvalue (Actor|GetLifeSpan))
  (Utilities|FlowControl|Sequence
    (:then_0
      (Utilities|FlowControl|DoOnce false
        (:Completed
          (bind _returnvalue_2 (Rendering|Material|CreateDynamicMaterialInstance (Variables|SkeletalMeshActor|GetSkeletalMeshComponent) 0 "/Game/Mordhau/Assets/Interactables/Mesh/BrChests/BrChestTier1_Inst.BrChestTier1_Inst" "None" :!class /Script/Engine.PrimitiveComponent))
          (Variables|Default|SetDynamicMaterial _returnvalue_2))))
    (:then_1
      (if (< _returnvalue 1.0)
        (Rendering|Material|SetScalarParameterValue (Variables|Default|GetDynamicMaterial) "Dissolve" (/ _returnvalue 1.0) :!class /Script/Engine.MaterialInstanceDynamic)))))

(fn ConstructionScript)