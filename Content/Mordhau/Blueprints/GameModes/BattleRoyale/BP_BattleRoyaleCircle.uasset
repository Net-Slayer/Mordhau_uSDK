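; Battle Royale shrinking zone that periodically damages living characters outside its capsule, tracked by overlaps.
; ActivateCircle precomputes nested centers backwards from a random final spot, using rejection sampling with a circle-intersection fallback.
; The server advances timed levels through replicated CircleState and deals damage.
; Tick interpolates mesh, capsule and "PPBR" post-process volume by server time, keeping audio on the edge toward the local camera.
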(event EventBeginPlay
  (bind _outactors (Actor|GetAllActorsOfClass "/Script/Engine.PostProcessVolume"))
  (bind _array_element (Utilities|Array|ForEachLoopwithBreak _outactors :!label _label)
    (:LoopBody
      (if (Utilities|Enum|Equal(Enum) (Utilities|GetObjectName _array_element) "PPBR")
        (Variables|Default|SetCirclePostProcess _array_element)
        (goto _label Break)))
    (:Completed
      (Variables|Default|SetInitialRadius (.radius (Utilities|Array|Get(acopy) (Variables|Default|GetCircleInfoPerLevel)))))))

(event Collision|EventActorBeginOverlap
  (params (OtherActor :type Actor%20Object%20Reference))
  (bind _asadvanced_character (Utilities|Casting|CastToAdvancedCharacter OtherActor))
  (Utilities|Set|Remove (Variables|Default|GetUnsafeCharacters) _asadvanced_character)
  (Utilities|IsValid _asadvanced_character
    (:Is%20Valid
      (if (not (Class|AdvancedCharacter|GetIsDead _asadvanced_character))
        (Utilities|Set|Add (Variables|Default|GetSafeCharacters) _asadvanced_character)))))

(event EventTick
  (params (DeltaSeconds :type Float%20%28single-precision%29))
  (bind _returnvalue (Game|GetPlayerCameraManager 0))
  (bind _returnvalue_2 (Transformation|GetActorLocation))
  (bind _audio (Variables|Default|GetAudio))
  (bind _damageinterval (Variables|Default|GetDamageInterval))
  (bind _circlestate (Variables|Default|GetCircleState))
  (bind (_currentcirclelevel _circlestartservertime) (Utilities|Struct|BreakBP_BattleRoyaleCircleState _circlestate))
  (bind _returnvalue_3 (Transformation|GetActorLocation _returnvalue))
  (bind _asbp_battle_royale_game_state (Utilities|Casting|CastToBP_BattleRoyaleGameState (Game|GetGameState)))
  (if (not (Variables|/Game/Mordhau/Blueprints/GameModes/BP_MordhauGameState.BP_MordhauGameState_C|GetMatchEndInfoReplicated _asbp_battle_royale_game_state))
    (Utilities|FlowControl|Sequence
      (:then_0
        (Networking|SwitchHasAuthority
          (:Authority
            (Utilities|FlowControl|Sequence
              (:then_0
                (if (>= (Utilities|Time|GetTimeSeconds) (+ (.Duration (Utilities|Struct|BreakBP_BattleRoyaleCircleInfo (Utilities|Array|Get(acopy) (Variables|Default|GetCircleInfoPerLevel) (Math|Conversions|ToInteger(Byte) _currentcirclelevel)))) _circlestartservertime))
                  (CallFunction|BeginCircleLevel (+ _currentcirclelevel 1))))
              (:then_1
                (Variables|Default|SetDamageDealTick (+ (Variables|Default|GetDamageDealTick) DeltaSeconds))
                (if (>= (Variables|Default|GetDamageDealTick) _damageinterval)
                  (Variables|Default|SetDamageDealTick (- (Variables|Default|GetDamageDealTick) _damageinterval))
                  (CallFunction|DealDamage)))))))
      (:then_1
        (CallFunction|InterpCircle))
      (:then_2
        (Networking|CanExecuteCosmeticEvents
          (:True
            (Utilities|FlowControl|Sequence
              (:then_0
                (Utilities|FlowControl|DoOnce false
                  (:Completed
                    (Components|Activation|Activate _audio false))))
              (:then_1
                (Transformation|SetWorldLocation _audio (Math|Conversions|ToVector(Vector2D) (+ (* (Math|Vector2D|Normalize2D (Math|Conversions|ToVector2D(Vector) (- _returnvalue_3 _returnvalue_2))) (Variables|/Script/Engine.CapsuleComponent|GetCapsuleRadius (Variables|Default|GetCapsule))) (Math|Conversions|ToVector2D(Vector) _returnvalue_2)) (.Z (Math|Vector|BreakVector _returnvalue_3))) false false)))))))))

(event Collision|EventActorEndOverlap
  (params (OtherActor :type Actor%20Object%20Reference))
  (bind _asadvanced_character (Utilities|Casting|CastToAdvancedCharacter OtherActor))
  (Utilities|Set|Remove (Variables|Default|GetSafeCharacters) _asadvanced_character)
  (Utilities|IsValid _asadvanced_character
    (:Is%20Valid
      (if (not (Class|AdvancedCharacter|GetIsDead _asadvanced_character))
        (Utilities|Set|Add (Variables|Default|GetUnsafeCharacters) _asadvanced_character)))))

(fn ConstructionScript
  (bind _circleinfoperlevel (Variables|Default|GetCircleInfoPerLevel))
  (bind _capsule (Variables|Default|GetCapsule))
  (bind _staticmesh (Variables|Default|GetStaticMesh))
  (bind _output (Utilities|Array|Get(acopy) _circleinfoperlevel))
  (bind _radius (Utilities|Struct|BreakBP_BattleRoyaleCircleInfo _output))
  (bind _returnvalue (* _radius 0.002))
  (if (Utilities|Array|IsValidIndex _circleinfoperlevel)
    (Transformation|SetRelativeScale3D _staticmesh (Math|Vector|MakeVector _returnvalue _returnvalue (.Z (Math|Vector|BreakVector (Variables|/Script/Engine.SceneComponent|GetRelativeScale3D _staticmesh)))))
    (Components|Capsule|SetCapsuleRadius _capsule _radius false)
    (Components|Capsule|SetCapsuleHalfHeight _capsule 2.4e+04 false)))

(fn DealDamage
  (bind _unsafecharacters (Variables|Default|GetUnsafeCharacters))
  (bind _result (Utilities|Set|ToArray _unsafecharacters))
  (for _array_element _result
    (Utilities|IsValid _array_element
      (:Is%20Valid
        (if (Class|AdvancedCharacter|GetIsDead _array_element)
          (Utilities|Set|Remove _unsafecharacters _array_element :!label _label)
          (else
            (bind _asmordhau_character (Utilities|Casting|CastToMordhauCharacter _array_element))
            (Utilities|IsValid (Variables|/Script/Mordhau.MordhauCharacter|GetCurrentVehicle _asmordhau_character)
              (:Is%20Valid
                (if (not (Utilities|Set|Contains (Variables|Default|GetSafeCharacters) (Variables|/Script/Mordhau.MordhauCharacter|GetCurrentVehicle _asmordhau_character)))
                  (Class|AdvancedCharacter|OffsetHealth _array_element (* (Variables|Default|GetDamagePerTick) -1) true :!label _label_2)
                  (if (== (Variables|/Script/Mordhau.AdvancedCharacter|GetHealth _array_element) 0)
                    (Class|AdvancedCharacter|Suicide _array_element)
                    (goto _label))))
              (:Is%20Not%20Valid
                (goto _label_2))))))
      (:Is%20Not%20Valid
        (goto _label)))))

(fn ActivateCircle
  (bind _circlecentersperlevel (Variables|Default|GetCircleCentersPerLevel))
  (bind _circleinfoperlevel (Variables|Default|GetCircleInfoPerLevel))
  (bind _circleinfoperlevel_2 (Variables|Default|GetCircleInfoPerLevel))
  (bind _returnvalue (Utilities|Array|Length _circlecentersperlevel))
  (bind _output (Utilities|Array|Get(acopy) _circleinfoperlevel_2))
  (bind _output_2 (Utilities|Array|Get(acopy) _circlecentersperlevel))
  (bind _radius (Utilities|Struct|BreakBP_BattleRoyaleCircleInfo _output))
  (bind _returnvalue_2 (- _returnvalue 1))
  (Utilities|FlowControl|Sequence
    (:then_0
      ;[1 1 1] Find circle spots working backwards from final spot
      (for _array_element _circleinfoperlevel
        (Utilities|Array|Add :TargetArray _circlecentersperlevel))
      (Utilities|Array|SetArrayElem _circlecentersperlevel 0 (Transformation|GetActorLocation))
      (bind _subcirclecenter (CallFunction|FindRandomCircleCenterInside _radius _output_2 (.Radius (Utilities|Struct|BreakBP_BattleRoyaleCircleInfo (Utilities|Array|Get(acopy) _circleinfoperlevel _returnvalue_2)))))
      (Utilities|Array|SetArrayElem _circlecentersperlevel _returnvalue_2 _subcirclecenter)
      (for _index (range 0 (- _returnvalue 3))
        (bind _desiredcirclecenter (CallFunction|FindRandomCircleBetweenCircles _radius _output_2 (.Radius (Utilities|Struct|BreakBP_BattleRoyaleCircleInfo (Utilities|Array|Get(acopy) _circleinfoperlevel_2 (+ (- (- _returnvalue 2) _index) 1)))) (Utilities|Array|Get(acopy) _circlecentersperlevel (+ (- (- _returnvalue 2) _index) 1)) (.Radius (Utilities|Struct|BreakBP_BattleRoyaleCircleInfo (Utilities|Array|Get(acopy) _circleinfoperlevel_2 (- (- _returnvalue 2) _index))))))
        (Utilities|Array|SetArrayElem _circlecentersperlevel (- (- _returnvalue 2) _index) _desiredcirclecenter)))
    (:then_1
      (CallFunction|BeginCircleLevel)
      (Collision|SetCollisionEnabled (Variables|Default|GetCapsule) "QueryOnly"))))

(fn BeginCircleLevel
  (params (NewLevel :type Byte))
  (bind _returnvalue (Math|Conversions|ToInteger(Byte) NewLevel))
  (bind _circlecentersperlevel (Variables|Default|GetCircleCentersPerLevel))
  (bind _circlecentersperlevel_2 (Variables|Default|GetCircleCentersPerLevel))
  (bind _returnvalue_2 (+ _returnvalue 1))
  (bind _output (Utilities|Array|Get(acopy) _circlecentersperlevel _returnvalue))
  (bind (_x _y _z) (Math|Vector|BreakVector _output))
  (bind _output_2 (Utilities|Array|Get(acopy) _circlecentersperlevel_2 _returnvalue_2))
  (bind (_x_2 _y_2 _z_2) (Math|Vector|BreakVector _output_2))
  (if (Utilities|Array|IsValidIndex (Variables|Default|GetCircleInfoPerLevel) _returnvalue)
    (Utilities|FlowControl|Sequence
      (:then_0
        ;[1 1 1] Find circle start
        (if (== NewLevel 0)
          (LocalVariables|SetNewCircleStart (Math|Vector|MakeVectorNetQuantize _x _y _z))
          (else
            (LocalVariables|SetNewCircleStart (.CircleEndLocation (Utilities|Struct|BreakBP_BattleRoyaleCircleState (Variables|Default|GetCircleState)))))))
      (:then_1
        ;[1 1 1] Find circle end
        (if (Utilities|Array|IsValidIndex (Variables|Default|GetCircleInfoPerLevel) _returnvalue_2)
          (LocalVariables|SetNewCircleEnd (Math|Vector|MakeVectorNetQuantize _x_2 _y_2 _z_2))
          (else
            (LocalVariables|SetNewCircleEnd (LocalVariables|GetNewCircleStart)))))
      (:then_2
        (Variables|Default|SetCircleState (Utilities|Struct|MakeBP_BattleRoyaleCircleState NewLevel (Utilities|Time|GetTimeSeconds) (LocalVariables|GetNewCircleStart) (LocalVariables|GetNewCircleEnd)))))))

(fn OnRepCircleState
  (bind _circlestate (Variables|Default|GetCircleState))
  (bind _circleinfoperlevel (Variables|Default|GetCircleInfoPerLevel))
  (bind _currentcirclelevel (Utilities|Struct|BreakBP_BattleRoyaleCircleState _circlestate))
  (bind _returnvalue (Math|Conversions|ToInteger(Byte) _currentcirclelevel))
  (bind _output (Utilities|Array|Get(acopy) _circleinfoperlevel _returnvalue))
  (bind (_radius _duration _damagepertick _damagetickinterval) (Utilities|Struct|BreakBP_BattleRoyaleCircleInfo _output))
  (Actor|Tick|SetActorTickEnabled true)
  (Utilities|FlowControl|Sequence
    (:then_0
      (Variables|Default|SetDamagePerTick _damagepertick)
      (Variables|Default|SetDamageInterval _damagetickinterval))
    (:then_1
      (if (Math|Float|NearlyEqual(Float) _radius 0.0 1e-06)
        (Collision|SetCollisionEnabled (Variables|Default|GetCapsule) "NoCollision")
        (Development|SetHiddeninGame (Variables|Default|GetStaticMesh) true false)))))

(fn InterpCircle
  (bind _returnvalue (Game|GetGameState))
  (bind _circlepostprocess (Variables|Default|GetCirclePostProcess))
  (bind _circlestate (Variables|Default|GetCircleState))
  (bind _circleinfoperlevel (Variables|Default|GetCircleInfoPerLevel))
  (bind _staticmesh (Variables|Default|GetStaticMesh))
  (bind (_currentcirclelevel _circlestartservertime _circlestartlocation _circleendlocation) (Utilities|Struct|BreakBP_BattleRoyaleCircleState _circlestate))
  (bind _returnvalue_2 (Transformation|GetWorldScale _staticmesh))
  (bind _returnvalue_3 (Math|Conversions|ToInteger(Byte) _currentcirclelevel))
  (bind _z (Math|Vector|BreakVector _returnvalue_2))
  (bind _returnvalue_4 (+ _returnvalue_3 1))
  (bind _output (Utilities|Array|Get(acopy) _circleinfoperlevel _returnvalue_3))
  (bind (_radius _duration) (Utilities|Struct|BreakBP_BattleRoyaleCircleInfo _output))
  (bind _returnvalue_5 (* _radius 0.002))
  (Utilities|IsValid _returnvalue
    (:Is%20Valid
      (if (Utilities|Array|IsValidIndex _circleinfoperlevel _returnvalue_4)
        (LocalVariables|SetNextRadius (.Radius (Utilities|Struct|BreakBP_BattleRoyaleCircleInfo (Utilities|Array|Get(acopy) _circleinfoperlevel _returnvalue_4))))
        (else
          (LocalVariables|SetNextRadius 0.0)))
      (bind _returnvalue_6 (Class|MordhauUtilityLibrary|GetNormalizedTime _circlestartservertime (+ _circlestartservertime _duration) (GameState|GetServerWorldTimeSeconds _returnvalue)))
      (Transformation|SetActorLocation (Math|Vector|Lerp(Vector) _circlestartlocation _circleendlocation _returnvalue_6) false false)
      (Transformation|SetWorldScale3D _staticmesh (Math|Vector|Lerp(Vector) (Math|Vector|MakeVector _returnvalue_5 _returnvalue_5 _z) (Math|Vector|MakeVector (* (LocalVariables|GetNextRadius) 0.002) (* (LocalVariables|GetNextRadius) 0.002) _z) _returnvalue_6))
      (Components|Capsule|SetCapsuleRadius (Variables|Default|GetCapsule) (Math|Float|Lerp _radius (LocalVariables|GetNextRadius) _returnvalue_6) false)
      (Utilities|IsValid _circlepostprocess
        (:Is%20Valid
          (Transformation|SetWorldScale3D (Variables|/Script/Engine.Brush|GetBrushComponent _circlepostprocess) (Math|Vector|MakeVector (/ (Math|Float|Lerp _radius (LocalVariables|GetNextRadius) _returnvalue_6) (Variables|Default|GetInitialRadius)) (/ (Math|Float|Lerp _radius (LocalVariables|GetNextRadius) _returnvalue_6) (Variables|Default|GetInitialRadius)) 1.0))
          (Transformation|SetActorLocation _circlepostprocess (Math|Vector|Lerp(Vector) _circlestartlocation _circleendlocation _returnvalue_6) false false))))))

(fn FindRandomCircleCenterInside
  (params (InCircleRadius :type Float%20%28single-precision%29) (InCircleCenter :type Vector) (SubCircleRadius :type Float%20%28single-precision%29))
  (bind _output_get (LocalVariables|SetNewLoc (* (* (Math|Random|RandomUnitVector) (Math|Random|RandomFloat)) (- InCircleRadius SubCircleRadius))))
  (return (+ InCircleCenter (Math|Vector|MakeVector (.X (Math|Vector|BreakVector _output_get)) (.Y (Math|Vector|BreakVector _output_get)) 0.0))))

(fn FindRandomCircleBetweenCircles
  (params (BigCircleRadius :type Float%20%28single-precision%29) (BigCircleCenter :type Vector) (SmallCircleRadius :type Float%20%28single-precision%29) (SmallCircleCenter :type Vector) (DesiredCircleRadius :type Float%20%28single-precision%29))
  (bind _output_get (LocalVariables|SetAB (- BigCircleRadius DesiredCircleRadius)))
  (bind _output_get_2 (LocalVariables|SetBC (- DesiredCircleRadius SmallCircleRadius)))
  ;[1 1 1] Try rejection sampling first for 100 tries. If we can't find a good random, fallback to randomizing along the intersection line which is always correct, but less random.
  (Utilities|FlowControl|ForLoopwithBreak 0 100
    (:LoopBody
      (bind _output_get_3 (LocalVariables|SetNewLoc (* (* (Math|Random|RandomUnitVector) (Math|Random|RandomFloat)) _output_get_2)))
      (bind _output_get_4 (LocalVariables|SetNewLoc (+ SmallCircleCenter (Math|Vector|MakeVector (.X (Math|Vector|BreakVector _output_get_3)) (.Y (Math|Vector|BreakVector _output_get_3)) 0.0))))
      (if (<= (Math|Vector|VectorLength (- _output_get_4 BigCircleCenter)) _output_get)
        (bind _output_get_5 (LocalVariables|SetNewQuality (Math|Vector|VectorLength (- SmallCircleCenter (LocalVariables|GetNewLoc)))))
        (if (LocalVariables|GetFoundWithRejectionSampling)
          (if (> _output_get_5 (LocalVariables|GetRejectionSamplingQuality))
            (LocalVariables|SetRejectionSamplingLoc (LocalVariables|GetNewLoc) :!label _label)
            (LocalVariables|SetRejectionSamplingQuality _output_get_5))
          (else
            (LocalVariables|SetFoundWithRejectionSampling true)
            (goto _label)))))
    (:Completed
      (if (LocalVariables|GetFoundWithRejectionSampling)
        (return (LocalVariables|GetRejectionSamplingLoc))
        (else
          (bind (_pointa _pointb _returnvalue) (Class|MordhauUtilityLibrary|FindCircleIntersectionPoints (Math|Conversions|ToVector2D(Vector) BigCircleCenter) _output_get (Math|Conversions|ToVector2D(Vector) SmallCircleCenter) _output_get_2))
          (if _returnvalue
            (bind _output_get_6 (LocalVariables|SetRandomPointOnIntersectionLine (Math|Conversions|ToVector2D(Vector) (Math|Vector|Lerp(Vector) (Math|Conversions|ToVector(Vector2D) _pointa) (Math|Conversions|ToVector(Vector2D) _pointb) (Math|Random|RandomFloat)))))
            (bind _output_get_7 (LocalVariables|SetNewLoc (Math|Vector|Lerp(Vector) (Math|Conversions|ToVector(Vector2D) _pointa) (Math|Conversions|ToVector(Vector2D) _pointb) (Math|Random|RandomFloat))))
            (return (Math|Vector|MakeVector (.X (Math|Vector|BreakVector _output_get_7)) (.Y (Math|Vector|BreakVector _output_get_7)) (.Z (Math|Vector|BreakVector BigCircleCenter))))
            (else
              (bind _output_get_8 (LocalVariables|SetNewLoc (* (* (Math|Random|RandomUnitVector) (Math|Random|RandomFloat)) _output_get_2)))
              (return (+ SmallCircleCenter (Math|Vector|MakeVector (.X (Math|Vector|BreakVector _output_get_8)) (.Y (Math|Vector|BreakVector _output_get_8)) 0.0))))))))))