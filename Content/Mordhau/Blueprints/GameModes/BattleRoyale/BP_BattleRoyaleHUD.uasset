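; Battle Royale game mode HUD that extends its parent HUD with a mode-specific in-game widget and end screen.
; On BeginPlay it replaces the parent's end screen with a collapsed Battle Royale one, exposed through ShowBattleRoyaleEndScreen.
; The in-game widget is created once game state replicates, and its visibility follows minimal/full HUD and main menu events.
; Closing the menu restores cursor and UI-only input if the end screen is visible.
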(event EventBeginPlay
  (|CallParentFunction)
  (Widget|RemovefromParent (Variables|Default|GetEnd%20Screen))
  (bind _returnvalue (UserInterface|CreateWidget "/Game/Mordhau/Blueprints/GameModes/BattleRoyale/BP_BattleRoyaleEndScreen.BP_BattleRoyaleEndScreen_C" (Game|GetPlayerController 0)))
  (bind _output_get (Variables|Default|SetBattleRoyaleEndScreen _returnvalue))
  (Widget|SetVisibility _output_get "Collapsed")
  (Widget|Panel|AddChild (Variables|/Game/Mordhau/UI/BP_HUDWidget.BP_HUDWidget_C|GetPostMatchScreenContainer (Variables|Default|GetHUD)) _output_get))

(event EventOnGameStateReplicated
  (|CallParentFunction)
  (bind _returnvalue (UserInterface|CreateWidget "/Game/Mordhau/Blueprints/GameModes/BattleRoyale/BP_BattleRoyaleHUDWidget.BP_BattleRoyaleHUDWidget_C" (Game|GetPlayerController 0)))
  (bind _output_get (Variables|Default|SetBattleRoyaleHUDWidget _returnvalue))
  (UserInterface|Viewport|AddtoViewport _output_get -5)
  (if (Variables|Default|GetIsHUDMinimal)
    (Widget|SetVisibility _output_get "Collapsed")))

(event EventHideMainMenu
  (bind _returnvalue (Game|GetPlayerController 0))
  (bind _battleroyaleendscreen (Variables|Default|GetBattleRoyaleEndScreen))
  (|CallParentFunction)
  (Widget|SetVisibility (Variables|Default|GetBattleRoyaleHUDWidget) "Visible")
  (if (Widget|IsVisible _battleroyaleendscreen)
    (Variables|/Script/Engine.PlayerController|SetbShowMouseCursor _returnvalue true)
    (Input|SetInputModeUIOnly _returnvalue _battleroyaleendscreen "DoNotLock")))

(event EventShowMainMenu
  (params (Armory%20State :type E_ArmoryStates%20Enum :default "NewEnumerator0"))
  (|CallParentFunction Armory%20State)
  (Widget|SetVisibility (Variables|Default|GetBattleRoyaleHUDWidget) "Collapsed"))

(event EventUseMinimalHUD
  (|CallParentFunction)
  (Utilities|IsValid (Variables|Default|GetBattleRoyaleHUDWidget)
    (:Is%20Valid
      (Widget|SetVisibility (Variables|Default|GetBattleRoyaleHUDWidget) "Collapsed"))))

(event EventUseFullHUD
  (|CallParentFunction)
  (Utilities|IsValid (Variables|Default|GetBattleRoyaleHUDWidget)
    (:Is%20Valid
      (Widget|SetVisibility (Variables|Default|GetBattleRoyaleHUDWidget) "Visible"))))

(fn ConstructionScript
  (|CallParentFunction))

(fn ShowBattleRoyaleEndScreen
  (Default|Show (Variables|Default|GetBattleRoyaleEndScreen)))