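; BP_EconomyPlayerState is the player state for the economy game mode, holding each player's coin balance.
; GiveCoins adds an amount to the replicated Coins variable.
; When Coins replicates, its OnRep casts the owner to BP_EconomyPlayerController and refreshes that controller's shop menu if it is valid and visible.
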(event EventBeginPlay
  (|CallParentFunction) ; This node is disabled and will not be called.\nDrag off pins to build functionality.
)

(event EventTick
  (params (DeltaSeconds :type Float%20%28single-precision%29))
  (|CallParentFunction DeltaSeconds) ; This node is disabled and will not be called.\nDrag off pins to build functionality.
)

(fn ConstructionScript
  (|CallParentFunction))

(fn OnRepCoins
  (bind _asbp_economy_player_controller (Utilities|Casting|CastToBP_EconomyPlayerController (Components|GetOwner)))
  (Utilities|IsValid (Variables|/Game/Mordhau/Blueprints/GameModes/BP_EconomyPlayerController.BP_EconomyPlayerController_C|GetShopMenu _asbp_economy_player_controller)
    (:Is%20Valid
      (if (Widget|IsVisible (Variables|/Game/Mordhau/Blueprints/GameModes/BP_EconomyPlayerController.BP_EconomyPlayerController_C|GetShopMenu _asbp_economy_player_controller))
        (Default|Refresh (Variables|/Game/Mordhau/Blueprints/GameModes/BP_EconomyPlayerController.BP_EconomyPlayerController_C|GetShopMenu _asbp_economy_player_controller))))))

(fn GiveCoins
  (params (Amount :type Integer))
  (Variables|Default|SetCoins (+ (Variables|Default|GetCoins) Amount)))