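; BP_EconomyBuyZone is a team-specific buy zone volume for the Economy game mode.
; Begin and end overlap events cast the other actor to BP_EconomyCharacter and increment or decrement one of its zone counters.
; TeamRestriction picks the counter: zero uses the Team 1 counter, any other value the Team 2 counter.
; Using counters instead of booleans keeps track of overlapping zones.
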(event EventBeginPlay)

(event Collision|EventActorBeginOverlap
  (params (OtherActor :type Actor%20Object%20Reference))
  (bind _asbp_economy_character (Utilities|Casting|CastToBP_EconomyCharacter OtherActor))
  (if (== (Variables|Default|GetTeamRestriction) 0)
    (Variables|/Game/Mordhau/Blueprints/GameModes/BP_EconomyCharacter.BP_EconomyCharacter_C|SetTeam1EconomyZoneCounter _asbp_economy_character (+ (Variables|/Game/Mordhau/Blueprints/GameModes/BP_EconomyCharacter.BP_EconomyCharacter_C|GetTeam1EconomyZoneCounter _asbp_economy_character) 1))
    (else
      (Variables|/Game/Mordhau/Blueprints/GameModes/BP_EconomyCharacter.BP_EconomyCharacter_C|SetTeam2EconomyZoneCounter _asbp_economy_character (+ (Variables|/Game/Mordhau/Blueprints/GameModes/BP_EconomyCharacter.BP_EconomyCharacter_C|GetTeam2EconomyZoneCounter _asbp_economy_character) 1)))))

(event Collision|EventActorEndOverlap
  (params (OtherActor :type Actor%20Object%20Reference))
  (bind _asbp_economy_character (Utilities|Casting|CastToBP_EconomyCharacter OtherActor))
  (if (== (Variables|Default|GetTeamRestriction) 0)
    (Variables|/Game/Mordhau/Blueprints/GameModes/BP_EconomyCharacter.BP_EconomyCharacter_C|SetTeam1EconomyZoneCounter _asbp_economy_character (- (Variables|/Game/Mordhau/Blueprints/GameModes/BP_EconomyCharacter.BP_EconomyCharacter_C|GetTeam1EconomyZoneCounter _asbp_economy_character) 1))
    (else
      (Variables|/Game/Mordhau/Blueprints/GameModes/BP_EconomyCharacter.BP_EconomyCharacter_C|SetTeam2EconomyZoneCounter _asbp_economy_character (- (Variables|/Game/Mordhau/Blueprints/GameModes/BP_EconomyCharacter.BP_EconomyCharacter_C|GetTeam2EconomyZoneCounter _asbp_economy_character) 1)))))

(fn ConstructionScript)