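; BP_ScenarioGameState is the game state Blueprint for Mordhau's Scenario game mode.
; It overrides the objective title, goal, progress and hint getters to return empty text, and always hides the spawn info text.
; It adds no runtime logic: BeginPlay and Tick are disabled stubs, and the construction script only calls its parent.
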(event EventBeginPlay
  (|CallParentFunction) ; This node is disabled and will not be called.\nDrag off pins to build functionality.
)

(event EventTick
  (params (DeltaSeconds :type Float%20%28single-precision%29))
  (|CallParentFunction DeltaSeconds) ; This node is disabled and will not be called.\nDrag off pins to build functionality.
)

(fn ConstructionScript
  (|CallParentFunction))

(fn GetObjectiveTitle
  (return ""))

(fn GetObjectiveGoal
  (return ""))

(fn GetObjectiveProgress
  (return ""))

(fn GetObjectiveHint
  (return ""))

(fn ShouldHideSpawnInfoText
  (return true))