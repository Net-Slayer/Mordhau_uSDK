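; BP_ScenarioCharacter is a scenario-mode character with a preset loadout and looping patrol route.
; On BeginPlay, the server offsets health by -1, applies DefaultProfile with equipment through the Mordhau singleton, then holsters any right-hand item.
; GetTargetPatrolLocation returns the current patrol point, advancing cyclically once the character is within a fixed radius.
; Without patrol points, it returns the character's own location.
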(event EventBeginPlay
  (bind _righthandequipment (Variables|Default|GetRightHandEquipment))
  (Utilities|FlowControl|Sequence
    (:then_0
      (Networking|SwitchHasAuthority
        (:Authority
          (Class|AdvancedCharacter|OffsetHealth -1 true)
          (bind _asbp_mordhau_singleton (Utilities|Casting|CastToBP_MordhauSingleton (Class|MordhauUtilityLibrary|GetMordhauSingleton)))
          (Class|MordhauSingleton|ApplyProfileto _asbp_mordhau_singleton (Variables|Default|GetDefaultProfile) self 0 true)
          (Utilities|IsValid _righthandequipment
            (:Is%20Valid
              (Class|MordhauCharacter|Holster _righthandequipment))))))
    (:then_1
      (|CallParentFunction))))

(fn ConstructionScript
  (|CallParentFunction))

(fn GetTargetPatrolLocation
  (bind _patrolpoints (Variables|Default|GetPatrolPoints))
  (bind _patrolpoints_2 (Variables|Default|GetPatrolPoints))
  (if (> (Utilities|Array|Length _patrolpoints) 0)
    (if (< (Math|Vector|VectorLength (- (Transformation|GetActorLocation) (Transformation|GetActorLocation (Utilities|Array|Get(acopy) _patrolpoints (Variables|Default|GetCurrentPatrolPointIdx))))) 4e+02)
      (Variables|Default|SetCurrentPatrolPointIdx (Math|Integer|%(Integer) (+ (Variables|Default|GetCurrentPatrolPointIdx) 1) (Utilities|Array|Length _patrolpoints_2))))
    (return (Transformation|GetActorLocation (Utilities|Array|Get(acopy) _patrolpoints_2 (Variables|Default|GetCurrentPatrolPointIdx))))
    (else
      (return (Transformation|GetActorLocation)))))