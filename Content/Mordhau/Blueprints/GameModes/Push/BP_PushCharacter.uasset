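; Player character for the Push game mode that turns out-of-bounds deaths in the enemy team area into retreats while the game state's ForwardSpawnUntil window is active.
; On timeout, it has the game mode destroy the pawn and restart the player, otherwise deferring to parent handling.
; Warning text overrides show a pushed-back message and retreat countdown if the timeout will land inside that window.
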(event EventBeginPlay
  (|CallParentFunction) ; This node is disabled and will not be called.\nDrag off pins to build functionality.
)

(event Collision|EventActorBeginOverlap
  (params (OtherActor :type Actor%20Object%20Reference))
  (|CallParentFunction OtherActor) ; This node is disabled and will not be called.\nDrag off pins to build functionality.
)

(event EventTick
  (params (DeltaSeconds :type Float%20%28single-precision%29))
  (|CallParentFunction DeltaSeconds) ; This node is disabled and will not be called.\nDrag off pins to build functionality.
)

(event EventOnExceededTimeOutOfBounds
  (bind _asbp_push_game_state (Utilities|Casting|CastToBP_PushGameState (Game|GetGameState))
    (:then
      (if (and (< (Utilities|Time|GetTimeSeconds) (Variables|/Game/Mordhau/Blueprints/GameModes/Push/BP_PushGameState.BP_PushGameState_C|GetForwardSpawnUntil _asbp_push_game_state)) (Class|MordhauCharacter|IsinEnemyTeamArea))
        (bind _asbp_mordhau_game_mode (Utilities|Casting|CastToBP_MordhauGameMode (Game|GetGameMode))
          (:then
            (bind _asmordhau_player_controller (Utilities|Casting|CastToMordhauPlayerController (Pawn|GetController))
              (:then
                (Default|UnpossessandDestroyPawn _asbp_mordhau_game_mode _asmordhau_player_controller true))
              (:CastFailed
                (|CallParentFunction :!label _label))))
          (:CastFailed
            (goto _label)))
        (else
          (goto _label))))
    (:CastFailed
      (goto _label))))

(fn ConstructionScript
  (|CallParentFunction))

(fn GetOutOfBoundsSubtext
  (bind _asbp_push_game_state (Utilities|Casting|CastToBP_PushGameState (Game|GetGameState))
    (:then
      (if (and (Class|MordhauCharacter|IsinEnemyTeamArea) (< (+ (Class|AdvancedCharacter|GetOutOfBoundsTimeUntilDeath) (Utilities|Time|GetTimeSeconds)) (Variables|/Game/Mordhau/Blueprints/GameModes/Push/BP_PushGameState.BP_PushGameState_C|GetForwardSpawnUntil _asbp_push_game_state)))
        (return (Utilities|Text|FormatText "Retreating in {a} seconds" (Math|Float|Ceil (Class|AdvancedCharacter|GetOutOfBoundsTimeUntilDeath))))
        (else
          _)))
    (:CastFailed
      _))
  (bind _subtext (|CallParentFunction))
  (return _subtext))

(fn GetOutOfBoundsText
  (bind _asbp_push_game_state (Utilities|Casting|CastToBP_PushGameState (Game|GetGameState))
    (:then
      (if (and (Class|MordhauCharacter|IsinEnemyTeamArea) (< (+ (Class|AdvancedCharacter|GetOutOfBoundsTimeUntilDeath) (Utilities|Time|GetTimeSeconds)) (Variables|/Game/Mordhau/Blueprints/GameModes/Push/BP_PushGameState.BP_PushGameState_C|GetForwardSpawnUntil _asbp_push_game_state)))
        (return "We are being pushed back!")
        (else
          _)))
    (:CastFailed
      _))
  (bind _header (|CallParentFunction))
  (return _header))