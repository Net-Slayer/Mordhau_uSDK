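; Objective point for the Push game mode that reacts to team ownership changes and objective completion.
; An ownership change re-toggles team spawn protection, disabling all first for clean overlaps, briefly opens forward spawn, and, for a valid team, records remaining stage time and extends the timer.
; Completion switches linked spawns on the authority.
; HUD events announce next, completed or failed objectives, and construction clears the capture area.
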(event EventBeginPlay
  (|CallParentFunction)
  (CallFunction|UpdateSpawnProtection))

(event Collision|EventActorBeginOverlap
  (params (OtherActor :type Actor%20Object%20Reference)))

(event EventTick
  (params (DeltaSeconds :type Float%20%28single-precision%29)))

(event EventOnObjectivesCompleted
  (|CallParentFunction)
  (Networking|SwitchHasAuthority
    (:Authority
      (for _array_element (Variables|Default|GetSpawnsToActivateOnCompletion)
        (Utilities|IsValid _array_element
          (:Is%20Valid
            (Default|Activate _array_element))))
      (for _array_element_2 (Variables|Default|GetSpawnsToDeactivateOnCompletion)
        (Utilities|IsValid _array_element_2
          (:Is%20Valid
            (Default|Deactivate _array_element_2)))))))

(event EventEnemyGainedPrerequisites
  (|CallParentFunction)
  (Networking|CanExecuteCosmeticEvents
    (:True
      (if (not (< (Utilities|Time|GetTimeSeconds) 5.0))
        (bind _relevance (CallFunction|GetTeamRelevance (Variables|Default|GetOwningTeam)))
        (bind _asbp_frontline_hud (Utilities|Casting|CastToBP_FrontlineHUD (Class|MordhauUtilityLibrary|GetMordhauHUD)))
        (Utilities|FlowControl|Delay 4.1)
        (Audio|PlaySound2D 0 1.0 1.0 0.0 0 0)
        (Default|ShowAnnouncement _asbp_frontline_hud "NEXT OBJECTIVE" (select (== _relevance 0) (Variables|Default|GetAnnouncementDefendersText) (Variables|Default|GetAnnouncementAttackersText)) 4.0 "NewEnumerator1")
        (Utilities|FlowControl|Delay 4.0)
        (Default|ShowObjectives _asbp_frontline_hud)))))

(event EventOnOwningTeamChanged
  (bind _returnvalue (Game|GetPlayerController 0))
  (bind _returnvalue_2 (Game|GetGameState))
  (bind _timeboostoncapture (Variables|Default|GetTimeBoostOnCapture))
  (|CallParentFunction)
  (Utilities|FlowControl|Sequence
    (:then_0
      (CallFunction|UpdateSpawnProtection)
      (if (!= (Variables|Default|GetOwningTeam) 255)
        (Utilities|FlowControl|Sequence
          (:then_0
            (Networking|SwitchHasAuthority
              (:Authority
                (Utilities|FlowControl|Sequence
                  (:then_0
                    (bind _asbp_push_game_state (Utilities|Casting|CastToBP_PushGameState _returnvalue_2))
                    (Utilities|Array|Add (Variables|/Game/Mordhau/Blueprints/GameModes/Push/BP_PushGameState.BP_PushGameState_C|GetTimeLeftPerCompletedStage _asbp_push_game_state) (Math|Float|Max(Float) (- (Variables|/Game/Mordhau/Blueprints/GameModes/Battle/BP_FrontlineGameState.BP_FrontlineGameState_C|GetStageEndTime _asbp_push_game_state) (Utilities|Time|GetTimeSeconds)) 0.0)))
                  (:then_1
                    (bind _asbp_frontline_game_state (Utilities|Casting|CastToBP_FrontlineGameState _returnvalue_2))
                    (Variables|/Game/Mordhau/Blueprints/GameModes/Battle/BP_FrontlineGameState.BP_FrontlineGameState_C|SetStageEndTime _asbp_frontline_game_state (+ (Variables|/Game/Mordhau/Blueprints/GameModes/Battle/BP_FrontlineGameState.BP_FrontlineGameState_C|GetStageEndTime _asbp_frontline_game_state) _timeboostoncapture)))))))
          (:then_1
            (Utilities|IsValid _returnvalue
              (:Is%20Valid
                (if (Pawn|IsLocalPlayerController _returnvalue)
                  (bind _asbp_frontline_hud (Utilities|Casting|CastToBP_FrontlineHUD (Class|MordhauUtilityLibrary|GetMordhauHUD)))
                  (Utilities|IsValid (Variables|/Game/Mordhau/Blueprints/GameModes/Battle/BP_FrontlineHUD.BP_FrontlineHUD_C|GetPushHUDWidget _asbp_frontline_hud)
                    (:Is%20Valid
                      (Default|AddTime (Variables|/Game/Mordhau/Blueprints/GameModes/Battle/BP_FrontlineHUD.BP_FrontlineHUD_C|GetPushHUDWidget _asbp_frontline_hud) _timeboostoncapture))))))))))
    (:then_1
      ;[1 1 1] Enable the forward spawn for those stuck inside spawn protection now
      (bind _asbp_push_game_state_2 (Utilities|Casting|CastToBP_PushGameState (Game|GetGameState)))
      (Variables|/Game/Mordhau/Blueprints/GameModes/Push/BP_PushGameState.BP_PushGameState_C|SetForwardSpawnUntil _asbp_push_game_state_2 (+ (Utilities|Time|GetTimeSeconds) 6.0)))))

(event EventShowPushAttackerAnnouncement
  (bind _asbp_frontline_hud (Utilities|Casting|CastToBP_FrontlineHUD (Class|MordhauUtilityLibrary|GetMordhauHUD)))
  (Default|ShowAnnouncement _asbp_frontline_hud "COMPLETED" (Variables|Default|GetAnnouncementAttackersText) 3.5 "NewEnumerator1"))

(event EventShowPushDefenderAnnouncement
  (bind _asbp_frontline_hud (Utilities|Casting|CastToBP_FrontlineHUD (Class|MordhauUtilityLibrary|GetMordhauHUD)))
  (Default|ShowAnnouncement _asbp_frontline_hud "FAILED" (Variables|Default|GetAnnouncementDefendersText) 3.5 "NewEnumerator1"))

(fn ConstructionScript
  (|CallParentFunction)
  (Variables|Default|SetCaptureArea 0))

(fn UpdateSpawnProtection
  ;[1 1 1] Disable both first, this forces the overlaps to update nicer, since we rely on a certain order (spawn protection boxes should not overlap normally, but they do in this case...)
  (for _array_element (Variables|Default|GetTeam1SpawnProtection)
    (Default|Disable _array_element))
  (for _array_element_2 (Variables|Default|GetTeam2SpawnProtection)
    (Default|Disable _array_element_2))
  (if (== (Variables|Default|GetOwningTeam) 0)
    (for _array_element_3 (Variables|Default|GetTeam1SpawnProtection)
      (Default|Enable _array_element_3))
    (elif (== (Variables|Default|GetOwningTeam) 1)
      (for _array_element_4 (Variables|Default|GetTeam2SpawnProtection)
        (Default|Enable _array_element_4)))))