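; Game mode for Push that records whether a killed player died near an active objective.
; On each kill it finds the first capture point in the game state that has incomplete objectives and is not owned by the attacking team.
; It flags the victim's Push character as close to objective on death if inside any uncompleted objective's area.
; Parent kill handling runs afterwards through a sequence.
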(event EventBeginPlay
  (|CallParentFunction) ; This node is disabled and will not be called.\nDrag off pins to build functionality.
)

(event EventTick
  (params (DeltaSeconds :type Float%20%28single-precision%29))
  (|CallParentFunction DeltaSeconds) ; This node is disabled and will not be called.\nDrag off pins to build functionality.
)

(event EventOnKilled
  (params (Killer :type Controller%20Object%20Reference) (KilledPlayer :type Controller%20Object%20Reference) (KilledPawn :type Pawn%20Object%20Reference) (Type :type EMordhauDamageType%20Enum :default "Generic") (SubType :type Byte :default 0) (DamageSource :type Actor%20Object%20Reference) (DamageAgent :type Actor%20Object%20Reference))
  (Utilities|FlowControl|Sequence
    (:then_0
      (bind _asbp_push_character (Utilities|Casting|CastToBP_PushCharacter KilledPawn))
      (bind _asbp_push_game_state (Utilities|Casting|CastToBP_PushGameState (Game|GetGameState)))
      (bind _array_element (Utilities|Array|ForEachLoopwithBreak (Variables|/Script/Mordhau.MordhauGameState|GetAllCapturePoints _asbp_push_game_state) :!label _label)
        (:LoopBody
          (bind _asbp_capture_point (Utilities|Casting|CastToBP_CapturePoint _array_element))
          (if (and (not (Variables|/Game/Mordhau/Blueprints/GameModes/Battle/BP_CapturePoint.BP_CapturePoint_C|GetObjectivesCompleted _asbp_capture_point)) (!= (Variables|/Game/Mordhau/Blueprints/GameModes/Battle/BP_FrontlineGameState.BP_FrontlineGameState_C|GetAttackingTeam _asbp_push_game_state) (Variables|/Script/Mordhau.ControlPoint|GetOwningTeam _asbp_capture_point)))
            (for _array_element_2 (Variables|/Game/Mordhau/Blueprints/GameModes/Battle/BP_CapturePoint.BP_CapturePoint_C|GetObjectives _asbp_capture_point)
              (Utilities|IsValid (Utilities|ToObject(Interface) _array_element_2)
                (:Is%20Valid
                  ;[1 1 1] needs some way to find if objective is already completed.. at the moment, we have no way of doing this.
                  (bind _completed (Default|IsCompleted _array_element_2))
                  (if (not _completed)
                    (bind _inarea (Default|IsinObjectiveArea _array_element_2 (Transformation|GetActorLocation _asbp_push_character)))
                    (if _inarea
                      (Variables|/Game/Mordhau/Blueprints/GameModes/Push/BP_PushCharacter.BP_PushCharacter_C|SetCloseToObjectiveOnDeath _asbp_push_character true))))))
            (goto _label Break)))))
    (:then_1
      (|CallParentFunction Killer KilledPlayer KilledPawn Type SubType DamageSource DamageAgent))))

(fn ConstructionScript
  (|CallParentFunction))