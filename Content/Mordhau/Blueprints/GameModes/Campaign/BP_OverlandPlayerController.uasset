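; Player controller for the campaign overland mode.
; On BeginPlay it waits briefly, spawns an overland group at its own transform, possesses it and switches input to game and UI.
; It overrides the spectator action and tips events with empty bodies.
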(event EventBeginPlay
  (|CallParentFunction)
  (Utilities|FlowControl|Delay 0.2)
  (bind _returnvalue (Game|SpawnActorfromClass "/Game/Mordhau/Blueprints/GameModes/Campaign/BP_OverlandGroup.BP_OverlandGroup_C" (Transformation|GetActorTransform) "Undefined" 0 0))
  (Pawn|Possess _returnvalue)
  (Input|SetInputModeGameandUI self 0 "DoNotLock" false))

(event EventTick
  (params (DeltaSeconds :type Float%20%28single-precision%29))
  (|CallParentFunction DeltaSeconds))

(event EventOnSpectatorAction
  (params (Action :type Byte :default 0)))

(event EventShowTips)

(event Input|ActionEvents|InputActionShowTeamSelect
  (params (Key :type Key%20Structure)))

(fn ConstructionScript
  (|CallParentFunction))