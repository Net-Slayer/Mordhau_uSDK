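; HUD for the Teamfight (Group3v3) game mode, adding a Teamfight widget on top of the parent HUD's behavior.
; Once game state replicates, it creates the widget and opens the main menu if it is not already showing.
; Player-killed events update the widget's players-remaining popup.
; The widget collapses for minimal HUD or main menu and reappears on full HUD or menu close, without rechecking minimal mode on close.
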(event Custom|Player%20Killed
  (params (Victim :type Player%20State%20Object%20Reference))
  (bind _teamfighthudwidget (Variables|Default|GetTeamfightHUDWidget))
  (bind _bp_playersremainingpopup (Variables|/Game/Mordhau/Blueprints/GameModes/Group3v3/BP_TeamfightHUDWidget.BP_TeamfightHUDWidget_C|GetBP_PlayersRemainingPopup _teamfighthudwidget))
  (Utilities|IsValid _bp_playersremainingpopup
    (:Is%20Valid
      (Default|Update _bp_playersremainingpopup Victim))))

(event EventBeginPlay
  (|CallParentFunction)
  (EventDispatchers|BindEventtoOnPlayerKilledEvent (delegate Custom|Player%20Killed)))

(event EventOnGameStateReplicated
  (Utilities|FlowControl|Sequence
    (:then_0
      (bind _returnvalue (UserInterface|CreateWidget "/Game/Mordhau/Blueprints/GameModes/Group3v3/BP_TeamfightHUDWidget.BP_TeamfightHUDWidget_C" (Game|GetPlayerController 0)))
      (bind _output_get (Variables|Default|SetTeamfightHUDWidget _returnvalue))
      (UserInterface|Viewport|AddtoViewport _output_get -5)
      (if (Variables|Default|GetIsHUDMinimal)
        (Widget|SetVisibility _output_get "Collapsed")))
    (:then_1
      (bind _bisvisible (CallFunction|IsMainMenuVisible))
      (if (not _bisvisible)
        (CallFunction|ShowMainMenu "NewEnumerator0")))))

(event EventHideMainMenu
  (Utilities|FlowControl|Sequence
    (:then_0
      (Widget|SetVisibility (Variables|Default|GetTeamfightHUDWidget) "Visible"))
    (:then_1
      (|CallParentFunction))))

(event EventShowMainMenu
  (params (Armory%20State :type E_ArmoryStates%20Enum :default "NewEnumerator0"))
  (bind _teamfighthudwidget (Variables|Default|GetTeamfightHUDWidget))
  (|CallParentFunction Armory%20State)
  (Utilities|IsValid _teamfighthudwidget
    (:Is%20Valid
      (Widget|SetVisibility _teamfighthudwidget "Collapsed"))))

(event EventUseMinimalHUD
  (|CallParentFunction)
  (Utilities|IsValid (Variables|Default|GetTeamfightHUDWidget)
    (:Is%20Valid
      (Widget|SetVisibility (Variables|Default|GetTeamfightHUDWidget) "Collapsed"))))

(event EventUseFullHUD
  (|CallParentFunction)
  (Utilities|IsValid (Variables|Default|GetTeamfightHUDWidget)
    (:Is%20Valid
      (Widget|SetVisibility (Variables|Default|GetTeamfightHUDWidget) "Visible"))))

(fn ConstructionScript
  (|CallParentFunction))