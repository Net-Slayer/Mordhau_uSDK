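; Game state for the Group 3v3 mode, adapting scoreboard, input blocking and profile changes to the player's room game.
; It reads the replicated room game on the duel player controller, showing that room's team wins as "Points" on the scoreboard.
; During one specific round stage it blocks pawn input and allows immediate profile changes, otherwise deferring to parent behavior.
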(event EventBeginPlay)

(event EventTick
  (params (DeltaSeconds :type Float%20%28single-precision%29))
  (|CallParentFunction DeltaSeconds))

(fn ConstructionScript
  (|CallParentFunction))

(fn GetScoreboardObjectiveName
  (return "Points"))

(fn GetScoreboardTeamObjectiveValue
  (params (Team :type Integer))
  (bind _asbp_duel_player_controller (Utilities|Casting|CastToBP_DuelPlayerController (Game|GetPlayerController 0))
    (:then
      (if (Pawn|IsLocalPlayerController _asbp_duel_player_controller)
        (return (Utilities|String|ToString(Byte) (Utilities|Select :Index Team :Option%200 (.Team1Wins (Utilities|Struct|BreakST_DuelRoomGame (Variables|/Game/Mordhau/Blueprints/GameModes/Duel/BP_DuelPlayerController.BP_DuelPlayerController_C|GetReplicatedRoomGame _asbp_duel_player_controller))) :Option%201 (.Team2Wins (Utilities|Struct|BreakST_DuelRoomGame (Variables|/Game/Mordhau/Blueprints/GameModes/Duel/BP_DuelPlayerController.BP_DuelPlayerController_C|GetReplicatedRoomGame _asbp_duel_player_controller))))))
        (else
          _)))
    (:CastFailed
      _))
  (return (|CallParentFunction Team)))

(fn ShouldBlockPawnInput
  (bind _asbp_duel_player_controller (Utilities|Casting|CastToBP_DuelPlayerController (Game|GetPlayerController 0))
    (:then
      (if (Pawn|IsLocalPlayerController _asbp_duel_player_controller)
        (if (Utilities|Enum|Equal(Enum) (.Stage (Utilities|Struct|BreakSTRUCT_DuelRoundInfo (.RoundInfo (Utilities|Struct|BreakST_DuelRoomGame (Variables|/Game/Mordhau/Blueprints/GameModes/Duel/BP_DuelPlayerController.BP_DuelPlayerController_C|GetReplicatedRoomGame _asbp_duel_player_controller))))) "NewEnumerator1")
          (return true)
          (else
            _))))
    (:CastFailed
      _))
  (bind _returnvalue (|CallParentFunction))
  (return _returnvalue))

(fn CanImmediatelyChangeProfile
  (params (Controller :type Controller%20Object%20Reference))
  (bind _returnvalue (|CallParentFunction Controller))
  (if _returnvalue
    _
    (else
      (bind _asbp_duel_player_controller (Utilities|Casting|CastToBP_DuelPlayerController Controller)
        (:then
          (if (Utilities|Enum|Equal(Enum) (.Stage (Utilities|Struct|BreakSTRUCT_DuelRoundInfo (.RoundInfo (Utilities|Struct|BreakST_DuelRoomGame (Variables|/Game/Mordhau/Blueprints/GameModes/Duel/BP_DuelPlayerController.BP_DuelPlayerController_C|GetReplicatedRoomGame _asbp_duel_player_controller))))) "NewEnumerator1")
            _
            (else
              (return false))))
        (:CastFailed
          (return false)))))
  (return true))