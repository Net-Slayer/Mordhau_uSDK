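; Game mode for ranked 3v3 teamfight matches, run in rooms with matchmade teams.
; Assigns teams by matching each player's PlayFab entity to the matchmaking match's member list.
; Computes per-team average MMR from teamfight rank stats, substituting a default for players without rank history.
; Finishing a room awards score, MMR against the opposing average and reward drops; leavers take a loss, with an extra penalty for the first.
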(event EventBeginPlay
  (|CallParentFunction) ; This node is disabled and will not be called.\nDrag off pins to build functionality.
)

(event EventTick
  (params (DeltaSeconds :type Float%20%28single-precision%29))
  (|CallParentFunction DeltaSeconds) ; This node is disabled and will not be called.\nDrag off pins to build functionality.
)

(event EventAssignTeam
  (params (RoomIndex :type Integer) (Controller :type Mordhau%20Player%20Controller%20Object%20Reference))
  (bind _matchmakingmatchid (Variables|/Script/Mordhau.MordhauPlayerController|GetMatchmakingMatchID Controller))
  (bind _matches (Variables|Default|GetMatches))
  (bind (_value _returnvalue) (Utilities|Map|Find _matches _matchmakingmatchid))
  (bind _asmordhau_player_state (Utilities|Casting|CastToMordhauPlayerState (Variables|/Script/Engine.Controller|GetPlayerState Controller)))
  (if _returnvalue
    (bind _array_element (Utilities|Array|ForEachLoopwithBreak (Utilities|Struct|Break _value) :!label _label)
      (:LoopBody
        (if (Utilities|Enum|Equal(Enum) (.id (.entity _array_element)) (.id (Utilities|Struct|Break (Class|MordhauUtilityLibrary|GetPlayFabPlayer _asmordhau_player_state))))
          (Class|MordhauPlayerState|SetTeam _asmordhau_player_state (select (Utilities|Enum|Equal(Enum) (.teamid _array_element) "FreeGuard") 1 0))
          (goto _label Break))))
    (elif (Class|MordhauUtilityLibrary|IsPlayinEditor)
      (Class|MordhauPlayerState|SetTeam _asmordhau_player_state)
      (else
        (Class|MordhauUtilityLibrary|PrinttoConsoleandLog (Utilities|String|Append "AssignTeam: Failed to find match " _matchmakingmatchid " for player " (.id (Utilities|Struct|Break (Class|MordhauUtilityLibrary|GetPlayFabPlayer _asmordhau_player_state)))))))))

(event EventFinishRoomGame
  (params (RoomIndex :type Integer) (Winner :type Byte :default 0))
  (bind _rooms (Variables|Default|GetRooms))
  (bind _output (Utilities|Array|Get(acopy) _rooms RoomIndex))
  (bind (_controllers _team1mmr _team2mmr) (Utilities|Struct|BreakST_DuelRoom _output))
  (CallFunction|SetRoomTerminated RoomIndex)
  (Class|MordhauUtilityLibrary|PrinttoConsoleandLog (Utilities|String|Append "Successfully finished match with Team1 MMR: " (Utilities|String|ToString(Integer) _team1mmr) " and Team2 MMR: " (Utilities|String|ToString(Integer) _team2mmr)))
  (for _array_element _controllers
    (bind _asbp_group_3v_3player_controller (Utilities|Casting|CastToBP_Group3v3PlayerController _array_element))
    (bind _asbp_mordhau_player_state (Utilities|Casting|CastToBP_MordhauPlayerState (Variables|/Script/Engine.Controller|GetPlayerState _array_element)))
    (Class|MordhauPlayerState|AddScore _asbp_mordhau_player_state (select (== (Variables|/Script/Mordhau.MordhauPlayerState|GetTeam _asbp_mordhau_player_state) (Math|Conversions|ToInteger(Byte) Winner)) 100000 0))
    (bind _newmmr (Class|MordhauUtilityLibrary|AwardTeamfightMMR (== (Variables|/Script/Mordhau.MordhauPlayerState|GetTeam _asbp_mordhau_player_state) (Math|Conversions|ToInteger(Byte) Winner)) (Utilities|Struct|Break (Class|MordhauUtilityLibrary|GetPlayFabPlayer _asbp_mordhau_player_state)) (select (== (Variables|/Script/Mordhau.MordhauPlayerState|GetTeam _asbp_mordhau_player_state) 0) _team2mmr _team1mmr)))
    (Variables|/Game/Mordhau/Blueprints/GameModes/Duel/BP_DuelPlayerController.BP_DuelPlayerController_C|SetNewMMR _asbp_group_3v_3player_controller _newmmr)
    (Class|MordhauGameSession|TriggerRewardDropforPlayer (Class|MordhauUtilityLibrary|GetMordhauGameSession) _asbp_group_3v_3player_controller)))

(event EventPenalizeforLeavingActiveGame
  (params (Controller :type Mordhau%20Player%20Controller%20Object%20Reference) (RoomIdx :type Integer) (IsFirstLeaver :type Boolean))
  (bind _rooms (Variables|Default|GetRooms))
  (bind _output (Utilities|Array|Get(acopy) _rooms RoomIdx))
  (bind (_controllers _game _team1mmr _team2mmr) (Utilities|Struct|BreakST_DuelRoom _output))
  (bind _asbp_duel_player_controller (Utilities|Casting|CastToBP_DuelPlayerController Controller))
  (bind _asmordhau_player_state (Utilities|Casting|CastToMordhauPlayerState (Variables|/Script/Engine.Controller|GetPlayerState Controller)))
  (bind _newmmr (Class|MordhauUtilityLibrary|AwardTeamfightMMR (Class|KismetSystemLibrary|MakeLiteralBool false) (.PlayFabID (Utilities|Struct|Break (Class|MordhauUtilityLibrary|GetPlayFabPlayer _asmordhau_player_state))) (select (== (Variables|/Script/Mordhau.MordhauPlayerState|GetTeam _asmordhau_player_state) 0) _team2mmr _team1mmr)))
  (Variables|/Game/Mordhau/Blueprints/GameModes/Duel/BP_DuelPlayerController.BP_DuelPlayerController_C|SetNewMMR _asbp_duel_player_controller _newmmr)
  (Class|MordhauGameSession|TriggerRewardDropforPlayer (Class|MordhauUtilityLibrary|GetMordhauGameSession) Controller)
  (if IsFirstLeaver
    (|PenalizeforLeavingActiveMatch (.Entity (Utilities|Struct|Break (Class|MordhauUtilityLibrary|GetPlayFabPlayer _asmordhau_player_state))))))

(fn ConstructionScript
  (|CallParentFunction))

(fn ComputeTeamMMR
  (params (RoomIndex :type Integer))
  (bind _returnvalue (Class|MordhauUtilityLibrary|GetMordhauStats))
  (bind _maxpeopleperroom (Variables|Default|GetMaxPeoplePerRoom))
  (bind _returnvalue_2 (/ _maxpeopleperroom 2))
  (bind _returnvalue_3 (Math|Conversions|ToFloat(Integer) _returnvalue_2))
  (for _array_element (Utilities|Struct|BreakST_DuelRoom (Utilities|Array|Get(acopy) (Variables|Default|GetRooms) RoomIndex))
    (bind _asmordhau_player_state (Utilities|Casting|CastToMordhauPlayerState (Variables|/Script/Engine.Controller|GetPlayerState _array_element)))
    (bind _value (Class|MordhauStats|GetPlayerValue _returnvalue (Utilities|Struct|Break (Class|MordhauUtilityLibrary|GetPlayFabPlayer _asmordhau_player_state)) (Variables|/Script/Mordhau.MordhauStats|GetTeamfightRankSamples _returnvalue))
      (:Success
        (bind _value_2 (Class|MordhauStats|GetPlayerValue _returnvalue (Utilities|Struct|Break (Class|MordhauUtilityLibrary|GetPlayFabPlayer _asmordhau_player_state)) (Variables|/Script/Mordhau.MordhauStats|GetTeamfightRank _returnvalue))
          (:Success
            (if (== (Variables|/Script/Mordhau.MordhauPlayerState|GetTeam _asmordhau_player_state) 0)
              (LocalVariables|SetTeam1MMRValue (+ (LocalVariables|GetTeam1MMRValue) (select (and (== _value 0) (== _value_2 0)) 1500 _value_2)))
              (else
                (LocalVariables|SetTeam2MMRValue (+ (LocalVariables|GetTeam2MMRValue) (select (and (== _value 0) (== _value_2 0)) 1500 _value_2))))))))))
  (return (Math|Float|Truncate (/ (Math|Conversions|ToFloat(Integer) (LocalVariables|GetTeam1MMRValue)) _returnvalue_3)) (Math|Float|Truncate (/ (Math|Conversions|ToFloat(Integer) (LocalVariables|GetTeam2MMRValue)) _returnvalue_3)) false))