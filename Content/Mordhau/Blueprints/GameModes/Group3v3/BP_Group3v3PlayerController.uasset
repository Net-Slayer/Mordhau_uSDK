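; Player controller for the Group 3v3 game mode, which here only adds logging of Teamfight MMR updates.
; When new MMR is received, it reads the TeamfightRank value from Mordhau stats and prints both new and old ratings to console and log.
; If the read fails it logs that instead, though that message prints the failed lookup's value as the new MMR.
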(event EventBeginPlay
  (|CallParentFunction) ; This node is disabled and will not be called.\nDrag off pins to build functionality.
)

(event EventTick
  (params (DeltaSeconds :type Float%20%28single-precision%29))
  (|CallParentFunction DeltaSeconds) ; This node is disabled and will not be called.\nDrag off pins to build functionality.
)

(event EventOnReceivedMMR
  (bind _returnvalue (Class|MordhauUtilityLibrary|GetMordhauStats))
  (bind _value (Class|MordhauStats|GetValue _returnvalue (Variables|/Script/Mordhau.MordhauStats|GetTeamfightRank _returnvalue))
    (:Success
      (Class|MordhauUtilityLibrary|PrinttoConsoleandLog (Utilities|String|Append "Received new Teamfight MMR: " (Utilities|String|ToString(Integer) (Variables|Default|GetNewMMR)) ", old Teamfight MMR was: " (Utilities|String|ToString(Integer) _value))))
    (:Failure
      (Class|MordhauUtilityLibrary|PrinttoConsoleandLog (Utilities|String|Append "Received new Teamfight MMR: " (Utilities|String|ToString(Integer) _value) ", but failed to get old Teamfight MMR")))))

(fn ConstructionScript
  (|CallParentFunction))