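; BP_VolleySignalProjectile is a Horde mode projectile that marks the spot for a volley by spawning a BP_VolleyArea where it hits.
; On hit, a short vertical trace against WorldStatic finds the ground, and the area spawns there with the owning controller as instigator.
; The area's damage multiplier scales with a skill level read from the owner's BP_HordePlayerController.
; The parent hit handling runs afterwards.
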(event EventOnProjectileHit
  (params (HitLocation :type Vector%20%28by%20ref%29 :default "0, 0, 0") (HitNormal :type Vector%20%28by%20ref%29 :default "0, 0, 0") (BounceForce :type Float%20%28single-precision%29) (Surface :type Byte :default 0) (bHasHitWorld :type Boolean) (bHasStopped :type Boolean))
  (Utilities|FlowControl|Sequence
    (:then_0
      (bind _returnvalue (Class|MordhauProjectile|GetProjectileOwningController))
      (bind (_outhit _returnvalue_2) (Collision|LineTraceForObjects (+ HitLocation "0, 0,50.000000") (- HitLocation "0, 0,200.000000") (Utilities|Array|MakeArray "ObjectTypeQuery1") false 0 "None"))
      (if _returnvalue_2
        (bind _returnvalue_3 (Game|SpawnActorfromClass "/Game/Mordhau/Blueprints/GameModes/Horde/BP_VolleyArea.BP_VolleyArea_C" (Math|Transform|MakeTransform (.ImpactPoint (Collision|BreakHitResult _outhit))) "AlwaysSpawn" 0 _returnvalue 0))
        (bind _asbp_horde_player_controller (Utilities|Casting|CastToBP_HordePlayerController _returnvalue))
        (Variables|/Game/Mordhau/Blueprints/GameModes/Horde/BP_VolleyArea.BP_VolleyArea_C|SetDamageMultiplier _returnvalue_3 (+ (* (Default|GetSkillLevelFloat _asbp_horde_player_controller "NewEnumerator42") 0.2) 1.0))))
    (:then_1
      (|CallParentFunction HitLocation HitNormal BounceForce Surface bHasHitWorld bHasStopped))))

(event EventBeginPlay)

(event Collision|EventActorBeginOverlap
  (params (OtherActor :type Actor%20Object%20Reference)))

(event EventTick
  (params (DeltaSeconds :type Float%20%28single-precision%29)))

(fn ConstructionScript
  (|CallParentFunction))