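; Player state for Horde mode, holding a player's coins, skill points, skill array and last equipment with ammo.
; The construction script zero-fills the replicated skill array from the skill enum, and its RepNotify tells the owning Horde controller that skills changed.
; CopyProperties carries these values to a new player state, though the armor copy is disconnected.
; Discounted price lookups defer to the owning controller, falling back to base price.
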(event EventBeginPlay
  (|CallParentFunction) ; This node is disabled and will not be called.\nDrag off pins to build functionality.
)

(event EventTick
  (params (DeltaSeconds :type Float%20%28single-precision%29))
  (|CallParentFunction DeltaSeconds) ; This node is disabled and will not be called.\nDrag off pins to build functionality.
)

(event EventCopyProperties
  (params (NewPlayerState :type Player%20State%20Object%20Reference))
  (|CallParentFunction NewPlayerState)
  (bind _asbp_horde_player_state (Utilities|Casting|CastToBP_HordePlayerState NewPlayerState))
  (CallFunction|CopyfromOtherState _asbp_horde_player_state self))

(fn ConstructionScript
  (|CallParentFunction)
  (Utilities|Array|Clear (Variables|Default|GetReplicatedSkills))
  (for _index (range 0 (- (Math|Conversions|ToInteger(Byte) (Utilities|Enum|LiteralenumE_HordeSkill "NewEnumerator4")) 1))
    (Utilities|Array|Add (Variables|Default|GetReplicatedSkills) 0)))

(fn OnRepCoins)

(fn GetDiscountedPrice
  (params (BasePrice :type Integer))
  (bind _asbp_horde_player_controller (Utilities|Casting|CastToBP_HordePlayerController (Components|GetOwner))
    (:then
      (return (Default|GetDiscountedPrice _asbp_horde_player_controller BasePrice)))
    (:CastFailed
      (return BasePrice))))

(fn OnRepSkillPoints)

(fn OnRepReplicatedSkills
  (bind _asbp_horde_player_controller (Utilities|Casting|CastToBP_HordePlayerController (Components|GetOwner)))
  (Default|SkillsUpdated _asbp_horde_player_controller))

(fn CopyfromOtherState
  (params (OtherState :type BP%20Horde%20Player%20State%20Object%20Reference))
  (Variables|Default|SetCoins (Variables|BP_HordePlayerState_C|GetCoins OtherState))
  (Variables|Default|SetSkillPoints (Variables|BP_HordePlayerState_C|GetSkillPoints OtherState))
  (Variables|Default|SetLastEquipment (Variables|BP_HordePlayerState_C|GetLastEquipment OtherState))
  (Variables|Default|SetLastEquipmentAmmo (Variables|BP_HordePlayerState_C|GetLastEquipmentAmmo OtherState))
  (Variables|Default|SetReplicatedSkills (Variables|BP_HordePlayerState_C|GetReplicatedSkills OtherState)))