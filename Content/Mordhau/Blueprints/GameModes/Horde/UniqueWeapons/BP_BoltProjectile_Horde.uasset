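; Crossbow bolt projectile for Horde mode that gains penetration and crippling effects from the owning player's skills.
; On firing, a skill level from BP_HordePlayerController sets the penetration limit and enables pass-through on SurfaceType1.
; The authority counts hits on that surface and removes pass-through once the limit is reached.
; Damaging a BP_HordeEnemy cripples it, scaled by a second skill's level.
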(event EventBeginPlay
  (|CallParentFunction) ; This node is disabled and will not be called.\nDrag off pins to build functionality.
)

(event Collision|EventActorBeginOverlap
  (params (OtherActor :type Actor%20Object%20Reference))
  (|CallParentFunction OtherActor) ; This node is disabled and will not be called.\nDrag off pins to build functionality.
)

(event EventTick
  (params (DeltaSeconds :type Float%20%28single-precision%29))
  (|CallParentFunction DeltaSeconds) ; This node is disabled and will not be called.\nDrag off pins to build functionality.
)

(event EventOnProjectileHit
  (params (HitLocation :type Vector%20%28by%20ref%29 :default "0, 0, 0") (HitNormal :type Vector%20%28by%20ref%29 :default "0, 0, 0") (BounceForce :type Float%20%28single-precision%29) (Surface :type Byte :default 0) (bHasHitWorld :type Boolean) (bHasStopped :type Boolean))
  (|CallParentFunction HitLocation HitNormal BounceForce Surface bHasHitWorld bHasStopped)
  (Networking|SwitchHasAuthority
    (:Authority
      (if (== Surface (Utilities|Enum|LiteralenumEPhysicalSurface "SurfaceType1"))
        (bind _output_get (Variables|Default|SetPenetrations (+ (Variables|Default|GetPenetrations) 1)))
        (if (>= _output_get (Variables|Default|GetMaxPenetrations))
          (Utilities|Array|RemoveItem (Variables|Default|GetWillPassThroughOn) "SurfaceType1"))))))

(event EventOnProjectileFired
  (|CallParentFunction)
  (bind _returnvalue (Class|MordhauProjectile|GetProjectileOwningController))
  (bind _asbp_horde_player_controller (Utilities|Casting|CastToBP_HordePlayerController _returnvalue))
  (bind _output_get (Variables|Default|SetMaxPenetrations (Math|Conversions|ToInteger(Byte) (Default|GetSkillLevel _asbp_horde_player_controller "NewEnumerator32"))))
  (if (> _output_get 0)
    (Utilities|Array|Add (Variables|Default|GetWillPassThroughOn) "SurfaceType1")))

(event EventOnProjectileDamagedCharacter
  (params (Character :type Advanced%20Character%20Object%20Reference) (bWillKill :type Boolean) (WorldLocation :type Vector%20%28by%20ref%29 :default "0, 0, 0") (bone :type Name%20%28by%20ref%29 :default "None"))
  (|CallParentFunction Character bWillKill WorldLocation bone)
  (bind _returnvalue (Class|MordhauProjectile|GetProjectileOwningController))
  (bind _asbp_horde_player_controller (Utilities|Casting|CastToBP_HordePlayerController _returnvalue))
  (if (> (Default|GetSkillLevel _asbp_horde_player_controller "NewEnumerator36") 0)
    (bind _asbp_horde_enemy (Utilities|Casting|CastToBP_HordeEnemy Character))
    (Default|Cripple _asbp_horde_enemy (* (Default|GetSkillLevelFloat _asbp_horde_player_controller "NewEnumerator36") 1.0))))

(fn ConstructionScript
  (|CallParentFunction))