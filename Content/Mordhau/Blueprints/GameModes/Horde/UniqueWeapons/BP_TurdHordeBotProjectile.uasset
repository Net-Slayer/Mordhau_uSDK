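; Projectile for Horde mode bots, a "turd" unique weapon that deals small area damage on impact.
; On hit, the server applies radial damage at the hit location, credited to the owning controller and ignoring friendlies.
; Equal minimum and base damage and matching radii make the damage flat across the area.
; The parent projectile's hit handling then runs on all sides.
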(event EventBeginPlay
  (|CallParentFunction) ; This node is disabled and will not be called.\nDrag off pins to build functionality.
)

(event Collision|EventActorBeginOverlap
  (params (OtherActor :type Actor%20Object%20Reference))
  (|CallParentFunction OtherActor) ; This node is disabled and will not be called.\nDrag off pins to build functionality.
)

(event EventTick
  (params (DeltaSeconds :type Float%20%28single-precision%29))
  (|CallParentFunction DeltaSeconds) ; This node is disabled and will not be called.\nDrag off pins to build functionality.
)

(event EventOnProjectileHit
  (params (HitLocation :type Vector%20%28by%20ref%29 :default "0, 0, 0") (HitNormal :type Vector%20%28by%20ref%29 :default "0, 0, 0") (BounceForce :type Float%20%28single-precision%29) (Surface :type Byte :default 0) (bHasHitWorld :type Boolean) (bHasStopped :type Boolean))
  (Utilities|FlowControl|Sequence
    (:then_0
      (Networking|SwitchHasAuthority
        (:Authority
          (bind _returnvalue (Class|MordhauProjectile|GetProjectileOwningController))
          (Class|MordhauUtilityLibrary|MordhauApplyRadialDamagewithFalloff 0 3.0 3.0 0.0 0.0 HitLocation 1.7e+02 1.7e+02 5.0 0 0.0 0.0 0.0 self _returnvalue "ECC_WorldStatic" true))))
    (:then_1
      (|CallParentFunction HitLocation HitNormal BounceForce Surface bHasHitWorld bHasStopped))))

(fn ConstructionScript
  (|CallParentFunction))