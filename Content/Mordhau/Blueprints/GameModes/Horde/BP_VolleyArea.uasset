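; BP_VolleyArea is a Horde mode area effect that deals timed volley damage to characters inside its box.
; After an activation delay, a looping timer damages each living overlapping AdvancedCharacter, crediting the instigator's controller.
; A long downward line trace onto each character must hit that character first, so overhead cover blocks damage.
; Particles deactivate shortly before the duration ends, then the timer clears and a short lifespan removes the actor.
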(event Custom|DamageTick
  (bind _self self)
  (bind _output_get (Variables|Default|SetOverlaps (Collision|GetOverlappingActors (Variables|Default|GetBox) "/Script/Mordhau.AdvancedCharacter" :!class /Script/Engine.PrimitiveComponent)))
  (for _array_element _output_get
    (bind _asadvanced_character (Utilities|Casting|CastToAdvancedCharacter _array_element))
    (if (not (Class|AdvancedCharacter|GetIsDead _asadvanced_character))
      (bind _outhit (Collision|LineTraceForObjects (+ (Transformation|GetWorldLocation (Variables|/Script/Engine.Character|GetCapsuleComponent _asadvanced_character)) "0, 0,100000.000000") (Transformation|GetWorldLocation (Variables|/Script/Engine.Character|GetCapsuleComponent _asadvanced_character)) (Utilities|Array|MakeArray "ObjectTypeQuery1" "ObjectTypeQuery3" "ObjectTypeQuery5") false 0 "None"))
      (if (== (.HitActor (Collision|BreakHitResult _outhit)) _asadvanced_character)
        (Class|AdvancedCharacter|MordhauTakeDamage _asadvanced_character (* (Variables|Default|GetDamage) (Variables|Default|GetDamageMultiplier)) (Collision|MakeHitResult false false 0.0 0.0 "0, 0, 0" "0, 0, 0" "0,0,1" "0,0,1" 0 0) "Generic" 0 _self _self (Variables|Default|GetInstigatorController))))))

(event EventBeginPlay
  (Utilities|FlowControl|Delay (Variables|Default|GetActivationDelay))
  (bind _returnvalue (Utilities|Time|SetTimerbyEvent (delegate Custom|DamageTick) (Variables|Default|GetInterval) true))
  (Utilities|FlowControl|Sequence
    (:then_0
      (Utilities|FlowControl|Delay (- (Variables|Default|GetDuration) 3.25))
      (Components|Activation|Deactivate (Variables|Default|GetParticleSystem)))
    (:then_1
      (Utilities|FlowControl|Delay (Variables|Default|GetDuration))
      (Utilities|Time|ClearandInvalidateTimerbyHandle _returnvalue)
      (Actor|SetLifeSpan 6.0))))

(event Collision|EventActorBeginOverlap
  (params (OtherActor :type Actor%20Object%20Reference)))

(event EventTick
  (params (DeltaSeconds :type Float%20%28single-precision%29)))

(fn ConstructionScript)