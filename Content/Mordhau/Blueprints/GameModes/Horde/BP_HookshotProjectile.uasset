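; Hookshot projectile for Horde mode that drags struck enemies back to the player who fired it.
; On a non-lethal hit to a Horde enemy, the server stores the victim as the pull target and trips it.
; Tick then moves the victim toward the creator at constant speed while both are alive, releasing it once it is close.
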(event EventBeginPlay
  (|CallParentFunction) ; This node is disabled and will not be called.\nDrag off pins to build functionality.
)

(event Collision|EventActorBeginOverlap
  (params (OtherActor :type Actor%20Object%20Reference))
  (|CallParentFunction OtherActor) ; This node is disabled and will not be called.\nDrag off pins to build functionality.
)

(event EventTick
  (params (DeltaSeconds :type Float%20%28single-precision%29))
  (|CallParentFunction DeltaSeconds)
  (Utilities|IsValid (Variables|Default|GetPulling)
    (:Is%20Valid
      (if (not (Class|AdvancedCharacter|GetIsDead (Variables|Default|GetPulling)))
        (bind _returnvalue (Class|MordhauProjectile|GetProjectileCreator))
        (bind _asbp_horde_character (Utilities|Casting|CastToBP_HordeCharacter _returnvalue))
        (if (not (Class|AdvancedCharacter|GetIsDead _asbp_horde_character))
          (if (Math|Vector|Equal(Vector) (Transformation|GetActorLocation (Variables|Default|GetPulling)) (Transformation|GetActorLocation _asbp_horde_character) 1.5e+02)
            (Variables|Default|SetPulling 0)
            (else
              (Transformation|SetActorLocation (Variables|Default|GetPulling) (Math|Interpolation|VInterptoConstant (Transformation|GetActorLocation (Variables|Default|GetPulling)) (Transformation|GetActorLocation _asbp_horde_character) DeltaSeconds 2e+03) false false))))))))

(event EventOnProjectileDamagedCharacter
  (params (Character :type Advanced%20Character%20Object%20Reference) (bWillKill :type Boolean) (WorldLocation :type Vector%20%28by%20ref%29 :default "0, 0, 0") (bone :type Name%20%28by%20ref%29 :default "None"))
  (|CallParentFunction Character bWillKill WorldLocation bone)
  (if (not bWillKill)
    (Utilities|Casting|CastToBP_HordeEnemy Character)
    (Networking|SwitchHasAuthority
      (:Authority
        (bind _output_get (Variables|Default|SetPulling Character))
        (Class|AdvancedCharacter|Trip _output_get)))))

(fn ConstructionScript
  (|CallParentFunction))