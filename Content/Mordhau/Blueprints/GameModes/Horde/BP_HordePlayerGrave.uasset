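; Horde mode grave for a player that another character can revive through a held interaction before its timer expires.
; The server counts down the revive period, pausing while interaction is maintained, replicates whole seconds left and destroys the grave at zero.
; Interaction start awards assist score, respawns the owner at the grave with an incremented revive count, then destroys it.
; An OnRep links the grave to its player state.
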(event EventTick
  (params (DeltaSeconds :type Float%20%28single-precision%29))
  (Networking|SwitchHasAuthority
    (:Authority
      (Utilities|FlowControl|Sequence
        (:then_0
          (if (not (Variables|Default|GetBeingInteractedWith))
            (Variables|Default|SetRevivePeriod (- (Variables|Default|GetRevivePeriod) DeltaSeconds))))
        (:then_1
          (Variables|Default|SetBeingInteractedWith false))
        (:then_2
          (Variables|Default|SetReplicatedLifeSpanSeconds (Math|Conversions|ToByte(Integer) (Math|Float|Ceil (Variables|Default|GetRevivePeriod)))))
        (:then_3
          (if (<= (Variables|Default|GetRevivePeriod) 0.0)
            (Actor|DestroyActor)))))))

(event EventOnHeldInteractionStart
  (params (Character :type Mordhau%20Character%20Object%20Reference))
  (bind _associatedplayerstate (Variables|Default|GetAssociatedPlayerState))
  (Utilities|FlowControl|Sequence
    (:then_0
      (Utilities|IsValid Character
        (:Is%20Valid
          (Utilities|IsValid _associatedplayerstate
            (:Is%20Valid
              (bind _asmordhau_player_controller (Utilities|Casting|CastToMordhauPlayerController (Components|GetOwner _associatedplayerstate)))
              (bind _asbp_mordhau_game_mode (Utilities|Casting|CastToBP_MordhauGameMode (Game|GetGameMode)))
              (Utilities|FlowControl|Sequence
                (:then_0
                  (bind _asmordhau_player_controller_2 (Utilities|Casting|CastToMordhauPlayerController (Pawn|GetController Character)))
                  (Class|MordhauPlayerController|GiveClientScoreBP _asmordhau_player_controller_2 "Assist" 250))
                (:then_1
                  (Default|UnpossessandDestroyPawn _asbp_mordhau_game_mode _asmordhau_player_controller false)
                  (Class|GameModeBase|RestartPlayeratTransform _asbp_mordhau_game_mode _asmordhau_player_controller (Transformation|GetActorTransform))
                  (bind _asbp_horde_character (Utilities|Casting|CastToBP_HordeCharacter (Pawn|GetControlledPawn _asmordhau_player_controller)))
                  (Variables|/Game/Mordhau/Blueprints/Characters/BP_HordeCharacter.BP_HordeCharacter_C|SetRevivedCount _asbp_horde_character (Math|Conversions|ToByte(Integer) (+ (Variables|Default|GetPreviousRevivedCount) 1))))))))))
    (:then_1
      (Actor|DestroyActor))))

(event EventOnInteractionMaintained
  (params (Character :type Mordhau%20Character%20Object%20Reference))
  (Variables|Default|SetBeingInteractedWith true))

(fn ConstructionScript)

(fn CanInteract
  (params (Character :type Mordhau%20Character%20Object%20Reference))
  (return false))

(fn OnRepAssociatedPlayerState
  (bind _asbp_horde_player_state (Utilities|Casting|CastToBP_HordePlayerState (Variables|Default|GetAssociatedPlayerState)))
  (Variables|/Game/Mordhau/Blueprints/GameModes/Horde/BP_HordePlayerState.BP_HordePlayerState_C|SetGrave _asbp_horde_player_state self))