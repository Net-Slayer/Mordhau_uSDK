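; Horde-mode enemy character that picks a random valid task from the game mode and reacts to player skills.
; Damage, parry, block and kill hooks query the attacking Horde character or controller for lifesteal, damage scaling, parry bypass and rewards.
; Timed cripple and enrage effects join trips and stuns, with bosses exempt from these.
; It knocks back nearby players on possession and damages blocking destroyables or pavises, massively after climbing or possession.
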(event Custom|CompleteTask
  (Variables|Default|SetCurrentTask 0))

(event Custom|LegSweep
  (if (not (Variables|Default|GetIsBoss))
    (Utilities|FlowControl|Delay 0.001)
    (if (not (Class|AdvancedCharacter|GetIsDead))
      (Class|AdvancedCharacter|Trip))))

(event Custom|Recoil
  (if (not (Class|AdvancedCharacter|GetIsDead))
    (Utilities|FlowControl|Delay 0.001)
    (if (not (Variables|Default|GetIsBoss))
      (Class|MordhauCharacter|AssignNetMotionSimple (Utilities|Enum|LiteralenumEMotionType "Stunned") 127)
      (Variables|Default|SetStunnedBySkillCounter (+ (Variables|Default|GetStunnedBySkillCounter) 1)))))

(event Custom|Cripple
  (params (Duration :type Float%20%28single-precision%29))
  (bind _charactermovement (Variables|Character|GetCharacterMovement))
  (if (not (Class|AdvancedCharacter|GetIsDead))
    (if (not (Variables|Default|GetIsBoss))
      (Utilities|FlowControl|Sequence
        (:then_0
          (if (not (Variables|Default|GetIsCrippled))
            (Variables|Default|SetPreCrippleMaxWalkSpeed (Variables|/Script/Engine.CharacterMovementComponent|GetMaxWalkSpeed _charactermovement))
            (Variables|Default|SetIsCrippled true)
            (Variables|/Script/Engine.CharacterMovementComponent|SetMaxWalkSpeed _charactermovement (* (Variables|/Script/Engine.CharacterMovementComponent|GetMaxWalkSpeed _charactermovement) 0.5))))
        (:then_1
          (Utilities|FlowControl|RetriggerableDelay Duration)
          (if (not (Class|AdvancedCharacter|GetIsDead))
            (Variables|Default|SetIsCrippled false)
            (Variables|/Script/Engine.CharacterMovementComponent|SetMaxWalkSpeed _charactermovement (Variables|Default|GetPreCrippleMaxWalkSpeed))))))))

(event Custom|Enrage
  (params (Target :type Mordhau%20Character%20Object%20Reference) (Duration :type Float%20%28single-precision%29))
  (if (not (Variables|Default|GetIsBoss))
    (Variables|Default|SetRageTarget Target)
    (Utilities|FlowControl|RetriggerableDelay Duration)
    (Variables|Default|SetRageTarget 0)))

(event EventBeginPlay
  (|CallParentFunction)
  (Networking|SwitchHasAuthority
    (:Authority
      (bind _asbp_horde_game_mode (Utilities|Casting|CastToBP_HordeGameMode (Game|GetGameMode)))
      (if (> (Utilities|Array|Length (Variables|/Game/Mordhau/Blueprints/GameModes/Horde/BP_HordeGameMode.BP_HordeGameMode_C|GetHordeTasks _asbp_horde_game_mode)) 0)
        (bind _output_get (Variables|Default|SetCurrentTask (Utilities|Array|Get(acopy) (Variables|/Game/Mordhau/Blueprints/GameModes/Horde/BP_HordeGameMode.BP_HordeGameMode_C|GetHordeTasks _asbp_horde_game_mode) (Math|Random|RandomIntegerinRange 0 (- (Utilities|Array|Length (Variables|/Game/Mordhau/Blueprints/GameModes/Horde/BP_HordeGameMode.BP_HordeGameMode_C|GetHordeTasks _asbp_horde_game_mode)) 1)))))
        (Utilities|IsValid _output_get
          (:Is%20Valid
            (if (not (Default|IsTaskValidfor _output_get self))
              (Variables|Default|SetCurrentTask 0))))))))

(event Collision|EventActorBeginOverlap
  (params (OtherActor :type Actor%20Object%20Reference))
  (|CallParentFunction OtherActor) ; This node is disabled and will not be called.\nDrag off pins to build functionality.
)

(event EventTick
  (params (DeltaSeconds :type Float%20%28single-precision%29))
  (|CallParentFunction DeltaSeconds) ; This node is disabled and will not be called.\nDrag off pins to build functionality.
)

(event EventOnDied
  (params (Angle :type Float%20%28single-precision%29) (Type :type EMordhauDamageType%20Enum :default "Generic") (SubType :type Byte :default 0) (bone :type Name%20%28by%20ref%29 :default "None") (Point :type Vector%20%28by%20ref%29 :default "0, 0, 0") (Source :type Actor%20Object%20Reference) (Agent :type Actor%20Object%20Reference))
  (Variables|/Script/Mordhau.MordhauWidgetComponent|SetOverrideVisible (Variables|Default|GetMordhauWidget) 0)
  (|CallParentFunction Angle Type SubType bone Point Source Agent))

(event EventMoveBlockedbySlow
  (params (Impact :type Hit%20Result%20Structure%20%28by%20ref%29))
  (CallFunction|HandleObstructionRemoval Impact))

(event EventMordhauDamage
  (params (Damage :type Float%20%28single-precision%29) (HitResult :type Hit%20Result%20Structure%20%28by%20ref%29) (DamageType :type EMordhauDamageType%20Enum :default "Generic") (SubDamageType :type Byte :default 0) (Source :type Actor%20Object%20Reference) (Agent :type Actor%20Object%20Reference) (EventInstigator :type Controller%20Object%20Reference))
  (bind _hitbonename (Collision|BreakHitResult HitResult))
  (|CallParentFunction Damage HitResult DamageType SubDamageType Source Agent EventInstigator)
  (if (and (Utilities|Enum|Equal(Enum) DamageType "Melee") (> Damage 0.0))
    (bind _asbp_horde_character (Utilities|Casting|CastToBP_HordeCharacter Source))
    (Utilities|FlowControl|Sequence
      (:then_0
        (if (> (Default|GetSkill _asbp_horde_character "NewEnumerator19") 0)
          (Class|AdvancedCharacter|OffsetHealth _asbp_horde_character (Math|Float|Ceil (* (Default|GetSkillFloat _asbp_horde_character "NewEnumerator19") Damage 0.02)) true)))
      (:then_1
        (if (<= (Math|Random|RandomFloat) (* (Default|GetSkillFloat _asbp_horde_character "NewEnumerator27") 0.1))
          (if (Math|Boolean|ORBoolean (Utilities|Name|Equal(Name) _hitbonename "RightFoot") (Utilities|Name|Equal(Name) _hitbonename "LeftFoot") (Utilities|Name|Equal(Name) _hitbonename "RightLeg") (Utilities|Name|Equal(Name) _hitbonename "LeftLeg"))
            (CallFunction|LegSweep)))))))

(event EventOnBlockedMelee
  (params (HitResult :type Hit%20Result%20Structure%20%28by%20ref%29) (Attacker :type Mordhau%20Character%20Object%20Reference))
  (|CallParentFunction HitResult Attacker)
  (if (not (Class|AdvancedCharacter|GetIsDead))
    (bind _asbp_horde_character (Utilities|Casting|CastToBP_HordeCharacter Attacker))
    (Utilities|FlowControl|Sequence
      (:then_0
        (if (<= (Math|Random|RandomFloat) (* (Default|GetSkillFloat _asbp_horde_character "NewEnumerator29") 0.1))
          (if (not (Variables|Default|GetIsBoss))
            (Class|MordhauCharacter|AssignNetMotionSimple (Utilities|Enum|LiteralenumEMotionType "Stunned") 127)
            (Variables|Default|SetStunnedBySkillCounter (+ (Variables|Default|GetStunnedBySkillCounter) 1))))))))

(event EventOnKilled
  (params (EventInstigator :type Controller%20Object%20Reference))
  (|CallParentFunction EventInstigator)
  (Utilities|FlowControl|Sequence
    (:then_0
      (bind _returnvalue (Class|AdvancedCharacter|GetLastNetDamageType))
      (if (Utilities|Enum|Equal(Enum) _returnvalue "Melee")
        (bind _returnvalue_2 (Class|AdvancedCharacter|GetLastNetDamageSource))
        (bind _asbp_horde_character (Utilities|Casting|CastToBP_HordeCharacter _returnvalue_2))
        (Default|AwardHealthonKilltoTeammates _asbp_horde_character)))
    (:then_1
      (bind _asbp_horde_player_controller (Utilities|Casting|CastToBP_HordePlayerController EventInstigator))
      (bind _asbp_horde_character_2 (Utilities|Casting|CastToBP_HordeCharacter (Pawn|GetControlledPawn _asbp_horde_player_controller)))
      (Default|OnKilledEnemy _asbp_horde_character_2 self))))

(event EventPossessed
  (params (NewController :type Controller%20Object%20Reference))
  (bind _self self)
  (|CallParentFunction NewController)
  (bind _outactors (Collision|SphereOverlapActors (Transformation|GetActorLocation) 1e+02 (Utilities|Array|MakeArray "ObjectTypeQuery3") "/Game/Mordhau/Blueprints/Characters/BP_HordeCharacter.BP_HordeCharacter_C"))
  (for _array_element _outactors
    (bind _asmordhau_character (Utilities|Casting|CastToMordhauCharacter _array_element))
    (if (not (Class|AdvancedCharacter|GetIsDead _asmordhau_character))
      (bind _returnvalue (Class|MordhauCharacter|IsinKnockback _asmordhau_character))
      (if (not _returnvalue)
        (Class|AdvancedCharacter|Knockback _asmordhau_character (* (Math|Vector|Normalize (- (Transformation|GetActorLocation _asmordhau_character) (Transformation|GetActorLocation))) 1e+03))
        (Class|AdvancedCharacter|Trip _asmordhau_character)
        (Class|AdvancedCharacter|MordhauTakeDamage _asmordhau_character 3e+01 (Collision|MakeHitResult false false 0.0 0.0 "0, 0, 0" "0, 0, 0" "0,0,1" "0,0,1" 0 0) "Generic" 0 _self _self NewController)))))

(fn ConstructionScript
  (|CallParentFunction))

(fn ModifyDamage
  (params (DamageAmount :type Float%20%28single-precision%29) (DamageInfo :type Mordhau%20Damage%20Info%20Structure%20%28by%20ref%29) (EventInstigator :type Controller%20Object%20Reference))
  (bind (_hit _type _subtype _damagesource _damageagent) (Utilities|Struct|BreakMordhauDamageInfo DamageInfo))
  (bind _returnvalue (|CallParentFunction DamageAmount DamageInfo EventInstigator))
  (bind _output_get (LocalVariables|SetDamage _returnvalue))
  (Utilities|FlowControl|Sequence
    (:then_0
      (bind _asbp_horde_character (Utilities|Casting|CastToBP_HordeCharacter _damagesource))
      (bind _outdamage (Default|ModifyOutgoingDamage _asbp_horde_character self _type _hit _damageagent _output_get))
      (LocalVariables|SetDamage _outdamage))
    (:then_1
      (return (LocalVariables|GetDamage)))
    (:then_2
      (if (Utilities|Enum|Equal(Enum) _type "Fire")
        (bind _asbp_horde_player_controller (Utilities|Casting|CastToBP_HordePlayerController EventInstigator))
        (LocalVariables|SetDamage (* (LocalVariables|GetDamage) (+ (* (Default|GetSkillLevelFloat _asbp_horde_player_controller "NewEnumerator20") 0.2) 1.0)))))))

(fn ModifyParryResult
  (params (InResult :type Boolean) (HitResult :type Hit%20Result%20Structure%20%28by%20ref%29) (Attacker :type Mordhau%20Character%20Object%20Reference))
  (Utilities|FlowControl|Sequence
    (:then_0
      (if InResult
        (bind _asbp_horde_character (Utilities|Casting|CastToBP_HordeCharacter Attacker))
        (if (Variables|/Game/Mordhau/Blueprints/Characters/BP_HordeCharacter.BP_HordeCharacter_C|GetLastAttackBypassesParry _asbp_horde_character)
          (return false))))
    (:then_1
      (bind _returnvalue (|CallParentFunction InResult HitResult Attacker))
      (return _returnvalue))))

(fn GetEnragedTarget
  (bind _ragetarget (Variables|Default|GetRageTarget))
  (Utilities|IsValid _ragetarget
    (:Is%20Valid
      (if (Class|AdvancedCharacter|GetIsDead _ragetarget)
        _
        (else
          (return _ragetarget))))
    (:Is%20Not%20Valid
      _))
  (return 0))

(fn OnRepStunnedbySkillCounter
  (Audio|SpawnSoundAttached 0 (Variables|Default|GetCapsuleComponent) "None" "0, 0, 0" "0, 0, 0" "SnapToTarget" false 1.0 1.0 0.0 0 0))

(fn HandleObstructionRemoval
  (params (Impact :type Hit%20Result%20Structure))
  (bind _hitactor (Collision|BreakHitResult Impact))
  (LocalVariables|SetDamageToApply (Variables|Default|GetWoodDamageForPathClearing))
  (bind _output_get (LocalVariables|SetExtraDamageMode (or (> (+ (Variables|Default|GetLastClimbTime) 3.0) (Utilities|Time|GetTimeSeconds)) (> (+ (Variables|Default|GetLastPossessionTime) 1.0) (Utilities|Time|GetRealTimeSeconds)))))
  (Utilities|FlowControl|Sequence
    (:then_0
      (if _output_get
        (LocalVariables|SetDamageToApply 99999.0)))
    (:then_1
      (Utilities|Casting|CastToBP_DestroyableActor _hitactor
        (:then
          _)
        (:CastFailed
          (Utilities|Casting|CastToBP_PaviseShield _hitactor)))
      (Game|Damage|ApplyDamage _hitactor (LocalVariables|GetDamageToApply) (Pawn|GetController) self))))

(fn AttemptClimb
  (Variables|Default|SetLastClimbTime (Utilities|Time|GetTimeSeconds))
  (bind _succeeded (|CallParentFunction))
  (return _succeeded))