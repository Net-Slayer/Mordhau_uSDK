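; BP_HordeSpectator is the Horde mode spectator, which restricts spectating while the player has a grave.
; GetGrave reads the Grave reference from the controller's BP_HordePlayerState.
; Primary, secondary and tertiary spectator actions run only when no valid grave exists.
; With a valid grave, SwitchtoFreeCam makes the grave the view target and sets the Mordhau camera manager's style; otherwise it calls the parent free-cam switch.
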(event EventSwitchtoFreeCam
  (bind _grave (CallFunction|GetGrave))
  (Utilities|IsValid _grave
    (:Is%20Valid
      (bind _asplayer_controller (Utilities|Casting|CastToPlayerController (Pawn|GetController)))
      (Game|Player|SetViewTargetwithBlend _asplayer_controller _grave 0.0 "VTBlend_Linear" 0.0 false)
      (bind _asmordhau_camera_manager (Utilities|Casting|CastToMordhauCameraManager (Variables|/Script/Engine.PlayerController|GetPlayerCameraManager _asplayer_controller)))
      (Class|MordhauCameraManager|SetCameraStyleBP _asmordhau_camera_manager "FreeCam_Mordhau"))
    (:Is%20Not%20Valid
      (|CallParentFunction))))

(event Collision|EventActorBeginOverlap
  (params (OtherActor :type Actor%20Object%20Reference))
  (|CallParentFunction OtherActor) ; This node is disabled and will not be called.\nDrag off pins to build functionality.
)

(event EventTick
  (params (DeltaSeconds :type Float%20%28single-precision%29))
  (|CallParentFunction DeltaSeconds) ; This node is disabled and will not be called.\nDrag off pins to build functionality.
)

(event Input|ActionEvents|InputActionPrimarySpectatorAction
  (params (Key :type Key%20Structure))
  (:Pressed
    (bind _grave (CallFunction|GetGrave))
    (Utilities|IsValid _grave
      (:Is%20Not%20Valid
        (Class|MordhauSpectator|PrimarySpectatorAction)))))

(event Input|ActionEvents|InputActionSecondarySpectatorAction
  (params (Key :type Key%20Structure))
  (:Pressed
    (bind _grave (CallFunction|GetGrave))
    (Utilities|IsValid _grave
      (:Is%20Not%20Valid
        (Class|MordhauSpectator|SecondarySpectatorAction)))))

(event Input|ActionEvents|InputActionTertiarySpectatorAction
  (params (Key :type Key%20Structure))
  (:Pressed
    (bind _grave (CallFunction|GetGrave))
    (Utilities|IsValid _grave
      (:Is%20Not%20Valid
        (Class|MordhauSpectator|TertiarySpectatorAction)))))

(fn ConstructionScript
  (|CallParentFunction))

(fn GetGrave
  (bind _returnvalue (Pawn|GetController))
  (Utilities|IsValid _returnvalue
    (:Is%20Valid
      (bind _asbp_horde_player_state (Utilities|Casting|CastToBP_HordePlayerState (Variables|/Script/Engine.Controller|GetPlayerState _returnvalue))
        (:then
          (return (Variables|/Game/Mordhau/Blueprints/GameModes/Horde/BP_HordePlayerState.BP_HordePlayerState_C|GetGrave _asbp_horde_player_state)))
        (:CastFailed
          _)))
    (:Is%20Not%20Valid
      _))
  (return 0))