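; Horde mode objective character on team 0 that players defend; its death triggers defeat.
; On BeginPlay the server gives it an AI controller and customization actor, then starts wave progression.
; Each wave sets DefenseUpgrades, whose RepNotify lowers damage taken and swaps appearance profiles, and replaces equipment from a per-wave map.
; Health feeds a floating defend widget and, every tick, the Horde HUD progress bar.
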(event EventBeginPlay
  (bind _mordhauwidget (Variables|Default|GetMordhauWidget))
  (|CallParentFunction)
  (Utilities|FlowControl|Sequence
    (:then_0
      (Utilities|IsValid _mordhauwidget
        (:Is%20Valid
          (bind _asbp_horde_defend_widget_floater (Utilities|Casting|CastToBP_HordeDefendWidgetFloater (UserInterface|GetUserWidgetObject _mordhauwidget)))
          (Default|UpdateHealth _asbp_horde_defend_widget_floater (Math|Conversions|ToFloat(Byte) (Variables|Default|GetHealth))))))
    (:then_1
      (Networking|SwitchHasAuthority
        (:Authority
          (Utilities|FlowControl|Delay 0.2)
          (bind _returnvalue (Game|SpawnActorfromClass "/Game/Mordhau/Blueprints/GameModes/Horde/Objectives/BP_HordeKillObjectiveAIController.BP_HordeKillObjectiveAIController_C" (Math|Transform|MakeTransform "0, 0, 0") "Undefined" 0 0))
          (bind _returnvalue_2 (Game|ConstructObjectfromClass (Variables|Default|GetBehaviorProfile) _returnvalue))
          (Variables|/Script/Mordhau.MordhauAIController|SetBehaviorProfile _returnvalue _returnvalue_2)
          (bind _returnvalue_3 (Game|SpawnActorfromClass "/Script/Mordhau.CustomizationReplicationActor" (Math|Transform|MakeTransform "0, 0, 0") "Undefined" 0 0))
          (bind _output_get (Variables|/Script/Mordhau.MordhauAIController|SetCustomizationReplicationActor _returnvalue _returnvalue_3))
          (bind _returnvalue_4 (Class|MordhauUtilityLibrary|MakeEmptyProfile "/Game/Mordhau/Blueprints/Characters/BP_MordhauCharacter.BP_MordhauCharacter_C" false))
          (Class|CustomizationReplicationActor|AssignDatafromProfile _returnvalue_3 _returnvalue_4)
          (Class|MordhauCharacter|SetCustomizationReplicationActor _output_get)
          (Pawn|Possess _returnvalue self)
          (CallFunction|OnWaveProgressed)
          (Class|MordhauCharacter|OnPostProfileAssigned))))))

(event Collision|EventActorBeginOverlap
  (params (OtherActor :type Actor%20Object%20Reference)))

(event EventTick
  (params (DeltaSeconds :type Float%20%28single-precision%29))
  (|CallParentFunction DeltaSeconds)
  (bind _asbp_horde_hud (Utilities|Casting|CastToBP_HordeHUD (Class|MordhauUtilityLibrary|GetMordhauHUD)))
  (Utilities|IsValid (Variables|/Game/Mordhau/Blueprints/GameModes/Horde/BP_HordeHUD.BP_HordeHUD_C|GetHordeHUDWidget _asbp_horde_hud)
    (:Is%20Valid
      (Variables|/Game/Mordhau/Blueprints/GameModes/Horde/BP_HordeHUDWidget.BP_HordeHUDWidget_C|SetObjectiveProgress (Variables|/Game/Mordhau/Blueprints/GameModes/Horde/BP_HordeHUD.BP_HordeHUD_C|GetHordeHUDWidget _asbp_horde_hud) (/ (Math|Conversions|ToFloat(Byte) (Variables|Default|GetHealth)) 1e+02)))))

(event EventOnDied
  (params (Angle :type Float%20%28single-precision%29) (Type :type EMordhauDamageType%20Enum :default "Generic") (SubType :type Byte :default 0) (bone :type Name%20%28by%20ref%29 :default "None") (Point :type Vector%20%28by%20ref%29 :default "0, 0, 0") (Source :type Actor%20Object%20Reference) (Agent :type Actor%20Object%20Reference))
  (bind _mordhauwidget (Variables|Default|GetMordhauWidget))
  (Utilities|FlowControl|Sequence
    (:then_0
      (Variables|/Script/Mordhau.MordhauWidgetComponent|SetOverrideVisible _mordhauwidget 0)
      (Variables|/Script/Mordhau.MordhauWidgetComponent|SetbIsSlowHideOverride _mordhauwidget true)
      (Variables|/Script/Mordhau.MordhauWidgetComponent|SetVisibilityWeightInterpolationSpeed _mordhauwidget 1.0)
      (bind _asbp_horde_defend_widget_floater (Utilities|Casting|CastToBP_HordeDefendWidgetFloater (UserInterface|GetUserWidgetObject (Variables|Default|GetMordhauWidget))))
      (Default|UpdateHealth _asbp_horde_defend_widget_floater 0.0))
    (:then_1
      (|CallParentFunction Angle Type SubType bone Point Source Agent))
    (:then_2
      (bind _asbp_horde_game_mode (Utilities|Casting|CastToBP_HordeGameMode (Game|GetGameMode)))
      (Default|TriggerDefeat _asbp_horde_game_mode))))

(event EventOnHealthChanged
  (bind _mordhauwidget (Variables|Default|GetMordhauWidget))
  (if (not (Class|AdvancedCharacter|GetIsDead))
    (Utilities|IsValid _mordhauwidget
      (:Is%20Valid
        (bind _asbp_horde_defend_widget_floater (Utilities|Casting|CastToBP_HordeDefendWidgetFloater (UserInterface|GetUserWidgetObject _mordhauwidget)))
        (Default|UpdateHealth _asbp_horde_defend_widget_floater (Math|Conversions|ToFloat(Byte) (Variables|Default|GetHealth)))))))

(fn ConstructionScript
  (|CallParentFunction)
  (Variables|Default|SetTeam 0))

(fn SpawnOurEquipment
  (for _array_element (Variables|Default|GetEquipmentToSpawn)
    (if (Utilities|IsValidClass _array_element)
      (bind _returnvalue (Game|SpawnActorfromClass _array_element (Math|Transform|MakeTransform "0, 0, 0") "Undefined" 0 0))
      (bind _returnvalue_2 (Class|MordhauEquipment|GetRandomCustomization _returnvalue false))
      (Class|MordhauEquipment|AssignCustomization _returnvalue _returnvalue_2)
      (Class|MordhauCharacter|PickUp _returnvalue))))

(fn OnRepDefenseUpgrades
  (bind _defenseupgrades (Variables|Default|GetDefenseUpgrades))
  (bind _defenseleveltoprofilemap (Variables|Default|GetDefenseLevelToProfileMap))
  (bind _returnvalue (Math|Conversions|ToInteger(Byte) _defenseupgrades))
  (Variables|Default|SetReceivedDamageModifier (- 1.0 (* (Math|Conversions|ToFloat(Byte) _defenseupgrades) 0.05)))
  (Networking|SwitchHasAuthority
    (:Authority
      (if (Utilities|Map|Contains _defenseleveltoprofilemap _returnvalue)
        (bind _returnvalue_2 (Class|MordhauCharacter|GetCustomizationReplicationActor))
        (Class|CustomizationReplicationActor|AssignDatafromProfile _returnvalue_2 (.Value (Utilities|Map|Find _defenseleveltoprofilemap _returnvalue)))))))

(fn OnRepOffenseUpgrades)

(fn OnWaveProgressed
  (params (NewWave :type Integer))
  (bind _wavetoequipmentmap (Variables|Default|GetWaveToEquipmentMap))
  (Variables|Default|SetDefenseUpgrades (Math|Conversions|ToByte(Integer) NewWave))
  (if (Utilities|Map|Contains _wavetoequipmentmap NewWave)
    (Utilities|FlowControl|Sequence
      (:then_0
        (Utilities|IsValid (Variables|Default|GetLastSpawnedEquipment)
          (:Is%20Valid
            (Class|MordhauCharacter|DropEquipment (Variables|Default|GetLastSpawnedEquipment) true)
            (Actor|DestroyActor (Variables|Default|GetLastSpawnedEquipment)))))
      (:then_1
        (bind _returnvalue (Game|SpawnActorfromClass (.Value (Utilities|Map|Find _wavetoequipmentmap NewWave)) (Math|Transform|MakeTransform "0, 0, 0") "Undefined" 0 0))
        (Utilities|IsValid _returnvalue
          (:Is%20Valid
            (bind _output_get (Variables|Default|SetLastSpawnedEquipment _returnvalue))
            (Variables|/Script/Mordhau.MordhauEquipment|SetbAllowDrop _output_get false)
            (bind _returnvalue_2 (Class|MordhauEquipment|GetRandomCustomization _output_get false))
            (Class|MordhauEquipment|AssignCustomization _output_get _returnvalue_2)
            (Class|MordhauCharacter|PickUp _output_get)))))))