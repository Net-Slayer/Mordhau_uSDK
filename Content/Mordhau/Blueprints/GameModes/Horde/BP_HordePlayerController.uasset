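; Player controller for Horde mode that owns the player's skill tree and carries loadout between pawns.
; On first possession the server copies skills, armor, equipment and ammo from BP_HordePlayerState, and EndPlay saves equipment back.
; Server-side upgrades spend skill points, checking prerequisites, a level cap and one ultimate.
; Scaled skill levels drive discounts, tougher built structures and bow perks, while rep notifies trigger sounds and ultimate HUD feedback.
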(event Custom|RequestUpgradeSkill
  (params (Skill :type E_HordeSkill%20Enum :default "NewEnumerator0"))
  (CallFunction|UpgradeSkill Skill))

(event EventBeginPlay
  (|CallParentFunction))

(event EventTick
  (params (DeltaSeconds :type Float%20%28single-precision%29))
  (|CallParentFunction DeltaSeconds) ; This node is disabled and will not be called.\nDrag off pins to build functionality.
)

(event EventOnAfterPossess
  (params (APawn :type Pawn%20Object%20Reference))
  (Utilities|FlowControl|Sequence
    (:then_0
      (bind _asbp_horde_character (Utilities|Casting|CastToBP_HordeCharacter APawn))
      (if (not (Variables|/Game/Mordhau/Blueprints/Characters/BP_HordeCharacter.BP_HordeCharacter_C|GetAlreadyGaveDefaults _asbp_horde_character))
        (Variables|/Game/Mordhau/Blueprints/Characters/BP_HordeCharacter.BP_HordeCharacter_C|SetAlreadyGaveDefaults _asbp_horde_character true)
        (Networking|SwitchHasAuthority
          (:Authority
            (bind _asbp_horde_player_state (Utilities|Casting|CastToBP_HordePlayerState (Variables|Default|GetPlayerState)))
            (Utilities|FlowControl|Sequence
              (:then_0
                (Variables|/Game/Mordhau/Blueprints/Characters/BP_HordeCharacter.BP_HordeCharacter_C|SetReplicatedSkills _asbp_horde_character (Variables|/Game/Mordhau/Blueprints/GameModes/Horde/BP_HordePlayerState.BP_HordePlayerState_C|GetReplicatedSkills _asbp_horde_player_state))
                (Utilities|FlowControl|Sequence
                  (:then_0
                    (if (> (CallFunction|GetSkillLevel "NewEnumerator3") 0)
                      (Variables|/Script/Mordhau.AdvancedCharacter|SetbHasLastChance _asbp_horde_character true)))))
              (:then_1
                (if (Utilities|IsValidClass (Variables|/Game/Mordhau/Blueprints/GameModes/Horde/BP_HordePlayerState.BP_HordePlayerState_C|GetLastHeadArmor _asbp_horde_player_state))
                  (Variables|/Game/Mordhau/Blueprints/Characters/BP_BattleRoyaleCharacter.BP_BattleRoyaleCharacter_C|SetHeadArmor _asbp_horde_character (Variables|/Game/Mordhau/Blueprints/GameModes/Horde/BP_HordePlayerState.BP_HordePlayerState_C|GetLastHeadArmor _asbp_horde_player_state))))
              (:then_2
                (if (Utilities|IsValidClass (Variables|/Game/Mordhau/Blueprints/GameModes/Horde/BP_HordePlayerState.BP_HordePlayerState_C|GetLastChestArmor _asbp_horde_player_state))
                  (Variables|/Game/Mordhau/Blueprints/Characters/BP_BattleRoyaleCharacter.BP_BattleRoyaleCharacter_C|SetChestArmor _asbp_horde_character (Variables|/Game/Mordhau/Blueprints/GameModes/Horde/BP_HordePlayerState.BP_HordePlayerState_C|GetLastChestArmor _asbp_horde_player_state))))
              (:then_3
                (if (Utilities|IsValidClass (Variables|/Game/Mordhau/Blueprints/GameModes/Horde/BP_HordePlayerState.BP_HordePlayerState_C|GetLastLegArmor _asbp_horde_player_state))
                  (Variables|/Game/Mordhau/Blueprints/Characters/BP_BattleRoyaleCharacter.BP_BattleRoyaleCharacter_C|SetLegArmor _asbp_horde_character (Variables|/Game/Mordhau/Blueprints/GameModes/Horde/BP_HordePlayerState.BP_HordePlayerState_C|GetLastLegArmor _asbp_horde_player_state))))
              (:then_4
                (for (_array_element _array_index) (Variables|/Game/Mordhau/Blueprints/GameModes/Horde/BP_HordePlayerState.BP_HordePlayerState_C|GetLastEquipment _asbp_horde_player_state)
                  (if (Utilities|IsValidClass _array_element)
                    (bind _returnvalue (Game|SpawnActorfromClass _array_element (Math|Transform|MakeTransform "0, 0, 0") "Undefined" 0 0))
                    (Utilities|FlowControl|Sequence
                      (:then_0
                        (CallFunction|CustomizeEquipment _returnvalue))
                      (:then_1
                        (Class|MordhauCharacter|PickUptoSlot _asbp_horde_character _returnvalue (Math|Conversions|ToByte(Integer) _array_index))
                        (if (!= (Utilities|Array|Get(acopy) (Variables|/Game/Mordhau/Blueprints/GameModes/Horde/BP_HordePlayerState.BP_HordePlayerState_C|GetLastEquipmentAmmo _asbp_horde_player_state) _array_index) (Class|MordhauEquipment|GetAmmo _returnvalue))
                          (Class|MordhauEquipment|SetAmmo _returnvalue (Utilities|Array|Get(acopy) (Variables|/Game/Mordhau/Blueprints/GameModes/Horde/BP_HordePlayerState.BP_HordePlayerState_C|GetLastEquipmentAmmo _asbp_horde_player_state) _array_index)))))))))))))
    (:then_1
      (|CallParentFunction APawn))))

(event EventOnBuilt
  (params (Structure :type Actor%20Object%20Reference))
  (bind _skilllevel (CallFunction|GetSkillLevelFloat "NewEnumerator50"))
  (bind _returnvalue (* _skilllevel 0.05))
  (bind _returnvalue_2 (- 1.0 _returnvalue))
  (|CallParentFunction Structure)
  (bind _asbp_destroyable_actor (Utilities|Casting|CastToBP_DestroyableActor Structure)
    (:then
      (Variables|/Game/Mordhau/Blueprints/Interactables/Environment/BP_DestroyableActor.BP_DestroyableActor_C|SetDamageFactor _asbp_destroyable_actor (* (Variables|/Game/Mordhau/Blueprints/Interactables/Environment/BP_DestroyableActor.BP_DestroyableActor_C|GetDamageFactor _asbp_destroyable_actor) _returnvalue_2)))
    (:CastFailed
      (bind _asbp_deployable_ballista (Utilities|Casting|CastToBP_DeployableBallista Structure))
      (Variables|/Script/Mordhau.AdvancedCharacter|SetReceivedDamageModifier _asbp_deployable_ballista (* (Variables|/Script/Mordhau.AdvancedCharacter|GetReceivedDamageModifier _asbp_deployable_ballista) _returnvalue_2)))))

(event EventEndPlay
  (params (EndPlayReason :type EEndPlayReason%20Enum :default "Destroyed"))
  (bind _asbp_horde_character (Utilities|Casting|CastToBP_HordeCharacter (Pawn|GetControlledPawn)))
  (Default|SaveEquipmenttoPlayerState _asbp_horde_character))

(event Input|ActionEvents|InputActionBattlecry
  (params (Key :type Key%20Structure)))

(event Input|ActionEvents|InputActionShowProfileSelect
  (params (Key :type Key%20Structure))
  (:Pressed
    (if (Variables|Default|GetNewHorde)
      (bind _asbp_horde_hud (Utilities|Casting|CastToBP_HordeHUD (Class|MordhauUtilityLibrary|GetMordhauHUD)))
      (Default|ShowSkillTree _asbp_horde_hud))))

(fn ConstructionScript
  (|CallParentFunction))

(fn OnRepPurchaseTrigger
  (Networking|CanExecuteCosmeticEvents
    (:True
      (Audio|PlaySound2D "/Game/Mordhau/Audio/Cues/UI/SC_HordePurchase.SC_HordePurchase" 1.0 1.0 0.0 0 0))))

(fn CustomizeEquipment
  (params (Equipment :type Mordhau%20Equipment%20Object%20Reference))
  (bind _characterprofile (Variables|Default|GetCharacterProfile))
  (bind _appearancecustomization (Utilities|Struct|BreakCharacterProfile _characterprofile))
  (bind (_emblem _emblemcolors) (Utilities|Struct|BreakAppearanceCustomization _appearancecustomization))
  (bind _returnvalue (Class|MordhauEquipment|GetRandomCustomization Equipment true))
  (LocalVariables|SetCustomization _returnvalue)
  (Utilities|FlowControl|Sequence
    (:then_0
      (LocalVariables|SetEmblem _emblem)
      (LocalVariables|SetEmblemColor1 (Utilities|Array|Get(acopy) _emblemcolors))
      (LocalVariables|SetEmblemColor2 (Utilities|Array|Get(acopy) _emblemcolors 1))
      (bind (_outcustomization _returnvalue_2) (Class|MordhauPlayerController|GetDefaultEquipmentCustomizationfor (Utilities|GetClass Equipment)))
      (if _returnvalue_2
        (LocalVariables|SetCustomization _outcustomization)))
    (:then_1
      (Class|MordhauEquipment|AssignCustomization Equipment (LocalVariables|GetCustomization) (Math|Conversions|ToByte(Integer) (LocalVariables|GetEmblem)) (LocalVariables|GetEmblemColor1) (LocalVariables|GetEmblemColor2)))))

(fn UpgradeSkill
  (params (Skill :type E_HordeSkill%20Enum :default "NewEnumerator0"))
  (bind _returnvalue (Math|Conversions|ToInteger(Byte) Skill))
  (bind _specialskill (Variables|Default|GetSpecialSkill))
  (bind _asbp_horde_player_state (Utilities|Casting|CastToBP_HordePlayerState (Variables|Default|GetPlayerState))
    (:then
      (Networking|SwitchHasAuthority
        (:Authority
          (if (and (> (Variables|/Game/Mordhau/Blueprints/GameModes/Horde/BP_HordePlayerState.BP_HordePlayerState_C|GetSkillPoints _asbp_horde_player_state) 0) (Utilities|Array|IsValidIndex (Variables|/Game/Mordhau/Blueprints/GameModes/Horde/BP_HordePlayerState.BP_HordePlayerState_C|GetReplicatedSkills _asbp_horde_player_state) _returnvalue))
            (if (CallFunction|HasPrerequisite Skill)
              (if (Math|Boolean|ANDBoolean (Utilities|Enum|NotEqual(Enum) _specialskill "NewEnumerator0") (Utilities|Enum|NotEqual(Enum) _specialskill Skill) (.Ultimate (Utilities|Struct|BreakSTRUCT_HordeSkillInfo (.Value (Utilities|Map|Find (Variables|Default|GetSkillInfo) Skill)))))
                (return false)
                (elif (< (Utilities|Array|Get(acopy) (Variables|/Game/Mordhau/Blueprints/GameModes/Horde/BP_HordePlayerState.BP_HordePlayerState_C|GetReplicatedSkills _asbp_horde_player_state) _returnvalue) 5)
                  (Utilities|FlowControl|Sequence
                    (:then_0
                      (if (== (Utilities|Array|Get(acopy) (Variables|/Game/Mordhau/Blueprints/GameModes/Horde/BP_HordePlayerState.BP_HordePlayerState_C|GetReplicatedSkills _asbp_horde_player_state) _returnvalue) 0)
                        (if (Utilities|Enum|Equal(Enum) Skill "NewEnumerator3")
                          (bind _asbp_horde_character (Utilities|Casting|CastToBP_HordeCharacter (Pawn|GetControlledPawn)))
                          (Variables|/Script/Mordhau.AdvancedCharacter|SetbHasLastChance _asbp_horde_character true))))
                    (:then_1
                      (Utilities|Array|SetArrayElem (Variables|/Game/Mordhau/Blueprints/GameModes/Horde/BP_HordePlayerState.BP_HordePlayerState_C|GetReplicatedSkills _asbp_horde_player_state) _returnvalue (+ (Utilities|Array|Get(acopy) (Variables|/Game/Mordhau/Blueprints/GameModes/Horde/BP_HordePlayerState.BP_HordePlayerState_C|GetReplicatedSkills _asbp_horde_player_state) _returnvalue) 1))
                      (CallFunction|SkillsUpdated)
                      (Variables|/Game/Mordhau/Blueprints/GameModes/Horde/BP_HordePlayerState.BP_HordePlayerState_C|SetSkillPoints _asbp_horde_player_state (- (Variables|/Game/Mordhau/Blueprints/GameModes/Horde/BP_HordePlayerState.BP_HordePlayerState_C|GetSkillPoints _asbp_horde_player_state) 1))
                      (return true)))
                  (else
                    (return false))))
              (else
                (return false)))
            (else
              (return false))))
        (:Remote
          (return false))))
    (:CastFailed
      (return false))))

(fn GetSkillLevel
  (params (Skill :type E_HordeSkill%20Enum :default "NewEnumerator0"))
  (bind _returnvalue (Math|Conversions|ToInteger(Byte) Skill))
  (bind _asbp_horde_player_state (Utilities|Casting|CastToBP_HordePlayerState (Variables|Default|GetPlayerState))
    (:then
      (if (Utilities|Array|IsValidIndex (Variables|/Game/Mordhau/Blueprints/GameModes/Horde/BP_HordePlayerState.BP_HordePlayerState_C|GetReplicatedSkills _asbp_horde_player_state) _returnvalue)
        (return (Utilities|Array|Get(acopy) (Variables|/Game/Mordhau/Blueprints/GameModes/Horde/BP_HordePlayerState.BP_HordePlayerState_C|GetReplicatedSkills _asbp_horde_player_state) _returnvalue))
        (else
          _)))
    (:CastFailed
      _))
  (return 0))

(fn HasPrerequisite
  (params (Skill :type E_HordeSkill%20Enum :default "NewEnumerator0"))
  (bind _skillprerequisites (Variables|Default|GetSkillPrerequisites))
  (bind (_value _returnvalue) (Utilities|Map|Find _skillprerequisites Skill))
  (if _returnvalue
    (if (or (> (CallFunction|GetSkillLevel _value) 0) (Utilities|Enum|Equal(Enum) _value "NewEnumerator0"))
      _
      (else
        (return false))))
  (return true))

(fn SkillsUpdated
  (bind _asbp_horde_player_state (Utilities|Casting|CastToBP_HordePlayerState (Variables|Default|GetPlayerState)))
  (Utilities|FlowControl|Sequence
    (:then_0
      (Variables|Default|SetSpecialSkill "NewEnumerator0")
      (bind (_array_element _array_index) (Utilities|Array|ForEachLoopwithBreak (Variables|/Game/Mordhau/Blueprints/GameModes/Horde/BP_HordePlayerState.BP_HordePlayerState_C|GetReplicatedSkills _asbp_horde_player_state) :!label _label)
        (:LoopBody
          (if (> _array_element 0)
            (if (and (.ReturnValue (Utilities|Map|Find (Variables|Default|GetSkillInfo) (Utilities|Enum|ByteToEnumE_HordeSkill (Math|Conversions|ToByte(Integer) _array_index)))) (.Ultimate (Utilities|Struct|BreakSTRUCT_HordeSkillInfo (.Value (Utilities|Map|Find (Variables|Default|GetSkillInfo) (Utilities|Enum|ByteToEnumE_HordeSkill (Math|Conversions|ToByte(Integer) _array_index)))))))
              (Variables|Default|SetSpecialSkill (Utilities|Enum|ByteToEnumE_HordeSkill (Math|Conversions|ToByte(Integer) _array_index)))
              (goto _label Break))))))
    (:then_1
      (Networking|SwitchHasAuthority
        (:Authority
          (bind _asbp_horde_character (Utilities|Casting|CastToBP_HordeCharacter (Pawn|GetControlledPawn)))
          (Variables|/Game/Mordhau/Blueprints/Characters/BP_HordeCharacter.BP_HordeCharacter_C|SetReplicatedSkills _asbp_horde_character (Variables|/Game/Mordhau/Blueprints/GameModes/Horde/BP_HordePlayerState.BP_HordePlayerState_C|GetReplicatedSkills _asbp_horde_player_state)))))
    (:then_2
      (bind _asbp_horde_hud (Utilities|Casting|CastToBP_HordeHUD (Class|MordhauUtilityLibrary|GetMordhauHUD)))
      (Utilities|IsValid (stale _skilltree)
        (:Is%20Valid
          (bind _skilltree (|SkillTree>refreshNodes _asbp_horde_hud)))))))

(fn GetSkillLevelFloat
  (params (Skill :type E_HordeSkill%20Enum :default "NewEnumerator0"))
  (return (Math|Conversions|ToFloat(Byte) (CallFunction|GetSkillLevel Skill))))

(fn TryFletcherRestock
  (Networking|SwitchHasAuthority
    (:Authority
      (if (<= (Math|Random|RandomFloat) (.PercentA (CallFunction|GetScaledSkillLevelParams "NewEnumerator33")))
        (bind _returnvalue (Class|MordhauPlayerController|GetLastControlledCharacter))
        (Utilities|IsValid _returnvalue
          (:Is%20Valid
            (if (Class|AdvancedCharacter|GetIsDead _returnvalue)
              (bind _asbp_bow (Utilities|Casting|CastToBP_Bow (Variables|/Script/Mordhau.MordhauCharacter|GetLeftHandEquipment _returnvalue)))
              (Class|MordhauEquipment|SetAmmo _asbp_bow (Class|KismetMathLibrary|BMin (+ (Class|MordhauEquipment|GetAmmo _asbp_bow) 1) (Class|MordhauEquipment|GetCurrentMaxAmmo _asbp_bow))))))))))

(fn TryScatterShot
  (params (SourceProjectile :type Mordhau%20Projectile%20Object%20Reference))
  (bind _returnvalue (Utilities|GetClass SourceProjectile))
  (bind _returnvalue_2 (Transformation|GetActorTransform SourceProjectile))
  (bind (_location _rotation _scale) (Math|Transform|BreakTransform _returnvalue_2))
  (bind (_roll _pitch _yaw) (Math|Rotator|BreakRotator _rotation))
  (bind (_roll_2 _pitch_2 _yaw_2) (Math|Rotator|BreakRotator _rotation))
  (Networking|SwitchHasAuthority
    (:Authority
      (if (not (Variables|Default|GetAvoidScattershotRecursion))
        (Variables|Default|SetAvoidScattershotRecursion true)
        (Utilities|FlowControl|Sequence
          (:then_0
            (if (<= (Math|Random|RandomFloat) (.PercentA (CallFunction|GetScaledSkillLevelParams "NewEnumerator34")))
              (bind _returnvalue_3 (Class|MordhauPlayerController|GetLastControlledCharacter))
              (Utilities|IsValid _returnvalue_3
                (:Is%20Valid
                  (Utilities|FlowControl|Sequence
                    (:then_0
                      (bind _returnvalue_4 (Game|SpawnActorfromClass _returnvalue (Math|Transform|MakeTransform (Math|Transform|TransformLocation _returnvalue_2 "50.000000,10.000000, 0") (Math|Rotator|MakeRotator _roll _pitch (+ _yaw 2.5)) _scale) "Undefined" 0 0))
                      (Variables|/Script/Mordhau.MordhauProjectile|SetbUsesLocalProjectileBlending _returnvalue_4 false)
                      (CallFunction|AssignFireArrowValues _returnvalue_4)
                      (Class|MordhauProjectile|InitializeProjectile _returnvalue_4 self false _returnvalue_3)
                      (Class|MordhauProjectile|Fire _returnvalue_4))
                    (:then_1
                      (bind _returnvalue_5 (Game|SpawnActorfromClass _returnvalue (Math|Transform|MakeTransform (Math|Transform|TransformLocation _returnvalue_2 "50.000000,-10.000000, 0") (Math|Rotator|MakeRotator _roll_2 _pitch_2 (+ _yaw_2 -2.5)) _scale) "Undefined" 0 0))
                      (Variables|/Script/Mordhau.MordhauProjectile|SetbUsesLocalProjectileBlending _returnvalue_5 false)
                      (CallFunction|AssignFireArrowValues _returnvalue_5)
                      (Class|MordhauProjectile|InitializeProjectile _returnvalue_5 self false _returnvalue_3)
                      (Class|MordhauProjectile|Fire _returnvalue_5)))))))
          (:then_1
            (Variables|Default|SetAvoidScattershotRecursion false)))))))

(fn AssignFireArrowValues
  (params (Arrow :type Actor%20Object%20Reference))
  (bind _asbp_arrow_projectile (Utilities|Casting|CastToBP_ArrowProjectile Arrow))
  (if (> (CallFunction|GetSkillLevel "NewEnumerator35") 0)
    (Variables|/Game/Mordhau/Blueprints/BP_MordhauProjectile.BP_MordhauProjectile_C|SetFireDamage _asbp_arrow_projectile 1e+01)
    (Variables|/Game/Mordhau/Blueprints/BP_MordhauProjectile.BP_MordhauProjectile_C|SetFireDuration _asbp_arrow_projectile (* (.TimeA (CallFunction|GetScaledSkillLevelParams "NewEnumerator35")) 0.5))
    (Variables|/Game/Mordhau/Blueprints/BP_MordhauProjectile.BP_MordhauProjectile_C|SetFireTick _asbp_arrow_projectile 0.5)))

(fn GetDiscountedPrice
  (params (BasePrice :type Integer))
  (return (Math|Float|Truncate (* BasePrice (- 1.0 (.PercentA (CallFunction|GetScaledSkillLevelParams "NewEnumerator41")))))))

(fn OnRepBackstabCounter
  (Audio|PlaySound2D 0 1.0 1.0 0.0 0 0))

(fn OnRepCriticalCounter
  (Audio|PlaySound2D 0 1.0 1.0 0.0 0 0))

(fn OnRepNextSpecialTime
  (bind _asbp_horde_game_state (Utilities|Casting|CastToBP_HordeGameState (Game|GetGameState)))
  (Variables|Default|SetSpecialTriggeredTime (GameState|GetServerWorldTimeSeconds _asbp_horde_game_state))
  (bind _asbp_horde_hud (Utilities|Casting|CastToBP_HordeHUD (Class|MordhauUtilityLibrary|GetMordhauHUD)))
  (Default|UltimateUsed (Variables|/Game/Mordhau/Blueprints/GameModes/Horde/BP_HordeHUDWidget.BP_HordeHUDWidget_C|GetBP_UltimateDisplay (Variables|/Game/Mordhau/Blueprints/GameModes/Horde/BP_HordeHUD.BP_HordeHUD_C|GetHordeHUDWidget _asbp_horde_hud))))

(fn GetScaledSkillLevelParams
  (params (Skill :type E_HordeSkill%20Enum :default "NewEnumerator0") (Bias :type Integer))
  (bind _returnvalue (Math|Conversions|ToInteger(Byte) Skill))
  (bind _skillinfo (Variables|Default|GetSkillInfo))
  (bind _value (Utilities|Map|Find _skillinfo Skill))
  (bind (_name _description _nextleveldescription _icon _ultimate _percenta _percentb _integera _timea) (Utilities|Struct|BreakSTRUCT_HordeSkillInfo _value))
  (bind _asbp_horde_player_state (Utilities|Casting|CastToBP_HordePlayerState (Variables|Default|GetPlayerState))
    (:then
      (if (Utilities|Array|IsValidIndex (Variables|/Game/Mordhau/Blueprints/GameModes/Horde/BP_HordePlayerState.BP_HordePlayerState_C|GetReplicatedSkills _asbp_horde_player_state) _returnvalue)
        (if (> (+ Bias (Math|Conversions|ToInteger(Byte) (Utilities|Array|Get(acopy) (Variables|/Game/Mordhau/Blueprints/GameModes/Horde/BP_HordePlayerState.BP_HordePlayerState_C|GetReplicatedSkills _asbp_horde_player_state) _returnvalue))) 0)
          (return (* _percenta (Math|Conversions|ToFloat(Integer) (+ Bias (Math|Conversions|ToInteger(Byte) (Utilities|Array|Get(acopy) (Variables|/Game/Mordhau/Blueprints/GameModes/Horde/BP_HordePlayerState.BP_HordePlayerState_C|GetReplicatedSkills _asbp_horde_player_state) _returnvalue))))) (* _percentb (Math|Conversions|ToFloat(Integer) (+ Bias (Math|Conversions|ToInteger(Byte) (Utilities|Array|Get(acopy) (Variables|/Game/Mordhau/Blueprints/GameModes/Horde/BP_HordePlayerState.BP_HordePlayerState_C|GetReplicatedSkills _asbp_horde_player_state) _returnvalue))))) (* _integera (+ Bias (Math|Conversions|ToInteger(Byte) (Utilities|Array|Get(acopy) (Variables|/Game/Mordhau/Blueprints/GameModes/Horde/BP_HordePlayerState.BP_HordePlayerState_C|GetReplicatedSkills _asbp_horde_player_state) _returnvalue)))) (* _timea (Math|Conversions|ToFloat(Integer) (+ Bias (Math|Conversions|ToInteger(Byte) (Utilities|Array|Get(acopy) (Variables|/Game/Mordhau/Blueprints/GameModes/Horde/BP_HordePlayerState.BP_HordePlayerState_C|GetReplicatedSkills _asbp_horde_player_state) _returnvalue))))))
          (else
            _))))
    (:CastFailed
      _))
  (return 0.0 0.0 0 0.0))