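; Horde mode spawn actor that briefly shows a floating enemy-spawn marker when it is activated.
; Replication of the spawn activation counter clears the MordhauWidget visibility override and plays the floater's SizeBounce animation.
; A retriggerable delay then hides the widget a few seconds later, so repeated activations keep it visible.
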(event Custom|HideFloaterDelayed
  (Utilities|FlowControl|RetriggerableDelay 4.0)
  (Variables|/Script/Mordhau.MordhauWidgetComponent|SetOverrideVisible (Variables|Default|GetMordhauWidget) 0))

(event EventBeginPlay)

(event Collision|EventActorBeginOverlap
  (params (OtherActor :type Actor%20Object%20Reference)))

(event EventTick
  (params (DeltaSeconds :type Float%20%28single-precision%29)))

(fn ConstructionScript)

(fn OnRepSpawnActivatedCounter
  (bind _mordhauwidget (Variables|Default|GetMordhauWidget))
  (Variables|/Script/Mordhau.MordhauWidgetComponent|SetOverrideVisible _mordhauwidget -1)
  (bind _asbp_horde_enemy_spawn_floater (Utilities|Casting|CastToBP_HordeEnemySpawnFloater (UserInterface|GetUserWidgetObject _mordhauwidget)))
  (UserInterface|Animation|PlayAnimation _asbp_horde_enemy_spawn_floater (Variables|/Game/Mordhau/Blueprints/GameModes/Horde/BP_HordeEnemySpawnFloater.BP_HordeEnemySpawnFloater_C|GetSizeBounce _asbp_horde_enemy_spawn_floater) 0.0 1 "Forward" 1.0)
  (CallFunction|HideFloaterDelayed))