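; Battering ram objective for Battle mode that players use by held interaction to break down a linked RamDoor.
; Each interaction change plays the ram animation, then after a timed delay plays the door's hit animation, or its death once the required count is reached.
; An IsAnimating flag blocks use mid-swing and stays set after the final hit.
; Valid characters must also be near UsePoint to interact.
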(event EventOnInteractionsChanged
  (bind _skeletalmesh (Variables|Default|GetSkeletalMesh))
  (|CallParentFunction)
  (Variables|Default|SetIsAnimating true)
  (Components|Animation|SetPosition _skeletalmesh 0.0 false)
  (Audio|Components|Audio|Play _skeletalmesh false)
  (Utilities|FlowControl|RetriggerableDelay 2.353)
  (CallFunction|DoDoorHit)
  (bind _output_get (Variables|Default|SetCompletedInteractionsWithDelay (Variables|Default|GetInteractions)))
  (if (not (== _output_get (Variables|Default|GetRequiredInteractions)))
    (Utilities|FlowControl|RetriggerableDelay 1.0)
    (Variables|Default|SetIsAnimating false)))

(fn ConstructionScript
  (|CallParentFunction))

(fn DoDoorHit
  (bind _ramdoor (Variables|Default|GetRamDoor))
  (Utilities|IsValid _ramdoor
    (:Is%20Valid
      (if (== (Variables|Default|GetInteractions) (Variables|Default|GetRequiredInteractions))
        (Default|PlayDeath _ramdoor)
        (else
          (Default|PlayAnim _ramdoor))))))

(fn CanHeldInteract
  (params (Character :type Mordhau%20Character%20Object%20Reference))
  (if (Variables|Default|GetIsAnimating)
    _
    (else
      (Utilities|IsValid Character
        (:Is%20Valid
          (if (<= (Math|Vector|VectorLength (- (Transformation|GetActorLocation Character) (Transformation|GetWorldLocation (Variables|Default|GetUsePoint)))) 2e+02)
            (return (|CallParentFunction Character))
            (else
              _)))
        (:Is%20Not%20Valid
          (return (|CallParentFunction Character))))))
  (return false))