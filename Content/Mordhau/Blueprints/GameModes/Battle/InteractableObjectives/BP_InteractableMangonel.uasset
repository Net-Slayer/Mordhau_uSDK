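; An interactable battle objective mangonel that loads and fires a rock as players progress the objective.
; Progress changes scrub the skeletal mesh animation, and one interaction before completion the rock snaps to the projectile socket.
; On the final interaction it plays the firing animation, detaches the rock and moves it along a spline by timeline.
; When the timeline ends, a particle effect activates at a spline point and the rock is destroyed.
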(event EventBeginPlay)

(event Collision|EventActorBeginOverlap
  (params (OtherActor :type Actor%20Object%20Reference))
  (|CallParentFunction OtherActor) ; This node is disabled and will not be called.\nDrag off pins to build functionality.
)

(event EventTick
  (params (DeltaSeconds :type Float%20%28single-precision%29))
  (|CallParentFunction DeltaSeconds))

(event EventOnAnyObjectiveProgressChanged
  (bind _requiredinteractions (Variables|Default|GetRequiredInteractions))
  (bind _spline (Variables|Default|GetSpline))
  (bind _sk_mangonel (Variables|Default|GetSK_Mangonel))
  (bind _spline_2 (Variables|/Game/Mordhau/Blueprints/Interactables/BP_SplineActor.BP_SplineActor_C|GetSpline _spline))
  (bind _progress (CallFunction|GetObjectiveProgress))
  (Utilities|FlowControl|Sequence
    (:then_0
      (Components|Animation|SetPosition (Variables|Default|GetSK_Mangonel) _progress true))
    (:then_1
      (if (== (Variables|Default|GetInteractions) (- _requiredinteractions 1))
        (Utilities|FlowControl|DoOnce false
          (:Completed
            (Transformation|AttachComponentToComponent (Variables|Default|GetCatapultRock) (Variables|Default|GetSK_Mangonel) "Projectile" "SnapToTarget" "SnapToTarget" "SnapToTarget" false)))))
    (:then_2
      (if (== _requiredinteractions (Variables|Default|GetInteractions))
        (Utilities|FlowControl|DoOnce false
          (:Completed
            (Components|Animation|PlayAnimation _sk_mangonel 0 false)
            (Components|Timeline|SetPlayRate _sk_mangonel 2.0)
            (Utilities|FlowControl|Delay 0.3)
            (Components|Animation|PlayAnimation _sk_mangonel 0 false)
            (Transformation|DetachFromComponent (Variables|Default|GetCatapultRock) "KeepRelative" "KeepRelative" "KeepRelative" true)
            (bind _track (Timeline|Timeline_0 Play)
              (:Update
                (Transformation|SetWorldLocationAndRotation (Variables|Default|GetCatapultRock) (Spline|GetLocationatDistanceAlongSpline _spline_2 (* (Spline|GetSplineLength _spline_2) _track) "World") "0, 0, 0" false false))
              (:Finished
                (Transformation|SetWorldLocation (Variables|Default|GetParticleSystem) (Spline|GetLocationatSplinePoint _spline_2 2 "World") false false)
                (Components|Activation|Activate (Variables|Default|GetParticleSystem) false)
                (Components|DestroyComponent (Variables|Default|GetCatapultRock))))))))))

(fn ConstructionScript
  (|CallParentFunction))