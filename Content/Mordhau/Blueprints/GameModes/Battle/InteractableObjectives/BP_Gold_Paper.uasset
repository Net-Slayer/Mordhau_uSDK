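; BP_Gold_Paper is an interactable objective for Battle mode, a gold pile with coins, props and a crate lid that visibly empties as players interact with it.
; Each interaction change plays a coin sound and splash effect, skipped during the first four seconds of world time.
; Props hide in stages at the first interaction, past half the required count and on completion, when the pile and lid also lose collision.
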(event EventBeginPlay)

(event Collision|EventActorBeginOverlap
  (params (OtherActor :type Actor%20Object%20Reference))
  (|CallParentFunction OtherActor) ; This node is disabled and will not be called.\nDrag off pins to build functionality.
)

(event EventTick
  (params (DeltaSeconds :type Float%20%28single-precision%29))
  (|CallParentFunction DeltaSeconds) ; This node is disabled and will not be called.\nDrag off pins to build functionality.
)

(event EventOnInteractionsChanged
  (bind _interactions (Variables|Default|GetInteractions))
  (bind _requiredinteractions (Variables|Default|GetRequiredInteractions))
  (bind _pile (Variables|Default|GetPile))
  (|CallParentFunction)
  (Utilities|FlowControl|Sequence
    (:then_0
      (if (> (Utilities|Time|GetTimeSeconds) 4.0)
        (Audio|Components|Audio|Play (Variables|Default|GetSC_CoinObjective) 0.0)
        (Components|Activation|Activate (Variables|Default|GetP_CoinSplash) false)))
    (:then_1
      (if (> _interactions 0)
        (Development|SetHiddeninGame (Variables|Default|Getchalice_02) true false)
        (if (> _interactions (/ _requiredinteractions 2))
          (Development|SetHiddeninGame (Variables|Default|Gettr_book_01) true false)
          (if (>= _interactions _requiredinteractions)
            (Development|SetHiddeninGame _pile true false)
            (Collision|SetCollisionEnabled _pile "NoCollision")))))))

(fn ConstructionScript
  (|CallParentFunction))