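; Destroyable cog ship for Frontline battles that sails a looping spline route and sinks when destroyed.
; Each tick derives its spline position and heading from replicated server world time, keeping movement in sync without replicating transforms.
; At zero replicated health it stops ticking, deactivates the bow wave, then after a delay eases the mesh downward into a roll.
; An unconnected authority-only trace that would destroy destroyables and ballistas at the mesh never runs.
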(event EventBeginPlay
  (|CallParentFunction) ; This node is disabled and will not be called.\nDrag off pins to build functionality.
)

(event Collision|EventActorBeginOverlap
  (params (OtherActor :type Actor%20Object%20Reference))
  (|CallParentFunction OtherActor) ; This node is disabled and will not be called.\nDrag off pins to build functionality.
)

(event EventTick
  (params (DeltaSeconds :type Float%20%28single-precision%29))
  (bind _returnvalue (Game|GetGameState))
  (bind _spline (Variables|Default|GetSpline))
  (bind _spline_2 (Variables|/Game/Mordhau/Blueprints/Interactables/BP_SplineActor.BP_SplineActor_C|GetSpline _spline))
  (bind _returnvalue_2 (Spline|GetSplineLength _spline_2))
  (|CallParentFunction DeltaSeconds)
  (Utilities|IsValid _returnvalue
    (:Is%20Valid
      (if (== (Variables|Default|GetReplicatedHealth) 0)
        (Actor|Tick|SetActorTickEnabled false)
        (Components|Activation|Deactivate (Variables|Default|GetP_BowWave))
        (Utilities|FlowControl|Delay 7.0)
        (Components|MoveComponentTo (Variables|Default|GetSkeletalMesh) "0.000000, 0,-750.000000" "0,180.000000, 0" true true 5.0 false)
        (else
          (Variables|Default|SetTrack (Math|Float|%(Float) (/ (GameState|GetServerWorldTimeSeconds _returnvalue) (/ _returnvalue_2 (Variables|Default|GetMoveSpeed))) 1.0))
          (Transformation|SetActorLocationAndRotation self (Spline|GetLocationatDistanceAlongSpline _spline_2 (Math|Float|Lerp 0.0 _returnvalue_2 (Variables|Default|GetTrack)) "World") (Math|Rotator|MakeRotator 0.0 (.Roll (Math|Rotator|BreakRotator (Spline|GetRotationatDistanceAlongSpline _spline_2 (Math|Float|Lerp 0.0 _returnvalue_2 (Variables|Default|GetTrack)) "World"))) (- (.Yaw (Math|Rotator|BreakRotator (Spline|GetRotationatDistanceAlongSpline _spline_2 (Math|Float|Lerp 0.0 _returnvalue_2 (Variables|Default|GetTrack)) "World"))) 9e+01))))))))

(fn ConstructionScript
  (|CallParentFunction))