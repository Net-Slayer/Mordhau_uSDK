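; Battle-mode objective where players deliver BP_DeliverableEquipment into an area to advance a linked capture point.
; On authority, overlaps consume each item, score its last carrier and increment a replicated count.
; The OnRep updates progress, widget and staged visuals, notifies the capture point and disables the completed spot.
; Enemy prerequisites toggle the spot and its delivery spawns, and the progress bar flips according to the local player's team.
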(event OnComponentBeginOverlap(Area)
  (params (OverlappedComponent :type Primitive%20Component%20Object%20Reference) (OtherActor :type Actor%20Object%20Reference) (OtherComp :type Primitive%20Component%20Object%20Reference) (OtherBodyIndex :type Integer) (bFromSweep :type Boolean) (SweepResult :type Hit%20Result%20Structure%20%28by%20ref%29))
  (Networking|SwitchHasAuthority
    (:Authority
      (if (< (Variables|Default|GetDeliverables) (Variables|Default|GetRequiredDeliveries))
        (bind _asbp_deliverable_equipment (Utilities|Casting|CastToBP_DeliverableEquipment OtherActor))
        (if (not (Variables|/Game/Mordhau/Blueprints/GameModes/Battle/BP_DeliverableEquipment.BP_DeliverableEquipment_C|GetConsumed _asbp_deliverable_equipment))
          (Utilities|FlowControl|Sequence
            (:then_0
              (Utilities|IsValid (Variables|/Game/Mordhau/Blueprints/GameModes/Battle/BP_DeliverableEquipment.BP_DeliverableEquipment_C|GetLastEquippedByPlayerController _asbp_deliverable_equipment)
                (:Is%20Valid
                  (Class|MordhauPlayerController|GiveClientScoreBP (Variables|/Game/Mordhau/Blueprints/GameModes/Battle/BP_DeliverableEquipment.BP_DeliverableEquipment_C|GetLastEquippedByPlayerController _asbp_deliverable_equipment) "Objective" (Variables|Default|GetScoreAwardPerDelivery)))))
            (:then_1
              (Default|Consume _asbp_deliverable_equipment))
            (:then_2
              (Variables|Default|SetDeliverables (+ (Variables|Default|GetDeliverables) 1))
              (Networking|ForceNetUpdate))))))))

(event Custom|OnDeliverablesChanged)

(event Custom|ProgressVisualStage)

(event EventOnAnyObjectiveProgressChanged
  (CallFunction|AnyObjectiveProgressChanged))

(event Collision|EventActorBeginOverlap
  (params (OtherActor :type Actor%20Object%20Reference)))

(event EventTick
  (params (DeltaSeconds :type Float%20%28single-precision%29)))

(event EventOnInitialize
  (params (Point :type BP%20Capture%20Point%20Object%20Reference))
  (CallFunction|Initialize Point))

(event EventOnEnemyGainedPrerequisites
  (CallFunction|EnemyGainedPrerequisites))

(event EventOnEnemyLostPrerequisites
  (CallFunction|EnemyLostPrerequisites))

(event EventOnUpdateUIWidgets
  (bind _capturepoint (Variables|Default|GetCapturePoint))
  (Utilities|IsValid _capturepoint
    (:Is%20Valid
      (if (not (== (Variables|/Game/Mordhau/Blueprints/GameModes/Battle/BP_CapturePoint.BP_CapturePoint_C|GetObjectiveProgress _capturepoint) 1.0))
        (CallFunction|UpdateFlipProgressBarState)
        (CallFunction|UpdateFloater)))))

(fn ConstructionScript
  (|CallParentFunction)
  (Variables|Default|SetOriginalFlipProgressBar (Variables|Default|GetFlipProgressBar)))

(fn OnRepDeliverables
  (bind _capturepoint (Variables|Default|GetCapturePoint))
  (Utilities|FlowControl|Sequence
    (:then_0
      (Variables|Default|SetProgress (/ (Math|Conversions|ToFloat(Byte) (Variables|Default|GetDeliverables)) (Math|Conversions|ToFloat(Byte) (Variables|Default|GetRequiredDeliveries)))))
    (:then_1
      (if (>= (Variables|Default|GetDeliverables) (Variables|Default|GetRequiredDeliveries))
        (CallFunction|Disable true)))
    (:then_2
      (Utilities|IsValid _capturepoint
        (:Is%20Valid
          (Default|ObjectivesChanged _capturepoint)
          (bind _isdone (CallFunction|IsCapturePointDone))
          (if _isdone
            (CallFunction|DisableSpawns)))))
    (:then_3
      (CallFunction|UpdateFloater))
    (:then_4
      (CallFunction|UpdateDeliverySpotVisuals))
    (:then_5
      (CallFunction|OnDeliverablesChanged))))

(fn Activate
  (if (< (Variables|Default|GetDeliverables) (Variables|Default|GetRequiredDeliveries))
    (Collision|SetCollisionEnabled (Variables|Default|GetArea) "QueryOnly")
    (Variables|/Script/Mordhau.MordhauWidgetComponent|SetOverrideVisible (Variables|Default|GetMordhauWidget) -1)
    (Development|SetHiddeninGame (Variables|Default|GetDecal) false false)))

(fn Disable
  (params (SlowDisable :type Boolean))
  (bind _mordhauwidget (Variables|Default|GetMordhauWidget))
  (Collision|SetCollisionEnabled (Variables|Default|GetArea) "NoCollision")
  (Variables|/Script/Mordhau.MordhauWidgetComponent|SetOverrideVisible _mordhauwidget 0)
  (Development|SetHiddeninGame (Variables|Default|GetDecal) true false)
  (if SlowDisable
    (Variables|/Script/Mordhau.MordhauWidgetComponent|SetbIsSlowHideOverride _mordhauwidget true)
    (Variables|/Script/Mordhau.MordhauWidgetComponent|SetVisibilityWeightInterpolationSpeed _mordhauwidget 1.0)))

(fn Initialize
  (params (CapturePoint :type BP%20Capture%20Point%20Object%20Reference))
  (Variables|Default|SetCapturePoint CapturePoint)
  (for _array_element (Variables|Default|GetDeliverySpawns)
    (Utilities|IsValid _array_element
      (:Is%20Valid
        (Variables|/Game/Mordhau/Blueprints/GameModes/Battle/BP_ItemDeliverySpawn.BP_ItemDeliverySpawn_C|SetCapturePoint _array_element CapturePoint))))
  (CallFunction|UpdateFlipProgressBarState))

(fn EnemyGainedPrerequisites
  (bind _isdone (CallFunction|IsCapturePointDone))
  (if (not _isdone)
    (CallFunction|Activate)
    (CallFunction|ActivateSpawns)))

(fn EnemyLostPrerequisites
  (CallFunction|Disable false)
  (CallFunction|DisableSpawns))

(fn UpdateDeliverySpotVisuals
  (bind _requireddeliveries (Variables|Default|GetRequiredDeliveries))
  (bind _deliverables (Variables|Default|GetDeliverables))
  (bind _returnvalue (Math|Conversions|ToFloat(Byte) _requireddeliveries))
  (while (< (Variables|Default|GetVisualStage) (Math|Integer|Max(Integer) (Math|Float|Truncate (Math|Float|MapRangeClamped (Math|Conversions|ToFloat(Byte) _deliverables) 0.0 _returnvalue 0.0 (Math|Float|Min(Float) _returnvalue (Math|Conversions|ToFloat(Integer) (Variables|Default|GetMaxVisualStage))))) (Math|Conversions|ToInteger(Byte) (Math|Conversions|ToByte(Integer) (>= _deliverables 1)))))
    (CallFunction|ProgressVisualStage)
    (Variables|Default|SetVisualStage (+ (Variables|Default|GetVisualStage) 1))))

(fn DisableSpawns
  (for _array_element (Variables|Default|GetDeliverySpawns)
    (Utilities|IsValid _array_element
      (:Is%20Valid
        (Default|Disable _array_element)))))

(fn ActivateSpawns
  (for _array_element (Variables|Default|GetDeliverySpawns)
    (Utilities|IsValid _array_element
      (:Is%20Valid
        (Default|Activate _array_element)))))

(fn IsCapturePointDone
  (bind _capturepoint (Variables|Default|GetCapturePoint))
  (Utilities|IsValid _capturepoint
    (:Is%20Valid
      (return (== (Variables|/Game/Mordhau/Blueprints/GameModes/Battle/BP_CapturePoint.BP_CapturePoint_C|GetObjectiveProgress _capturepoint) 1.0)))
    (:Is%20Not%20Valid
      (return false))))

(fn AnyObjectiveProgressChanged
  (bind _capturepoint (Variables|Default|GetCapturePoint))
  (Utilities|IsValid _capturepoint
    (:Is%20Valid
      (if (== (Variables|/Game/Mordhau/Blueprints/GameModes/Battle/BP_CapturePoint.BP_CapturePoint_C|GetObjectiveProgress _capturepoint) 1.0)
        (CallFunction|EnemyLostPrerequisites)
        (else
          (bind _array_element (Utilities|Array|ForEachLoopwithBreak (Variables|/Game/Mordhau/Blueprints/GameModes/Battle/BP_CapturePoint.BP_CapturePoint_C|GetDeliverySpots _capturepoint) :!label _label)
            (:LoopBody
              (Utilities|IsValid _array_element
                (:Is%20Valid
                  (bind _progress (CallFunction|GetObjectiveProgress _array_element))
                  (if (!= _progress 1.0)
                    (LocalVariables|SetAllDeliveriesFinished false)
                    (goto _label Break)))))
            (:Completed
              (if (LocalVariables|GetAllDeliveriesFinished)
                (CallFunction|EnemyLostPrerequisites)))))))))

(fn UpdateFloater
  (bind _progress (Variables|Default|GetProgress))
  (bind _asbp_delivery_spot_widget_floater (Utilities|Casting|CastToBP_DeliverySpotWidgetFloater (UserInterface|GetUserWidgetObject (Variables|Default|GetMordhauWidget))))
  (Default|UpdateProgress _asbp_delivery_spot_widget_floater (select (Variables|Default|GetFlipProgressBar) _progress (- 1.0 _progress)) true))

(fn UpdateFlipProgressBarState
  (bind _capturepoint (Variables|Default|GetCapturePoint))
  (Utilities|IsValid _capturepoint
    (:Is%20Valid
      (bind _asmordhau_player_controller (Utilities|Casting|CastToMordhauPlayerController (Game|GetPlayerController 0)))
      (bind _asbp_mordhau_player_state (Utilities|Casting|CastToBP_MordhauPlayerState (Variables|/Script/Engine.Controller|GetPlayerState _asmordhau_player_controller)))
      (if (== (Variables|/Script/Mordhau.ControlPoint|GetOwningTeam _capturepoint) (Math|Conversions|ToByte(Integer) (Variables|/Script/Mordhau.MordhauPlayerState|GetTeam _asbp_mordhau_player_state)))
        (Variables|Default|SetFlipProgressBar false)
        (else
          (Variables|Default|SetFlipProgressBar (Variables|Default|GetOriginalFlipProgressBar)))))))

(fn GetObjectiveProgress
  (return (* (Variables|Default|GetProgress) (Variables|Default|GetObjectiveWeight))))

(fn IsCompleted
  (return (== (Variables|Default|GetProgress) 1.0)))

(fn IsinObjectiveArea
  (params (Location :type Vector :default "0, 0, 0"))
  (return (< (Math|Vector|VectorLengthXY (- Location (Transformation|GetActorLocation))) 1e+03)))