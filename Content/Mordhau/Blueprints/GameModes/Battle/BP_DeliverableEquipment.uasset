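; Team-restricted equipment for Battle mode that is carried or thrown as a deliverable and can be broken by opponents.
; The UsableByTeam team gets normal interaction; others get a held interaction that sets replicated Broke, whose notify clears the mesh and expires the actor.
; DeliverableCollision optionally stays off until thrown.
; Consume removes that collision, switches the carrier to fists, and destroys or drops the item; pickup records the last player controller.
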(event Custom|OnBroken
  (bind _skeletalmeshcomponent (Variables|Default|GetSkeletalMeshComponent))
  (bind _deliverablecollision (Variables|Default|GetDeliverableCollision))
  (Variables|Default|SetbIsInteractable false)
  (Utilities|FlowControl|Sequence
    (:then_0
      (Networking|SwitchHasAuthority
        (:Authority
          (Actor|SetLifeSpan 2.0)
          (Utilities|IsValid _deliverablecollision
            (:Is%20Valid
              (Components|DestroyComponent _deliverablecollision))))))
    (:then_1
      (Utilities|IsValid (Variables|/Script/Engine.SkinnedMeshComponent|GetSkeletalMesh _skeletalmeshcomponent)
        (:Is%20Valid
          (Class|SkinnedMeshComponent|SetSkeletalMesh _skeletalmeshcomponent 0 true))))
    (:then_2
      (Class|MordhauEquipment|UpdateEquipmentState))))

(event EventOnThud
  (|CallParentFunction))

(event EventFireProjectile
  (params (Origin :type Vector%20%28by%20ref%29 :default "0, 0, 0") (Orientation :type Rotator%20%28by%20ref%29 :default "0, 0, 0") (OwningController :type Controller%20Object%20Reference) (ExpectedDelay :type Float%20%28single-precision%29))
  (bind _deliverablecollision (Variables|Default|GetDeliverableCollision))
  (|CallParentFunction Origin Orientation OwningController ExpectedDelay)
  (Networking|SwitchHasAuthority
    (:Authority
      (Utilities|IsValid _deliverablecollision
        (:Is%20Valid
          (if (and (not (Class|PrimitiveComponent|IsQueryCollisionEnabled _deliverablecollision)) (Variables|Default|GetMustThrow))
            (Collision|SetCollisionEnabled _deliverablecollision "QueryOnly")))))))

(event EventOnPickedUp
  (params (Character :type Mordhau%20Character%20Object%20Reference))
  (|CallParentFunction Character)
  (bind _asmordhau_player_controller (Utilities|Casting|CastToMordhauPlayerController (Pawn|GetController Character)))
  (Variables|Default|SetLastEquippedByPlayerController _asmordhau_player_controller))

(event EventOnHeldInteractionStart
  (params (Character :type Mordhau%20Character%20Object%20Reference))
  (CallFunction|Break))

(fn ConstructionScript
  (|CallParentFunction)
  (if (Variables|Default|GetMustThrow)
    (Collision|SetCollisionEnabled (Variables|Default|GetDeliverableCollision) "NoCollision")))

(fn Consume
  (bind _deliverablecollision (Variables|Default|GetDeliverableCollision))
  (if (not (Variables|Default|GetConsumed))
    (Variables|Default|SetConsumed true)
    (Utilities|FlowControl|Sequence
      (:then_0
        (Utilities|IsValid _deliverablecollision
          (:Is%20Valid
            (Components|DestroyComponent _deliverablecollision))))
      (:then_1
        (bind _output_get (LocalVariables|SetParentCharDeref (Class|MordhauEquipment|GetParentCharacter)))
        (if (Variables|Default|GetDestroysOnDelivery)
          (Utilities|FlowControl|Sequence
            (:then_0
              (Utilities|IsValid _output_get
                (:Is%20Valid
                  (Class|MordhauCharacter|SwitchtoFists _output_get))))
            (:then_1
              (Actor|DestroyActor)))
          (else
            (Utilities|IsValid _output_get
              (:Is%20Valid
                (Class|MordhauCharacter|DropEquipment _output_get self false)
                (Class|MordhauCharacter|SwitchtoFists _output_get)))))))))

(fn OnRepBroke
  (CallFunction|OnBroken))

(fn Break
  (if (not (Variables|Default|GetBroke))
    (Variables|Default|SetBroke true)
    (Networking|ForceNetUpdate)))

(fn CanHeldInteract
  (params (Character :type Mordhau%20Character%20Object%20Reference))
  (Utilities|IsValid Character
    (:Is%20Valid
      (if (!= (Variables|/Script/Mordhau.AdvancedCharacter|GetTeam Character) (Variables|Default|GetUsableByTeam))
        _
        (else
          (return false))))
    (:Is%20Not%20Valid
      _))
  (return (|CallParentFunction Character)))

(fn CanInteract
  (params (Character :type Mordhau%20Character%20Object%20Reference))
  (Utilities|IsValid Character
    (:Is%20Valid
      (if (== (Variables|/Script/Mordhau.AdvancedCharacter|GetTeam Character) (Variables|Default|GetUsableByTeam))
        _
        (else
          (return false))))
    (:Is%20Not%20Valid
      _))
  (return (|CallParentFunction Character)))