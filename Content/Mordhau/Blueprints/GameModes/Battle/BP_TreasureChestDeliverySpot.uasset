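; Battle mode delivery spot for treasure chests that shows more chest meshes as its visual stage progresses.
; On each ProgressVisualStage event, a switch on VisualStage reveals one of five static mesh components and enables its query and physics collision.
; The stage value is only read here, and the construction script just calls the parent.
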(event EventBeginPlay)

(event Collision|EventActorBeginOverlap
  (params (OtherActor :type Actor%20Object%20Reference))
  (|CallParentFunction OtherActor) ; This node is disabled and will not be called.\nDrag off pins to build functionality.
)

(event EventTick
  (params (DeltaSeconds :type Float%20%28single-precision%29))
  (|CallParentFunction DeltaSeconds) ; This node is disabled and will not be called.\nDrag off pins to build functionality.
)

(event EventProgressVisualStage
  (bind _sm_chestdeliverable1 (Variables|Default|GetSM_ChestDeliverable1))
  (bind _sm_chestdeliverable (Variables|Default|GetSM_ChestDeliverable))
  (bind _sm_chestdeliverable2 (Variables|Default|GetSM_ChestDeliverable2))
  (bind _staticmesh (Variables|Default|GetStaticMesh))
  (bind _staticmesh1 (Variables|Default|GetStaticMesh1))
  (switch int (Variables|Default|GetVisualStage)
    (:0
      (Rendering|SetVisibility _sm_chestdeliverable true false)
      (Collision|SetCollisionEnabled _sm_chestdeliverable "QueryAndPhysics"))
    (:1
      (Rendering|SetVisibility _sm_chestdeliverable1 true false)
      (Collision|SetCollisionEnabled _sm_chestdeliverable1 "QueryAndPhysics"))
    (:2
      (Rendering|SetVisibility _sm_chestdeliverable2 true false)
      (Collision|SetCollisionEnabled _sm_chestdeliverable2 "QueryAndPhysics"))
    (:3
      (Rendering|SetVisibility _staticmesh true false)
      (Collision|SetCollisionEnabled _staticmesh "QueryAndPhysics"))
    (:4
      (Rendering|SetVisibility _staticmesh1 true false)
      (Collision|SetCollisionEnabled _staticmesh1 "QueryAndPhysics"))))

(fn ConstructionScript
  (|CallParentFunction))