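; Team base capture point for the Battle game modes that refreshes the player's objective display when the enemy's capture prerequisites change.
; When the enemy gains or loses prerequisites, it runs the parent logic, then calls ShowObjectives on the Frontline HUD.
; The HUD call runs only where cosmetic events can execute and the HUD casts to BP_FrontlineHUD; all other behavior comes from the parent class.
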(event EventBeginPlay
  (|CallParentFunction) ; This node is disabled and will not be called.\nDrag off pins to build functionality.
)

(event Collision|EventActorBeginOverlap
  (params (OtherActor :type Actor%20Object%20Reference)))

(event EventTick
  (params (DeltaSeconds :type Float%20%28single-precision%29)))

(event EventEnemyGainedPrerequisites
  (|CallParentFunction)
  (Networking|CanExecuteCosmeticEvents
    (:True
      (bind _asbp_frontline_hud (Utilities|Casting|CastToBP_FrontlineHUD (Class|MordhauUtilityLibrary|GetMordhauHUD)))
      (Default|ShowObjectives _asbp_frontline_hud))))

(event EventEnemyLostPrerequisites
  (|CallParentFunction)
  (Networking|CanExecuteCosmeticEvents
    (:True
      (bind _asbp_frontline_hud (Utilities|Casting|CastToBP_FrontlineHUD (Class|MordhauUtilityLibrary|GetMordhauHUD)))
      (Default|ShowObjectives _asbp_frontline_hud))))

(fn ConstructionScript
  (|CallParentFunction))