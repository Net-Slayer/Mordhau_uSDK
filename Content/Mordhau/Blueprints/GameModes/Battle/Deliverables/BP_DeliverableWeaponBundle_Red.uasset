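; Red-variant deliverable weapon bundle for the Battle game mode, judging by its name and folder.
; When broken, it runs the parent logic, then spawns a particle emitter and an armor foley sound at its location.
; It adds no other logic of its own: BeginPlay, overlap and Tick are disabled stubs, and construction only calls the parent.
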(event EventBeginPlay
  (|CallParentFunction) ; This node is disabled and will not be called.\nDrag off pins to build functionality.
)

(event Collision|EventActorBeginOverlap
  (params (OtherActor :type Actor%20Object%20Reference))
  (|CallParentFunction OtherActor) ; This node is disabled and will not be called.\nDrag off pins to build functionality.
)

(event EventTick
  (params (DeltaSeconds :type Float%20%28single-precision%29))
  (|CallParentFunction DeltaSeconds) ; This node is disabled and will not be called.\nDrag off pins to build functionality.
)

(event EventOnBroken
  (bind _returnvalue (Transformation|GetActorLocation))
  (|CallParentFunction)
  (Effects|SpawnEmitteratLocation 0 _returnvalue (Transformation|GetActorRotation))
  (Audio|SpawnSoundatLocation "/Game/Mordhau/Audio/Cues/Foley/SC_SnappyArmorFoley.SC_SnappyArmorFoley" _returnvalue "0, 0, 0" 1.0 1.0 0.0 0 0))

(fn ConstructionScript
  (|CallParentFunction))