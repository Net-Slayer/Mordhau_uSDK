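; Containment volume for the Battle game mode that tracks whether one designated kill objective stays inside its allowed area.
; Overlap events ignore every actor except the referenced objective, and only notify it once that objective has begun play.
; Leaving the box tells the objective it entered an out-of-bounds area, and entering the box tells it that it left one.
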(event EventBeginPlay)

(event Collision|EventActorBeginOverlap
  (params (OtherActor :type Actor%20Object%20Reference))
  (bind _killobjectivetocontain (Variables|Default|GetKillObjectiveToContain))
  (if (== _killobjectivetocontain OtherActor)
    (if (Class|MordhauUtilityLibrary|HasActorBegunPlay _killobjectivetocontain)
      (Class|AdvancedCharacter|LeftOutOfBoundsArea _killobjectivetocontain))))

(event Collision|EventActorEndOverlap
  (params (OtherActor :type Actor%20Object%20Reference))
  (bind _killobjectivetocontain (Variables|Default|GetKillObjectiveToContain))
  (if (== OtherActor _killobjectivetocontain)
    (if (Class|MordhauUtilityLibrary|HasActorBegunPlay _killobjectivetocontain)
      (Class|AdvancedCharacter|EnteredOutOfBoundsArea _killobjectivetocontain))))

(fn ConstructionScript)