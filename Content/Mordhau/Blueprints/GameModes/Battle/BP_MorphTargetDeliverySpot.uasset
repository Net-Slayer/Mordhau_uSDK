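; Battle-mode delivery spot that shows delivery progress cosmetically on a skeletal mesh through a morph target and a material parameter, each optional.
; When deliverables change, the morph goal becomes the delivered fraction of the required count, while the material goal is looked up per count in a weight array.
; Tick eases both at constant speed, optionally remapping the morph through a curve, and switches itself off once both settle.
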(event EventBeginPlay
  (|CallParentFunction)
  (if (not (Utilities|Name|Equal(Name) (Variables|Default|GetProgressMaterialName) "None"))
    (bind _returnvalue (Rendering|Material|CreateDynamicMaterialInstance (Variables|Default|GetSkeletalMesh) (Variables|Default|GetMaterialIndex) 0 "None" :!class /Script/Engine.PrimitiveComponent))
    (Variables|Default|SetMaterialInstance _returnvalue)))

(event EventTick
  (params (DeltaSeconds :type Float%20%28single-precision%29))
  (bind _morphtargetname (Variables|Default|GetMorphTargetName))
  (bind _progressmaterialname (Variables|Default|GetProgressMaterialName))
  (bind _skeletalmesh (Variables|Default|GetSkeletalMesh))
  (|CallParentFunction DeltaSeconds)
  (Utilities|FlowControl|Sequence
    (:then_0
      (if (not (Utilities|Name|Equal(Name) (Variables|Default|GetMorphTargetName) "None"))
        (bind _output_get (Variables|Default|SetCurrentMorphTargetWeight (Math|Interpolation|FInterptoConstant (Variables|Default|GetCurrentMorphTargetWeight) (Variables|Default|GetDesiredMorphTargetWeight) DeltaSeconds (Variables|Default|GetMorphTargetInterpSpeed))))
        (Utilities|IsValid (Variables|Default|GetMorphTargetCurve)
          (:Is%20Valid
            (Components|SkeletalMesh|SetMorphTarget _skeletalmesh _morphtargetname (Math|Curves|GetFloatValue (Variables|Default|GetMorphTargetCurve) _output_get) true))
          (:Is%20Not%20Valid
            (Components|SkeletalMesh|SetMorphTarget _skeletalmesh _morphtargetname _output_get true)))))
    (:then_1
      (if (not (Utilities|Name|Equal(Name) _progressmaterialname "None"))
        (bind _output_get_2 (Variables|Default|SetCurrentMaterialTargetWeight (Math|Interpolation|FInterptoConstant (Variables|Default|GetCurrentMaterialTargetWeight) (Variables|Default|GetDesiredMaterialTargetWeight) DeltaSeconds (Variables|Default|GetMaterialTargetInterpSpeed))))
        (Rendering|Material|SetScalarParameterValue (Variables|Default|GetMaterialInstance) _progressmaterialname _output_get_2 :!class /Script/Engine.MaterialInstanceDynamic)))
    (:then_2
      (if (and (Math|Float|NearlyEqual(Float) (Variables|Default|GetCurrentMorphTargetWeight) (Variables|Default|GetDesiredMorphTargetWeight) 1e-06) (Math|Float|NearlyEqual(Float) (Variables|Default|GetCurrentMaterialTargetWeight) (Variables|Default|GetDesiredMaterialTargetWeight) 1e-06))
        (Actor|Tick|SetActorTickEnabled false)))))

(event EventOnDeliverablesChanged
  (bind _deliverables (Variables|Default|GetDeliverables))
  (bind _materialtargetweights (Variables|Default|GetMaterialTargetWeights))
  (bind _returnvalue (Math|Conversions|ToInteger(Byte) _deliverables))
  (Networking|CanExecuteCosmeticEvents
    (:True
      (Utilities|FlowControl|Sequence
        (:then_0
          (if (not (Utilities|Name|Equal(Name) (Variables|Default|GetMorphTargetName) "None"))
            (Variables|Default|SetDesiredMorphTargetWeight (/ (Math|Conversions|ToFloat(Byte) (Variables|Default|GetDeliverables)) (Math|Conversions|ToFloat(Byte) (Variables|Default|GetRequiredDeliveries))))))
        (:then_1
          (if (not (Utilities|Name|Equal(Name) (Variables|Default|GetProgressMaterialName) "None"))
            (if (Utilities|Array|IsValidIndex _materialtargetweights _returnvalue)
              (Variables|Default|SetDesiredMaterialTargetWeight (Utilities|Array|Get(acopy) _materialtargetweights _returnvalue)))))
        (:then_2
          (if (not (and (Math|Float|NearlyEqual(Float) (Variables|Default|GetCurrentMorphTargetWeight) (Variables|Default|GetDesiredMorphTargetWeight) 1e-06) (Math|Float|NearlyEqual(Float) (Variables|Default|GetCurrentMaterialTargetWeight) (Variables|Default|GetDesiredMaterialTargetWeight) 1e-06)))
            (if (not (Class|Actor|IsActorTickEnabled))
              (Actor|Tick|SetActorTickEnabled true))))))))

(fn ConstructionScript
  (|CallParentFunction))