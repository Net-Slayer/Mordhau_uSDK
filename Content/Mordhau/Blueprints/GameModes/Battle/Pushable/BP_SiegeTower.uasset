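; Pushable siege tower for Battle mode that travels along a spline and drops its gangplank on arrival.
; Tick derives wheel spin from spline distance, fades rolling audio by speed, and animates the gangplank fall with a bounce curve.
; Arrival starts the fall, then after a delay triggers impact effects, camera shake and radial damage at three points.
; The authority also spawns replicated ladders and optionally kills characters inside two kill areas.
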(event EventBeginPlay
  (|CallParentFunction))

(event EventPushableArrivedatDestination
  (bind _array (Utilities|Array|MakeArray "ObjectTypeQuery3" "ObjectTypeQuery5"))
  (bind _self self)
  (bind _scene2 (Variables|Default|GetScene2))
  (bind _killarea1 (Variables|Default|GetKillArea1))
  (bind _scene (Variables|Default|GetScene))
  (bind _gangplank_target (Variables|Default|GetGangplank_Target))
  (bind _killarea2 (Variables|Default|GetKillArea2))
  (bind _returnvalue (Transformation|GetWorldLocation _scene2))
  (bind _returnvalue_2 (Transformation|GetWorldLocation _scene))
  (bind _returnvalue_3 (Transformation|GetWorldLocation _gangplank_target))
  (|CallParentFunction)
  (Utilities|FlowControl|Sequence
    (:then_0
      (Audio|Components|Audio|FadeOut (Variables|Default|GetAudio) 0.2 0.0 :!class /Script/Engine.AudioComponent)
      (Variables|Default|SetFalling%20Bridge%20Origin (Transformation|GetRelativeTransform (Variables|Default|GetGangplank_Origin)))
      (Variables|Default|SetStart%20Fall%20Time (Utilities|Time|GetTimeSeconds))
      (Audio|PlaySoundatLocation 0 _returnvalue_3 "0, 0, 0" 1.0 1.0 0.0 0 0 0)
      (Effects|SpawnEmitteratLocation 0 _returnvalue_3)
      (Utilities|FlowControl|Delay 3.3)
      (Effects|SpawnEmitteratLocation 0 _returnvalue_2 "90.000000, 0,0.000000")
      (Audio|PlaySoundatLocation 0 _returnvalue_2 "0, 0, 0" 1.0 1.0 0.0 0 0 0)
      (Class|MordhauUtilityLibrary|MordhauApplyRadialDamagewithFalloff 0 2.5e+03 1.0 4e+02 2e+01 _returnvalue_2 5e+01 1e+02 5.0 0 1e+03 5e+02 2e+02 _self 0 "ECC_WorldStatic" false)
      (Class|MordhauUtilityLibrary|MordhauApplyRadialDamagewithFalloff 0 2.5e+03 1.0 4e+02 2e+01 (Transformation|GetWorldLocation (Variables|Default|GetScene1)) 5e+01 1e+02 5.0 0 1e+03 5e+02 2e+02 _self 0 "ECC_WorldStatic" false)
      (Class|MordhauUtilityLibrary|MordhauApplyRadialDamagewithFalloff 0 2.5e+03 1.0 4e+02 2e+01 _returnvalue 5e+01 1e+02 5.0 0 1e+03 5e+02 2e+02 _self 0 "ECC_WorldStatic" false)
      (Camera|PlayWorldCameraShake "/Game/Mordhau/Blueprints/CameraShakes/ImpactShake.ImpactShake_C" _returnvalue 2.5e+02 7.5e+03 1e+01))
    (:then_1
      (Networking|SwitchHasAuthority
        (:Authority
          (bind _returnvalue_4 (Game|SpawnActorfromClass "/Game/Mordhau/Blueprints/Interactables/SiegeEngines/BP_Ladder_6m.BP_Ladder_6m_C" (Math|Transform|ComposeTransforms (Math|Transform|MakeTransform "-805.590027,-184.100006,68.000000" "-11.900000, 0, 0") (Transformation|GetActorTransform)) "Undefined" 0 0))
          (Networking|SetReplicates _returnvalue_4 true)
          (Transformation|AddRelativeLocation (Variables|/Game/Mordhau/Blueprints/Interactables/SiegeEngines/BP_Ladder.BP_Ladder_C|GetLadderExit _returnvalue_4) "0, 0,50.000000" false false)
          (bind _returnvalue_5 (Game|SpawnActorfromClass "/Game/Mordhau/Blueprints/Interactables/SiegeEngines/BP_Ladder_7m.BP_Ladder_7m_C" (Math|Transform|ComposeTransforms (Math|Transform|MakeTransform "-49.500000,173.000000,1633.480591" "-7.752000, 0, 0") (Transformation|GetActorTransform)) "Undefined" 0 0))
          (Networking|SetReplicates _returnvalue_5 true)
          (if (Variables|Default|GetKillOnComplete)
            (bind _outactors (Collision|ComponentOverlapActors _killarea1 (Transformation|GetWorldTransform _killarea1) _array "/Script/Mordhau.AdvancedCharacter"))
            (for _array_element _outactors
              (bind _asadvanced_character (Utilities|Casting|CastToAdvancedCharacter _array_element))
              (if (not (Class|AdvancedCharacter|GetIsDead _asadvanced_character))
                (Class|AdvancedCharacter|Suicide _asadvanced_character)))
            (bind _outactors_2 (Collision|ComponentOverlapActors _killarea2 (Transformation|GetWorldTransform _killarea2) _array "/Script/Mordhau.AdvancedCharacter"))
            (for _array_element_2 _outactors_2
              (bind _asadvanced_character_2 (Utilities|Casting|CastToAdvancedCharacter _array_element_2))
              (if (not (Class|AdvancedCharacter|GetIsDead _asadvanced_character_2))
                (Class|AdvancedCharacter|Suicide _asadvanced_character_2)))))))))

(event EventTick
  (params (DeltaSeconds :type Float%20%28single-precision%29))
  (bind _progress (Variables|Default|GetProgress))
  (bind _targetsplineactor (Variables|Default|GetTargetSplineActor))
  (bind _start_fall_time (Variables|Default|GetStart%20Fall%20Time))
  (bind _audio (Variables|Default|GetAudio))
  (bind _returnvalue (Audio|Components|Audio|IsPlaying _audio))
  (bind _spline (Variables|/Game/Mordhau/Blueprints/Interactables/BP_SplineActor.BP_SplineActor_C|GetSpline _targetsplineactor))
  (bind _returnvalue_2 (Spline|GetSplineLength _spline))
  (|CallParentFunction DeltaSeconds)
  (Utilities|FlowControl|Sequence
    (:then_0
      (bind _output_get (Variables|Default|SetWheelRotator (Math|Rotator|MakeRotator (* (/ (* _returnvalue_2 _progress) (Math|Float|MultiplybyPi 1.9e+02)) -3.6e+02) 0.0 9e+01)))
      (Transformation|SetRelativeRotation (Variables|Default|Getwheel_01) _output_get false false)
      (if (> (/ (* _returnvalue_2 (- _progress (Variables|Default|GetPreviousProgress))) DeltaSeconds) 1.0)
        (if (not _returnvalue)
          (Audio|Components|Audio|FadeIn _audio 1.0 1.0 0.0 :!class /Script/Engine.AudioComponent))
        (elif _returnvalue
          (Audio|Components|Audio|FadeOut _audio 0.2 0.0 :!class /Script/Engine.AudioComponent))))
    (:then_1
      (if (not (== _start_fall_time -1.0))
        (bind _returnvalue_3 (Class|MordhauUtilityLibrary|GetNormalizedTime _start_fall_time (+ _start_fall_time 5.0) (Utilities|Time|GetTimeSeconds)))
        (Transformation|SetRelativeTransform (Variables|Default|GetGangplank_Origin) (Math|Transform|Lerp(Transform) (Variables|Default|GetFalling%20Bridge%20Origin) (Transformation|GetRelativeTransform (Variables|Default|GetGangplank_Target)) (Math|Curves|GetFloatValue (Variables|Default|GetBounce%20Curve) _returnvalue_3)) false false)
        (if (== _returnvalue_3 1.0)
          (Actor|Tick|SetActorTickEnabled false))))
    (:then_2
      (Variables|Default|SetPreviousProgress (Variables|Default|GetProgress)))))

(fn ConstructionScript
  (|CallParentFunction))