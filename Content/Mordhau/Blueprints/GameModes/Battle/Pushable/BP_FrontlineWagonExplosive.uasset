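; An explosive pushable wagon, filed under Battle game mode pushables, that blows up after arriving at its destination.
; Arrival activates fuse sparks and sound, then after a short delay swaps them for explosion, fire, smoke and debris effects.
; The blast disables skeletal mesh collision, hides the wagon and keg meshes and reveals a decal.
; It then applies falloff radial damage with knockback and ragdoll, plus a world camera shake.
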(event EventBeginPlay
  (|CallParentFunction) ; This node is disabled and will not be called.\nDrag off pins to build functionality.
)

(event Collision|EventActorBeginOverlap
  (params (OtherActor :type Actor%20Object%20Reference))
  (|CallParentFunction OtherActor) ; This node is disabled and will not be called.\nDrag off pins to build functionality.
)

(event EventTick
  (params (DeltaSeconds :type Float%20%28single-precision%29))
  (|CallParentFunction DeltaSeconds) ; This node is disabled and will not be called.\nDrag off pins to build functionality.
)

(event EventPushableArrivedatDestination
  (bind _p_explosivespark (Variables|Default|GetP_ExplosiveSpark))
  (bind _p_explosion (Variables|Default|GetP_Explosion))
  (bind _returnvalue (Transformation|GetWorldLocation _p_explosion))
  (Components|Activation|Activate _p_explosivespark false)
  (Utilities|FlowControl|Delay 5.0)
  (Components|Activation|Deactivate _p_explosivespark)
  (Components|Activation|Activate _p_explosion false)
  (Collision|SetCollisionEnabled (Variables|Default|GetSkeletalMesh) "NoCollision")
  (Rendering|SetVisibility (Variables|Default|GetSkeletalMesh) false false)
  (Rendering|SetVisibility (Variables|Default|GetDecal1) true false)
  (Class|MordhauUtilityLibrary|MordhauApplyRadialDamagewithFalloff 0 2.5e+03 3e+01 0.0 0.0 _returnvalue 6e+02 2.2e+03 6.0 0 1.2e+04 9e+03 2.2e+03 self 0 "ECC_WorldStatic" false)
  (Camera|PlayWorldCameraShake "/Game/Mordhau/Blueprints/CameraShakes/ExplosionShake.ExplosionShake_C" _returnvalue 1e+03 1e+04))

(fn ConstructionScript
  (|CallParentFunction))