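; Pushable wagon for the Frontline game mode that moves along a target spline, adding wheel animation and rolling sound.
; On cosmetic-capable instances, Tick converts spline progress into travelled distance and wheel circumference into a rotation fed to the wagon's AnimBP.
; The change in progress since the last tick gives a speed that fades the wheel sound in or out.
; Arrival at the destination disables Tick and fades the sound out.
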(event EventTick
  (params (DeltaSeconds :type Float%20%28single-precision%29))
  (bind _splinerange (Variables|Default|GetSplineRange))
  (bind _wheelssound (Variables|Default|GetWheelsSound))
  (bind _targetsplineactor (Variables|Default|GetTargetSplineActor))
  (bind (_x _y) (Math|Vector2D|BreakVector2D _splinerange))
  (bind _returnvalue (Audio|Components|Audio|IsPlaying _wheelssound))
  (bind _spline (Variables|/Game/Mordhau/Blueprints/Interactables/BP_SplineActor.BP_SplineActor_C|GetSpline _targetsplineactor))
  (|CallParentFunction DeltaSeconds)
  (Networking|CanExecuteCosmeticEvents
    (:True
      (if (not (Math|Float|NearlyEqual(Float) DeltaSeconds 0.0 1e-06))
        (Utilities|FlowControl|Sequence
          (:then_0
            (bind _asab_empty_wagon (Utilities|Casting|CastToAB_EmptyWagon (Components|SkeletalMesh|GetAnimInstance (Variables|Default|GetSkeletalMesh))))
            (Variables|/Game/Mordhau/Animations/Blueprints/AB_EmptyWagon.AB_EmptyWagon_C|SetWheels _asab_empty_wagon (Math|Rotator|MakeRotator (* (/ (* (Math|Float|Lerp _x _y (Variables|Default|GetProgress)) (Spline|GetSplineLength _spline)) (Math|Float|MultiplybyPi 1.2e+02)) -3.6e+02) 0.0 0.0))
            (if (> (/ (* (Spline|GetSplineLength _spline) (- (Variables|Default|GetProgress) (Variables|Default|GetPreviousProgress))) DeltaSeconds) 1.0)
              (if (not _returnvalue)
                (Audio|Components|Audio|FadeIn _wheelssound 1.0 1.0 0.0 :!class /Script/Engine.AudioComponent))
              (elif _returnvalue
                (Audio|Components|Audio|FadeOut _wheelssound 0.2 0.0 :!class /Script/Engine.AudioComponent))))
          (:then_1
            (Variables|Default|SetPreviousProgress (Variables|Default|GetProgress))))))))

(event EventPushableArrivedatDestination
  (Actor|Tick|SetActorTickEnabled false)
  (Audio|Components|Audio|FadeOut (Variables|Default|GetWheelsSound) 0.2 0.0 :!class /Script/Engine.AudioComponent))

(fn ConstructionScript
  (|CallParentFunction))