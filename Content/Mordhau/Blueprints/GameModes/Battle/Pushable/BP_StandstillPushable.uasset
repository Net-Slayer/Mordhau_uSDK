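; A stationary pushable objective for Battle game modes that shows its progress through animation rather than code-driven movement.
; On each progress update it sets the skeletal mesh's animation position to Progress, updates an optional dynamic material parameter created in the construction script, and forwards Progress to linked ProgressActors.
; The pushing sound starts on updates and stops through a retriggerable delay shortly after updates cease.
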(event EventBeginPlay
  (|CallParentFunction) ; This node is disabled and will not be called.\nDrag off pins to build functionality.
)

(event Collision|EventActorBeginOverlap
  (params (OtherActor :type Actor%20Object%20Reference))
  (|CallParentFunction OtherActor) ; This node is disabled and will not be called.\nDrag off pins to build functionality.
)

(event EventTick
  (params (DeltaSeconds :type Float%20%28single-precision%29))
  (|CallParentFunction DeltaSeconds) ; This node is disabled and will not be called.\nDrag off pins to build functionality.
)

(event EventOnProgressUpdated
  (params (OldProgress :type Float%20%28single-precision%29))
  (bind _progress (Variables|Default|GetProgress))
  (bind _animatedmaterial (Variables|Default|GetAnimatedMaterial))
  (bind _pushingsound (Variables|Default|GetPushingSound))
  (bind _returnvalue (Audio|Components|Audio|IsPlaying _pushingsound))
  (|CallParentFunction OldProgress)
  (Components|Animation|SetPosition (Variables|Default|GetSkeletalMesh) _progress false)
  (Utilities|FlowControl|Sequence
    (:then_0
      (Utilities|IsValid _animatedmaterial
        (:Is%20Valid
          (Rendering|Material|SetScalarParameterValue _animatedmaterial (Variables|Default|GetAnimatedParameter) _progress :!class /Script/Engine.MaterialInstanceDynamic))))
    (:then_1
      (if (not _returnvalue)
        (Audio|Components|Audio|Play _pushingsound 0.0)))
    (:then_2
      (Utilities|FlowControl|RetriggerableDelay 0.3)
      (if _returnvalue
        (Audio|Components|Audio|Stop _pushingsound)))
    (:then_3
      (for _array_element (Variables|Default|GetProgressActors)
        (Utilities|IsValid _array_element
          (:Is%20Valid
            (Default|ProgressUpdatedInternal _array_element _progress)))))))

(fn ConstructionScript
  (bind _animatedmaterialindex (Variables|Default|GetAnimatedMaterialIndex))
  (|CallParentFunction)
  (if (>= _animatedmaterialindex 0)
    (bind _returnvalue (Rendering|Material|CreateDynamicMaterialInstance (Variables|Default|GetSkeletalMesh) _animatedmaterialindex 0 "None" :!class /Script/Engine.PrimitiveComponent))
    (Variables|Default|SetAnimatedMaterial _returnvalue)))