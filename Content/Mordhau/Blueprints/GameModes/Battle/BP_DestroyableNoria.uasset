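; Destroyable noria (water wheel) for Battle mode that visibly winds down as it takes damage.
; Tick picks a health tier, slowing the wheel, increasing its cosine wobble and thinning water splash particles as health drops.
; At zero the splash deactivates, the wheel only rocks, and a one-shot timeline drives post-process blend weight.
; The top tier reads Health, while lower tiers read ReplicatedHealth.
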(event EventBeginPlay
  (|CallParentFunction))

(event Collision|EventActorBeginOverlap
  (params (OtherActor :type Actor%20Object%20Reference))
  (|CallParentFunction OtherActor) ; This node is disabled and will not be called.\nDrag off pins to build functionality.
)

(event EventTick
  (params (DeltaSeconds :type Float%20%28single-precision%29))
  (|CallParentFunction DeltaSeconds)
  (if (>= (Variables|Default|GetHealth) 75.0)
    (Transformation|AddLocalRotation (Variables|Default|GetStaticMesh) (Math|Rotator|MakeRotator 0.0 0.15 (* (Math|Trig|Cos(Radians) (* (Utilities|Time|GetGameTimeinSeconds) 4.0)) 0.005)) false false)
    (Effects|Components|ParticleSystem|SetFloatParameter (Variables|Default|GetFX) "SpawnRate" 1.0)
    (elif (>= (Variables|Default|GetReplicatedHealth) 50)
      (Effects|Components|ParticleSystem|SetFloatParameter (Variables|Default|GetFX) "SpawnRate" 0.6)
      (Transformation|AddLocalRotation (Variables|Default|GetStaticMesh) (Math|Rotator|MakeRotator 0.0 0.075 (* (Math|Trig|Cos(Radians) (* (Utilities|Time|GetGameTimeinSeconds) 4.0)) 0.01)) false false)
      (elif (>= (Variables|Default|GetReplicatedHealth) 25)
        (Effects|Components|ParticleSystem|SetFloatParameter (Variables|Default|GetFX) "SpawnRate" 0.15)
        (Transformation|AddLocalRotation (Variables|Default|GetStaticMesh) (Math|Rotator|MakeRotator 0.0 0.04 (* (Math|Trig|Cos(Radians) (* (Utilities|Time|GetGameTimeinSeconds) 4.0)) 0.015)) false false)
        (elif (> (Variables|Default|GetReplicatedHealth) 0)
          (Effects|Components|ParticleSystem|SetFloatParameter (Variables|Default|GetFX) "SpawnRate" 0.01)
          (Transformation|AddLocalRotation (Variables|Default|GetStaticMesh) (Math|Rotator|MakeRotator 0.0 0.015 (* (Math|Trig|Cos(Radians) (* (Utilities|Time|GetGameTimeinSeconds) 4.0)) 0.02)) false false)
          (else
            (Components|Activation|Deactivate (Variables|Default|GetFX))
            (Transformation|AddLocalRotation (Variables|Default|GetStaticMesh) (Math|Rotator|MakeRotator 0.0 (* (Math|Trig|Cos(Radians) (* (Utilities|Time|GetGameTimeinSeconds) 0.6)) 0.025) (* (Math|Trig|Cos(Radians) (* (Utilities|Time|GetGameTimeinSeconds) 4.0)) 0.02)) false false)
            (Utilities|FlowControl|DoOnce false
              (:Completed
                (bind _blend (Timeline|Timeline_0 Play)
                  (:Update
                    (Variables|/Script/Engine.PostProcessComponent|SetBlendWeight (Variables|Default|GetPostProcess) _blend)))))))))))

(fn ConstructionScript
  (|CallParentFunction))