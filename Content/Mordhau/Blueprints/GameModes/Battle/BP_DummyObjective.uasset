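; Placeholder Battle-mode objective that toggles a marker widget for a linked capture point and never reports progress or completion of its own.
; When the enemy gains prerequisites it clears the widget's visibility override, unless the point is already fully captured.
; It hides the widget when those prerequisites are lost or the point's progress reaches full.
; Its objective area is a fixed horizontal radius around the actor, ignoring height.
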(event EventOnAnyObjectiveProgressChanged
  (CallFunction|AnyObjectiveProgressChanged))

(event Collision|EventActorBeginOverlap
  (params (OtherActor :type Actor%20Object%20Reference)))

(event EventTick
  (params (DeltaSeconds :type Float%20%28single-precision%29)))

(event EventOnInitialize
  (params (Point :type BP%20Capture%20Point%20Object%20Reference))
  (CallFunction|Initialize Point))

(event EventOnEnemyGainedPrerequisites
  (CallFunction|EnemyGainedPrerequisites))

(event EventOnEnemyLostPrerequisites
  (CallFunction|EnemyLostPrerequisites))

(event EventOnUpdateUIWidgets
  (bind _capturepoint (Variables|Default|GetCapturePoint))
  (Utilities|IsValid _capturepoint
    (:Is%20Valid
      (if (== (Variables|/Game/Mordhau/Blueprints/GameModes/Battle/BP_CapturePoint.BP_CapturePoint_C|GetObjectiveProgress _capturepoint) 1.0)
        _))))

(fn ConstructionScript
  (|CallParentFunction))

(fn Activate
  (Variables|/Script/Mordhau.MordhauWidgetComponent|SetOverrideVisible (Variables|Default|GetMordhauWidget) -1))

(fn Disable
  (Variables|/Script/Mordhau.MordhauWidgetComponent|SetOverrideVisible (Variables|Default|GetMordhauWidget) 0))

(fn Initialize
  (params (CapturePoint :type BP%20Capture%20Point%20Object%20Reference))
  (Variables|Default|SetCapturePoint CapturePoint))

(fn EnemyGainedPrerequisites
  (bind _isdone (CallFunction|IsCapturePointDone))
  (if (not _isdone)
    (CallFunction|Activate)))

(fn EnemyLostPrerequisites
  (CallFunction|Disable))

(fn IsCapturePointDone
  (bind _capturepoint (Variables|Default|GetCapturePoint))
  (Utilities|IsValid _capturepoint
    (:Is%20Valid
      (return (== (Variables|/Game/Mordhau/Blueprints/GameModes/Battle/BP_CapturePoint.BP_CapturePoint_C|GetObjectiveProgress _capturepoint) 1.0)))
    (:Is%20Not%20Valid
      (return false))))

(fn AnyObjectiveProgressChanged
  (bind _capturepoint (Variables|Default|GetCapturePoint))
  (Utilities|IsValid _capturepoint
    (:Is%20Valid
      (if (== (Variables|/Game/Mordhau/Blueprints/GameModes/Battle/BP_CapturePoint.BP_CapturePoint_C|GetObjectiveProgress _capturepoint) 1.0)
        (CallFunction|Disable)))))

(fn GetObjectiveProgress
  (return 0.0))

(fn IsCompleted
  (return false))

(fn IsinObjectiveArea
  (params (Location :type Vector :default "0, 0, 0"))
  (return (< (Math|Vector|VectorLengthXY (- Location (Transformation|GetActorLocation))) 1e+03)))