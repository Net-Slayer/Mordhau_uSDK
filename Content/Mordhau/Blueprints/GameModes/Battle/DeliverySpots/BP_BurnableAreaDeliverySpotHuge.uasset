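; Huge variant of a burnable area delivery spot for the Battle game modes, which visibly catches fire in stages.
; ProgressVisualStage switches on VisualStage across seven steps, each raising post-process blend weight, playing a hit sound and activating more fire, smoke or flare effects.
; Most stages also spawn a BP_EnvFireField at the newly lit fire's transform, and fire audio starts and adjusts in early stages.
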(event EventBeginPlay
  (|CallParentFunction) ; This node is disabled and will not be called.\nDrag off pins to build functionality.
)

(event Collision|EventActorBeginOverlap
  (params (OtherActor :type Actor%20Object%20Reference))
  (|CallParentFunction OtherActor) ; This node is disabled and will not be called.\nDrag off pins to build functionality.
)

(event EventTick
  (params (DeltaSeconds :type Float%20%28single-precision%29))
  (|CallParentFunction DeltaSeconds) ; This node is disabled and will not be called.\nDrag off pins to build functionality.
)

(event EventProgressVisualStage
  (bind _fire1 (Variables|Default|GetFire1))
  (bind _fire4 (Variables|Default|GetFire4))
  (bind _fire6 (Variables|Default|GetFire6))
  (bind _fire2 (Variables|Default|GetFire2))
  (bind _fire2sound (Variables|Default|GetFire2Sound))
  (bind _fire3 (Variables|Default|GetFire3))
  (switch int (Variables|Default|GetVisualStage)
    (:0
      (Variables|/Script/Engine.PostProcessComponent|SetBlendWeight (Variables|Default|GetPostProcess) 0.1)
      (Audio|Components|Audio|Play (Variables|Default|GetSC_FireHitSound) 0.0)
      (Components|Activation|Activate _fire1 false)
      (Game|SpawnActorfromClass "/Game/Mordhau/Blueprints/Fields/BP_EnvFireField.BP_EnvFireField_C" (Transformation|GetWorldTransform _fire1) "Undefined" 0 0))
    (:1
      (Variables|/Script/Engine.PostProcessComponent|SetBlendWeight (Variables|Default|GetPostProcess) 0.3)
      (Audio|Components|Audio|Play (Variables|Default|GetSC_FireHitSound) 0.0)
      (Components|Activation|Activate _fire2 false)
      (Components|Activation|Activate _fire2sound false)
      (Components|Activation|Activate (Variables|Default|GetGpuFlares) false)
      (Game|SpawnActorfromClass "/Game/Mordhau/Blueprints/Fields/BP_EnvFireField.BP_EnvFireField_C" (Transformation|GetWorldTransform _fire2) "Undefined" 0 0))
    (:2
      (Variables|/Script/Engine.PostProcessComponent|SetBlendWeight (Variables|Default|GetPostProcess) 0.5)
      (Audio|Components|Audio|Play (Variables|Default|GetSC_FireHitSound) 0.0)
      (Components|Activation|Activate _fire3 false)
      (Components|Activation|Activate (Variables|Default|GetSmoke) false)
      (Audio|Components|Audio|AdjustVolume _fire2sound 0.0 1.0 :!class /Script/Engine.AudioComponent)
      (Game|SpawnActorfromClass "/Game/Mordhau/Blueprints/Fields/BP_EnvFireField.BP_EnvFireField_C" (Transformation|GetWorldTransform _fire3) "Undefined" 0 0))
    (:3
      (Variables|/Script/Engine.PostProcessComponent|SetBlendWeight (Variables|Default|GetPostProcess) 0.6)
      (Audio|Components|Audio|Play (Variables|Default|GetSC_FireHitSound) 0.0)
      (Components|Activation|Activate (Variables|Default|GetGpuFlares2) false)
      (Game|SpawnActorfromClass "/Game/Mordhau/Blueprints/Fields/BP_EnvFireField.BP_EnvFireField_C" (Transformation|GetWorldTransform (Variables|Default|GetFire5)) "Undefined" 0 0))
    (:4
      (Variables|/Script/Engine.PostProcessComponent|SetBlendWeight (Variables|Default|GetPostProcess) 0.7)
      (Audio|Components|Audio|Play (Variables|Default|GetSC_FireHitSound) 0.0)
      (Components|Activation|Activate _fire4 false)
      (Game|SpawnActorfromClass "/Game/Mordhau/Blueprints/Fields/BP_EnvFireField.BP_EnvFireField_C" (Transformation|GetWorldTransform _fire4) "Undefined" 0 0))
    (:5
      (Variables|/Script/Engine.PostProcessComponent|SetBlendWeight (Variables|Default|GetPostProcess) 0.9)
      (Audio|Components|Audio|Play (Variables|Default|GetSC_FireHitSound) 0.0)
      (Components|Activation|Activate (Variables|Default|GetGpuFlares3) false))
    (:6
      (Variables|/Script/Engine.PostProcessComponent|SetBlendWeight (Variables|Default|GetPostProcess) 1.0)
      (Audio|Components|Audio|Play (Variables|Default|GetSC_FireHitSound) 0.0)
      (Components|Activation|Activate _fire6 false)
      (Game|SpawnActorfromClass "/Game/Mordhau/Blueprints/Fields/BP_EnvFireField.BP_EnvFireField_C" (Transformation|GetWorldTransform _fire6) "Undefined" 0 0))))

(fn ConstructionScript
  (|CallParentFunction))