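; Burnable building delivery spot for Battle game modes that shows the building catching fire in three escalating visual stages.
; ProgressVisualStage switches on VisualStage, raising post-process weight, playing fire audio, activating that stage's fire, smoke and flares, and toggling its burnt components' visibility.
; Each stage spawns BP_EnvFireField actors at its marker transforms, and later stages scale up fog, wispy smoke and earlier fires.
; BeginPlay skips the parent call, and several unconnected effect chains never run.
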(event EventBeginPlay)

(event Collision|EventActorBeginOverlap
  (params (OtherActor :type Actor%20Object%20Reference))
  (|CallParentFunction OtherActor) ; This node is disabled and will not be called.\nDrag off pins to build functionality.
)

(event EventTick
  (params (DeltaSeconds :type Float%20%28single-precision%29))
  (|CallParentFunction DeltaSeconds) ; This node is disabled and will not be called.\nDrag off pins to build functionality.
)

(event EventProgressVisualStage
  (bind _smokewispy (Variables|Default|GetSmokeWispy))
  (bind _stage1fire1 (Variables|Default|GetStage1Fire1))
  (bind _stage1fire2 (Variables|Default|GetStage1Fire2))
  (bind _stage1fire3 (Variables|Default|GetStage1Fire3))
  (bind _stage2fire1 (Variables|Default|GetStage2Fire1))
  (bind _stage2fire2 (Variables|Default|GetStage2Fire2))
  (bind _stage2fire3 (Variables|Default|GetStage2Fire3))
  (bind _stage1fire1_2 (Variables|Default|GetStage1Fire1))
  (bind _stage1fire2_2 (Variables|Default|GetStage1Fire2))
  (bind _stage1fire3_2 (Variables|Default|GetStage1Fire3))
  (bind _fog (Variables|Default|GetFog))
  (bind _smokewispy_2 (Variables|Default|GetSmokeWispy))
  (bind _fog_2 (Variables|Default|GetFog))
  (switch int (Variables|Default|GetVisualStage)
    (:0
      (Variables|/Script/Engine.PostProcessComponent|SetBlendWeight (Variables|Default|GetPostProcess) 0.1)
      (Components|Activation|Activate (Variables|Default|GetStage1Fire1Sound) false)
      (Audio|Components|Audio|Play (Variables|Default|GetSC_FireHitSound) 0.0)
      (Components|Activation|Activate (Variables|Default|GetStage1Fire1) false)
      (Components|Activation|Activate (Variables|Default|GetStage1Fire2) false)
      (Components|Activation|Activate (Variables|Default|GetStage1Fire3) false)
      (Components|Activation|Activate (Variables|Default|GetStage1Smoke1) false)
      (Components|Activation|Activate (Variables|Default|GetStage1Smoke2) false)
      (Components|Activation|Activate (Variables|Default|GetStage1Smoke3) false)
      (Components|Activation|Activate (Variables|Default|GetStage1Flares1) false)
      (Components|Activation|Activate (Variables|Default|GetStage1Flares2) false)
      (Components|Activation|Activate (Variables|Default|GetStage1Flares3) false)
      (Components|Activation|Activate (Variables|Default|GetSmokeWispy) false)
      (Components|Activation|Activate (Variables|Default|GetFog) false)
      (Rendering|ToggleVisibility (Variables|Default|GetStage1Burnt1) false)
      (Rendering|ToggleVisibility (Variables|Default|GetStage1Burnt2) false)
      (Rendering|ToggleVisibility (Variables|Default|GetStage1Burnt3) false)
      (Game|SpawnActorfromClass "/Game/Mordhau/Blueprints/Fields/BP_EnvFireField.BP_EnvFireField_C" (Transformation|GetWorldTransform (Variables|Default|GetStage1%20-%201)) "Undefined" 0 0)
      (Game|SpawnActorfromClass "/Game/Mordhau/Blueprints/Fields/BP_EnvFireField.BP_EnvFireField_C" (Transformation|GetWorldTransform (Variables|Default|GetStage1%20-%202)) "Undefined" 0 0)
      (Game|SpawnActorfromClass "/Game/Mordhau/Blueprints/Fields/BP_EnvFireField.BP_EnvFireField_C" (Transformation|GetWorldTransform (Variables|Default|GetStage1%20-%203)) "Undefined" 0 0))
    (:1
      (Variables|/Script/Engine.PostProcessComponent|SetBlendWeight (Variables|Default|GetPostProcess) 0.5)
      (Components|Activation|Activate (Variables|Default|GetStage1Fire1Sound) false)
      (Audio|Components|Audio|Play (Variables|Default|GetSC_FireHitSound) 0.0)
      (Components|Activation|Activate (Variables|Default|GetStage2Fire1) false)
      (Components|Activation|Activate (Variables|Default|GetStage2Fire2) false)
      (Components|Activation|Activate (Variables|Default|GetStage2Fire3) false)
      (Components|Activation|Activate (Variables|Default|GetStage2Fire4) false)
      (Components|Activation|Activate (Variables|Default|GetStage2Smoke1) false)
      (Components|Activation|Activate (Variables|Default|GetStage2Smoke2) false)
      (Components|Activation|Activate (Variables|Default|GetStage2Smoke3) false)
      (Components|Activation|Activate (Variables|Default|GetStage2Smoke4) false)
      (Components|Activation|Activate (Variables|Default|GetStage2Flares1) false)
      (Components|Activation|Activate (Variables|Default|GetStage2Flares2) false)
      (Components|Activation|Activate (Variables|Default|GetStage2Flares3) false)
      (Components|Activation|Activate (Variables|Default|GetStage2Flares4) false)
      (Rendering|ToggleVisibility (Variables|Default|GetStage2Burnt1) false)
      (Rendering|ToggleVisibility (Variables|Default|GetStage2Burnt2) false)
      (Rendering|ToggleVisibility (Variables|Default|GetStage2Burnt3) false)
      (Rendering|ToggleVisibility (Variables|Default|GetStage2Burnt4) false)
      (Transformation|SetWorldScale3D _fog_2 (* (Transformation|GetWorldScale _fog_2) 1.2))
      (Transformation|SetWorldScale3D _smokewispy (* (Transformation|GetWorldScale _smokewispy) 1.2))
      (Transformation|SetWorldScale3D _stage1fire1_2 (* (Transformation|GetWorldScale _stage1fire1_2) 1.5))
      (Transformation|SetWorldScale3D _stage1fire2_2 (* (Transformation|GetWorldScale _stage1fire2_2) 1.5))
      (Transformation|SetWorldScale3D _stage1fire3_2 (* (Transformation|GetWorldScale _stage1fire3_2) 1.5))
      (Game|SpawnActorfromClass "/Game/Mordhau/Blueprints/Fields/BP_EnvFireField.BP_EnvFireField_C" (Transformation|GetWorldTransform (Variables|Default|GetStage2%20-%201)) "Undefined" 0 0)
      (Game|SpawnActorfromClass "/Game/Mordhau/Blueprints/Fields/BP_EnvFireField.BP_EnvFireField_C" (Transformation|GetWorldTransform (Variables|Default|GetStage2%20-%202)) "Undefined" 0 0)
      (Game|SpawnActorfromClass "/Game/Mordhau/Blueprints/Fields/BP_EnvFireField.BP_EnvFireField_C" (Transformation|GetWorldTransform (Variables|Default|GetStage2%20-%203)) "Undefined" 0 0)
      (Game|SpawnActorfromClass "/Game/Mordhau/Blueprints/Fields/BP_EnvFireField.BP_EnvFireField_C" (Transformation|GetWorldTransform (Variables|Default|GetStage2%20-%204)) "Undefined" 0 0))
    (:2
      (Variables|/Script/Engine.PostProcessComponent|SetBlendWeight (Variables|Default|GetPostProcess) 1.0)
      (Components|Activation|Activate (Variables|Default|GetStage1Fire1Sound) false)
      (Audio|Components|Audio|Play (Variables|Default|GetSC_FireHitSound) 0.0)
      (Components|Activation|Activate (Variables|Default|GetStage3Fire1) false)
      (Components|Activation|Activate (Variables|Default|GetStage3Fire2) false)
      (Components|Activation|Activate (Variables|Default|GetStage3Fire3) false)
      (Components|Activation|Activate (Variables|Default|GetStage3Fire4) false)
      (Components|Activation|Activate (Variables|Default|GetStage3Fire5) false)
      (Components|Activation|Activate (Variables|Default|GetStage3Smoke1) false)
      (Components|Activation|Activate (Variables|Default|GetStage3Smoke2) false)
      (Components|Activation|Activate (Variables|Default|GetStage3Smoke3) false)
      (Components|Activation|Activate (Variables|Default|GetStage3Smoke4) false)
      (Components|Activation|Activate (Variables|Default|GetStage3Smoke5) false)
      (Components|Activation|Activate (Variables|Default|GetStage3Flares1) false)
      (Components|Activation|Activate (Variables|Default|GetStage3Flares2) false)
      (Components|Activation|Activate (Variables|Default|GetStage3Flares3) false)
      (Components|Activation|Activate (Variables|Default|GetStage3Flares4) false)
      (Components|Activation|Activate (Variables|Default|GetStage3Flares5) false)
      (Rendering|ToggleVisibility (Variables|Default|GetStage3Burnt1) false)
      (Rendering|ToggleVisibility (Variables|Default|GetStage3Burnt2) false)
      (Rendering|ToggleVisibility (Variables|Default|GetStage3Burnt3) false)
      (Rendering|ToggleVisibility (Variables|Default|GetStage3Burnt4) false)
      (Rendering|ToggleVisibility (Variables|Default|GetStage3Burnt5) false)
      (Transformation|SetWorldScale3D _fog (* (Transformation|GetWorldScale _fog) 1.5))
      (Transformation|SetWorldScale3D _smokewispy_2 (* (Transformation|GetWorldScale _smokewispy_2) 1.5))
      (Transformation|SetWorldScale3D _stage1fire1 (* (Transformation|GetWorldScale _stage1fire1) 2.0))
      (Transformation|SetWorldScale3D _stage1fire2 (* (Transformation|GetWorldScale _stage1fire2) 2.0))
      (Transformation|SetWorldScale3D _stage1fire3 (* (Transformation|GetWorldScale _stage1fire3) 2.0))
      (Transformation|SetWorldScale3D _stage2fire1 (* (Transformation|GetWorldScale _stage2fire1) 2.0))
      (Transformation|SetWorldScale3D _stage2fire2 (* (Transformation|GetWorldScale _stage2fire2) 2.0))
      (Transformation|SetWorldScale3D _stage2fire3 (* (Transformation|GetWorldScale _stage2fire3) 2.0))
      (Game|SpawnActorfromClass "/Game/Mordhau/Blueprints/Fields/BP_EnvFireField.BP_EnvFireField_C" (Transformation|GetWorldTransform (Variables|Default|GetStage3%20-%201)) "Undefined" 0 0)
      (Game|SpawnActorfromClass "/Game/Mordhau/Blueprints/Fields/BP_EnvFireField.BP_EnvFireField_C" (Transformation|GetWorldTransform (Variables|Default|GetStage3%20-%202)) "Undefined" 0 0)
      (Game|SpawnActorfromClass "/Game/Mordhau/Blueprints/Fields/BP_EnvFireField.BP_EnvFireField_C" (Transformation|GetWorldTransform (Variables|Default|GetStage3%20-%203)) "Undefined" 0 0)
      (Game|SpawnActorfromClass "/Game/Mordhau/Blueprints/Fields/BP_EnvFireField.BP_EnvFireField_C" (Transformation|GetWorldTransform (Variables|Default|GetStage3%20-%204)) "Undefined" 0 0)
      (Game|SpawnActorfromClass "/Game/Mordhau/Blueprints/Fields/BP_EnvFireField.BP_EnvFireField_C" (Transformation|GetWorldTransform (Variables|Default|GetStage3%20-%205)) "Undefined" 0 0))))

(fn ConstructionScript
  (|CallParentFunction))