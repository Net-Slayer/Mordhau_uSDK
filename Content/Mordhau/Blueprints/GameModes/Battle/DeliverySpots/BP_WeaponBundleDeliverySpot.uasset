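; BP_WeaponBundleDeliverySpot is a delivery spot for weapon bundles in Battle mode that visually fills up in stages.
; ProgressVisualStage switches on VisualStage to unhide one of three skeletal meshes, playing a sound at its location and spawning a dust emitter.
; The Blueprint only handles this presentation, with Tick and construction deferring to the parent class.
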(event EventBeginPlay)

(event Collision|EventActorBeginOverlap
  (params (OtherActor :type Actor%20Object%20Reference))
  (|CallParentFunction OtherActor) ; This node is disabled and will not be called.\nDrag off pins to build functionality.
)

(event EventTick
  (params (DeltaSeconds :type Float%20%28single-precision%29))
  (|CallParentFunction DeltaSeconds))

(event EventProgressVisualStage
  (bind _skeletalmesh2 (Variables|Default|GetSkeletalMesh2))
  (bind _skeletalmesh1 (Variables|Default|GetSkeletalMesh1))
  (bind _skeletalmesh3 (Variables|Default|GetSkeletalMesh3))
  (switch int (Variables|Default|GetVisualStage)
    (:0
      (Development|SetHiddeninGame _skeletalmesh1 false false)
      (Audio|PlaySoundatLocation 0 (Transformation|GetWorldLocation _skeletalmesh1) "0, 0, 0" 1.0 1.0 0.0 0 0 0)
      (Effects|SpawnEmitteratLocation "/Game/Mordhau/Particles/Dust/P_JumpDust.P_JumpDust" "0, 0, 0"))
    (:1
      (Development|SetHiddeninGame _skeletalmesh2 false false)
      (Audio|PlaySoundatLocation 0 (Transformation|GetWorldLocation _skeletalmesh2) "0, 0, 0" 1.0 1.0 0.0 0 0 0)
      (Effects|SpawnEmitteratLocation "/Game/Mordhau/Particles/Dust/P_JumpDust.P_JumpDust" "0, 0, 0"))
    (:2
      (Development|SetHiddeninGame _skeletalmesh3 false false)
      (Audio|PlaySoundatLocation 0 (Transformation|GetWorldLocation _skeletalmesh3) "0, 0, 0" 1.0 1.0 0.0 0 0 0)
      (Effects|SpawnEmitteratLocation "/Game/Mordhau/Particles/Dust/P_JumpDust.P_JumpDust" "0, 0, 0"))))

(fn ConstructionScript
  (|CallParentFunction))