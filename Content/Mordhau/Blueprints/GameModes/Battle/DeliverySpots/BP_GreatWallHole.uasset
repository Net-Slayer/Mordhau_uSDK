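; BP_GreatWallHole is a Battle-mode delivery spot where delivered explosives blow open a hole by removing a bridge tower cover.
; When the deliverable count changes and is above zero, it reveals a barrel and runs fuse audio and effects for a short delay.
; The barrel then explodes with sound, particles, and radial falloff damage with knockback and ragdolling, while the cover is hidden and loses collision.
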(event EventBeginPlay)

(event Collision|EventActorBeginOverlap
  (params (OtherActor :type Actor%20Object%20Reference))
  (|CallParentFunction OtherActor) ; This node is disabled and will not be called.\nDrag off pins to build functionality.
)

(event EventTick
  (params (DeltaSeconds :type Float%20%28single-precision%29))
  (|CallParentFunction DeltaSeconds) ; This node is disabled and will not be called.\nDrag off pins to build functionality.
)

(event EventOnDeliverablesChanged
  (bind _barrel (Variables|Default|GetBarrel))
  (bind _returnvalue (Transformation|GetWorldLocation _barrel))
  (|CallParentFunction)
  (if (> (Variables|Default|GetDeliverables) 0)
    (Audio|Components|Audio|Play (Variables|Default|GetAudio) 0.0)
    (Components|Activation|Activate (Variables|Default|GetFuse) false)
    (Development|SetHiddeninGame _barrel false false)
    (Utilities|FlowControl|Delay 4.0)
    (Development|SetHiddeninGame _barrel true false)
    (Collision|SetCollisionEnabled (Variables|Default|GetBridgeTowerCover) "NoCollision")
    (Components|Activation|Deactivate (Variables|Default|GetSC_Fuse))
    (Audio|PlaySoundatLocation "/Game/StarterContent/Audio/Explosion_Cue.Explosion_Cue" _returnvalue "0, 0, 0" 0.7 1.0 0.0 0 0 0)
    (Components|Activation|Activate (Variables|Default|GetP_ExplosionHuge) false)
    (Class|MordhauUtilityLibrary|MordhauApplyRadialDamagewithFalloff 0 2.5e+03 3e+01 0.0 0.0 _returnvalue 1.2e+02 7e+02 6.0 0 5e+03 3e+03 6e+02 0 0 "ECC_WorldStatic" false)))

(fn ConstructionScript
  (|CallParentFunction))