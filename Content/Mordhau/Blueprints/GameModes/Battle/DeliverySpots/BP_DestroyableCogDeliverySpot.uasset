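; Battle-mode delivery spot for a destroyable cog, where delivered explosive kegs accumulate until they blow up.
; Each change to the deliverable count reveals cumulative keg meshes and plays the barrel placement effect.
; At four deliverables, spark and fuse effects start, then a five-second delay ends in hidden kegs, falloff radial damage with knockback, a skeletal mesh animation and camera shake.
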(event EventBeginPlay
  (|CallParentFunction))

(event Collision|EventActorBeginOverlap
  (params (OtherActor :type Actor%20Object%20Reference))
  (|CallParentFunction OtherActor) ; This node is disabled and will not be called.\nDrag off pins to build functionality.
)

(event EventTick
  (params (DeltaSeconds :type Float%20%28single-precision%29))
  (|CallParentFunction DeltaSeconds) ; This node is disabled and will not be called.\nDrag off pins to build functionality.
)

(event EventOnDeliverablesChanged
  (bind _deliverables (Variables|Default|GetDeliverables))
  (bind _p_explosivespark (Variables|Default|GetP_ExplosiveSpark))
  (|CallParentFunction)
  (if (> _deliverables 0)
    (Development|SetHiddeninGame (Variables|Default|GetKeg1) false false)
    (Audio|Components|Audio|Play (Variables|Default|GetBarrelPut) 0.0)
    (if (> _deliverables 1)
      (Development|SetHiddeninGame (Variables|Default|GetKeg2) false false)
      (Audio|Components|Audio|Play (Variables|Default|GetBarrelPut) 0.0)
      (if (> _deliverables 2)
        (Development|SetHiddeninGame (Variables|Default|GetSkeletalMesh1) false false)
        (Audio|Components|Audio|Play (Variables|Default|GetBarrelPut) 0.0)
        (if (> _deliverables 3)
          (Development|SetHiddeninGame (Variables|Default|GetSkeletalMesh2) false false)
          (Audio|Components|Audio|Play (Variables|Default|GetBarrelPut) 0.0)
          (Components|Activation|Activate (Variables|Default|GetP_ExplosiveSpark) false)
          (Components|Activation|Activate (Variables|Default|GetSC_ExplosiveBarrelFuse) false)
          (Utilities|FlowControl|Delay 5.0)
          (Components|Activation|Deactivate _p_explosivespark)
          (Development|SetHiddeninGame (Variables|Default|GetKeg2) true false)
          (Class|MordhauUtilityLibrary|MordhauApplyRadialDamagewithFalloff 0 2.5e+03 3e+01 0.0 0.0 (Transformation|GetWorldLocation _p_explosivespark) 1.2e+02 7e+02 6.0 0 5e+03 3e+03 6e+02 self 0 "ECC_WorldStatic" false)
          (Components|Animation|PlayAnimation (Variables|Default|GetSkeletalMesh) (Variables|Default|GetAnimation) false)
          (Camera|PlayWorldCameraShake "/Game/Mordhau/Blueprints/CameraShakes/ExplosionShake.ExplosionShake_C" (Transformation|GetActorLocation) 0.0 3e+03))))))

(fn ConstructionScript
  (|CallParentFunction))