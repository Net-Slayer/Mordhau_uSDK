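; Delivery spot for Mordhau's Battle game mode that shows a siege tower being built in stages.
; ProgressVisualStage switches on VisualStage, revealing the next of six pre-placed build components and hiding the previous one.
; Each step also plays a sound at the new piece and spawns a dust emitter.
; Tick and the construction script only call their parent versions.
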(event EventBeginPlay)

(event Collision|EventActorBeginOverlap
  (params (OtherActor :type Actor%20Object%20Reference))
  (|CallParentFunction OtherActor) ; This node is disabled and will not be called.\nDrag off pins to build functionality.
)

(event EventTick
  (params (DeltaSeconds :type Float%20%28single-precision%29))
  (|CallParentFunction DeltaSeconds))

(event EventProgressVisualStage
  (bind _siegetowerbuild_02 (Variables|Default|GetSiegeTowerBuild_02))
  (bind _siegetowerbuild_03 (Variables|Default|GetSiegeTowerBuild_03))
  (bind _siegetowerbuild_04 (Variables|Default|GetSiegeTowerBuild_04))
  (bind _siegetowerbuild_05 (Variables|Default|GetSiegeTowerBuild_05))
  (bind _siegetowerbuild_06 (Variables|Default|GetSiegeTowerBuild_06))
  (switch int (Variables|Default|GetVisualStage)
    (:0
      (Development|SetHiddeninGame _siegetowerbuild_02 false false)
      (Development|SetHiddeninGame (Variables|Default|GetSiegeTowerBuild_01) true false)
      (Audio|PlaySoundatLocation 0 (Transformation|GetWorldLocation _siegetowerbuild_02) "0, 0, 0" 1.0 1.0 0.0 0 0 0)
      (Effects|SpawnEmitteratLocation "/Game/Mordhau/Particles/Dust/P_JumpDust.P_JumpDust" "0, 0, 0"))
    (:1
      (Development|SetHiddeninGame _siegetowerbuild_03 false false)
      (Development|SetHiddeninGame _siegetowerbuild_02 true false)
      (Audio|PlaySoundatLocation 0 (Transformation|GetWorldLocation _siegetowerbuild_03) "0, 0, 0" 1.0 1.0 0.0 0 0 0)
      (Effects|SpawnEmitteratLocation "/Game/Mordhau/Particles/Dust/P_JumpDust.P_JumpDust" "0, 0, 0"))
    (:2
      (Development|SetHiddeninGame _siegetowerbuild_04 false false)
      (Development|SetHiddeninGame _siegetowerbuild_03 true false)
      (Audio|PlaySoundatLocation 0 (Transformation|GetWorldLocation _siegetowerbuild_04) "0, 0, 0" 1.0 1.0 0.0 0 0 0)
      (Effects|SpawnEmitteratLocation "/Game/Mordhau/Particles/Dust/P_JumpDust.P_JumpDust" "0, 0, 0"))
    (:3
      (Development|SetHiddeninGame _siegetowerbuild_05 false false)
      (Development|SetHiddeninGame _siegetowerbuild_04 true false)
      (Audio|PlaySoundatLocation 0 (Transformation|GetWorldLocation _siegetowerbuild_05) "0, 0, 0" 1.0 1.0 0.0 0 0 0)
      (Effects|SpawnEmitteratLocation "/Game/Mordhau/Particles/Dust/P_JumpDust.P_JumpDust" "0, 0, 0"))
    (:4
      (Development|SetHiddeninGame _siegetowerbuild_06 false false)
      (Development|SetHiddeninGame _siegetowerbuild_05 true false)
      (Audio|PlaySoundatLocation 0 (Transformation|GetWorldLocation _siegetowerbuild_06) "0, 0, 0" 1.0 1.0 0.0 0 0 0)
      (Effects|SpawnEmitteratLocation "/Game/Mordhau/Particles/Dust/P_JumpDust.P_JumpDust" "0, 0, 0"))))

(fn ConstructionScript
  (|CallParentFunction))