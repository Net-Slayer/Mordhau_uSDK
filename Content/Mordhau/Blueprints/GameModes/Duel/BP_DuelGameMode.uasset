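; Duel game mode that hosts many matchmade duels on one server, each in its own room.
; Tick places joining players into rooms by matchmaking ID, then steps each room through timed round stages and copies its state to player controllers.
; A won game or opponent forfeit awards MMR and reward drops; team MMR and leave penalties are stubs.
; After the map-change timer, joining closes and the match ends once the server empties.
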(event Custom|RequestMatchmakingMatch
  (params (MatchID :type String))
  (bind _matchmakingqueuename (Variables|Default|GetMatchmakingQueueName))
  (if (not (Variables|Default|GetbRequestingMatch))
    (Variables|Default|SetbRequestingMatch true)
    (Class|MordhauUtilityLibrary|PrinttoConsoleandLog (Utilities|String|Append "Requesting " _matchmakingqueuename " match " MatchID))
    (bind _match (|GetMatchmakingMatch _matchmakingqueuename MatchID))))

(event EventBeginPlay
  (|CallParentFunction) ; This node is disabled and will not be called.\nDrag off pins to build functionality.
)

(event EventTick
  (params (DeltaSeconds :type Float%20%28single-precision%29))
  (bind _returnvalue (Class|MordhauUtilityLibrary|GetMordhauGameSession))
  (bind _rooms (Variables|Default|GetRooms))
  (|CallParentFunction DeltaSeconds)
  (if (Class|GameMode|IsMatchinProgress)
    (Utilities|FlowControl|Sequence
      (:then_0
        (CallFunction|HandleUnhandledPlayers))
      (:then_1
        ;[1 1 1] Rooms can be deleted, in this case some rooms can be skipped this tick due to index reordering. This is generally harmless, given that we don't rely on ticking every frame.
        (for _index (range 0 (- (Utilities|Array|Length _rooms) 1))
          (if (Utilities|Array|IsValidIndex _rooms _index)
            (CallFunction|TickRoom _index))))
      (:then_2
        (bind _output_get (Variables|Default|SetTimeUntilMapChange (- (Variables|Default|GetTimeUntilMapChange) DeltaSeconds)))
        (if (< _output_get 0.0)
          (Utilities|FlowControl|Sequence
            (:then_0
              (if (Class|MordhauGameSession|AllowsJoin _returnvalue)
                (Class|MordhauGameSession|AllowJoin _returnvalue false)))
            (:then_1
              (bind _asmordhau_game_instance (Utilities|Casting|CastToMordhauGameInstance (Game|GetGameInstance)))
              (bind _returnvalue_2 (Class|GameModeBase|GetNumPlayers))
              (if (and (== _returnvalue_2 0) (== (Class|MordhauGameInstance|GetNumReservedSlots _asmordhau_game_instance) 0))
                (Class|GameMode|EndMatch)))))))))

(event EventRequestedAssignTeam
  (params (Controller :type Controller%20Object%20Reference) (Team :type Integer)))

(event EventPostLogin
  (params (NewPlayer :type Player%20Controller%20Object%20Reference))
  (Utilities|FlowControl|Sequence
    (:then_0
      (|CallParentFunction NewPlayer))
    (:then_1
      (bind _asmordhau_player_controller (Utilities|Casting|CastToMordhauPlayerController NewPlayer))
      (Utilities|Array|Add (Variables|Default|GetUnhandledControllers) _asmordhau_player_controller))))

(event EventOnLogout
  (params (ExitingController :type Controller%20Object%20Reference))
  (Utilities|FlowControl|Sequence
    (:then_0
      (bind _asmordhau_player_controller (Utilities|Casting|CastToMordhauPlayerController ExitingController))
      (CallFunction|HandlePlayerLeaving _asmordhau_player_controller))
    (:then_1
      (|CallParentFunction ExitingController))))

(fn ConstructionScript
  (|CallParentFunction))

(fn HandleNewPlayer
  (params (NewPlayer :type Mordhau%20Player%20Controller%20Object%20Reference))
  (bind _matchmakingmatchid (Variables|/Script/Mordhau.MordhauPlayerController|GetMatchmakingMatchID NewPlayer))
  (bind _asmordhau_player_state (Utilities|Casting|CastToMordhauPlayerState (Variables|/Script/Engine.Controller|GetPlayerState NewPlayer)))
  (bind (_array_element _array_index) (Utilities|Array|ForEachLoopwithBreak (Variables|Default|GetRooms) :!label _label)
    (:LoopBody
      (if (Math|Boolean|ANDBoolean (> (Utilities|Array|Length (.Controllers (Utilities|Struct|BreakST_DuelRoom _array_element))) 0) (< (Utilities|Array|Length (.Controllers (Utilities|Struct|BreakST_DuelRoom _array_element))) (Variables|Default|GetMaxPeoplePerRoom)) (Utilities|Enum|Equal(Enum) (.RoomState (Utilities|Struct|BreakST_DuelRoom _array_element)) "NewEnumerator0"))
        (if (or (Utilities|Enum|Equal(Enum) (.MatchID (Utilities|Struct|BreakST_DuelRoom _array_element)) _matchmakingmatchid) (Class|MordhauUtilityLibrary|IsPlayinEditor))
          (Class|MordhauUtilityLibrary|PrinttoConsoleandLog (Utilities|String|Append "HandleNewPlayer: Player " (.id (Utilities|Struct|Break (Class|MordhauUtilityLibrary|GetPlayFabPlayer _asmordhau_player_state))) " found existing room " (Utilities|String|ToString(Integer) _array_index) " for match " _matchmakingmatchid))
          (LocalVariables|SetRoomIdx _array_index)
          (goto _label Break))))
    (:Completed
      (if (== (LocalVariables|GetRoomIdx) -1)
        (bind _returnvalue (Utilities|Array|Add (Variables|Default|GetRooms) (Utilities|Struct|MakeST_DuelRoom (Utilities|Array|MakeArray NewPlayer) (Utilities|Struct|MakeST_DuelRoomGame 0 0 (Utilities|Struct|MakeSTRUCT_DuelRoundInfo "NewEnumerator0" 0 (+ (Utilities|Time|GetTimeSeconds) (Variables|Default|GetTimeToWaitForPlayers)))) 0 0 "NewEnumerator0" _matchmakingmatchid)))
        (bind _output_get (LocalVariables|SetRoomIdx _returnvalue))
        (Class|MordhauUtilityLibrary|PrinttoConsoleandLog (Utilities|String|Append "HandleNewPlayer: Player " (.id (Utilities|Struct|Break (Class|MordhauUtilityLibrary|GetPlayFabPlayer _asmordhau_player_state))) " created new room " (Utilities|String|ToString(Integer) _output_get) " for match " _matchmakingmatchid))
        (else
          (CallFunction|AddControllertoRoom NewPlayer (LocalVariables|GetRoomIdx))
          (Class|MordhauUtilityLibrary|PrinttoConsoleandLog (Utilities|String|Append "HandleNewPlayer: Player " (.id (Utilities|Struct|Break (Class|MordhauUtilityLibrary|GetPlayFabPlayer _asmordhau_player_state))) " joined room " (Utilities|String|ToString(Integer) (LocalVariables|GetRoomIdx)) " for match " _matchmakingmatchid))))
      (CallFunction|AssignTeam (LocalVariables|GetRoomIdx) NewPlayer))))

(fn SetRoomGame
  (params (RoomIndex :type Integer) (NewGame :type ST%20Duel%20Room%20Game%20Structure%20%28by%20ref%29))
  (Utilities|Struct|SetmembersinST_DuelRoom (Utilities|Array|Get(acopy) (Variables|Default|GetRooms) RoomIndex) NewGame))

(fn SetRoomGameRound
  (params (RoomIndex :type Integer) (NewRound :type STRUCT%20Duel%20Round%20Info%20Structure%20%28by%20ref%29))
  (bind _rooms (Variables|Default|GetRooms))
  (bind _output (Utilities|Array|Get(acopy) _rooms RoomIndex))
  (bind _game (Utilities|Struct|BreakST_DuelRoom _output))
  (bind (_team1wins _team2wins) (Utilities|Struct|BreakST_DuelRoomGame _game))
  (CallFunction|SetRoomGame RoomIndex (Utilities|Struct|MakeST_DuelRoomGame _team1wins _team2wins NewRound)))

(fn FinishRoomGame
  (params (RoomIndex :type Integer) (Winner :type Byte))
  (bind _returnvalue (Class|MordhauUtilityLibrary|GetMordhauGameSession))
  (CallFunction|SetRoomTerminated RoomIndex)
  (for _array_element (Utilities|Struct|BreakST_DuelRoom (Utilities|Array|Get(acopy) (Variables|Default|GetRooms) RoomIndex))
    (bind _asbp_duel_player_controller (Utilities|Casting|CastToBP_DuelPlayerController _array_element))
    (bind _asmordhau_player_state (Utilities|Casting|CastToMordhauPlayerState (Variables|/Script/Engine.Controller|GetPlayerState _array_element)))
    (if (== Winner (Math|Conversions|ToByte(Integer) (Variables|/Script/Mordhau.MordhauPlayerState|GetTeam _asmordhau_player_state)))
      (LocalVariables|SetWinnerID (Utilities|Struct|Break (Class|MordhauUtilityLibrary|GetPlayFabPlayer _asmordhau_player_state)))
      (LocalVariables|SetWinnerPlayerController _asbp_duel_player_controller)
      (Class|MordhauPlayerState|AddScore _asmordhau_player_state 100000) ; 1st place
      (else
        (LocalVariables|SetLoserID (Utilities|Struct|Break (Class|MordhauUtilityLibrary|GetPlayFabPlayer _asmordhau_player_state)))
        (LocalVariables|SetLoserPlayerController _asbp_duel_player_controller))))
  (Utilities|IsValid (LocalVariables|GetWinnerPlayerController)
    (:Is%20Valid
      (Utilities|IsValid (LocalVariables|GetLoserPlayerController)
        (:Is%20Valid
          (bind (_newwinnermmr _newlosermmr) (Class|MordhauUtilityLibrary|AwardDuelMMR (LocalVariables|GetWinnerID) (LocalVariables|GetLoserID)))
          (Variables|/Game/Mordhau/Blueprints/GameModes/Duel/BP_DuelPlayerController.BP_DuelPlayerController_C|SetNewMMR (LocalVariables|GetWinnerPlayerController) _newwinnermmr)
          (Variables|/Game/Mordhau/Blueprints/GameModes/Duel/BP_DuelPlayerController.BP_DuelPlayerController_C|SetNewMMR (LocalVariables|GetLoserPlayerController) _newlosermmr)
          (Class|MordhauGameSession|TriggerRewardDropforPlayer _returnvalue (LocalVariables|GetWinnerPlayerController))
          (Class|MordhauGameSession|TriggerRewardDropforPlayer _returnvalue (LocalVariables|GetLoserPlayerController)))))))

(fn PrepareandStartRoom
  (params (RoomIndex :type Integer))
  (bind (_team1mmr _team2mmr) (CallFunction|ComputeTeamMMR RoomIndex))
  (Utilities|Struct|SetmembersinST_DuelRoom (Utilities|Array|Get(acopy) (Variables|Default|GetRooms) RoomIndex) _team1mmr _team2mmr "NewEnumerator1")
  (CallFunction|SetRoomGameRound RoomIndex (Utilities|Struct|MakeSTRUCT_DuelRoundInfo "NewEnumerator4" 0 (+ (Utilities|Time|GetTimeSeconds) 1e+01))))

(fn IsRoomReadytoStart
  (params (RoomIndex :type Integer))
  (bind _rooms (Variables|Default|GetRooms))
  (bind _output (Utilities|Array|Get(acopy) _rooms RoomIndex))
  (bind _controllers (Utilities|Struct|BreakST_DuelRoom _output))
  (if (== (Utilities|Array|Length _controllers) (Variables|Default|GetMaxPeoplePerRoom))
    (for _array_element _controllers
      (bind _returnvalue (Class|MordhauPlayerController|AreStatsAvailable _array_element))
      (if (not _returnvalue)
        (return false)))
    (return true)
    (else
      (return false))))

(fn TickRoom
  (params (RoomIndex :type Integer))
  (bind _returnvalue (Utilities|Time|GetTimeSeconds))
  (bind _rooms (Variables|Default|GetRooms))
  (bind _team1living (LocalVariables|GetTeam1Living))
  (bind _team2living (LocalVariables|GetTeam2Living))
  (bind _output (Utilities|Array|Get(acopy) _rooms RoomIndex))
  (bind (_controllers _game _roomstate) (Utilities|Struct|BreakST_DuelRoom _output))
  (bind _roundinfo (Utilities|Struct|BreakST_DuelRoomGame _game))
  (bind _returnvalue_2 (Utilities|Enum|Equal(Enum) _roomstate "NewEnumerator2"))
  (bind (_stage _winner _starttime) (Utilities|Struct|BreakSTRUCT_DuelRoundInfo _roundinfo))
  (bind _returnvalue_3 (< _starttime _returnvalue))
  (Utilities|FlowControl|Sequence
    (:then_0
      (if (not _returnvalue_2)
        (switch Utilities|FlowControl|Switch|SwitchonE_DuelRoundStage _stage
          (:NewEnumerator0
            (if _returnvalue_3
              (CallFunction|DestroyRoom RoomIndex true)
              (return)
              (elif (CallFunction|IsRoomReadytoStart RoomIndex)
                (CallFunction|PrepareandStartRoom RoomIndex))))
          (:NewEnumerator4
            (if _returnvalue_3
              (CallFunction|RestartRoom RoomIndex)))
          (:NewEnumerator1
            (if _returnvalue_3
              (CallFunction|SetRoomGameRound RoomIndex (Utilities|Struct|MakeSTRUCT_DuelRoundInfo "NewEnumerator2" 0 0.0))))
          (:NewEnumerator2
            (for _array_element _controllers
              (bind _asmordhau_player_state (Utilities|Casting|CastToMordhauPlayerState (Variables|/Script/Engine.Controller|GetPlayerState _array_element)))
              (if (== (Variables|/Script/Mordhau.MordhauPlayerState|GetTeam _asmordhau_player_state) 0)
                (if (Variables|/Script/Mordhau.MordhauPlayerState|GetbIsAlive _asmordhau_player_state)
                  (Math|Integer|IncrementInt (LocalVariables|GetTeam1Living)))
                (elif (Variables|/Script/Mordhau.MordhauPlayerState|GetbIsAlive _asmordhau_player_state)
                  (Math|Integer|IncrementInt (LocalVariables|GetTeam2Living)))))
            (if (or (== _team1living 0) (== _team2living 0))
              (CallFunction|AwardRoundWin RoomIndex (Math|Integer|SelectInt 0 1 (> _team1living _team2living)))))
          (:NewEnumerator3
            (if _returnvalue_3
              (CallFunction|RestartRoom RoomIndex))))))
    (:then_1
      (for _array_element_2 _controllers
        (bind _asbp_duel_player_controller (Utilities|Casting|CastToBP_DuelPlayerController _array_element_2))
        (Variables|/Game/Mordhau/Blueprints/GameModes/Duel/BP_DuelPlayerController.BP_DuelPlayerController_C|SetReplicatedRoomGame _asbp_duel_player_controller _game))
      (if _returnvalue_2
        (CallFunction|DestroyRoom RoomIndex false)))))

(fn AwardRoundWin
  (params (RoomIndex :type Integer) (Winner :type Integer))
  (bind _rooms (Variables|Default|GetRooms))
  (bind _roundstowin (Variables|Default|GetRoundsToWin))
  (bind _rooms_2 (Variables|Default|GetRooms))
  (bind _output (Utilities|Array|Get(acopy) _rooms_2 RoomIndex))
  (bind _output_2 (Utilities|Array|Get(acopy) _rooms RoomIndex))
  (bind _game (Utilities|Struct|BreakST_DuelRoom _output_2))
  (bind _game_2 (Utilities|Struct|BreakST_DuelRoom _output))
  (bind (_team1wins _team2wins) (Utilities|Struct|BreakST_DuelRoomGame _game))
  (bind (_team1wins_2 _team2wins_2) (Utilities|Struct|BreakST_DuelRoomGame _game_2))
  (bind _returnvalue (== _team1wins _roundstowin))
  (LocalVariables|SetNewTeam1Wins (+ _team1wins_2 (Utilities|Select :Index Winner :Option%200 1 :Option%201 0)))
  (LocalVariables|SetNewTeam2Wins (+ _team2wins_2 (Utilities|Select :Index Winner :Option%200 0 :Option%201 1)))
  (CallFunction|SetRoomGame RoomIndex (Utilities|Struct|MakeST_DuelRoomGame (LocalVariables|GetNewTeam1Wins) (LocalVariables|GetNewTeam2Wins) (Utilities|Struct|MakeSTRUCT_DuelRoundInfo "NewEnumerator3" (Math|Conversions|ToByte(Integer) Winner) (+ (Utilities|Time|GetTimeSeconds) 2.0))))
  (if (or _returnvalue (== _team2wins (Variables|Default|GetRoundsToWin)))
    (CallFunction|FinishRoomGame RoomIndex (Math|Conversions|ToByte(Integer) (Math|Integer|SelectInt 0 1 _returnvalue)))))

(fn RestartRoom
  (params (RoomIndex :type Integer))
  (bind _rooms (Variables|Default|GetRooms))
  (bind _output (Utilities|Array|Get(acopy) _rooms RoomIndex))
  (bind _controllers (Utilities|Struct|BreakST_DuelRoom _output))
  (Utilities|FlowControl|Sequence
    (:then_0
      (bind _outactors (Actor|GetAllActorsOfClass "/Script/Mordhau.MordhauActor"))
      (for _array_element _outactors
        (if (Class|MordhauActor|IsAnyInstanceOwner _array_element _controllers)
          (Actor|DestroyActor _array_element))))
    (:then_1
      (for _array_element_2 _controllers
        (CallFunction|UnpossessandDestroyPawn _array_element_2 true)))
    (:then_2
      (CallFunction|SetRoomGameRound RoomIndex (Utilities|Struct|MakeSTRUCT_DuelRoundInfo "NewEnumerator1" 0 (+ (Utilities|Time|GetTimeSeconds) 5.0))))))

(fn DestroyRoom
  (params (RoomIndex :type Integer) (KickPlayers :type Boolean))
  (bind _rooms (Variables|Default|GetRooms))
  (bind _output (Utilities|Array|Get(acopy) _rooms RoomIndex))
  (bind (_controllers _matchid) (Utilities|Struct|BreakST_DuelRoom _output))
  (CallFunction|SetRoomTerminated RoomIndex)
  (Utilities|FlowControl|Sequence
    (:then_0
      (if KickPlayers
        (for _array_element _controllers
          (Class|MordhauGameSession|KickPlayer (Class|MordhauUtilityLibrary|GetMordhauGameSession) _array_element (Utilities|Text|MakeLiteralText "Match ended")))))
    (:then_1
      (Utilities|Map|Remove (Variables|Default|GetMatches) _matchid)
      (Class|MordhauUtilityLibrary|PrinttoConsoleandLog (Utilities|String|Append "DestroyRoom: Destroyed room " (Utilities|String|ToString(Integer) RoomIndex) " for match " _matchid " (KickPlayers: " (Utilities|String|ToString(Boolean) KickPlayers) ")")))
    (:then_2
      (Utilities|Array|RemoveIndex _rooms RoomIndex))))

(fn HandlePlayerLeaving
  (params (Player :type Mordhau%20Player%20Controller%20Object%20Reference))
  (Utilities|Array|RemoveItem (Variables|Default|GetUnhandledControllers) Player)
  (bind _asmordhau_player_state (Utilities|Casting|CastToMordhauPlayerState (Variables|/Script/Engine.Controller|GetPlayerState Player)))
  (Class|MordhauUtilityLibrary|PrinttoConsoleandLog (Utilities|String|Append "HandlePlayerLeaving: Player " (.id (Utilities|Struct|Break (Class|MordhauUtilityLibrary|GetPlayFabPlayer _asmordhau_player_state))) " from match " (Variables|/Script/Mordhau.MordhauPlayerController|GetMatchmakingMatchID Player) " is leaving"))
  (bind (_array_element _array_index) (Utilities|Array|ForEachLoopwithBreak (Variables|Default|GetRooms) :!label _label)
    (:LoopBody
      (if (and (Utilities|Array|ContainsItem (.Controllers (Utilities|Struct|BreakST_DuelRoom _array_element)) Player) (Utilities|Enum|NotEqual(Enum) (.RoomState (Utilities|Struct|BreakST_DuelRoom _array_element)) "NewEnumerator2"))
        (LocalVariables|SetFoundRoomIdx _array_index)
        (goto _label Break)))
    (:Completed
      (if (!= (LocalVariables|GetFoundRoomIdx) -1)
        (if (Utilities|Enum|Equal(Enum) (Utilities|Struct|BreakST_DuelRoom (Utilities|Array|Get(acopy) (Variables|Default|GetRooms) (LocalVariables|GetFoundRoomIdx))) "NewEnumerator1")
          (for _array_element_2 (.Controllers (Utilities|Struct|BreakST_DuelRoom (Utilities|Array|Get(acopy) (Variables|Default|GetRooms) (LocalVariables|GetFoundRoomIdx))))
            (bind _asmordhau_player_state_2 (Utilities|Casting|CastToMordhauPlayerState (Variables|/Script/Engine.Controller|GetPlayerState _array_element_2)))
            (if (and (!= _array_element_2 Player) (== (Variables|/Script/Mordhau.MordhauPlayerState|GetTeam _asmordhau_player_state_2) (Variables|/Script/Mordhau.MordhauPlayerState|GetTeam _asmordhau_player_state)))
              (LocalVariables|SetHasOtherTeamMembers true)))
          (if (LocalVariables|GetHasOtherTeamMembers)
            (CallFunction|PenalizeforLeavingActiveGame Player (LocalVariables|GetFoundRoomIdx) (== (Utilities|Array|Length (.Controllers (Utilities|Struct|BreakST_DuelRoom (Utilities|Array|Get(acopy) (Variables|Default|GetRooms) (LocalVariables|GetFoundRoomIdx))))) (Variables|Default|GetMaxPeoplePerRoom)))
            (LocalVariables|SetNewControllersArray (.Controllers (Utilities|Struct|BreakST_DuelRoom (Utilities|Array|Get(acopy) (Variables|Default|GetRooms) (LocalVariables|GetFoundRoomIdx)))))
            (Utilities|Array|RemoveItem (LocalVariables|GetNewControllersArray) Player)
            (Utilities|Struct|SetmembersinST_DuelRoom (Utilities|Array|Get(acopy) (Variables|Default|GetRooms) (LocalVariables|GetFoundRoomIdx)) (LocalVariables|GetNewControllersArray))
            (else
              (CallFunction|FinishRoomGame (LocalVariables|GetFoundRoomIdx) (Utilities|Select :Index (Variables|/Script/Mordhau.MordhauPlayerState|GetTeam _asmordhau_player_state) :Option%200 1 :Option%201 0))))
          (elif (Utilities|Enum|Equal(Enum) (Utilities|Struct|BreakST_DuelRoom (Utilities|Array|Get(acopy) (Variables|Default|GetRooms) (LocalVariables|GetFoundRoomIdx))) "NewEnumerator0")
            (CallFunction|DestroyRoom (LocalVariables|GetFoundRoomIdx) true)))))))

(fn AddControllertoRoom
  (params (NewController :type Mordhau%20Player%20Controller%20Object%20Reference) (RoomIndex :type Integer))
  (bind _rooms (Variables|Default|GetRooms))
  (bind _output (Utilities|Array|Get(acopy) _rooms RoomIndex))
  (bind _output_get (LocalVariables|SetNewArray (.Controllers (Utilities|Struct|BreakST_DuelRoom _output))))
  (for _array_element _output_get
    (Utilities|Set|Add (Variables|/Script/Mordhau.MordhauPlayerController|GetInInstanceWithControllers NewController) _array_element)
    (Utilities|Set|Add (Variables|/Script/Mordhau.MordhauPlayerController|GetInInstanceWithControllers _array_element) NewController))
  (Utilities|Array|Add (LocalVariables|GetNewArray) NewController)
  (Utilities|Struct|SetmembersinST_DuelRoom _output (LocalVariables|GetNewArray)))

(fn HandleUnhandledPlayers
  (bind _unhandledcontrollers (Variables|Default|GetUnhandledControllers))
  (for _array_element _unhandledcontrollers
    (if (Utilities|Enum|NotEqual(Enum) (Variables|/Script/Mordhau.MordhauPlayerController|GetMatchmakingMatchID _array_element) "")
      (if (.ReturnValue (Utilities|Map|Find (Variables|Default|GetMatches) (Variables|/Script/Mordhau.MordhauPlayerController|GetMatchmakingMatchID _array_element)))
        (CallFunction|HandleNewPlayer _array_element :!label _label)
        (Class|MordhauUtilityLibrary|ResetController _array_element)
        (Utilities|Array|Add (LocalVariables|GetToRemove) _array_element)
        (else
          (CallFunction|RequestMatchmakingMatch (Variables|/Script/Mordhau.MordhauPlayerController|GetMatchmakingMatchID _array_element))))
      (elif (Class|MordhauUtilityLibrary|IsPlayinEditor)
        (goto _label))))
  (for _array_element_2 (LocalVariables|GetToRemove)
    (Utilities|Array|RemoveItem _unhandledcontrollers _array_element_2)))

(fn SetRoomTerminated
  (params (Index :type Integer))
  (Utilities|Struct|SetmembersinST_DuelRoom (Utilities|Array|Get(acopy) (Variables|Default|GetRooms) Index) "NewEnumerator2"))

(fn AssignTeam
  (params (RoomIndex :type Integer) (Controller :type Mordhau%20Player%20Controller%20Object%20Reference))
  (bind _asmordhau_player_state (Utilities|Casting|CastToMordhauPlayerState (Variables|/Script/Engine.Controller|GetPlayerState Controller)))
  (Class|MordhauPlayerState|SetTeam _asmordhau_player_state (- (Utilities|Array|Length (Utilities|Struct|BreakST_DuelRoom (Utilities|Array|Get(acopy) (Variables|Default|GetRooms) RoomIndex))) 1)))

(fn ComputeTeamMMR
  (params (RoomIndex :type Integer))
  (return 1000 1000 false))

(fn PenalizeforLeavingActiveGame
  (params (Controller :type Mordhau%20Player%20Controller%20Object%20Reference) (RoomIdx :type Integer) (IsFirstLeaver :type Boolean)))