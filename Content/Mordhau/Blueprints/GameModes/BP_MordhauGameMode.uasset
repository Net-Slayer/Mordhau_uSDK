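; Mordhau game mode Blueprint that handles kill events, bot population, player logout and post-match cleanup.
; Kills report team kills to the victim's controller and post kill notifies to the game state, crediting the victim when no valid killer exists.
; Bots are spawned onto a team or removed with optional team filtering, and all are destroyed after the post-match delay unless map change is disabled.
; Logout resolves vote kicks against the leaver; a helper destroys pawns, exiting vehicles first.
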(event EventOnMatchStateChanged
  (params (OldState :type Name%20%28by%20ref%29 :default "None") (NewState :type Name%20%28by%20ref%29 :default "None"))
  (if (Utilities|Name|Equal(Name) NewState "WaitingPostMatch")
    (bind _asbp_mordhau_game_state (Utilities|Casting|CastToBP_MordhauGameState (Game|GetGameState)))
    (if (not (Variables|/Script/Mordhau.MordhauGameState|GetbDoNotGoToNextMapOnMatchEnd _asbp_mordhau_game_state))
      (Utilities|FlowControl|Delay (Variables|/Script/Mordhau.MordhauGameState|GetPostMatchScreenDelay _asbp_mordhau_game_state))
      (bind _outactors (Actor|GetAllActorsOfClass "/Game/Mordhau/AI/BP_MordhauAIController.BP_MordhauAIController_C"))
      (for _array_element _outactors
        (Class|MordhauAIController|DestroyController _array_element)))))

(event EventOnLogout
  (params (ExitingController :type Controller%20Object%20Reference))
  (Utilities|FlowControl|Sequence
    (:then_0
      (if (Class|GameMode|IsMatchinProgress)
        (bind _asmordhau_player_state (Utilities|Casting|CastToMordhauPlayerState (Variables|/Script/Engine.Controller|GetPlayerState ExitingController)))
        (bind _asbp_mordhau_game_state (Utilities|Casting|CastToBP_MordhauGameState (Game|GetGameState)))
        (if (Variables|/Game/Mordhau/Blueprints/GameModes/BP_MordhauGameState.BP_MordhauGameState_C|GetIsVoteOngoing _asbp_mordhau_game_state)
          (if (== (.Target (Utilities|Struct|BreakSTRUCT_VoteKickInfo (Variables|/Game/Mordhau/Blueprints/GameModes/BP_MordhauGameState.BP_MordhauGameState_C|GetVoteKickInfo _asbp_mordhau_game_state))) _asmordhau_player_state)
            (Default|FinishVoteKick _asbp_mordhau_game_state "NewEnumerator3")))))
    (:then_1
      (|CallParentFunction ExitingController))))

(event EventBeginPlay
  (|CallParentFunction))

(event EventRemoveBots
  (params (Amount :type Integer) (Team :type Integer))
  (if (> Amount 0)
    (bind _outactors (Actor|GetAllActorsOfClass "/Game/Mordhau/AI/BP_MordhauAIController.BP_MordhauAIController_C"))
    (if (> (Utilities|Array|Length _outactors) 0)
      (Variables|Default|SetMaxRemoveCount (Math|Integer|Min(Integer) (Utilities|Array|Length _outactors) Amount))
      (Variables|Default|SetRemoveCount 0)
      (bind _asmordhau_game_state (Utilities|Casting|CastToMordhauGameState (Game|GetGameState))
        (:then
          (Variables|Default|SetbCheckTeam (and (< Team (Math|Conversions|ToInteger(Byte) (Variables|/Script/Mordhau.MordhauGameState|GetTeamCount _asmordhau_game_state))) (> Team -1))))
        (:CastFailed
          (Variables|Default|SetbCheckTeam false)))
      (bind _array_element (Utilities|Array|ForEachLoopwithBreak _outactors :!label _label)
        (:LoopBody
          (Utilities|IsValid (Variables|/Script/Engine.Controller|GetPlayerState _array_element)
            (:Is%20Valid
              (if (Variables|Default|GetbCheckTeam)
                (bind _returnvalue (Class|MordhauAIController|GetTeam _array_element))
                (if (== _returnvalue Team)
                  (Class|MordhauAIController|DestroyController _array_element :!label _label_2)
                  (bind _result (Math|Integer|IncrementInt (Variables|Default|GetRemoveCount))
                    (:%20%20
                      (if (== _result (Variables|Default|GetMaxRemoveCount))
                        (goto _label Break)))))
                (else
                  (goto _label_2))))))))))

(event EventAddBots
  (params (Amount :type Integer) (Team :type Integer))
  (if (> Amount 0)
    (for _index (range 1 Amount)
      (bind _returnvalue (Game|SpawnActorfromClass (Variables|Default|GetAIControllerClass) (Math|Transform|MakeTransform "0, 0, 0") "Undefined" 0 0))
      (Class|MordhauGameMode|RequestedAssignTeam _returnvalue Team))))

(event EventOnKilled
  (params (Killer :type Controller%20Object%20Reference) (KilledPlayer :type Controller%20Object%20Reference) (KilledPawn :type Pawn%20Object%20Reference) (Type :type EMordhauDamageType%20Enum :default "Generic") (SubType :type Byte :default 0) (DamageSource :type Actor%20Object%20Reference) (DamageAgent :type Actor%20Object%20Reference))
  (bind _playerstate (Variables|/Script/Engine.Controller|GetPlayerState KilledPlayer))
  (bind _playerstate_2 (Variables|/Script/Engine.Controller|GetPlayerState Killer))
  (|CallParentFunction Killer KilledPlayer KilledPawn Type SubType DamageSource DamageAgent)
  (bind _asbp_mordhau_game_state (Utilities|Casting|CastToBP_MordhauGameState (Game|GetGameState)))
  (Utilities|FlowControl|Sequence
    (:then_0
      (bind _asbp_mordhau_player_controller (Utilities|Casting|CastToBP_MordhauPlayerController KilledPlayer))
      (bind _asbp_mordhau_player_controller_2 (Utilities|Casting|CastToBP_MordhauPlayerController Killer))
      (bind _returnvalue (Class|MordhauGameState|IsFriendly _asbp_mordhau_game_state _asbp_mordhau_player_controller _asbp_mordhau_player_controller_2))
      (if _returnvalue
        (bind _asmordhau_player_state (Utilities|Casting|CastToMordhauPlayerState (Variables|/Script/Engine.Controller|GetPlayerState _asbp_mordhau_player_controller_2)))
        (Default|HandleTeamKill _asbp_mordhau_player_controller _asmordhau_player_state DamageAgent 5e+01)))
    (:then_1
      (Utilities|IsValid KilledPlayer
        (:Is%20Valid
          (Utilities|IsValid _playerstate
            (:Is%20Valid
              (Utilities|IsValid Killer
                (:Is%20Valid
                  (Utilities|IsValid _playerstate_2
                    (:Is%20Valid
                      (Default|AddKillNotify _asbp_mordhau_game_state _playerstate_2 _playerstate DamageAgent Type))
                    (:Is%20Not%20Valid
                      (Default|AddKillNotify _asbp_mordhau_game_state _playerstate _playerstate DamageAgent Type :!label _label))))
                (:Is%20Not%20Valid
                  (goto _label))))))))))

(fn ConstructionScript)

(fn UnpossessandDestroyPawn
  (params (Controller :type Controller%20Object%20Reference) (RestartPlayer :type Boolean))
  (bind _returnvalue (Pawn|GetControlledPawn Controller))
  (Utilities|FlowControl|Sequence
    (:then_0
      (bind _output_get (LocalVariables|SetPawn _returnvalue))
      (bind _asmordhau_vehicle (Utilities|Casting|CastToMordhauVehicle _output_get)
        (:then
          (Class|MordhauVehicle|StopDriving _asmordhau_vehicle)
          (LocalVariables|SetPawn _returnvalue))
        (:CastFailed
          _))
      (Utilities|IsValid (LocalVariables|GetPawn)
        (:Is%20Valid
          (Actor|DestroyActor (LocalVariables|GetPawn)))))
    (:then_1
      (Pawn|UnPossess Controller)
      (if RestartPlayer
        (Class|GameModeBase|RestartPlayer Controller)))))