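; Player controller for economy game modes that runs a coin-based shop and restores the player's last gear on respawn.
; The shop opens when allowed, optionally limited by team zone and a time left, which is a -1 stub here.
; Purchases deduct PlayerState coins, then spawn and equip customized items, while a replicated counter's OnRep plays the purchase sound.
; On first possession of a character, the authority re-grants saved armor, equipment and optionally ammo counts.
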(event Custom|BuyShopItem
  (params (ToBuy :type Actor%20Class%20Reference))
  (bind _purchaseables (Variables|Default|GetPurchaseables))
  (bind (_value _returnvalue) (Utilities|Map|Find _purchaseables ToBuy))
  (if _returnvalue
    (bind _success (CallFunction|SpendCoins _value))
    (if _success
      (bind _asmordhau_actor (Utilities|Casting|CastToMordhauActorClass ToBuy))
      (CallFunction|GiveItem _asmordhau_actor))))

(event EventBeginPlay
  (|CallParentFunction))

(event EventTick
  (params (DeltaSeconds :type Float%20%28single-precision%29))
  (bind _shopmenu (Variables|Default|GetShopMenu))
  (|CallParentFunction DeltaSeconds)
  (if (Pawn|IsLocalPlayerController)
    (Utilities|IsValid _shopmenu
      (:Is%20Valid
        (if (and (Variables|Default|GetIsShopTimeLimited) (Widget|IsVisible _shopmenu))
          (bind _seconds (CallFunction|GetShopTimeLeft))
          (if (<= _seconds 0.0)
            (CallFunction|Hide (.ShopMenu (Variables|Default|GetShopMenu)))))))))

(event EventOnAfterPossess
  (params (APawn :type Pawn%20Object%20Reference))
  (bind _lastheadarmor (Variables|Default|GetLastHeadArmor))
  (bind _lastchestarmor (Variables|Default|GetLastChestArmor))
  (bind _lastlegarmor (Variables|Default|GetLastLegArmor))
  (Utilities|FlowControl|Sequence
    (:then_0
      (bind _asbp_economy_character (Utilities|Casting|CastToBP_EconomyCharacter APawn))
      (if (not (Variables|/Game/Mordhau/Blueprints/GameModes/BP_EconomyCharacter.BP_EconomyCharacter_C|GetAlreadyGaveDefaults _asbp_economy_character))
        (Variables|/Game/Mordhau/Blueprints/GameModes/BP_EconomyCharacter.BP_EconomyCharacter_C|SetAlreadyGaveDefaults _asbp_economy_character true)
        (Networking|SwitchHasAuthority
          (:Authority
            (if (Variables|Default|GetGiveLastGearOnRespawn)
              (Utilities|FlowControl|Sequence
                (:then_0
                  (if (Utilities|IsValidClass _lastheadarmor)
                    (Variables|/Game/Mordhau/Blueprints/Characters/BP_BattleRoyaleCharacter.BP_BattleRoyaleCharacter_C|SetHeadArmor _asbp_economy_character _lastheadarmor)))
                (:then_1
                  (if (Utilities|IsValidClass _lastchestarmor)
                    (Variables|/Game/Mordhau/Blueprints/Characters/BP_BattleRoyaleCharacter.BP_BattleRoyaleCharacter_C|SetChestArmor _asbp_economy_character _lastchestarmor)))
                (:then_2
                  (if (Utilities|IsValidClass _lastlegarmor)
                    (Variables|/Game/Mordhau/Blueprints/Characters/BP_BattleRoyaleCharacter.BP_BattleRoyaleCharacter_C|SetLegArmor _asbp_economy_character _lastlegarmor)))
                (:then_3
                  (for (_array_element _array_index) (Variables|Default|GetLastEquipment)
                    (if (Utilities|IsValidClass _array_element)
                      (bind _returnvalue (Game|SpawnActorfromClass _array_element (Math|Transform|MakeTransform "0, 0, 0") "Undefined" 0 0))
                      (Utilities|FlowControl|Sequence
                        (:then_0
                          (CallFunction|CustomizeEquipment _returnvalue))
                        (:then_1
                          (Class|MordhauCharacter|PickUptoSlot _asbp_economy_character _returnvalue (Math|Conversions|ToByte(Integer) _array_index))
                          (if (!= (Utilities|Array|Get(acopy) (Variables|Default|GetLastEquipmentAmmo) _array_index) (Class|MordhauEquipment|GetAmmo _returnvalue))
                            (if (not (Variables|Default|GetRefillAmmoOnRespawn))
                              (Class|MordhauEquipment|SetAmmo _returnvalue (Utilities|Array|Get(acopy) (Variables|Default|GetLastEquipmentAmmo) _array_index)))))))))))))))
    (:then_1
      (|CallParentFunction APawn))))

(event Input|ActionEvents|InputActionShowProfileSelect
  (params (Key :type Key%20Structure))
  (:Pressed
    (CallFunction|ShowShop)))

(fn ConstructionScript
  (|CallParentFunction))

(fn OnRepPurchaseTrigger
  (Networking|CanExecuteCosmeticEvents
    (:True
      (Audio|PlaySound2D "/Game/Mordhau/Audio/Cues/UI/SC_HordePurchase.SC_HordePurchase" 1.0 1.0 0.0 0 0))))

(fn CustomizeEquipment
  (params (Equipment :type Mordhau%20Equipment%20Object%20Reference))
  (bind _characterprofile (Variables|Default|GetCharacterProfile))
  (bind _appearancecustomization (Utilities|Struct|BreakCharacterProfile _characterprofile))
  (bind (_emblem _emblemcolors) (Utilities|Struct|BreakAppearanceCustomization _appearancecustomization))
  (bind _returnvalue (Class|MordhauEquipment|GetRandomCustomization Equipment true))
  (LocalVariables|SetCustomization _returnvalue)
  (Utilities|FlowControl|Sequence
    (:then_0
      (LocalVariables|SetEmblem _emblem)
      (LocalVariables|SetEmblemColor1 (Utilities|Array|Get(acopy) _emblemcolors))
      (LocalVariables|SetEmblemColor2 (Utilities|Array|Get(acopy) _emblemcolors 1))
      (bind (_outcustomization _returnvalue_2) (Class|MordhauPlayerController|GetDefaultEquipmentCustomizationfor (Utilities|GetClass Equipment)))
      (if _returnvalue_2
        (LocalVariables|SetCustomization _outcustomization)))
    (:then_1
      (Class|MordhauEquipment|AssignCustomization Equipment (LocalVariables|GetCustomization) (Math|Conversions|ToByte(Integer) (LocalVariables|GetEmblem)) (LocalVariables|GetEmblemColor1) (LocalVariables|GetEmblemColor2)))))

(fn GiveItem
  (params (ClassToBuy :type Mordhau%20Actor%20Class%20Reference))
  (bind _characterprofile (Variables|Default|GetCharacterProfile))
  (bind _appearancecustomization (Utilities|Struct|BreakCharacterProfile _characterprofile))
  (bind (_emblem _emblemcolors) (Utilities|Struct|BreakAppearanceCustomization _appearancecustomization))
  (bind _asbp_economy_character (Utilities|Casting|CastToBP_EconomyCharacter (Pawn|GetControlledPawn)))
  (if (Utilities|IsValidClass ClassToBuy)
    (bind _returnvalue (Game|SpawnActorfromClass ClassToBuy (Transformation|GetActorTransform _asbp_economy_character) "Undefined" 0 0))
    (bind _asmordhau_equipment (Utilities|Casting|CastToMordhauEquipment _returnvalue)
      (:then
        (bind _returnvalue_2 (Class|MordhauEquipment|GetRandomCustomization _asmordhau_equipment true))
        (LocalVariables|SetCustomization _returnvalue_2)
        (Utilities|FlowControl|Sequence
          (:then_0
            (LocalVariables|SetEmblem _emblem)
            (LocalVariables|SetEmblemColor1 (Utilities|Array|Get(acopy) _emblemcolors))
            (LocalVariables|SetEmblemColor2 (Utilities|Array|Get(acopy) _emblemcolors 1))
            (bind (_outcustomization _returnvalue_3) (Class|MordhauPlayerController|GetDefaultEquipmentCustomizationfor (Utilities|GetClass _asmordhau_equipment)))
            (if _returnvalue_3
              (LocalVariables|SetCustomization _outcustomization)))
          (:then_1
            (Class|MordhauEquipment|AssignCustomization _asmordhau_equipment (LocalVariables|GetCustomization) (Math|Conversions|ToByte(Integer) (LocalVariables|GetEmblem)) (LocalVariables|GetEmblemColor1) (LocalVariables|GetEmblemColor2))
            (bind _returnvalue_4 (Class|MordhauCharacter|PickUp _asbp_economy_character _asmordhau_equipment))
            (if _returnvalue_4
              (Class|MordhauCharacter|SwitchEquipment _asbp_economy_character _asmordhau_equipment)
              (else
                (Variables|/Script/Mordhau.MordhauEquipment|SetbCanRagdoll _asmordhau_equipment true)
                (Class|MordhauEquipment|UpdateEquipmentState _asmordhau_equipment))))))
      (:CastFailed
        (bind _asbp_wearable_pickup (Utilities|Casting|CastToBP_WearablePickup _returnvalue))
        (Default|Equip _asbp_wearable_pickup _asbp_economy_character)))))

(fn ShowShop
  (bind _available (CallFunction|IsShopAvailable))
  (if _available
    (Utilities|IsValid (.ShopMenu (Variables|Default|GetShopMenu))
      (:Is%20Valid
        _)
      (:Is%20Not%20Valid
        (bind _returnvalue (UserInterface|CreateWidget 0 self))
        (UserInterface|Viewport|AddtoViewport _returnvalue 0)
        (Variables|Default|SetShopMenu 0 _returnvalue)))
    (CallFunction|Show (.ShopMenu (Variables|Default|GetShopMenu)))
    (else
      (Class|MordhauPlayerController|OnActionFailed (Utilities|Name|MakeLiteralName "None")))))

(fn GetShopTimeLeft
  (return -1.0))

(fn IsShopAvailable
  (Utilities|FlowControl|Sequence
    (:then_0
      (bind _asmordhau_character (Utilities|Casting|CastToMordhauCharacter (Pawn|GetControlledPawn))
        (:then
          (if (Class|AdvancedCharacter|GetIsDead _asmordhau_character)
            (return false)
            (elif (Variables|Default|GetShopOnlyInTeamZone)
              (bind _asbp_economy_character (Utilities|Casting|CastToBP_EconomyCharacter _asmordhau_character)
                (:then
                  (if (not (or (and (== (Variables|/Script/Mordhau.AdvancedCharacter|GetTeam _asmordhau_character) 0) (> (Variables|/Game/Mordhau/Blueprints/GameModes/BP_EconomyCharacter.BP_EconomyCharacter_C|GetTeam1EconomyZoneCounter _asbp_economy_character) 0)) (and (== (Variables|/Script/Mordhau.AdvancedCharacter|GetTeam _asmordhau_character) 1) (> (Variables|/Game/Mordhau/Blueprints/GameModes/BP_EconomyCharacter.BP_EconomyCharacter_C|GetTeam2EconomyZoneCounter _asbp_economy_character) 0))))
                    (return false)))
                (:CastFailed
                  (return false))))))
        (:CastFailed
          (return false))))
    (:then_1
      (if (Variables|Default|GetIsShopTimeLimited)
        (bind _seconds (CallFunction|GetShopTimeLeft))
        (if (not (> _seconds 0.0))
          (return false))))
    (:then_2
      (return (Variables|Default|GetAllowShop)))))

(fn SpendCoins
  (params (Amount :type Integer))
  (Utilities|FlowControl|Sequence
    (:then_0
      (bind _asbp_economy_player_state (Utilities|Casting|CastToBP_EconomyPlayerState (Variables|Default|GetPlayerState)))
      (if (>= (Variables|/Game/Mordhau/Blueprints/GameModes/BP_EconomyPlayerState.BP_EconomyPlayerState_C|GetCoins _asbp_economy_player_state) Amount)
        (Variables|/Game/Mordhau/Blueprints/GameModes/BP_EconomyPlayerState.BP_EconomyPlayerState_C|SetCoins _asbp_economy_player_state (- (Variables|/Game/Mordhau/Blueprints/GameModes/BP_EconomyPlayerState.BP_EconomyPlayerState_C|GetCoins _asbp_economy_player_state) Amount))
        (Variables|Default|SetPurchaseTrigger (+ (Variables|Default|GetPurchaseTrigger) 1))
        (return true)))
    (:then_1
      (return false))))

(fn ResetEconomy
  (Utilities|FlowControl|Sequence
    (:then_0
      (bind _asbp_economy_player_state (Utilities|Casting|CastToBP_EconomyPlayerState (Variables|Default|GetPlayerState)))
      (Variables|/Game/Mordhau/Blueprints/GameModes/BP_EconomyPlayerState.BP_EconomyPlayerState_C|SetCoins _asbp_economy_player_state (Utilities|GetClassDefaults (Utilities|GetClass _asbp_economy_player_state))))
    (:then_1
      (Variables|Default|SetLastHeadArmor 0)
      (Variables|Default|SetLastChestArmor 0)
      (Variables|Default|SetLastLegArmor 0)
      (Utilities|Array|Clear (Variables|Default|GetLastEquipment))
      (Utilities|Array|Clear (Variables|Default|GetLastEquipmentAmmo)))))