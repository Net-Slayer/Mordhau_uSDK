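; Mordhau game instance Blueprint that drives the dialog flow for joining a server session.
; Lazily created password, joining and network error dialogs are queued on the HUD; an entered password is stored before joining starts.
; The joining dialog starts a cancellable delay timer that fires Join into AsyncJoin.
; Full-server retry, password join and error-handling chains are disconnected, and several helper functions are empty.
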(event Custom|OnPasswordOKClicked
  (bind _passworddialog (Variables|MordhauGameInstance|GetPasswordDialog))
  ;[0.04831 0 0.7822] Password Dialog
  (Class|MordhauDialog|Hide _passworddialog)
  (bind _text (Default|GetEnteredText _passworddialog))
  (Variables|Default|SetServerPassword (Utilities|String|ToString(Text) _text))
  (Class|MordhauGameInstance|ShowJoiningDialog (Variables|Default|GetSessionToJoin)))

(event Custom|OnJoiningCancelClick
  ;[0.1256 0 0.704] Joining Dialog
  (Utilities|Time|ClearandInvalidateTimerbyHandle (Variables|MordhauGameInstance|GetJoinDelayTimer))
  (Variables|Default|SetSessionToJoin "")
  (Class|MordhauDialog|Hide (Variables|MordhauGameInstance|GetJoiningDialog)))

(event Custom|OnPasswordCancelClicked
  ;[0.04831 0 0.7822] Password Dialog
  (Class|MordhauDialog|Hide (Variables|MordhauGameInstance|GetPasswordDialog)))

(event Custom|OnPasswordTextEntered
  (params (CommitMethod :type ETextCommit%20Enum :default "Default"))
  (bind _passworddialog (Variables|MordhauGameInstance|GetPasswordDialog))
  ;[0.04831 0 0.7822] Password Dialog
  (switch Utilities|FlowControl|Switch|SwitchonETextCommit CommitMethod
    (:OnEnter
      (Class|MordhauDialog|Hide _passworddialog)
      (bind _text (Default|GetEnteredText _passworddialog))
      (Variables|Default|SetServerPassword (Utilities|String|ToString(Text) _text))
      (Class|MordhauGameInstance|ShowJoiningDialog (Variables|Default|GetSessionToJoin)))
    (:OnCleared
      (Class|MordhauDialog|Hide _passworddialog))))

(event Custom|CreateJoiningDialog
  ;[0.1256 0 0.704] Joining Dialog
  (bind _informationdialog (CallFunction|CreateInformationDialog (Game|GetPlayerController 0) "Joining" "" "cancel"))
  (bind _output_get (Variables|MordhauGameInstance|SetJoiningDialog _informationdialog))
  (EventDispatchers|BindEventtoButtonClicked _output_get (delegate Custom|OnJoiningCancelClick)))

(event Custom|OnErrorOkClicked
  ;[0 0.4058 0.4155] Network Error Dialog
  (Class|MordhauDialog|Hide (Variables|MordhauGameInstance|GetNetworkErrorDialog)))

(event Custom|Join
  ;[0.1256 0 0.704] Joining Dialog
  (|AsyncJoin (Variables|Default|GetSessionToJoin) (Class|MordhauGameInstance|GetPartyMemberEntities)))

(event Custom|CreatePasswordDialog
  ;[0.04831 0 0.7822] Password Dialog
  (bind _textinputdialog (CallFunction|CreateTextInputDialog (Game|GetPlayerController 0) "Enter Password" "Password" "ok" "cancel" true))
  (bind _output_get (Variables|MordhauGameInstance|SetPasswordDialog _textinputdialog))
  (EventDispatchers|BindEventtoLeftButtonClicked _output_get (delegate Custom|OnPasswordOKClicked))
  (EventDispatchers|BindEventtoTextCommitted _output_get (delegate Custom|OnPasswordTextEntered))
  (EventDispatchers|BindEventtoRightButtonClicked _output_get (delegate Custom|OnPasswordCancelClicked)))

(event Custom|CreateNetworkErrorDialog
  ;[0 0.4058 0.4155] Network Error Dialog
  (bind _informationdialog (CallFunction|CreateInformationDialog (Game|GetPlayerController 0) "Error" "" "ok"))
  (bind _output_get (Variables|MordhauGameInstance|SetNetworkErrorDialog _informationdialog))
  (EventDispatchers|BindEventtoButtonClicked _output_get (delegate Custom|OnErrorOkClicked)))

(event EventJoinSessionSearchResult
  (params (SearchResult :type Server%20Search%20Result%20Structure%20%28by%20ref%29))
  ;[0.1256 0 0.704] Joining Dialog
  (Class|MordhauGameInstance|ShowJoiningDialog SearchResult))

(event EventShowPasswordDialog
  (params (SearchResult :type Server%20Search%20Result%20Structure%20%28by%20ref%29))
  ;[0.04831 0 0.7822] Password Dialog
  (Variables|Default|SetSessionToJoin SearchResult)
  (Utilities|IsValid (Variables|MordhauGameInstance|GetPasswordDialog)
    (:Is%20Valid
      _)
    (:Is%20Not%20Valid
      (CallFunction|CreatePasswordDialog)))
  (Class|MordhauHUD|EnqueueMordhauDialog (Class|MordhauUtilityLibrary|GetMordhauHUD) (Variables|MordhauGameInstance|GetPasswordDialog)))

(event EventShowNetworkErrorDialog
  (bind _networkerrordialog (Variables|MordhauGameInstance|GetNetworkErrorDialog))
  ;[0 0.4058 0.4155] Network Error Dialog
  (Utilities|IsValid (Variables|MordhauGameInstance|GetNetworkErrorDialog)
    (:Is%20Valid
      _)
    (:Is%20Not%20Valid
      (CallFunction|CreateNetworkErrorDialog)))
  (Variables|/Game/Mordhau/UI/BP_InformationDialog.BP_InformationDialog_C|SetInfoText _networkerrordialog (Variables|Default|GetNetworkErrorText))
  (Class|MordhauHUD|EnqueueMordhauDialog (Class|MordhauUtilityLibrary|GetMordhauHUD) _networkerrordialog))

(event EventShowJoiningDialog
  (params (SearchResult :type Server%20Search%20Result%20Structure%20%28by%20ref%29))
  (bind _joiningdialog (Variables|MordhauGameInstance|GetJoiningDialog))
  ;[0.1256 0 0.704] Joining Dialog
  (bind _output_get (Variables|Default|SetSessionToJoin SearchResult))
  (Utilities|IsValid (Variables|MordhauGameInstance|GetJoiningDialog)
    (:Is%20Valid
      _)
    (:Is%20Not%20Valid
      (CallFunction|CreateJoiningDialog)))
  (bind _text (CallFunction|GetJoiningText (== (.GetCurrentPlayers (|PlayerNumbers _output_get _output_get)) (.GetMaxPlayers (|PlayerNumbers _output_get _output_get)))))
  (Variables|/Game/Mordhau/UI/BP_InformationDialog.BP_InformationDialog_C|SetInfoText _joiningdialog _text)
  (Widget|SetIsEnabled (Variables|/Game/Mordhau/UI/BP_OneButtonDialog.BP_OneButtonDialog_C|GetButton (Variables|/Game/Mordhau/UI/BP_InformationDialog.BP_InformationDialog_C|GetBP_OneButtonDialog _joiningdialog)) true)
  (Class|MordhauHUD|EnqueueMordhauDialog (Class|MordhauUtilityLibrary|GetMordhauHUD) _joiningdialog)
  (bind _returnvalue (Utilities|Time|SetTimerbyEvent (delegate Custom|Join) (Variables|MordhauGameInstance|GetJoinDelay)))
  (Variables|MordhauGameInstance|SetJoinDelayTimer _returnvalue))

(fn GetJoiningTextOld
  (params (Session :type Server%20Search%20Result%20Structure))
  (bind (_getservername _getcurrentplayers _getmaxplayers) (|GetServerDetails Session))
  (return (Utilities|Text|ToText(String) (select (< _getcurrentplayers _getmaxplayers) (Utilities|String|Append "Joining server \"" _getservername "\"...") (Utilities|String|Append "Server \"" _getservername "\" is full, retrying...")))))

(fn GetJoiningText
  (params (bIsFull :type Boolean))
  (return (Utilities|Text|ToText(String) (select bIsFull "Server is full, retrying..." "Joining server..."))))