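; Bandage equipment that heals the character carrying it.
; Firing runs ApplyHeal on the authority only, adding replicated health to a living parent character and spending one ammo, except at 255, which is never decremented.
; Fire and mode-switch requests are refused when a valid character has healing items disabled or health of 100 or more, otherwise they defer to the parent class.
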(event EventFireProjectile
  (params (Origin :type Vector%20%28by%20ref%29 :default "0, 0, 0") (Orientation :type Rotator%20%28by%20ref%29 :default "0, 0, 0") (OwningController :type Controller%20Object%20Reference) (ExpectedDelay :type Float%20%28single-precision%29))
  (Networking|SwitchHasAuthority
    (:Authority
      (CallFunction|ApplyHeal))))

(event EventBeginPlay)

(event Collision|EventActorBeginOverlap
  (params (OtherActor :type Actor%20Object%20Reference)))

(event EventTick
  (params (DeltaSeconds :type Float%20%28single-precision%29)))

(fn ConstructionScript
  (|CallParentFunction))

(fn ApplyHeal
  (bind _returnvalue (Class|MordhauEquipment|GetAmmo))
  (if (> (Class|MordhauEquipment|GetAmmo) 0)
    (bind _output_get (LocalVariables|SetChar (Class|MordhauEquipment|GetParentCharacter)))
    (Utilities|IsValid _output_get
      (:Is%20Valid
        (if (not (Class|AdvancedCharacter|GetIsDead _output_get))
          (Class|AdvancedCharacter|OffsetHealth _output_get (Variables|Default|GetHealAmount) true)
          (if (!= _returnvalue 255)
            (Class|MordhauEquipment|SetAmmo (- _returnvalue 1))))))))

(fn OnRequestFire
  (params (Character :type Mordhau%20Character%20Object%20Reference))
  (Utilities|IsValid Character
    (:Is%20Valid
      (if (and (not (Variables|/Script/Mordhau.AdvancedCharacter|GetbDisableHealingItems Character)) (< (Variables|/Script/Mordhau.AdvancedCharacter|GetHealth Character) 100))
        _
        (else
          (return false))))
    (:Is%20Not%20Valid
      _))
  (bind _returnvalue (|CallParentFunction Character))
  (return _returnvalue))

(fn OnRequestModeSwitch
  (params (Character :type Mordhau%20Character%20Object%20Reference))
  (Utilities|IsValid Character
    (:Is%20Valid
      (if (and (not (Variables|/Script/Mordhau.AdvancedCharacter|GetbDisableHealingItems Character)) (< (Variables|/Script/Mordhau.AdvancedCharacter|GetHealth Character) 100))
        _
        (else
          (return false))))
    (:Is%20Not%20Valid
      _))
  (bind _returnvalue (|CallParentFunction Character))
  (return _returnvalue))