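; Display actor that cycles through a list of equipment customizations, showing one non-interactable piece at a time while spinning it.
; On a timer it destroys the current piece and spawns the next through the Mordhau singleton, wrapping around the list.
; The spawned piece snaps to the root and has its physics proxy removed.
; Tick sets its relative rotation on the chosen axis from a float curve sampled over the switch interval.
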(event EventBeginPlay
  (Variables|Default|SetNextSwitchTime (+ (Utilities|Time|GetGameTimeinSeconds) (Variables|Default|GetSwitchTime)))
  (Variables|Default|SetCurrentId -1)
  (CallFunction|AdvanceEquipmentinList))

(event EventTick
  (params (DeltaSeconds :type Float%20%28single-precision%29))
  (bind _returnvalue (Utilities|Time|GetGameTimeinSeconds))
  (bind _spincurve (Variables|Default|GetSpinCurve))
  (if (< (Variables|Default|GetNextSwitchTime) (Utilities|Time|GetGameTimeinSeconds))
    (Variables|Default|SetNextSwitchTime (+ _returnvalue (Variables|Default|GetSwitchTime)))
    (Variables|Default|SetLastSwitchTime _returnvalue)
    (CallFunction|AdvanceEquipmentinList))
  (Utilities|IsValid (Variables|Default|GetCurrentInstance)
    (:Is%20Valid
      (Utilities|IsValid _spincurve
        (:Is%20Valid
          (bind _returnvalue_2 (Class|MordhauUtilityLibrary|GetNormalizedTime (Variables|Default|GetLastSwitchTime) (Variables|Default|GetNextSwitchTime) (Utilities|Time|GetTimeSeconds)))
          (Transformation|SetActorRelativeRotation (Variables|Default|GetCurrentInstance) (Math|Rotator|MakeRotator (Utilities|Select :Index (Variables|Default|GetSpinAxis) :X (Math|Curves|GetFloatValue _spincurve (* _returnvalue_2 (Variables|Default|GetSwitchTime))) :Y 0.0 :Z 0.0) (Utilities|Select :Index (Variables|Default|GetSpinAxis) :X 0.0 :Y (Math|Curves|GetFloatValue _spincurve (* _returnvalue_2 (Variables|Default|GetSwitchTime))) :Z 0.0) (Utilities|Select :Index (Variables|Default|GetSpinAxis) :X 0.0 :Y 0.0 :Z (Math|Curves|GetFloatValue _spincurve (* _returnvalue_2 (Variables|Default|GetSwitchTime)))))))))))

(fn ConstructionScript)

(fn AdvanceEquipmentinList
  (bind _equipmentlist (Variables|Default|GetEquipmentList))
  (Variables|Default|SetCurrentId (Math|Integer|%(Integer) (+ (Variables|Default|GetCurrentId) 1) (Utilities|Array|Length _equipmentlist)))
  (if (Utilities|Array|IsValidIndex _equipmentlist (Variables|Default|GetCurrentId))
    (Utilities|IsValid (Variables|Default|GetCurrentInstance)
      (:Is%20Valid
        (Actor|DestroyActor (Variables|Default|GetCurrentInstance)))
      (:Is%20Not%20Valid
        _))
    (bind _returnvalue (Class|MordhauSingleton|SpawnEquipment (Class|MordhauUtilityLibrary|GetMordhauSingleton) (Class|MordhauUtilityLibrary|GetWorldOf self) (Utilities|Array|Get(acopy) (Variables|Default|GetEquipmentList) (Variables|Default|GetCurrentId)) 0 0 0 false false))
    (bind _output_get (Variables|Default|SetCurrentInstance _returnvalue))
    (Variables|/Script/Mordhau.MordhauActor|SetbIsInteractable _output_get false)
    (Transformation|AttachComponentToComponent _output_get (Variables|Default|GetDefaultSceneRoot) "None" "SnapToTarget" "SnapToTarget" "SnapToTarget" false)
    (Class|MordhauEquipment|DestroyPhysicsProxy _output_get)))