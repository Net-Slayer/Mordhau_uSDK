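; Bow weapon Blueprint with a replicated fire-arrow mode.
; The FireArrows OnRep swaps the projectile class and fire sound, attaches flame particles and audio to the Missile component, and restores the originals when off.
; On authority, unloading the bow clears fire mode after a short retriggerable delay.
; Loaded and visual-state updates feed a first-person loaded flag to the bow's anim instance.
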(event EventDestroyed
  (CallFunction|ClearFireEffects)
  (|CallParentFunction))

(event EventBeginPlay
  (|CallParentFunction)
  (bind _asab_bow (Utilities|Casting|CastToAB_Bow (Components|SkeletalMesh|GetAnimInstance (Variables|Default|GetSkeletalMeshComponent))))
  (Variables|/Game/Mordhau/Animations/Blueprints/AB_Bow.AB_Bow_C|SetLoadedIn1P _asab_bow (Math|Conversions|ToFloat(Boolean) (and (Variables|Default|GetbIsLoaded) (Variables|Default|GetbIsParentInFirstPerson)))))

(event EventActorBeginOverlap
  (params (OtherActor :type Actor%20Object%20Reference)))

(event EventTick
  (params (DeltaSeconds :type Float%20%28single-precision%29)))

(event EventUpdateEquipmentVisualState
  (|CallParentFunction)
  (Networking|CanExecuteCosmeticEvents
    (:True
      (bind _asab_bow (Utilities|Casting|CastToAB_Bow (Components|SkeletalMesh|GetAnimInstance (Variables|Default|GetSkeletalMeshComponent))))
      (Variables|/Game/Mordhau/Animations/Blueprints/AB_Bow.AB_Bow_C|SetLoadedIn1P _asab_bow (Math|Conversions|ToFloat(Boolean) (and (Variables|Default|GetbIsLoaded) (Variables|Default|GetbIsParentInFirstPerson)))))))

(event EventOnLoadedChanged
  (|CallParentFunction)
  (Utilities|FlowControl|Sequence
    (:then_0
      (Networking|SwitchHasAuthority
        (:Authority
          (if (and (Variables|Default|GetFireArrows) (not (Variables|Default|GetbIsLoaded)))
            (Utilities|FlowControl|RetriggerableDelay 0.25)
            (CallFunction|SetUseFireArrows false)))))
    (:then_1
      (bind _asab_bow (Utilities|Casting|CastToAB_Bow (Components|SkeletalMesh|GetAnimInstance (Variables|Default|GetSkeletalMeshComponent))))
      (Variables|/Game/Mordhau/Animations/Blueprints/AB_Bow.AB_Bow_C|SetLoadedIn1P _asab_bow (Math|Conversions|ToFloat(Boolean) (and (Variables|Default|GetbIsLoaded) (Variables|Default|GetbIsParentInFirstPerson)))))))

(fn ConstructionScript
  (|CallParentFunction))

(fn SetUseFireArrows
  (params (UseFire :type Boolean))
  (if (Math|Boolean|NotEqual(Boolean) (Variables|Default|GetFireArrows) UseFire)
    (Variables|Default|SetFireArrows UseFire)
    (Networking|ForceNetUpdate)))

(fn GetUsesFireArrows
  (return (Variables|Default|GetFireArrows)))

(fn ClearFireEffects
  (Utilities|FlowControl|Sequence
    (:then_0
      (Utilities|IsValid (Variables|Default|GetFireEffectParticleComponent)
        (:Is%20Valid
          (Components|Activation|Deactivate (Variables|Default|GetFireEffectParticleComponent))
          (Variables|Default|SetFireEffectParticleComponent 0))))
    (:then_1
      (Utilities|IsValid (Variables|Default|GetFireEffectAudioComponent)
        (:Is%20Valid
          (Audio|Components|Audio|Stop (Variables|Default|GetFireEffectAudioComponent))
          (Variables|Default|SetFireEffectAudioComponent 0))))))

(fn OnRepFireArrows
  (bind _firearrows (Variables|Default|GetFireArrows))
  (bind _missile (Variables|Default|GetMissile))
  (bind _missile_2 (Variables|Default|GetMissile))
  (bind _firearrowstransform (Variables|Default|GetFireArrowsTransform))
  (bind _returnvalue (Transformation|GetWorldTransform _missile))
  (bind _returnvalue_2 (Math|Transform|ComposeTransforms _firearrowstransform _returnvalue))
  (bind (_location _rotation _scale) (Math|Transform|BreakTransform _returnvalue_2))
  (if (Math|Boolean|NotEqual(Boolean) _firearrows (Variables|Default|GetInternalUsingFireArrows))
    (bind _output_get (Variables|Default|SetInternalUsingFireArrows _firearrows))
    (if _output_get
      (Variables|Default|SetOriginalFireSound (Variables|Default|GetFireSound))
      (Variables|Default|SetFireSound (Variables|Default|GetFireArrowsFireSound))
      (Variables|Default|SetOriginalProjectileClass (Variables|Default|GetProjectileClass))
      (Variables|Default|SetProjectileClass (Variables|Default|GetFireArrowProjectile))
      (bind _returnvalue_3 (Effects|SpawnEmitterAttached (Variables|Default|GetFireArrowsParticleSystem) _missile_2 "None" _location _rotation _scale "KeepWorldPosition"))
      (bind _output_get_2 (Variables|Default|SetFireEffectParticleComponent _returnvalue_3))
      (Utilities|IsValid _output_get_2
        (:Is%20Valid
          (Class|PrimitiveComponent|SetSingleSampleShadowfromStationaryLights _output_get_2 true)
          (bind _returnvalue_4 (Audio|SpawnSoundAttached (Variables|Default|GetFireArrowsSound) _missile_2 "None" _location _rotation "KeepWorldPosition" true 1.0 1.0 0.0 0 0))
          (Variables|Default|SetFireEffectAudioComponent _returnvalue_4)))
      (else
        (CallFunction|ClearFireEffects)
        (Variables|Default|SetProjectileClass (Variables|Default|GetOriginalProjectileClass))
        (Variables|Default|SetFireSound (Variables|Default|GetOriginalFireSound))))))