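; Lute weapon that plays music outside alternate mode, where attacks and kicks pick chord samples, while blocking (by aim angle) and equipment commands play pitch-shifted single notes.
; Rate-limited tones play immediately for the local player and replicate to others through ReplicatedTone, offset by 128 on repeats so OnRep still fires.
; PlayTone cycles four audio components for overlapping sound and strums when the character is idle.
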(event Custom|ServerSetTone
  (params (Tone :type Byte))
  (Utilities|FlowControl|Sequence
    (:then_0
      (if (== Tone (Variables|Default|GetReplicatedTone))
        (Variables|Default|SetReplicatedTone (+ Tone 128))
        (else
          (Variables|Default|SetReplicatedTone Tone))))
    (:then_1
      (Networking|ForceNetUpdate))))

(event EventEquipmentCommand
  (params (Command :type Integer))
  (bind _returnvalue (Class|MordhauEquipment|GetParentCharacter))
  (Utilities|IsValid _returnvalue
    (:Is%20Valid
      (Utilities|Casting|CastToIdleMotion (Class|AdvancedCharacter|GetMotion _returnvalue))
      (if (not (Variables|Default|GetbIsUsingAlternateMode))
        (CallFunction|ServerSetToneandPlay (Math|Conversions|ToByte(Integer) (+ Command 9)))))))

(event EventRequestAttack
  (params (Move :type EAttackMove%20Enum :default "RightStrike") (Angle :type Float%20%28single-precision%29))
  (if (Variables|Default|GetbIsUsingAlternateMode)
    (|CallParentFunction Move Angle)
    (else
      (bind _tone (CallFunction|GetTonefromAttack Move Angle))
      (CallFunction|ServerSetToneandPlay _tone))))

(fn ConstructionScript
  (Variables|Default|SetAudioComponents (Utilities|Array|MakeArray (Variables|Default|GetAudio0) (Variables|Default|GetAudio1) (Variables|Default|GetAudio2) (Variables|Default|GetAudio3)))
  (|CallParentFunction))

(fn OnRepReplicatedTone
  (bind _returnvalue (Class|MordhauEquipment|GetParentCharacter))
  (bind _replicatedtone (Variables|Default|GetReplicatedTone))
  (Networking|CanExecuteCosmeticEvents
    (:True
      (Utilities|IsValid _returnvalue
        (:Is%20Valid
          (if (Class|MordhauCharacter|IsLocallyPlayerControlledIncludingVehicle _returnvalue)
            (return)
            (else
              _)))
        (:Is%20Not%20Valid
          _))
      (Utilities|FlowControl|Sequence
        (:then_0
          (if (>= _replicatedtone 128)
            (LocalVariables|SetTone (- _replicatedtone 128))
            (else
              (LocalVariables|SetTone _replicatedtone))))
        (:then_1
          (CallFunction|PlayTone (LocalVariables|GetTone)))))))

(fn PlayTone
  (params (Tone :type Byte))
  (bind _returnvalue (Class|MordhauEquipment|GetParentCharacter))
  (bind _returnvalue_2 (Math|Conversions|ToInteger(Byte) Tone))
  (bind _lutesounds (Variables|Default|GetLuteSounds))
  (bind _audiocomponents (Variables|Default|GetAudioComponents))
  (bind _output_get (Variables|Default|SetLastAudioComponent (Math|Integer|%(Integer) (+ (Variables|Default|GetLastAudioComponent) 1) (Utilities|Array|Length _audiocomponents))))
  (Audio|Components|Audio|Stop (Utilities|Array|Get(acopy) _audiocomponents _output_get))
  (if (> Tone 8)
    (Audio|Components|Audio|SetSound (Utilities|Array|Get(acopy) _audiocomponents _output_get) "/Game/Mordhau/Audio/Raw/Misc/Instruments/lute_C_3.lute_C_3")
    (Audio|Components|Audio|SetPitchMultiplier (Utilities|Array|Get(acopy) _audiocomponents _output_get) (Math|Float|Power 1.0594631 (Math|Conversions|ToFloat(Integer) (+ -12 (Math|Conversions|ToInteger(Byte) (- Tone 9))))))
    (Audio|Components|Audio|Play (Utilities|Array|Get(acopy) _audiocomponents _output_get) 0.0 :!label _label)
    (Utilities|IsValid _returnvalue
      (:Is%20Valid
        (if (not (Class|AdvancedCharacter|GetIsDead _returnvalue))
          (Utilities|Casting|CastToIdleMotion (Class|AdvancedCharacter|GetMotion _returnvalue))
          (Animation|PlayAnimMontage _returnvalue "/Game/Mordhau/Animations/RawClips/Lute/Strum3p_Montage.Strum3p_Montage" 1.0 "None"))))
    (elif (Utilities|Array|IsValidIndex _lutesounds _returnvalue_2)
      (Audio|Components|Audio|SetSound (Utilities|Array|Get(acopy) _audiocomponents _output_get) (Utilities|Array|Get(acopy) _lutesounds _returnvalue_2))
      (Audio|Components|Audio|SetPitchMultiplier (Utilities|Array|Get(acopy) _audiocomponents _output_get) 1.0)
      (goto _label))))

(fn GetTonefromAttack
  (params (Move :type EAttackMove%20Enum :default "RightStrike") (Angle :type Float%20%28single-precision%29))
  (bind _returnvalue (> Angle 3e+01))
  (bind _returnvalue_2 (< Angle -3e+01))
  (Utilities|FlowControl|Sequence
    (:then_0
      (switch Utilities|FlowControl|Switch|SwitchonEAttackMove Move
        (:RightStrike
          (if _returnvalue
            (return 1)
            (elif _returnvalue_2
              (return 2)
              (else
                (return 0)))))
        (:LeftStrike
          (if _returnvalue
            (return 5)
            (elif _returnvalue_2
              (return 3)
              (else
                (return 4)))))
        (:Stab
          (return 6))
        (:AltStab
          (return 7))
        (:Kick
          (return 8))))
    (:then_1
      (return 99))))

(fn RequestBlock
  (params (BlockType :type EBlockType%20Enum :default "Regular") (bAllowFTP :type Boolean))
  (bind _returnvalue (Class|MordhauEquipment|GetParentCharacter))
  (if (Variables|Default|GetbIsUsingAlternateMode)
    (bind _returnvalue_2 (|CallParentFunction BlockType bAllowFTP))
    (return _returnvalue_2)
    (else
      (Utilities|FlowControl|Sequence
        (:then_0
          (Utilities|IsValid _returnvalue
            (:Is%20Valid
              (bind _asbp_mordhau_player_controller (Utilities|Casting|CastToBP_MordhauPlayerController (Pawn|GetController _returnvalue)))
              (bind _returnvalue_3 (Class|MordhauPlayerController|GetAnglingAngle _asbp_mordhau_player_controller))
              (CallFunction|ServerSetToneandPlay (Math|Conversions|ToByte(Integer) (+ (Math|Float|Round (Math|Float|MapRangeClamped _returnvalue_3 -6e+01 6e+01 0.0 24.0)) 9))))))
        (:then_1
          (return true))))))

(fn ServerSetToneandPlay
  (params (Tone :type Byte))
  (bind _returnvalue (Utilities|Time|GetRealTimeSeconds))
  (bind _returnvalue_2 (Class|MordhauEquipment|GetParentCharacter))
  (if (>= _returnvalue (Variables|Default|GetNextPlayTime))
    (if (<= Tone 8)
      (if (>= _returnvalue (Variables|Default|GetNextChordTime))
        (Variables|Default|SetNextChordTime (+ _returnvalue (Variables|Default|GetChordCooldown)))
        (Variables|Default|SetNextPlayTime (+ _returnvalue (Variables|Default|GetToneCooldown)) :!label _label)
        (CallFunction|ServerSetTone Tone)
        (Utilities|IsValid _returnvalue_2
          (:Is%20Valid
            (if (Class|MordhauCharacter|IsLocallyPlayerControlledIncludingVehicle _returnvalue_2)
              (CallFunction|PlayTone Tone)))))
      (else
        (goto _label)))))