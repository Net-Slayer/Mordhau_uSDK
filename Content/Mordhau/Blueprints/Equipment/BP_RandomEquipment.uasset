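; BP_RandomEquipment is a spawner that places one piece of equipment of a set class with fully randomized cosmetic customization.
; On BeginPlay the server spawns it, disables its cleanup, and assigns a random skin up to Legendary with random parts, colors, pattern and emblem.
; A one-second timer then releases the equipment and destroys the spawner.
; External destruction before then, such as by a spawn controller, also destroys the equipment.
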(event Custom|OnDestroySpawner
  (Variables|Default|SetEquipment 0) ; unset equipment so it won't get destroyed along with the spawner
  (Actor|DestroyActor))

(event EventBeginPlay
  (bind _returnvalue (Class|MordhauUtilityLibrary|GetMordhauSingleton))
  (bind _emblemcolortable (Variables|/Script/Mordhau.MordhauSingleton|GetEmblemColorTable _returnvalue))
  (bind _returnvalue_2 (Utilities|Array|Length (.entries _emblemcolortable)))
  (bind _returnvalue_3 (Math|Random|RandomInteger _returnvalue_2))
  (bind _returnvalue_4 (Math|Conversions|ToByte(Integer) _returnvalue_3))
  (Networking|SwitchHasAuthority
    (:Authority
      (bind _returnvalue_5 (Game|SpawnActorfromClass (Variables|Default|GetEquipmentClass) (Transformation|GetActorTransform) "AlwaysSpawn" 0 0))
      (Utilities|IsValid _returnvalue_5
        (:Is%20Valid
          (Variables|Default|SetEquipment _returnvalue_5)
          (Variables|/Script/Mordhau.MordhauEquipment|SetbAllowCleanup _returnvalue_5 false)
          ;[1 1 1] skin
          (bind (_id _skin) (Class|MordhauUtilityLibrary|GetRandomSkin _returnvalue_5 "Legendary"))
          (Variables|Default|SetSkinId _id)
          ;[1 1 1] parts
          (for _array_element (.PartTypes (Utilities|Struct|BreakEquipmentSkinEntry _skin))
            (Utilities|Array|Add (Variables|Default|GetPartsIds) (Math|Conversions|ToByte(Integer) (Math|Random|RandomInteger (Utilities|Array|Length (.parts _array_element))))))
          ;[1 1 1] colors
          (for _array_element_2 (.ColorTables (Utilities|Struct|BreakEquipmentSkinEntry _skin))
            (Utilities|Array|Add (Variables|Default|GetColorIds) (Math|Conversions|ToByte(Integer) (Math|Random|RandomInteger (Utilities|Array|Length (.entries (Utilities|Array|Get(acopy) (Variables|/Script/Mordhau.MordhauSingleton|GetColorTables (Class|MordhauUtilityLibrary|GetMordhauSingleton)) (Math|Conversions|ToInteger(Byte) _array_element_2))))))))
          ;[1 1 1] pattern
          (Variables|Default|SetPatternId (Math|Conversions|ToByte(Integer) (Math|Random|RandomInteger (Utilities|Array|Length (.Patterns (Utilities|Struct|BreakEquipmentSkinEntry _skin))))))
          ;[1 1 1] emblem
          (Variables|Default|SetEmblemId (Math|Conversions|ToByte(Integer) (Math|Random|RandomInteger (Utilities|Array|Length (.Emblems (Variables|/Script/Mordhau.MordhauSingleton|GetEmblems _returnvalue))))))
          ;[1 1 1] emblem colors
          (Variables|Default|SetEmblemColor1 _returnvalue_4)
          (Variables|Default|SetEmblemColor2 _returnvalue_4)
          (Class|MordhauEquipment|AssignCustomization (Variables|Default|GetEquipment) (Utilities|Struct|MakeEquipmentCustomization 0 (Variables|Default|GetColorIds) (Variables|Default|GetPartsIds) (Variables|Default|GetPatternId) (Math|Conversions|ToByte(Integer) (Variables|Default|GetSkinId))) (Variables|Default|GetEmblemId) (Variables|Default|GetEmblemColor1) (Variables|Default|GetEmblemColor2))
          (Utilities|Time|SetTimerbyEvent (delegate Custom|OnDestroySpawner) 1.0) ; wait for external code (i.e. spawn controller) to handle destruction before destroying this spawner
        )
        (:Is%20Not%20Valid
          (Actor|DestroyActor))))))

(event EventDestroyed
  (bind _equipment (Variables|Default|GetEquipment))
  (Networking|SwitchHasAuthority
    (:Authority
      (Utilities|IsValid _equipment ; if still valid, destruction was initiated by external code so spawned equipment must be destroyed as well
        (:Is%20Valid
          (Actor|DestroyActor _equipment))))))

(fn ConstructionScript)