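; BP_ActorSpawnController randomizes how many placed equipment and vehicle actors remain in a level when play begins.
; On authority only, it shuffles each of its Equipment and Vehicles arrays and rolls a count between that category's min and max, clamped to the array length.
; Valid actors beyond that count are destroyed, so selection works by culling existing actors rather than spawning new ones.
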(event EventBeginPlay
  (bind _equipment (Variables|Default|GetEquipment))
  (bind _vehicles (Variables|Default|GetVehicles))
  (Networking|SwitchHasAuthority
    (:Authority
      (Utilities|FlowControl|Sequence
        (:then_0
          (Utilities|Array|Shuffle _equipment)
          (Variables|Default|SetVisibleEquipmentCount (Math|Integer|Clamp(Integer) (Math|Random|RandomIntegerinRange (Variables|Default|GetMinEquipmentSpawns) (Variables|Default|GetMaxEquipmentSpawns)) 0 (Utilities|Array|Length (Variables|Default|GetEquipment))))
          (for (_array_element _array_index) _equipment
            (Utilities|IsValid _array_element
              (:Is%20Valid
                (if (>= _array_index (Variables|Default|GetVisibleEquipmentCount))
                  (Actor|DestroyActor _array_element))))))
        (:then_1
          (Utilities|Array|Shuffle _vehicles)
          (Variables|Default|SetVisibleVehicleCount (Math|Integer|Clamp(Integer) (Math|Random|RandomIntegerinRange (Variables|Default|GetMinVehicleSpawns) (Variables|Default|GetMaxVehicleSpawns)) 0 (Utilities|Array|Length (Variables|Default|GetVehicles))))
          (for (_array_element_2 _array_index_2) _vehicles
            (Utilities|IsValid _array_element_2
              (:Is%20Valid
                (if (>= _array_index_2 (Variables|Default|GetVisibleVehicleCount))
                  (Actor|DestroyActor _array_element_2))))))))))

(fn ConstructionScript)