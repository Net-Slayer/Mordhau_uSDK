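; Pushable actor that travels along a target spline actor's spline as its progress updates, such as a payload-style objective.
; Progress maps into a spline range; differing front and back distance offsets orient it along the chord between two spline points.
; After each move, the server shifts overlapping characters by the movement delta, skipping those in vehicles.
; Other overlapping Mordhau actors, except Frontline destroyables, take massive damage to clear the path.
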(event EventBeginPlay
  (bind _skeletalmesh (Variables|Default|GetSkeletalMesh))
  (|CallParentFunction)
  (Utilities|IsValid (Variables|Default|GetTargetSplineActor)
    (:Is%20Valid
      (Variables|Default|SetPreviousLocation (Transformation|GetActorLocation))
      (bind _output (CallFunction|GetTransformAlongSplineOffset (Variables|Default|GetSplineOffsetA) (Variables|Default|GetSplineOffsetB)))
      (Transformation|SetActorTransform _output)
      (Networking|SwitchHasAuthority
        (:Authority
          (bind _outactors (Collision|ComponentOverlapActors _skeletalmesh (Transformation|GetWorldTransform _skeletalmesh) (Utilities|Array|MakeArray "ObjectTypeQuery3" "ObjectTypeQuery5" "ObjectTypeQuery1") 0))
          (for _array_element _outactors
            (bind _asmordhau_character (Utilities|Casting|CastToMordhauCharacter _array_element)
              (:then
                (Utilities|IsValid (Variables|/Script/Mordhau.MordhauCharacter|GetCurrentVehicle _asmordhau_character)
                  (:Is%20Not%20Valid
                    _)))
              (:CastFailed
                _))
            (bind _asadvanced_character (Utilities|Casting|CastToAdvancedCharacter _array_element)
              (:then
                (Transformation|AddActorWorldOffset _asadvanced_character (- (Transformation|GetActorLocation) (Variables|Default|GetPreviousLocation))))
              (:CastFailed
                (bind _asmordhau_actor (Utilities|Casting|CastToMordhauActor _array_element))
                (Utilities|Casting|CastToBP_FrontlineDestroyable _array_element
                  (:CastFailed
                    (Game|Damage|ApplyDamage _asmordhau_actor 1e+07 0 0)))))))))))

(event Collision|EventActorBeginOverlap
  (params (OtherActor :type Actor%20Object%20Reference)))

(event EventTick
  (params (DeltaSeconds :type Float%20%28single-precision%29)))

(event EventOnProgressUpdated
  (params (OldProgress :type Float%20%28single-precision%29))
  (bind _skeletalmesh (Variables|Default|GetSkeletalMesh))
  (Utilities|IsValid (Variables|Default|GetTargetSplineActor)
    (:Is%20Valid
      (Variables|Default|SetPreviousLocation (Transformation|GetActorLocation))
      (bind _output (CallFunction|GetTransformAlongSplineOffset (Variables|Default|GetSplineOffsetA) (Variables|Default|GetSplineOffsetB)))
      (Transformation|SetActorTransform _output)
      (Networking|SwitchHasAuthority
        (:Authority
          (bind _outactors (Collision|ComponentOverlapActors _skeletalmesh (Transformation|GetWorldTransform _skeletalmesh) (Utilities|Array|MakeArray "ObjectTypeQuery3" "ObjectTypeQuery5" "ObjectTypeQuery1") 0))
          (for _array_element _outactors
            (bind _asmordhau_character (Utilities|Casting|CastToMordhauCharacter _array_element)
              (:then
                (Utilities|IsValid (Variables|/Script/Mordhau.MordhauCharacter|GetCurrentVehicle _asmordhau_character)
                  (:Is%20Not%20Valid
                    _)))
              (:CastFailed
                _))
            (bind _asadvanced_character (Utilities|Casting|CastToAdvancedCharacter _array_element)
              (:then
                (Transformation|AddActorWorldOffset _asadvanced_character (- (Transformation|GetActorLocation) (Variables|Default|GetPreviousLocation))))
              (:CastFailed
                (bind _asmordhau_actor (Utilities|Casting|CastToMordhauActor _array_element))
                (Utilities|Casting|CastToBP_FrontlineDestroyable _array_element
                  (:CastFailed
                    (Game|Damage|ApplyDamage _asmordhau_actor 1e+07 0 0)))))))))))

(fn ConstructionScript
  (Variables|Default|SetPushArea (Variables|Default|GetArea)))

(fn GetTransformAlongSplineOffset
  (params (OffsetA :type Float%20%28single-precision%29) (OffsetB :type Float%20%28single-precision%29))
  (bind _progress (Variables|Default|GetProgress))
  (bind _targetsplineactor (Variables|Default|GetTargetSplineActor))
  (bind _splinerange (Variables|Default|GetSplineRange))
  (bind (_x _y) (Math|Vector2D|BreakVector2D _splinerange))
  (bind _spline (Variables|/Game/Mordhau/Blueprints/Interactables/BP_SplineActor.BP_SplineActor_C|GetSpline _targetsplineactor))
  (bind _returnvalue (Math|Float|Lerp _x _y _progress))
  (bind _returnvalue_2 (Spline|GetSplineLength _spline))
  (bind _returnvalue_3 (* _returnvalue _returnvalue_2))
  (bind _returnvalue_4 (+ _returnvalue_3 OffsetA))
  (bind _returnvalue_5 (Spline|GetLocationatDistanceAlongSpline _spline _returnvalue_4 "World"))
  (if (== OffsetA OffsetB)
    (return (Spline|GetTransformatTime _spline _returnvalue "World" true false))
    (else
      (return (Math|Transform|MakeTransform _returnvalue_5 (Math|Rotator|MakeRotfromXZ (Math|Vector|Normalize (- (Spline|GetLocationatDistanceAlongSpline _spline (+ _returnvalue_3 OffsetB) "World") _returnvalue_5)) (Math|Vector|GetUpVector (Spline|GetRotationatDistanceAlongSpline _spline _returnvalue_4 "World"))))))))