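; BP_HorseSpawner is a vehicle spawner that places a random horse at its location and respawns it after death.
; On BeginPlay, the authority builds the pool from allowed regular, medium and armored sets and reads respawn time from MordhauGameMode.
; Horses spawn far below, then teleport into place after a brief random delay, retrying if blocked.
; Color overrides apply only when the unused-dying time override is nonzero.
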(event Custom|OnHorseDied
  (params (Character :type Advanced%20Character%20Object%20Reference))
  (Utilities|FlowControl|Delay (Variables|Default|GetRespawnTime))
  (CallFunction|TrySpawnVehicle))

(event EventBeginPlay
  (Utilities|FlowControl|Sequence
    (:then_0
      (Networking|SwitchHasAuthority
        (:Authority
          (Utilities|FlowControl|Sequence
            (:then_0
              (if (Variables|HorseSpawner|GetbAllowRegular)
                (Utilities|Set|AddItems (Variables|HorseSpawner|GetHorses) (Variables|HorseSpawner|GetRegularHorses))))
            (:then_1
              (if (Variables|HorseSpawner|GetbAllowMedium)
                (Utilities|Set|AddItems (Variables|HorseSpawner|GetHorses) (Variables|HorseSpawner|GetMediumHorses))))
            (:then_2
              (if (Variables|HorseSpawner|GetbAllowArmored)
                (Utilities|Set|AddItems (Variables|HorseSpawner|GetHorses) (Variables|HorseSpawner|GetArmoredHorses))))
            (:then_3
              (bind _asmordhau_game_mode (Utilities|Casting|CastToMordhauGameMode (Game|GetGameMode)))
              (Variables|Default|SetRespawnTime (Variables|/Script/Mordhau.MordhauGameMode|GetHorseRespawnTime _asmordhau_game_mode)))))))
    (:then_1
      (|CallParentFunction))))

(event EventSpawnVehicle
  (bind _overridemintimetostartunuseddying (Variables|Default|GetOverrideMinTimeToStartUnusedDying))
  (bind _horses (Variables|HorseSpawner|GetHorses))
  (bind _overridehorsecolor1 (Variables|Default|GetOverrideHorseColor1))
  (bind _overridehorsecolor2 (Variables|Default|GetOverrideHorseColor2))
  (bind _returnvalue (Utilities|Set|Length _horses))
  (if (> _returnvalue 0)
    (bind _result (Utilities|Set|ToArray (Variables|HorseSpawner|GetHorses)))
    (bind _returnvalue_2 (Game|SpawnActorfromClass (Utilities|Array|Get(acopy) _result (Math|Random|RandomIntegerinRange 0 (- _returnvalue 1))) (Math|Transform|MakeTransform "0, 0,-3000.000000" "0, 0, 0" "1,1,1") "AlwaysSpawn" 0 0))
    (Variables|Default|SetSpawnedVehicle _returnvalue_2)
    (Utilities|FlowControl|Sequence
      (:then_0
        (if (!= _overridemintimetostartunuseddying 0.0)
          (bind _asbp_horse (Utilities|Casting|CastToBP_Horse _returnvalue_2))
          (Variables|/Script/Mordhau.MordhauVehicle|SetMinTimeToStartUnusedDying _asbp_horse _overridemintimetostartunuseddying)
          (Utilities|FlowControl|Sequence
            (:then_0
              (if (!= _overridehorsecolor1 -1)
                (Variables|/Game/Mordhau/Blueprints/Interactables/Animals/BP_Horse.BP_Horse_C|SetColor1 _asbp_horse (Math|Conversions|ToByte(Integer) _overridehorsecolor1))))
            (:then_1
              (if (!= _overridehorsecolor2 -1)
                (Variables|/Game/Mordhau/Blueprints/Interactables/Animals/BP_Horse.BP_Horse_C|SetColor2 _asbp_horse (Math|Conversions|ToByte(Integer) _overridehorsecolor2)))))))
      (:then_1
        (Utilities|FlowControl|Delay (Math|Random|RandomFloatinRange 0.0 0.1))
        (bind _returnvalue_3 (Transformation|Teleport _returnvalue_2 (Transformation|GetActorLocation) (Transformation|GetActorRotation)))
        (if _returnvalue_3
          (if (> (Variables|Default|GetRespawnTime) 0.0)
            (EventDispatchers|AssignOnCharacterDied _returnvalue_2 (delegate Custom|OnHorseDied)))
          (else
            (Utilities|FlowControl|Delay (Math|Random|RandomFloatinRange 0.1 0.5)) ; Not enough space; destroy actor and retry
            (Actor|DestroyActor _returnvalue_2)
            (Utilities|FlowControl|Delay (Math|Random|RandomFloatinRange 1.0 3.0))
            (CallFunction|TrySpawnVehicle)))))))

(fn ConstructionScript
  (|CallParentFunction))