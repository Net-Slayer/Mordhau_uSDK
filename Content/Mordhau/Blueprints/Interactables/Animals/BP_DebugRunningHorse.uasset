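; Debug horse Blueprint that keeps itself running forward without rider input.
; Every Tick it applies full forward movement input, caps DesiredGear at one above the integer TargetGear, and copies the result to UncontrolledGear.
; It has no other active logic of its own, as BeginPlay and overlap events are disabled and construction only calls the parent.
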(event EventBeginPlay
  (|CallParentFunction) ; This node is disabled and will not be called.\nDrag off pins to build functionality.
)

(event Collision|EventActorBeginOverlap
  (params (OtherActor :type Actor%20Object%20Reference)))

(event EventTick
  (params (DeltaSeconds :type Float%20%28single-precision%29))
  (Class|AdvancedCharacter|MoveForward 1.0)
  (bind _output_get (Variables|Default|SetDesiredGear (Math|Integer|Min(Integer) (Variables|Default|GetDesiredGear) (+ (Math|Conversions|ToInteger(Byte) (Variables|Default|GetTargetGear)) 1))))
  (Variables|Default|SetUncontrolledGear _output_get))

(fn ConstructionScript
  (|CallParentFunction))