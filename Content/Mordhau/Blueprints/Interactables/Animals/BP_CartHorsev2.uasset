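; Horse-drawn cart variant of the rideable horse: a pseudo-vehicle pawn that maps movement and look axes to turning and looking.
; On LOD tick it aligns the static mesh to the horse's Seat socket and spins a scene component, likely the wheels, from the anim rate while moving.
; BeginPlay widens the AnimBP's front-to-back leg distance, and construction registers the capsule as a secondary, step-capable movement component.
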(event EventBeginPlay
  (|CallParentFunction)
  (bind _asab_base_horse (Utilities|Casting|CastToAB_BaseHorse (Components|SkeletalMesh|GetAnimInstance (Variables|Character|GetMesh))))
  (Variables|/Script/Mordhau.HorseAnimInstance|SetFrontBackLegsDistance _asab_base_horse 5.4e+02))

(event Collision|EventActorBeginOverlap
  (params (OtherActor :type Actor%20Object%20Reference)))

(event EventTick
  (params (DeltaSeconds :type Float%20%28single-precision%29)))

(event EventBPLODTick
  (params (DeltaTime :type Float%20%28single-precision%29))
  (bind _returnvalue (Transformation|GetActorRightVector))
  (bind _staticmesh (Variables|Default|GetStaticMesh))
  (bind _mesh (Variables|Character|GetMesh))
  (bind _returnvalue_2 (* _returnvalue -1.0))
  (bind _returnvalue_3 (Transformation|GetWorldLocation _staticmesh))
  (bind _returnvalue_4 (Transformation|GetSocketLocation _mesh "Seat"))
  (bind _returnvalue_5 (- _returnvalue_4 _returnvalue_3))
  (bind _returnvalue_6 (Class|KismetMathLibrary|MakeRotfromYX _returnvalue_5 _returnvalue_2))
  (bind (_roll _pitch _yaw) (Math|Rotator|BreakRotator _returnvalue_6))
  (|CallParentFunction DeltaTime)
  (bind _asab_base_horse (Utilities|Casting|CastToAB_BaseHorse (Components|SkeletalMesh|GetAnimInstance (Variables|Character|GetMesh))))
  (Transformation|SetWorldRotation _staticmesh (Math|Rotator|MakeRotator _roll (.Pitch (Math|Rotator|BreakRotator (Transformation|GetSocketRotation _mesh "Seat"))) _yaw) false false)
  (Transformation|AddRelativeRotation (Variables|Default|GetScene) (Math|Rotator|MakeRotator (* (Variables|/Script/Mordhau.HorseAnimInstance|GetMovementAnimRate _asab_base_horse) DeltaTime 9e+01 (Math|Conversions|ToFloat(Boolean) (>= (Variables|/Script/Mordhau.HorseAnimInstance|GetHorseVelocity _asab_base_horse) 1.0))) 0.0 0.0) false false))

(event Input|AxisEvents|InputAxisMoveRight
  (params (AxisValue :type Float%20%28single-precision%29))
  (Class|AdvancedCharacter|Turn AxisValue false))

(event Input|AxisEvents|InputAxisLookUp
  (params (AxisValue :type Float%20%28single-precision%29))
  (Class|AdvancedCharacter|LookUp AxisValue false))

(event Input|AxisEvents|InputAxisTurnRight
  (params (AxisValue :type Float%20%28single-precision%29))
  (Class|MordhauVehicle|SecondaryTurn AxisValue false))

(fn ConstructionScript
  (bind _capsule (Variables|Default|GetCapsule))
  (|CallParentFunction)
  (bind _aspseudo_vehicle_movement_component (Utilities|Casting|CastToPseudoVehicleMovementComponent (Variables|Character|GetCharacterMovement)))
  (Variables|/Script/Mordhau.PseudoVehicleMovementComponent|SetSecondaryComponents _aspseudo_vehicle_movement_component (Utilities|Array|MakeArray _capsule))
  (Variables|/Script/Mordhau.PseudoVehicleMovementComponent|SetSecondaryStepCapableComponents _aspseudo_vehicle_movement_component (Utilities|Array|MakeArray _capsule)))