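; BP_SplineMovable is an environment actor that moves its static mesh continuously along a referenced target spline.
; Each tick, it derives spline distance from game time, speed and a fractional starting offset, subtracting accumulated lengths to loop back to the start.
; ApplyJiggle then eases mesh rotation toward a pitch based on world X movement since the last frame, with zero roll and yaw.
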(event EventBeginPlay)

(event Collision|EventActorBeginOverlap
  (params (OtherActor :type Actor%20Object%20Reference)))

(event EventTick
  (params (DeltaSeconds :type Float%20%28single-precision%29))
  (bind _targetspline (Variables|Default|GetTargetSpline))
  (bind _spline (Variables|/Game/Mordhau/Blueprints/Interactables/BP_SplineActor.BP_SplineActor_C|GetSpline _targetspline))
  (bind _returnvalue (Spline|GetSplineLength _spline))
  (Transformation|SetWorldLocation (Variables|Default|GetStaticMesh) (Spline|GetLocationatDistanceAlongSpline _spline (- (+ (* (Utilities|Time|GetGameTimeinSeconds) (Variables|Default|GetSpeed)) (* (Variables|Default|GetStartingPoint%28%25%29) _returnvalue)) (Variables|Default|GetRemovedLength)) "World") false false)
  (CallFunction|ApplyJiggle)
  (if (> (- (+ (* (Utilities|Time|GetGameTimeinSeconds) (Variables|Default|GetSpeed)) (* (Variables|Default|GetStartingPoint%28%25%29) _returnvalue)) (Variables|Default|GetRemovedLength)) _returnvalue)
    (Variables|Default|SetRemovedLength (+ (Variables|Default|GetRemovedLength) _returnvalue))))

(fn ConstructionScript)

(fn ApplyJiggle
  (bind _staticmesh (Variables|Default|GetStaticMesh))
  (Transformation|SetWorldRotation _staticmesh (Math|Rotator|Lerp(Rotator) (Transformation|GetWorldRotation _staticmesh) (Math|Rotator|MakeRotator 0.0 (.X (Math|Vector|BreakVector (* (- (.Location (Math|Transform|BreakTransform (Variables|Default|GetLastFrameTransform))) (.Location (Math|Transform|BreakTransform (Transformation|GetWorldTransform _staticmesh)))) 2.0))) 0.0) 0.05) false false)
  (Variables|Default|SetLastFrameTransform (Transformation|GetWorldTransform _staticmesh)))