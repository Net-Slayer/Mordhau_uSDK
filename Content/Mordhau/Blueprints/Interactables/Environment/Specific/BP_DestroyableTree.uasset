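; Destroyable tree that players chop down, falling to crush and knock back whatever it lands on.
; AnyDamage passes damage on only for hits in a height band on one side, otherwise zero.
; At zero replicated health, Tick lerps the log to the PreviewTree transform along a bounce curve.
; A delayed impact deals radial damage at three points, credited to the final chopper, with effects and damage skipped early in game time.
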(event Game|Damage|EventAnyDamage
  (params (Damage :type Float%20%28single-precision%29) (DamageType :type Damage%20Type%20Object%20Reference) (InstigatedBy :type Controller%20Object%20Reference) (DamageCauser :type Actor%20Object%20Reference))
  (bind _lastdamagelocation (Variables|Default|GetLastDamageLocation))
  (bind _returnvalue (- _lastdamagelocation "0, 0,160.000000"))
  (bind (_x _y _z) (Math|Vector|BreakVector _returnvalue))
  (if (and (< (Math|Float|Absolute(Float) _z) 5e+01) (> _y 0.0))
    (|CallParentFunction Damage DamageType InstigatedBy DamageCauser)
    (else
      (|CallParentFunction 0.0 DamageType InstigatedBy DamageCauser))))

(event Collision|EventActorBeginOverlap
  (params (OtherActor :type Actor%20Object%20Reference))
  (|CallParentFunction OtherActor) ; This node is disabled and will not be called.\nDrag off pins to build functionality.
)

(event EventTick
  (params (DeltaSeconds :type Float%20%28single-precision%29))
  (bind _fallstarttime (Variables|Default|GetFallStartTime))
  (|CallParentFunction DeltaSeconds)
  (if (not (== (Variables|Default|GetFallStartTime) -1.0))
    (bind _returnvalue (Class|MordhauUtilityLibrary|GetNormalizedTime _fallstarttime (+ _fallstarttime 5.0) (Utilities|Time|GetTimeSeconds)))
    (Transformation|SetRelativeTransform (Variables|Default|GetBreakableTree_Log) (Math|Transform|Lerp(Transform) (Variables|Default|GetFallingLogOrigin) (Transformation|GetRelativeTransform (Variables|Default|GetPreviewTree)) (Math|Curves|GetFloatValue (Variables|Default|GetBounceCurve) _returnvalue)) false false)
    (if (== _returnvalue 1.0)
      (Actor|Tick|SetActorTickEnabled false))))

(event EventOnReplicatedHealthChanged
  (bind _self self)
  (bind _breakabletree_log (Variables|Default|GetBreakableTree_Log))
  (bind _breakabletree_log1 (Variables|Default|GetBreakableTree_Log1))
  (bind _impact3 (Variables|Default|GetImpact3))
  (bind _impact2 (Variables|Default|GetImpact2))
  (bind _returnvalue (Transformation|GetWorldLocation _impact2))
  (bind _returnvalue_2 (Transformation|GetWorldLocation _impact3))
  (bind _returnvalue_3 (Transformation|GetWorldLocation _breakabletree_log))
  (bind _returnvalue_4 (Transformation|GetWorldLocation _breakabletree_log1))
  (|CallParentFunction)
  (Variables|Default|SetFinalChopperController (Variables|Default|GetLastHealthChangeInstigator))
  (if (== (Variables|Default|GetReplicatedHealth) 0)
    (if (== (Variables|Default|GetFallStartTime) -1.0)
      (Variables|Default|SetFallingLogOrigin (Transformation|GetRelativeTransform (Variables|Default|GetBreakableTree_Log)))
      (Variables|Default|SetFallStartTime (Utilities|Time|GetTimeSeconds))
      (Actor|Tick|SetActorTickEnabled true)
      (Development|SetHiddeninGame (Variables|Default|GetBreakableTree_Log) false false)
      (if (> (Utilities|Time|GetGameTimeinSeconds) 3.0)
        (Audio|PlaySoundatLocation 0 _returnvalue_3 "0, 0, 0" 1.0 1.0 0.0 0 0 0)
        (Effects|SpawnEmitteratLocation 0 _returnvalue_3)
        (Utilities|FlowControl|Delay 3.3)
        (Effects|SpawnEmitteratLocation 0 _returnvalue_2 "90.000000, 0,0.000000")
        (Audio|PlaySoundatLocation 0 _returnvalue_2 "0, 0, 0" 1.0 1.0 0.0 0 0 0)
        (Class|MordhauUtilityLibrary|MordhauApplyRadialDamagewithFalloff 0 2.5e+03 1.0 4e+02 2e+01 _returnvalue_2 5e+01 1e+02 5.0 0 1e+03 5e+02 2e+02 _self (Variables|Default|GetFinalChopperController) "ECC_WorldStatic" false)
        (Class|MordhauUtilityLibrary|MordhauApplyRadialDamagewithFalloff 0 2.5e+03 1.0 4e+02 2e+01 (Transformation|GetWorldLocation (Variables|Default|GetImpact1)) 5e+01 1e+02 5.0 0 1e+03 5e+02 2e+02 _self (Variables|Default|GetFinalChopperController) "ECC_WorldStatic" false)
        (Class|MordhauUtilityLibrary|MordhauApplyRadialDamagewithFalloff 0 2.5e+03 1.0 4e+02 2e+01 _returnvalue 5e+01 1e+02 5.0 0 1e+03 5e+02 2e+02 _self (Variables|Default|GetFinalChopperController) "ECC_WorldStatic" false)
        (Camera|PlayWorldCameraShake "/Game/Mordhau/Blueprints/CameraShakes/ImpactShake.ImpactShake_C" _returnvalue 2.5e+02 7.5e+03 1e+01)))
    (elif (> (Utilities|Time|GetGameTimeinSeconds) 3.0)
      (Audio|PlaySoundatLocation "/Game/Mordhau/Audio/Cues/Foley/SC_FallDamage.SC_FallDamage" _returnvalue_4 "0, 0, 0" 1.0 1.0 0.0 0 0 0)
      (Effects|SpawnEmitteratLocation 0 _returnvalue_4))))

(fn ConstructionScript
  (|CallParentFunction))