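; Interactable oil cauldron that tips to pour oil and spawns an oil fire, then reloads for reuse.
; Interaction, or a server-detected kick, activates it and records the user's controller, which becomes the fire's instigator.
; A replicated State's OnRep drives the idle, pour and recover cycle, toggling interactability and playing animations, sounds and particles.
; The authority advances State after each delay, with reload animation rate scaled to ReloadTime.
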(event Custom|ReleaseOil
  (bind _oil (Variables|Default|GetOil))
  (Components|Animation|PlayAnimation (Variables|Default|GetSkeletalMeshComponent) "/Game/Mordhau/Assets/SiegeEngines/OilKettle/Kettle_Tip.Kettle_Tip" false)
  (Components|Activation|Activate _oil false)
  (Audio|Components|Audio|Play (Variables|Default|GetSC_CauldronPour) 0.0)
  (Utilities|FlowControl|Delay (Variables|Default|GetSpawnFireTime))
  (bind _returnvalue (Game|SpawnActorfromClass "/Game/Mordhau/Blueprints/Fields/BP_OilFire.BP_OilFire_C" (Transformation|GetWorldTransform (Variables|Default|GetFire)) "Undefined" 0 0))
  (Variables|/Game/Mordhau/Blueprints/Fields/BP_MasterField.BP_MasterField_C|SetInstigatorController _returnvalue (Variables|Default|GetLastUserController))
  (Audio|Components|Audio|Play (Variables|Default|GetCauldronSplash) 0.0)
  (Components|Activation|Activate (Variables|Default|GetP_OilSplash) false)
  (Components|Activation|Deactivate _oil)
  (Networking|SwitchHasAuthority
    (:Authority
      (Variables|Default|SetState 2))))

(event Custom|Recover
  (bind _skeletalmeshcomponent (Variables|Default|GetSkeletalMeshComponent))
  (bind _reloadtime (Variables|Default|GetReloadTime))
  (Components|Animation|PlayAnimation _skeletalmeshcomponent "/Game/Mordhau/Assets/SiegeEngines/OilKettle/Kettle_Reload.Kettle_Reload" false)
  (Components|Timeline|SetPlayRate _skeletalmeshcomponent (/ 1.0 _reloadtime))
  (Utilities|FlowControl|Delay _reloadtime)
  (Audio|Components|Audio|Play (Variables|Default|GetCauldronReload) 0.0)
  (Networking|SwitchHasAuthority
    (:Authority
      (Variables|Default|SetState 0))))

(event Custom|Idle
  (Components|Animation|SetAnimation (Variables|Default|GetSkeletalMeshComponent) 0))

(event Custom|Activate
  (params (Char :type Mordhau%20Character%20Object%20Reference))
  (Utilities|IsValid Char
    (:Is%20Valid
      (bind _asplayer_controller (Utilities|Casting|CastToPlayerController (Pawn|GetController Char)))
      (Variables|Default|SetLastUserController _asplayer_controller)
      (Variables|Default|SetState 1))))

(event EventBeginPlay
  (|CallParentFunction) ; This node is disabled and will not be called.\nDrag off pins to build functionality.
)

(event Collision|EventActorBeginOverlap
  (params (OtherActor :type Actor%20Object%20Reference))
  (|CallParentFunction OtherActor) ; This node is disabled and will not be called.\nDrag off pins to build functionality.
)

(event EventTick
  (params (DeltaSeconds :type Float%20%28single-precision%29))
  (|CallParentFunction DeltaSeconds) ; This node is disabled and will not be called.\nDrag off pins to build functionality.
)

(event Game|Damage|EventAnyDamage
  (params (Damage :type Float%20%28single-precision%29) (DamageType :type Damage%20Type%20Object%20Reference) (InstigatedBy :type Controller%20Object%20Reference) (DamageCauser :type Actor%20Object%20Reference))
  (Utilities|FlowControl|Sequence
    (:then_0
      (Networking|SwitchHasAuthority
        (:Authority
          (bind _asmordhau_character (Utilities|Casting|CastToMordhauCharacter DamageCauser))
          (bind _asattack_motion (Utilities|Casting|CastToAttackMotion (Class|AdvancedCharacter|GetMotion _asmordhau_character)))
          (if (and (Utilities|Enum|Equal(Enum) (Variables|/Script/Mordhau.AttackMotion|GetMove _asattack_motion) "Kick") (Variables|Default|GetbIsInteractable))
            (CallFunction|Activate _asmordhau_character)))))
    (:then_1
      (|CallParentFunction Damage DamageType InstigatedBy DamageCauser))))

(event EventOnInteractionStart
  (params (Character :type Mordhau%20Character%20Object%20Reference))
  (CallFunction|Activate Character))

(fn ConstructionScript
  (|CallParentFunction))

(fn OnRepState
  (bind _state (Variables|Default|GetState))
  (Networking|ForceNetUpdate)
  (if (== _state 0)
    (Variables|Default|SetbIsInteractable true)
    (CallFunction|Idle)
    (else
      (Variables|Default|SetbIsInteractable false)
      (if (== _state 1)
        (CallFunction|ReleaseOil)
        (elif (== _state 2)
          (CallFunction|Recover))))))