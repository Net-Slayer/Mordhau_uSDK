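; Crank-style toggle interactable that drives linked progress actors and slave cranks between lowered and raised states.
; Toggling enables Tick, which moves progress at separate raise and lower speeds, updates linked actors and sleeps on arrival.
; Cosmetic updates map progress through an optional curve to scrub the skeletal animation and animated material, with movement and stop sounds.
; Flags control interaction at either end, mid-travel interruption and automatic re-toggling.
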(event EventBeginPlay
  (bind _self self)
  (bind _animatedmaterialindex (Variables|Default|GetAnimatedMaterialIndex))
  (bind _skeletalmesh (Variables|Default|GetSkeletalMesh))
  (Utilities|FlowControl|Sequence
    (:then_0
      (if (>= _animatedmaterialindex 0)
        (bind _returnvalue (Rendering|Material|CreateDynamicMaterialInstance _skeletalmesh 1 (Rendering|Material|GetMaterial _skeletalmesh _animatedmaterialindex) "None" :!class /Script/Engine.PrimitiveComponent))
        (Variables|Default|SetAnimatedMaterial _returnvalue)))
    (:then_1
      (for _array_element (Variables|Default|GetSlaveCranks)
        (Variables|/Game/Mordhau/Blueprints/Interactables/Environment/Specific/BP_SlaveProgressDriver.BP_SlaveProgressDriver_C|SetMasterCrank _array_element _self)))
    (:then_2
      (for _array_element_2 (Variables|Default|GetTargetProgressActors)
        (Variables|/Game/Mordhau/Blueprints/Interactables/Environment/BP_BaseProgressActor.BP_BaseProgressActor_C|SetDriver _array_element_2 _self)))
    (:then_3
      (|CallParentFunction))))

(event EventOnValueToggled
  (|CallParentFunction)
  (Actor|Tick|SetActorTickEnabled true))

(event EventTick
  (params (DeltaSeconds :type Float%20%28single-precision%29))
  (bind _skeletalmesh (Variables|Default|GetSkeletalMesh))
  (bind _animatedmaterial (Variables|Default|GetAnimatedMaterial))
  (bind _curve (Variables|Default|GetCurve))
  (bind _raisespeed (Variables|Default|GetRaiseSpeed))
  (bind _lowerspeed (Variables|Default|GetLowerSpeed))
  (bind _value (Variables|Default|GetValue))
  (bind _value_2 (Variables|Default|GetValue))
  (bind _returnvalue (Math|Conversions|ToFloat(Boolean) _value_2))
  (bind _returnvalue_2 (Transformation|GetSocketLocation _skeletalmesh "Crank"))
  (Utilities|FlowControl|Sequence
    (:then_0
      (if (== (Variables|Default|GetSmoothedValue) _returnvalue)
        (Actor|Tick|SetActorTickEnabled false)
        (if (Variables|Default|GetValue)
          (Audio|PlaySoundatLocation "/Game/Mordhau/Audio/Cues/Misc/SC_Crank_StopRaised.SC_Crank_StopRaised" _returnvalue_2 "0, 0, 0" 1.0 1.0 0.0 0 0 0)
          (else
            (Audio|PlaySoundatLocation "/Game/Mordhau/Audio/Cues/Misc/SC_Crank_StopLowered.SC_Crank_StopLowered" _returnvalue_2 "0, 0, 0" 1.0 1.0 0.0 0 0 0)))
        (Utilities|IsValid (Variables|Default|GetCurrentMovementSound)
          (:Is%20Valid
            (Audio|Components|Audio|FadeOut (Variables|Default|GetCurrentMovementSound) 0.2 0.0 :!class /Script/Engine.AudioComponent)
            (Variables|Default|SetCurrentMovementSound 0)))
        (else
          (bind _output_get (Variables|Default|SetSmoothedValue (Class|MordhauUtilityLibrary|FInterpConstanttoSeparate (Variables|Default|GetSmoothedValue) _returnvalue DeltaSeconds (Variables|Default|GetRaiseSpeed) (Variables|Default|GetLowerSpeed))))
          (Networking|CanExecuteCosmeticEvents
            (:True
              (Utilities|IsValid _curve
                (:Is%20Valid
                  (Variables|Default|SetPostCurveSmoothedValue (Math|Curves|GetFloatValue _curve _output_get)))
                (:Is%20Not%20Valid
                  (Variables|Default|SetPostCurveSmoothedValue _output_get)))
              (Utilities|FlowControl|Sequence
                (:then_0
                  (Utilities|IsValid (Variables|Default|GetCurrentMovementSound)
                    (:Is%20Not%20Valid
                      (bind _returnvalue_3 (Audio|SpawnSoundatLocation "/Game/Mordhau/Audio/Cues/Misc/SC_Crank_Movement.SC_Crank_Movement" _returnvalue_2 "0, 0, 0" 1.0 1.0 0.0 0 0))
                      (bind _output_get_2 (Variables|Default|SetCurrentMovementSound _returnvalue_3))
                      (Utilities|IsValid _output_get_2
                        (:Is%20Valid
                          (Audio|Parameter|SetFloatParameter _output_get_2 "Speed" (/ (Math|Float|MapRangeClamped _returnvalue 0.0 1.0 _lowerspeed _raisespeed) (Math|Float|Min(Float) _raisespeed _lowerspeed)) :!class /Script/Engine.AudioComponent))))))
                (:then_1
                  (Components|Animation|SetPosition (Variables|Default|GetSkeletalMesh) (* (Variables|Default|GetPostCurveSmoothedValue) 0.983) true)
                  (Utilities|IsValid _animatedmaterial
                    (:Is%20Valid
                      (Rendering|Material|SetScalarParameterValue _animatedmaterial "NormalizedTime" (Variables|Default|GetPostCurveSmoothedValue) :!class /Script/Engine.MaterialInstanceDynamic))))))))))
    (:then_1
      (for _array_element (Variables|Default|GetTargetProgressActors)
        (Utilities|IsValid _array_element
          (:Is%20Valid
            (Default|ProgressUpdatedInternal _array_element (Variables|Default|GetSmoothedValue)))))
      (for _array_element_2 (Variables|Default|GetSlaveCranks)
        (Default|UpdateProgress _array_element_2 (Variables|Default|GetSmoothedValue))))
    (:then_2
      (if (and (== (Variables|Default|GetSmoothedValue) (Math|Conversions|ToFloat(Boolean) (Variables|Default|GetValue))) (or (and _value (Variables|Default|GetAutoInteractRaised)) (and (not _value) (Variables|Default|GetAutoInteractLowered))))
        (CallFunction|ToggleValue)))))

(fn ConstructionScript
  (|CallParentFunction))

(fn CanInteract
  (params (Character :type Mordhau%20Character%20Object%20Reference))
  (bind _value (Variables|Default|GetValue))
  (bind _returnvalue (not _value))
  (if (== (Variables|Default|GetSmoothedValue) (Math|Conversions|ToFloat(Boolean) _value))
    (if (or (and (Variables|Default|GetPreventInteractRaised) _value) (and (Variables|Default|GetPreventInteractLowered) _returnvalue))
      _
      (else
        (return (|CallParentFunction Character))))
    (elif (or (and _value (Variables|Default|GetCanInterruptRaising)) (and _returnvalue (Variables|Default|GetCanInterruptLowering)))
      (return (|CallParentFunction Character))
      (else
        _)))
  (return false))