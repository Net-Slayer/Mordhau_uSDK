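; BP_FLFortification is a team-owned fortification with replicated health and a status widget.
; On BeginPlay it tints a configured mesh material slot with the owning team's color from the game state, via a dynamic material instance.
; The construction script restricts the widget to the owning team's viewers when a team is set.
; Health replication changes toggle the widget's visibility override around a disappear-health threshold.
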(event EventBeginPlay
  (bind _owningteam (Variables|Default|GetOwningTeam))
  (|CallParentFunction)
  (if (and (>= (Variables|Default|GetMaterialIndexForColor) 0) (or (== _owningteam 0) (== _owningteam 1)))
    (bind _returnvalue (Rendering|Material|CreateDynamicMaterialInstance (Variables|Default|GetStaticMesh) (Variables|Default|GetMaterialIndexForColor) 0 "None" :!class /Script/Engine.PrimitiveComponent))
    (bind _asmordhau_game_state (Utilities|Casting|CastToMordhauGameState (Game|GetGameState)))
    (bind _returnvalue_2 (Class|MordhauGameState|GetTeamColor _asmordhau_game_state (Math|Conversions|ToInteger(Byte) (Variables|Default|GetOwningTeam))))
    (Rendering|Material|SetVectorParameterValue _returnvalue "ColorA" _returnvalue_2 :!class /Script/Engine.MaterialInstanceDynamic)))

(event EventOnReplicatedHealthChanged
  (bind _mordhauwidget (Variables|Default|GetMordhauWidget))
  (|CallParentFunction)
  (if (>= (Variables|Default|GetReplicatedHealth) (Variables|Default|GetWidgetDisappearHealth))
    (Variables|/Script/Mordhau.MordhauWidgetComponent|SetOverrideVisible _mordhauwidget 0)
    (else
      (Variables|/Script/Mordhau.MordhauWidgetComponent|SetOverrideVisible _mordhauwidget -1))))

(fn ConstructionScript
  (bind _owningteam (Variables|Default|GetOwningTeam))
  (bind _mordhauwidget (Variables|Default|GetMordhauWidget))
  (|CallParentFunction)
  (if (!= _owningteam 255)
    (Variables|/Script/Mordhau.MordhauWidgetComponent|SetViewTargetTeamRestriction _mordhauwidget (Math|Conversions|ToInteger(Byte) _owningteam))
    (Variables|/Script/Mordhau.MordhauWidgetComponent|SetbUsesViewTargetTeamRestriction _mordhauwidget true)))