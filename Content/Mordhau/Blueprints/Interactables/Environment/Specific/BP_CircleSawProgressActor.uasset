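; An environmental circular saw hazard that deals lethal damage to whatever touches its kill box.
; On BeginPlay the Sawblade component loops its spin animation.
; KillBox overlaps deal massive damage to living AdvancedCharacters through MordhauTakeDamage, with the saw as source and agent, and to BP_DestroyableActors through standard ApplyDamage.
; The Blueprint itself contains no movement or progress logic beyond calls to its parent.
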(event OnComponentBeginOverlap(KillBox)
  (params (OverlappedComponent :type Primitive%20Component%20Object%20Reference) (OtherActor :type Actor%20Object%20Reference) (OtherComp :type Primitive%20Component%20Object%20Reference) (OtherBodyIndex :type Integer) (bFromSweep :type Boolean) (SweepResult :type Hit%20Result%20Structure%20%28by%20ref%29))
  (bind _self self)
  (bind _asadvanced_character (Utilities|Casting|CastToAdvancedCharacter OtherActor)
    (:then
      (if (not (Class|AdvancedCharacter|GetIsDead _asadvanced_character))
        (Class|AdvancedCharacter|MordhauTakeDamage _asadvanced_character 9999.0 SweepResult "Generic" 0 _self _self)))
    (:CastFailed
      (bind _asbp_destroyable_actor (Utilities|Casting|CastToBP_DestroyableActor OtherActor))
      (Game|Damage|ApplyDamage _asbp_destroyable_actor 9999.0 0 _self))))

(event EventBeginPlay
  (|CallParentFunction)
  (Components|Animation|PlayAnimation (Variables|Default|GetSawblade) "/Game/Mordhau/Assets/Environment/Props/SmallProps/StaticMeshes/Sawblade/SawSpin.SawSpin" true))

(event Collision|EventActorBeginOverlap
  (params (OtherActor :type Actor%20Object%20Reference))
  (|CallParentFunction OtherActor) ; This node is disabled and will not be called.\nDrag off pins to build functionality.
)

(fn ConstructionScript
  (|CallParentFunction))