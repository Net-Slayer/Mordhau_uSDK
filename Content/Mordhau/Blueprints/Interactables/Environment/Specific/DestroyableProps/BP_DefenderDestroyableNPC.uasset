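; Destroyable blue footsoldier NPC that acts as a pusher, apparently for a wagon, and respawns after being killed.
; Replicated health drops play a montage; death clears IsPushing and ragdolls the mesh.
; After a delay it restores health, snaps the mesh back to its attachment point and resumes pushing.
; Each tick feeds the mesh's frame-to-frame movement into the anim instance as WagonSpeed, without scaling by delta time.
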(event EventBeginPlay
  (|CallParentFunction) ; This node is disabled and will not be called.\nDrag off pins to build functionality.
)

(event Collision|EventActorBeginOverlap
  (params (OtherActor :type Actor%20Object%20Reference))
  (|CallParentFunction OtherActor) ; This node is disabled and will not be called.\nDrag off pins to build functionality.
)

(event EventTick
  (params (DeltaSeconds :type Float%20%28single-precision%29))
  (|CallParentFunction DeltaSeconds)
  (CallFunction|UpdatePusherAnimation))

(event EventOnReplicatedHealthChanged
  (bind _self self)
  (bind _sk_footsoldierblue (Variables|Default|GetSK_FootsoldierBlue))
  (bind _sk_footsoldierblue_2 (Variables|Default|GetSK_FootsoldierBlue))
  (bind _sk_footsoldierblue_3 (Variables|Default|GetSK_FootsoldierBlue))
  (if (>= (Variables|Default|GetHealth self) 1.0)
    (if (> (Variables|Default|GetLastReplicatedHealth) (Variables|Default|GetReplicatedHealth))
      (Utilities|Casting|CastTo (Components|SkeletalMesh|GetAnimInstance _sk_footsoldierblue))
      (Animation|Montage|PlayMontage _sk_footsoldierblue 0))
    (else
      (Variables|Default|SetIsPushing false)
      (Development|PrintString "Im dead, Oouchie")
      (Collision|SetCollisionProfileName _sk_footsoldierblue_3 "Ragdoll" :!class /Script/Engine.PrimitiveComponent)
      (Class|SkeletalMeshComponent|SetAllBodiesSimulatePhysics _sk_footsoldierblue_3 true)
      (Class|PrimitiveComponent|AddForceatLocation _sk_footsoldierblue_3 "0, 0, 0" "0, 0, 0" "None")
      (Utilities|FlowControl|Delay 3e+01)
      (Development|PrintString "Im alive")
      (Variables|Default|SetHealth _self 1e+02)
      (Default|UpdateReplicatedHealth _self)
      (Variables|Default|SetIsPushing true)
      (Class|SkeletalMeshComponent|SetAllBodiesSimulatePhysics _sk_footsoldierblue_2 false)
      (Transformation|AttachComponentToComponent _sk_footsoldierblue_2 (Variables|Default|GetAttachmentPoint) "None" "SnapToTarget" "SnapToTarget" "SnapToTarget" true)
      (Class|SkeletalMeshComponent|ResetAnimInstanceDynamics _sk_footsoldierblue_2 "ResetPhysics")
      (Variables|Default|SetOldPusherLocation (Transformation|GetWorldLocation (Variables|Default|GetSK_FootsoldierBlue))))))

(fn ConstructionScript
  (|CallParentFunction))

(fn UpdatePusherAnimation
  (bind _sk_footsoldierblue (Variables|Default|GetSK_FootsoldierBlue))
  (bind _returnvalue (Transformation|GetWorldLocation _sk_footsoldierblue))
  (bind _asab_pushing_cart_npc (Utilities|Casting|CastTo (Components|SkeletalMesh|GetAnimInstance _sk_footsoldierblue)))
  (Variables|Default|SetWagonSpeed _asab_pushing_cart_npc (* (Math|Vector|VectorLength (- _returnvalue (Variables|Default|GetOldPusherLocation))) 8e+01))
  (Variables|Default|SetOldPusherLocation _returnvalue))