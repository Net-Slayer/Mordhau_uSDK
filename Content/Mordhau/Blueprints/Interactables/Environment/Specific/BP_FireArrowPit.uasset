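; BP_FireArrowPit is an environmental fire pit that lets nearby ranged weapons shoot flaming projectiles.
; On the server, a looping half-second timer scans living AdvancedCharacter actors overlapping its Area.
; Characters holding a loaded BP_Bow get fire arrows enabled, while ballistas, deployable ballistas and catapults in state 0 get their Fire flag set.
; The pit only switches fire on and never clears it.
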(event Custom|GiveBuffs
  (bind _output_get (Variables|Default|SetOverlappingInternal (Collision|GetOverlappingActors (Variables|Default|GetArea) "/Script/Mordhau.AdvancedCharacter" :!class /Script/Engine.PrimitiveComponent)))
  (for _array_element _output_get
    (bind _asadvanced_character (Utilities|Casting|CastToAdvancedCharacter _array_element))
    (if (not (Class|AdvancedCharacter|GetIsDead _asadvanced_character))
      (bind _asmordhau_character (Utilities|Casting|CastToMordhauCharacter _array_element)
        (:then
          (bind _asbp_bow (Utilities|Casting|CastToBP_Bow (Variables|/Script/Mordhau.MordhauCharacter|GetLeftHandEquipment _asmordhau_character)))
          (if (Variables|/Script/Mordhau.MordhauEquipment|GetbIsLoaded _asbp_bow)
            (Default|SetUseFireArrows _asbp_bow true)))
        (:CastFailed
          (bind _asbp_ballista (Utilities|Casting|CastToBP_Ballista _array_element)
            (:then
              (if (and (not (Variables|/Game/Mordhau/Blueprints/Interactables/SiegeEngines/BP_Ballista.BP_Ballista_C|GetFire _asbp_ballista)) (== (Variables|/Game/Mordhau/Blueprints/Interactables/SiegeEngines/BP_Ballista.BP_Ballista_C|GetState _asbp_ballista) 0))
                (Variables|/Game/Mordhau/Blueprints/Interactables/SiegeEngines/BP_Ballista.BP_Ballista_C|SetFire _asbp_ballista true)))
            (:CastFailed
              (bind _asbp_deployable_ballista (Utilities|Casting|CastToBP_DeployableBallista _array_element)
                (:then
                  (if (and (not (Variables|/Game/Mordhau/Blueprints/Interactables/SiegeEngines/BP_DeployableBallista.BP_DeployableBallista_C|GetFire _asbp_deployable_ballista)) (== (Variables|/Game/Mordhau/Blueprints/Interactables/SiegeEngines/BP_DeployableBallista.BP_DeployableBallista_C|GetState _asbp_deployable_ballista) 0))
                    (Variables|/Game/Mordhau/Blueprints/Interactables/SiegeEngines/BP_DeployableBallista.BP_DeployableBallista_C|SetFire _asbp_deployable_ballista true)))
                (:CastFailed
                  (bind _asbp_catapult (Utilities|Casting|CastToBP_Catapult _array_element))
                  (if (and (not (Variables|/Game/Mordhau/Blueprints/Interactables/SiegeEngines/BP_Catapult.BP_Catapult_C|GetFire _asbp_catapult)) (== (Variables|/Game/Mordhau/Blueprints/Interactables/SiegeEngines/BP_Catapult.BP_Catapult_C|GetState _asbp_catapult) 0))
                    (Variables|/Game/Mordhau/Blueprints/Interactables/SiegeEngines/BP_Catapult.BP_Catapult_C|SetFire _asbp_catapult true)))))))))))

(event EventBeginPlay
  (|CallParentFunction)
  (Networking|SwitchHasAuthority
    (:Authority
      (Utilities|Time|SetTimerbyEvent (delegate Custom|GiveBuffs) 0.5 true))))

(event Collision|EventActorBeginOverlap
  (params (OtherActor :type Actor%20Object%20Reference))
  (|CallParentFunction OtherActor) ; This node is disabled and will not be called.\nDrag off pins to build functionality.
)

(event EventTick
  (params (DeltaSeconds :type Float%20%28single-precision%29))
  (|CallParentFunction DeltaSeconds) ; This node is disabled and will not be called.\nDrag off pins to build functionality.
)

(fn ConstructionScript
  (|CallParentFunction))