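; Interactable rock basket that tips over when used or kicked by a player, dumping a volley of rock projectiles, then reloads.
; A replicated State drives the idle, release and recover cycle through its OnRep, allowing interaction only when idle.
; Release plays the tip animation, hides the pile and has the server fire six staggered, randomly scattered projectiles credited to the last user.
; Recover plays the reload animation, restores the pile and returns to idle.
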(event Custom|Release
  (bind _rockposition (Variables|Default|GetRockPosition))
  (bind _returnvalue (Transformation|GetWorldTransform _rockposition))
  (Components|Animation|PlayAnimation (Variables|Default|GetSkeletalMeshComponent) "/Game/Mordhau/Assets/SiegeEngines/WickerBasket/WickerBasket_TipOver.WickerBasket_TipOver" false)
  (Utilities|FlowControl|Delay (Variables|Default|GetSpawnRocksTime))
  (Development|SetHiddeninGame (Variables|Default|GetRockPile) true false)
  (CallFunction|SpawnProjectile _returnvalue)
  (Utilities|FlowControl|Delay (Math|Random|RandomFloatinRange 0.11 0.17))
  (CallFunction|SpawnProjectile _returnvalue)
  (Utilities|FlowControl|Delay (Math|Random|RandomFloatinRange 0.11 0.17))
  (CallFunction|SpawnProjectile _returnvalue)
  (Utilities|FlowControl|Delay (Math|Random|RandomFloatinRange 0.11 0.17))
  (CallFunction|SpawnProjectile _returnvalue)
  (Utilities|FlowControl|Delay (Math|Random|RandomFloatinRange 0.11 0.17))
  (CallFunction|SpawnProjectile _returnvalue)
  (Utilities|FlowControl|Delay (Math|Random|RandomFloatinRange 0.11 0.17))
  (CallFunction|SpawnProjectile _returnvalue)
  (Utilities|FlowControl|Delay (Math|Random|RandomFloatinRange 0.11 0.17))
  (Utilities|FlowControl|Delay 1.0)
  (Networking|SwitchHasAuthority
    (:Authority
      (Variables|Default|SetState 2))))

(event Custom|Recover
  (Components|Animation|PlayAnimation (Variables|Default|GetSkeletalMeshComponent) "/Game/Mordhau/Assets/SiegeEngines/WickerBasket/WickerBasket_Reload.WickerBasket_Reload" false)
  (Utilities|FlowControl|Delay 1.6)
  (Utilities|FlowControl|Delay (- (Variables|Default|GetReloadTime) 1.8))
  (Development|SetHiddeninGame (Variables|Default|GetRockPile) false false)
  (Audio|PlaySoundatLocation 0 (Transformation|GetWorldLocation (Variables|Default|GetRockPile)) "0, 0, 0" 1.0 1.0 0.0 0 0 0)
  (Networking|SwitchHasAuthority
    (:Authority
      (Variables|Default|SetState 0))))

(event Custom|Idle
  (Components|Animation|SetAnimation (Variables|Default|GetSkeletalMeshComponent) 0)
  (Networking|SwitchHasAuthority
    (:Remote
      (Development|SetHiddeninGame (Variables|Default|GetRockPile) false false))))

(event Custom|Activate
  (params (Char :type Mordhau%20Character%20Object%20Reference))
  (Utilities|IsValid Char
    (:Is%20Valid
      (bind _asplayer_controller (Utilities|Casting|CastToPlayerController (Pawn|GetController Char)))
      (Variables|Default|SetLastUserController _asplayer_controller)
      (Variables|Default|SetState 1))))

(event Collision|EventActorBeginOverlap
  (params (OtherActor :type Actor%20Object%20Reference))
  (|CallParentFunction OtherActor) ; This node is disabled and will not be called.\nDrag off pins to build functionality.
)

(event Game|Damage|EventAnyDamage
  (params (Damage :type Float%20%28single-precision%29) (DamageType :type Damage%20Type%20Object%20Reference) (InstigatedBy :type Controller%20Object%20Reference) (DamageCauser :type Actor%20Object%20Reference))
  (Utilities|FlowControl|Sequence
    (:then_0
      (Networking|SwitchHasAuthority
        (:Authority
          (bind _asmordhau_character (Utilities|Casting|CastToMordhauCharacter DamageCauser))
          (bind _asattack_motion (Utilities|Casting|CastToAttackMotion (Class|AdvancedCharacter|GetMotion _asmordhau_character)))
          (if (and (Utilities|Enum|Equal(Enum) (Variables|/Script/Mordhau.AttackMotion|GetMove _asattack_motion) "Kick") (Variables|Default|GetbIsInteractable))
            (CallFunction|Activate _asmordhau_character)))))
    (:then_1
      (|CallParentFunction Damage DamageType InstigatedBy DamageCauser))))

(event EventOnInteractionStart
  (params (Character :type Mordhau%20Character%20Object%20Reference))
  (CallFunction|Activate Character))

(fn ConstructionScript
  (|CallParentFunction)
  (Transformation|AttachComponentToComponent (Variables|Default|GetRockPile) (Variables|Default|GetSkeletalMeshComponent) "Joint1" "KeepRelative" "KeepRelative" "KeepRelative" true))

(fn OnRepState
  (bind _state (Variables|Default|GetState))
  (Networking|ForceNetUpdate)
  (if (== _state 0)
    (Variables|Default|SetbIsInteractable true)
    (CallFunction|Idle)
    (else
      (Variables|Default|SetbIsInteractable false)
      (if (== _state 1)
        (CallFunction|Release)
        (elif (== _state 2)
          (CallFunction|Recover))))))

(fn SpawnProjectile
  (params (Projectile%20Transform%20Origin :type Transform))
  (Networking|SwitchHasAuthority
    (:Authority
      (bind _changed_transform (CallFunction|RandomizeRotation 4e+01 -4e+01 Projectile%20Transform%20Origin 25.0 -25.0))
      (bind _returnvalue (Game|SpawnActorfromClass "/Game/Mordhau/Blueprints/Equipment/Misc/BP_BasketRockProjectile.BP_BasketRockProjectile_C" _changed_transform "Undefined" 0 0))
      (Class|MordhauProjectile|InitializeProjectile _returnvalue (Variables|Default|GetLastUserController) false)
      (Class|MordhauProjectile|Fire _returnvalue))))

(fn RandomizeRotation
  (params (Top%20Span%20Rotation :type Float%20%28single-precision%29) (Bottom%20Span%20Rotation :type Float%20%28single-precision%29) (Original%20Transform :type Transform) (Top%20Span%20Location :type Float%20%28single-precision%29) (bottom%20Span%20Location :type Float%20%28single-precision%29))
  (bind (_location _rotation _scale) (Math|Transform|BreakTransform Original%20Transform))
  (bind (_roll _pitch _yaw) (Math|Rotator|BreakRotator _rotation))
  (bind (_x _y _z) (Math|Vector|BreakVector _location))
  (return (Math|Transform|MakeTransform (Math|Vector|MakeVector _x (+ (Math|Random|RandomFloatinRange Top%20Span%20Location bottom%20Span%20Location) _y) (+ (Math|Random|RandomFloatinRange Top%20Span%20Location bottom%20Span%20Location) _z)) (Math|Rotator|MakeRotator (+ _roll (Math|Random|RandomFloatinRange Top%20Span%20Rotation Bottom%20Span%20Rotation)) (+ _pitch (Math|Random|RandomFloatinRange Top%20Span%20Rotation Bottom%20Span%20Rotation)) (+ _yaw (Math|Random|RandomFloatinRange Top%20Span%20Rotation Bottom%20Span%20Rotation))) _scale)))