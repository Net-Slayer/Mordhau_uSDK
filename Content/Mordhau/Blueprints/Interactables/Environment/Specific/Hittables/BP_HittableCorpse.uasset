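; BP_HittableCorpse is a hittable environment corpse that animates in reaction to being hit.
; It extends a parent hittable's OnHit, playing a one-shot animation on its skeletal mesh, then switching to a looping animation after a short delay.
; The delay is retriggerable, so repeated hits postpone the return to the loop.
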(event EventBeginPlay
  (|CallParentFunction))

(event Collision|EventActorBeginOverlap
  (params (OtherActor :type Actor%20Object%20Reference))
  (|CallParentFunction OtherActor) ; This node is disabled and will not be called.\nDrag off pins to build functionality.
)

(event EventTick
  (params (DeltaSeconds :type Float%20%28single-precision%29))
  (|CallParentFunction DeltaSeconds) ; This node is disabled and will not be called.\nDrag off pins to build functionality.
)

(event EventOnHit
  (bind _skeletalmesh (Variables|Default|GetSkeletalMesh))
  (|CallParentFunction)
  (Components|Animation|PlayAnimation _skeletalmesh 0 false)
  (Utilities|FlowControl|RetriggerableDelay 1.4)
  (Components|Animation|PlayAnimation _skeletalmesh 0 true))

(fn ConstructionScript
  (|CallParentFunction))