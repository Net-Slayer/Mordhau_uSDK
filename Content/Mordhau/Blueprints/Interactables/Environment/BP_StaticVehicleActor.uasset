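; BP_StaticVehicleActor is an interactable static vehicle that puts an interacting character into a drivable vehicle.
; On interaction start it spawns CharacterClass at the VehicleSpawn transform with unit scale, always ignoring collision, links itself as that actor's StaticVehicleActor and calls StartDriving with the character.
; CanInteract refuses a valid character while VehicleCharacters is non-empty, otherwise deferring to the parent check.
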(event EventBeginPlay
  (|CallParentFunction) ; This node is disabled and will not be called.\nDrag off pins to build functionality.
)

(event Collision|EventActorBeginOverlap
  (params (OtherActor :type Actor%20Object%20Reference))
  (|CallParentFunction OtherActor) ; This node is disabled and will not be called.\nDrag off pins to build functionality.
)

(event EventTick
  (params (DeltaSeconds :type Float%20%28single-precision%29))
  (|CallParentFunction DeltaSeconds) ; This node is disabled and will not be called.\nDrag off pins to build functionality.
)

(event EventOnInteractionStart
  (params (Character :type Mordhau%20Character%20Object%20Reference))
  (bind _vehiclespawn (Variables|Default|GetVehicleSpawn))
  (bind _returnvalue (Transformation|GetWorldTransform _vehiclespawn))
  (bind (_location _rotation) (Math|Transform|BreakTransform _returnvalue))
  (bind _returnvalue_2 (Game|SpawnActorfromClass (Variables|Default|GetCharacterClass) (Math|Transform|MakeTransform _location _rotation) "AlwaysSpawn" 0 0))
  (Variables|/Game/Mordhau/Blueprints/Interactables/Environment/BP_StaticVehicleCharacter.BP_StaticVehicleCharacter_C|SetStaticVehicleActor _returnvalue_2 self)
  (Class|MordhauVehicle|StartDriving _returnvalue_2 Character))

(fn ConstructionScript
  (|CallParentFunction))

(fn CanInteract
  (params (Character :type Mordhau%20Character%20Object%20Reference))
  (Utilities|IsValid Character
    (:Is%20Valid
      (if (> (Utilities|Array|Length (Variables|Default|GetVehicleCharacters)) 0)
        (return false)
        (else
          _)))
    (:Is%20Not%20Valid
      _))
  (return (|CallParentFunction Character)))