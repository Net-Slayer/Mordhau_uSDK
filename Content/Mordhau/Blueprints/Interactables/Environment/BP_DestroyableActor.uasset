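; Destroyable environment actor that takes damage, can be repaired or regenerate, and awards team-based score for repairs and damage.
; Server float health is mirrored into a replicated byte, whose RepNotify swaps damage meshes, plays effects, controls regeneration and handles destruction.
; Segmented health caps repair and timer-driven regeneration.
; Mesh changes shed attached projectiles and equipment, while upgrades can destroy overlapping destroyables or teleport stuck characters out.
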(event Custom|RegenTickEvent
  (bind _regenerating (Variables|Combat|GetRegenerating))
  (bind _health (Variables|Combat|GetHealth))
  (if _regenerating
    (CallFunction|SetHealth (Math|Float|Min(Float) (+ _health (Variables|Combat|GetRegenPerTick)) (Math|Float|Max(Float) (Math|Conversions|ToFloat(Byte) (Variables|Combat|GetMaxHealthRepairableTo)) _health)))
    (if _regenerating
      (Utilities|Time|SetTimerbyEvent (delegate Custom|RegenTickEvent) (Variables|Combat|GetRegenTick)))))

(event Custom|StartRegenerating
  (Networking|SwitchHasAuthority
    (:Authority
      (Utilities|FlowControl|Sequence
        (:then_0
          (if (not (Variables|Combat|GetRegenerating))
            (Variables|Combat|SetRegenerating true)))
        (:then_1
          (Utilities|Time|SetTimerbyEvent (delegate Custom|RegenTickEvent) (Variables|Combat|GetRegenTick)))))))

(event Custom|DetachAfterShortDelay
  (Utilities|FlowControl|Delay 0.01)
  (CallFunction|DetachAttachedProjectiles))

(event Game|Damage|EventAnyDamage
  (params (Damage :type Float%20%28single-precision%29) (DamageType :type Damage%20Type%20Object%20Reference) (InstigatedBy :type Controller%20Object%20Reference) (DamageCauser :type Actor%20Object%20Reference))
  (bind _health (Variables|Combat|GetHealth))
  (if (or (>= Damage 0.0) (Variables|Combat|GetRepairable))
    (CallFunction|SetHealth (Math|Float|Min(Float) (- _health (* Damage (Variables|Combat|GetDamageFactor) (select (< Damage 0.0) (Variables|Combat|GetRepairFactor) 1.0))) (Math|Float|Max(Float) (Math|Conversions|ToFloat(Byte) (Variables|Combat|GetMaxHealthRepairableTo)) _health)) InstigatedBy)))

(event EventBeginPlay
  (Variables|Combat|SetSpawnHealth (Variables|Combat|GetHealth))
  (|CallParentFunction)
  (Utilities|FlowControl|Sequence
    (:then_0
      (Networking|SwitchHasAuthority
        (:Remote
          (Variables|/Script/Engine.PrimitiveComponent|SetbGenerateOverlapEvents (Variables|Default|GetStaticMesh) false))))
    (:then_1
      (if (Variables|Combat|GetRegenerating)
        (Utilities|FlowControl|Sequence
          (:then_0
            (Networking|SwitchHasAuthority
              (:Authority
                (Utilities|FlowControl|Delay (Variables|Combat|GetRegenStartDelay))
                (if (Variables|Combat|GetRegenerating)
                  (CallFunction|StartRegenerating)))))
          (:then_1
            (CallFunction|OnRepRegenerating)))))))

(fn ConstructionScript
  (|CallParentFunction)
  (bind _output_get (Variables|Combat|SetReplicatedHealth (Math|Conversions|ToByte(Integer) (Math|Integer|Clamp(Integer) (Math|Float|Floor (Variables|Combat|GetHealth)) 0 255))))
  (Variables|Combat|SetLastReplicatedHealth _output_get))

(fn UpdateReplicatedHealth
  (bind _output_get (LocalVariables|SetNewReplicatedHealth (Math|Conversions|ToByte(Integer) (Math|Integer|Clamp(Integer) (Math|Float|Floor (Variables|Combat|GetHealth)) 0 255))))
  (if (not (== _output_get (Variables|Combat|GetReplicatedHealth)))
    (Networking|ForceNetUpdate)
    (Variables|Combat|SetReplicatedHealth (LocalVariables|GetNewReplicatedHealth))
    (if (== (Variables|Combat|GetReplicatedHealth) 0)
      (if (Variables|Default|GetDeleteWhenDestroyed)
        (Actor|SetLifeSpan 1.0)))))

(fn OnRepReplicatedHealth
  (bind _staticmesh (Variables|Default|GetStaticMesh))
  (bind _replicatedhealth (Variables|Combat|GetReplicatedHealth))
  (bind _repairablehealthsegments (Variables|Default|GetRepairableHealthSegments))
  (bind _repairstatechangesound (Variables|Default|GetRepairStateChangeSound))
  (bind _damagestatechangesound (Variables|Default|GetDamageStateChangeSound))
  (bind _staticmesh_2 (Variables|Default|GetStaticMesh))
  (bind _damageaudioorigin (Variables|Default|GetDamageAudioOrigin))
  (bind _damagemesheshealth (Variables|Default|GetDamageMeshesHealth))
  (bind _damagemeshes (Variables|Default|GetDamageMeshes))
  (bind _staticmesh_3 (Variables|Default|GetStaticMesh))
  (bind _returnvalue (Transformation|GetWorldLocation _damageaudioorigin))
  (bind _returnvalue_2 (Math|Conversions|ToFloat(Byte) _repairablehealthsegments))
  (bind _returnvalue_3 (/ 1e+02 _returnvalue_2))
  (CallFunction|OnReplicatedHealthChanged)
  (Utilities|FlowControl|Sequence
    (:then_0
      (if (> (Variables|Default|GetRepairableHealthSegments) 1)
        (Variables|Combat|SetMaxHealthRepairableTo (Class|KismetMathLibrary|BMin (Math|Conversions|ToByte(Integer) (* (Math|Float|Ceil (/ (Math|Conversions|ToFloat(Byte) (Variables|Combat|GetReplicatedHealth)) _returnvalue_3)) (Math|Float|Ceil _returnvalue_3))) 100))))
    (:then_1
      (if (> (Utilities|Array|Length _damagemesheshealth) 0)
        (for (_array_element _array_index) _damagemesheshealth
          (if (<= (Variables|Combat|GetReplicatedHealth) _array_element)
            (LocalVariables|SetBestIdx _array_index)))
        (if (Utilities|Array|IsValidIndex _damagemeshes (LocalVariables|GetBestIdx))
          (if (!= (Variables|/Script/Engine.StaticMeshComponent|GetStaticMesh _staticmesh_3) (Utilities|Array|Get(acopy) _damagemeshes (LocalVariables|GetBestIdx)))
            (Components|StaticMesh|SetStaticMesh _staticmesh_3 (Utilities|Array|Get(acopy) _damagemeshes (LocalVariables|GetBestIdx)))
            (if (Class|MordhauUtilityLibrary|HasActorBegunPlay self)
              (Utilities|FlowControl|Sequence
                (:then_0
                  (Networking|CanExecuteCosmeticEvents
                    (:True
                      (if (> (Utilities|Time|GetGameTimeinSeconds) 3.0)
                        (CallFunction|PlayParticle)
                        (if (< (Variables|Combat|GetLastReplicatedHealth) (Variables|Combat|GetReplicatedHealth))
                          (Utilities|IsValid _repairstatechangesound
                            (:Is%20Valid
                              (Audio|PlaySoundatLocation _repairstatechangesound _returnvalue "0, 0, 0" 1.0 1.0 0.0 0 0 0)))
                          (else
                            (Utilities|IsValid _damagestatechangesound
                              (:Is%20Valid
                                (Audio|PlaySoundatLocation _damagestatechangesound _returnvalue "0, 0, 0" 1.0 1.0 0.0 0 0 0)))))))))
                (:then_1
                  (Networking|SwitchHasAuthority
                    (:Authority
                      (Utilities|FlowControl|Sequence
                        (:then_0
                          (CallFunction|DetachAfterShortDelay) ; Usually weps that did the damage will attach AFTER dealing damage, this waits for that..
                        )
                        (:then_1
                          (if (and (< (Variables|Combat|GetLastReplicatedHealth) (Variables|Combat|GetReplicatedHealth)) (Variables|Default|GetPerformsUnstuckProcess))
                            (bind _outactors (Collision|ComponentOverlapActors _staticmesh_2 (Transformation|GetWorldTransform _staticmesh_2) (Utilities|Array|MakeArray "ObjectTypeQuery1" "ObjectTypeQuery3" "ObjectTypeQuery5") 0 (Utilities|Array|MakeArray self)))
                            (for _array_element_2 _outactors
                              (bind _asbp_destroyable_actor (Utilities|Casting|CastToBP_DestroyableActor _array_element_2)
                                (:then
                                  (if (Variables|Default|GetDestroysOtherWhenUpgrading)
                                    (Game|Damage|ApplyDamage _asbp_destroyable_actor 1e+10 0 0)))
                                (:CastFailed
                                  (bind _asmordhau_character (Utilities|Casting|CastToMordhauCharacter _array_element_2)
                                    (:then
                                      (Utilities|IsValid (Variables|/Script/Mordhau.MordhauCharacter|GetCurrentVehicle _asmordhau_character)
                                        (:Is%20Not%20Valid
                                          _)))
                                    (:CastFailed
                                      _))
                                  (bind _asadvanced_character (Utilities|Casting|CastToAdvancedCharacter _array_element_2))
                                  (bind (_outhit _returnvalue_4) (Class|KismetSystemLibrary|CapsuleTraceSingleforObjects (+ (Transformation|GetActorLocation _asadvanced_character) "0, 0,500.000000") (Transformation|GetActorLocation _asadvanced_character) (* (Components|Capsule|GetScaledCapsuleRadius (Variables|/Script/Engine.Character|GetCapsuleComponent _asadvanced_character)) 0.8) (* (Components|Capsule|GetScaledCapsuleHalfHeight (Variables|/Script/Engine.Character|GetCapsuleComponent _asadvanced_character)) 0.9) (Utilities|Array|MakeArray "ObjectTypeQuery1") false 0 "None" false))
                                  (if _returnvalue_4
                                    (if (== (.HitActor (Collision|BreakHitResult _outhit)) self)
                                      (Transformation|Teleport _asadvanced_character (+ (.OutPointOnBody (Collision|GetClosestPointonCollision (Variables|Default|GetStaticMesh) (+ (Transformation|GetActorLocation _asadvanced_character) "0, 0,100.000000") "None")) (Math|Conversions|ToVector(Float) (Components|Capsule|GetUnscaledCapsuleHalfHeight (Variables|/Script/Engine.Character|GetCapsuleComponent _asadvanced_character)))) (Transformation|GetActorRotation _asadvanced_character)))))))))))))))))))
    (:then_2
      (Networking|CanExecuteCosmeticEvents
        (:True
          (if (Class|MordhauUtilityLibrary|HasActorBegunPlay self)
            (Rendering|Material|SetScalarParameterValueonMaterials _staticmesh "HitTime" (Utilities|Time|GetTimeSeconds))
            (Rendering|Material|SetScalarParameterValueonMaterials _staticmesh "HitDamage" (- (Math|Conversions|ToFloat(Byte) (Variables|Combat|GetLastReplicatedHealth)) (Math|Conversions|ToFloat(Byte) (Variables|Combat|GetReplicatedHealth))))))))
    (:then_3
      (Networking|SwitchHasAuthority
        (:Authority
          (if (or (and (Variables|Combat|GetStopRegeneratingOnDamage) (< _replicatedhealth (Variables|Combat|GetLastReplicatedHealth))) (>= _replicatedhealth (Variables|Combat|GetMaxHealthRepairableTo)))
            (CallFunction|StopRegenerating)
            (elif (and (Variables|Default|GetAutoResumeRegenerating) (< _replicatedhealth (Variables|Combat|GetMaxHealthRepairableTo)))
              (CallFunction|StartRegenerating))))))
    (:then_4
      (Variables|Combat|SetLastReplicatedHealth _replicatedhealth)
      (if (== (Variables|Combat|GetReplicatedHealth) 0)
        (Utilities|FlowControl|Sequence
          (:then_0
            (Networking|SwitchHasAuthority
              (:Authority
                (CallFunction|StopRegenerating))))
          (:then_1
            (if (Variables|Default|GetDeleteWhenDestroyed)
              (CallFunction|PlayParticle)
              (Development|SetHiddeninGame (Variables|Default|GetStaticMesh) true false)
              (Collision|SetActorEnableCollision false :!label _label)
              (elif (Variables|Default|GetDisableCollisionWhenDestroyed)
                (goto _label)))))))))

(fn SetHealth
  (params (NewHealth :type Float%20%28single-precision%29) (Instigator :type Controller%20Object%20Reference))
  (bind _owningteam (Variables|Default|GetOwningTeam))
  (Variables|Default|SetLastHealthChangeInstigator Instigator)
  (bind _output_get (LocalVariables|SetNewHealthAdjusted (Math|Float|Clamp(Float) NewHealth 0.0 255.0)))
  (Utilities|FlowControl|Sequence
    (:then_0
      (if (!= _owningteam 255)
        (bind _asmordhau_player_controller (Utilities|Casting|CastToMordhauPlayerController Instigator))
        (bind _asmordhau_player_state (Utilities|Casting|CastToMordhauPlayerState (Variables|/Script/Engine.Controller|GetPlayerState _asmordhau_player_controller)))
        (Utilities|FlowControl|Sequence
          (:then_0
            (if (== (Variables|/Script/Mordhau.MordhauPlayerState|GetTeam _asmordhau_player_state) (Math|Conversions|ToInteger(Byte) _owningteam))
              (if (< (- (Variables|Combat|GetHealth) (LocalVariables|GetNewHealthAdjusted)) 0.0)
                (LocalVariables|SetScoreAward (Math|Integer|Min(Integer) (Math|Float|Truncate (Math|Float|Absolute(Float) (- (Variables|Combat|GetHealth) (LocalVariables|GetNewHealthAdjusted)))) (Variables|Default|GetRepairScoreMax)))
                (LocalVariables|SetScoreType "Repair")
                (else
                  (return)))
              (elif (< (- (Variables|Combat|GetHealth) (LocalVariables|GetNewHealthAdjusted)) 0.0)
                (return)
                (else
                  (LocalVariables|SetScoreAward (Math|Integer|Min(Integer) (Math|Float|Truncate (- (Variables|Combat|GetHealth) (LocalVariables|GetNewHealthAdjusted))) (Variables|Default|GetDamageScoreMax)))
                  (LocalVariables|SetScoreType "OtherDamage")))))
          (:then_1
            (if (!= (LocalVariables|GetScoreAward) 0)
              (Class|MordhauPlayerController|GiveClientScoreBP _asmordhau_player_controller (LocalVariables|GetScoreType) (LocalVariables|GetScoreAward)))))))
    (:then_1
      (Variables|Combat|SetHealth _output_get)
      (CallFunction|UpdateReplicatedHealth))))

(fn PlayParticle
  (bind _damagemeshchangeparticle (Variables|Default|GetDamageMeshChangeParticle))
  (bind _damageparticletransform (Variables|Default|GetDamageParticleTransform))
  (Networking|CanExecuteCosmeticEvents
    (:True
      (if (Class|MordhauUtilityLibrary|HasActorBegunPlay self)
        (Utilities|IsValid _damagemeshchangeparticle
          (:Is%20Valid
            (bind _returnvalue (Effects|SpawnEmitteratLocation _damagemeshchangeparticle (Transformation|GetWorldLocation _damageparticletransform) (Transformation|GetWorldRotation _damageparticletransform)))
            (Utilities|IsValid _returnvalue
              (:Is%20Valid
                (Class|PrimitiveComponent|SetSingleSampleShadowfromStationaryLights _returnvalue true)))))))))

(fn StopRegenerating
  (if (Variables|Combat|GetRegenerating)
    (Variables|Combat|SetRegenerating false)))

(fn OnReplicatedHealthChanged)

(fn OnRepRegenerating
  (Networking|CanExecuteCosmeticEvents
    (:True
      (if (Variables|Combat|GetRegenerating)
        (Utilities|IsValid (Variables|Default|GetCurrentRegeneratingSound)
          (:Is%20Not%20Valid
            (Utilities|IsValid (Variables|Default|GetRegeneratingSoundCue)
              (:Is%20Valid
                (bind _returnvalue (Audio|SpawnSoundAttached (Variables|Default|GetRegeneratingSoundCue) (Variables|Default|GetDamageParticleTransform) "None" "0, 0, 0" "0, 0, 0" "SnapToTarget" true 1.0 1.0 0.0 0 0))
                (Variables|Default|SetCurrentRegeneratingSound _returnvalue)))))
        (else
          (Utilities|IsValid (Variables|Default|GetCurrentRegeneratingSound)
            (:Is%20Valid
              (Audio|Components|Audio|FadeOut (Variables|Default|GetCurrentRegeneratingSound) 0.4 0.0 :!class /Script/Engine.AudioComponent)
              (Variables|Default|SetCurrentRegeneratingSound 0))))))))

(fn DetachAttachedProjectiles
  (bind _output_get (LocalVariables|SetAttached (Actor|GetAttachedActors)))
  (for _array_element _output_get
    (bind _asmordhau_projectile (Utilities|Casting|CastToMordhauProjectile _array_element)
      (:then
        (Actor|DestroyActor _asmordhau_projectile))
      (:CastFailed
        (bind _asmordhau_equipment (Utilities|Casting|CastToMordhauEquipment _array_element))
        (Transformation|DetachFromActor _asmordhau_equipment "KeepWorld" "KeepWorld" "KeepWorld")))))