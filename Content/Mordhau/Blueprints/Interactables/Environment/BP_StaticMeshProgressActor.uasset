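; BP_StaticMeshProgressActor is an environment interactable that moves a static mesh between two poses as a progress value changes.
; BeginPlay stores the mesh's starting relative transform, and ProgressUpdated interpolates from it to TargetStaticMeshTransform using Progress as the alpha.
; With UseAbsoluteRotation set, rotation is lerped per axis as a vector toward AbsoluteRotation, bypassing the transform lerp's rotation, while location and scale still follow the target transform.
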(event EventBeginPlay
  (Variables|Default|SetStartStaticMeshTransform (Transformation|GetRelativeTransform (Variables|Default|GetStaticMesh))))

(event EventProgressUpdated
  (params (Progress :type Float%20%28single-precision%29))
  (bind _absoluterotation (Variables|Default|GetAbsoluteRotation))
  (bind _startstaticmeshtransform (Variables|Default|GetStartStaticMeshTransform))
  (bind _targetstaticmeshtransform (Variables|Default|GetTargetStaticMeshTransform))
  (bind _staticmesh (Variables|Default|GetStaticMesh))
  (bind _rotation (Math|Transform|BreakTransform _startstaticmeshtransform))
  (bind _returnvalue (Math|Transform|Lerp(Transform) _startstaticmeshtransform _targetstaticmeshtransform Progress))
  (bind (_location _rotation_2 _scale) (Math|Transform|BreakTransform _returnvalue))
  (bind (_roll _pitch _yaw) (Math|Rotator|BreakRotator _rotation))
  (bind _returnvalue_2 (Math|Vector|MakeVector _roll _pitch _yaw))
  (bind _returnvalue_3 (Math|Vector|Lerp(Vector) _returnvalue_2 _absoluterotation Progress))
  (bind (_x _y _z) (Math|Vector|BreakVector _returnvalue_3))
  (if (Variables|Default|GetUseAbsoluteRotation)
    (Transformation|SetRelativeTransform _staticmesh (Math|Transform|MakeTransform _location (Math|Rotator|MakeRotator _x _y _z) _scale) false false)
    (else
      (Transformation|SetRelativeTransform _staticmesh _returnvalue false false))))

(fn ConstructionScript)