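; BP_RagdollActor is an interactable environment prop that gets knocked around physically by weapon hits.
; On a cosmetic hit from a MordhauWeapon, it enables physics simulation on its static mesh if not already simulating.
; It then applies an impulse at the hit location along the weapon's last observed trace direction, scaled by the weapon's ragdoll force multiplier and the actor's own ForceMultiplier.
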(event EventBeginPlay)

(event Collision|EventActorBeginOverlap
  (params (OtherActor :type Actor%20Object%20Reference)))

(event EventTick
  (params (DeltaSeconds :type Float%20%28single-precision%29)))

(event EventOnReceiveCosmeticHit
  (params (Source :type Actor%20Object%20Reference) (Agent :type Actor%20Object%20Reference) (Move :type EAttackMove%20Enum :default "RightStrike") (Hit :type Hit%20Result%20Structure%20%28by%20ref%29))
  (bind _staticmeshcomponent (Variables|Default|GetStaticMeshComponent))
  (bind _asmordhau_weapon (Utilities|Casting|CastToMordhauWeapon Agent))
  (if (Physics|IsSimulatingPhysics _staticmeshcomponent "None")
    _
    (else
      (Physics|SetSimulatePhysics _staticmeshcomponent true)))
  (Physics|AddImpulseatLocation (Variables|Default|GetStaticMeshComponent) (* (* (Math|Vector|Normalize (Variables|/Script/Mordhau.MordhauWeapon|GetLastObservedTraceDirection _asmordhau_weapon)) (Variables|/Script/Mordhau.MordhauEquipment|GetRagdollForceMultiplier _asmordhau_weapon)) (Variables|Default|GetForceMultiplier)) (.Location (Collision|BreakHitResult Hit)) "None"))

(fn ConstructionScript)