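; Hittable environment prop that wobbles when a character damages it and can be severed when its health runs out.
; Damage updates a replicated Hit force and counter, whose OnRep plays force-scaled audio, sets a clamped tip target and calls the empty OnHit hook.
; Tick spring-interpolates the tip offset to rotate Holder, then disables itself when the animation ends.
; Severing removes Severable's children and can fire a projectile owned by the last hitter.
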(event EventTick
  (params (DeltaSeconds :type Float%20%28single-precision%29))
  (bind _tipdistanceclamp (Variables|Default|GetTipDistanceClamp))
  (bind (_x _y) (Math|Vector2D|BreakVector2D _tipdistanceclamp))
  (bind _output_get (Variables|Default|SetCurrentAnimationTime (- (Variables|Default|GetCurrentAnimationTime) DeltaSeconds)))
  (Utilities|FlowControl|Sequence
    (:then_0
      (if (> (Variables|Default|GetSpringTime) 0.0)
        (Variables|Default|SetSpringTime (Math|Float|Max(Float) (- (Variables|Default|GetSpringTime) DeltaSeconds) 0.0))
        (else
          (Variables|Default|SetTargetTipLocationOffset "0, 0, 0"))))
    (:then_1
      (bind _returnvalue (Class|KismetMathLibrary|VectorSpringInterp (Variables|Default|GetCurrentTipLocationOffset) (Variables|Default|GetTargetTipLocationOffset) (Variables|Default|GetSpringStateVector) (Variables|Default|GetSpringStiffness) (Variables|Default|GetSpringCriticalDampingFactor) DeltaSeconds (Variables|Default|GetSpringMass)))
      (Variables|Default|SetCurrentTipLocationOffset (Math|Vector|ClampVectorSize _returnvalue _x _y))
      (if (<= _output_get 0.0)
        (Variables|Default|SetCurrentTipLocationOffset "0, 0, 0")
        (Actor|Tick|SetActorTickEnabled false)
        (Class|KismetMathLibrary|ResetVectorSpringState (Variables|Default|GetSpringStateVector)))
      (Transformation|SetRelativeRotation (Variables|Default|GetHolder) (Math|Rotator|MakeRotfromZY (* (- (+ (Variables|Default|GetCurrentTipLocationOffset) (Variables|/Script/Engine.SceneComponent|GetRelativeLocation (Variables|Default|GetTip))) (Variables|/Script/Engine.SceneComponent|GetRelativeLocation (Variables|Default|GetHolder))) (Math|Float|Sign(Float) (- (.Z (Math|Vector|BreakVector (Variables|/Script/Engine.SceneComponent|GetRelativeLocation (Variables|Default|GetTip)))) (.Z (Math|Vector|BreakVector (Variables|/Script/Engine.SceneComponent|GetRelativeLocation (Variables|Default|GetHolder))))))) (Math|Vector|MakeVector 0.0 1.0 0.0)) false false))))

(event Game|Damage|EventAnyDamage
  (params (Damage :type Float%20%28single-precision%29) (DamageType :type Damage%20Type%20Object%20Reference) (InstigatedBy :type Controller%20Object%20Reference) (DamageCauser :type Actor%20Object%20Reference))
  (bind _returnvalue (Math|Float|Clamp(Float) Damage 1.0 1e+02))
  (bind _lastdamagenormal (Variables|Default|GetLastDamageNormal))
  (bind _returnvalue_2 (* _lastdamagenormal -1.0))
  (bind _returnvalue_3 (* _returnvalue_2 _returnvalue))
  (bind (_x _y _z) (Math|Vector|BreakVector _returnvalue_3))
  (Utilities|Casting|CastToMordhauCharacter DamageCauser)
  (Variables|Default|SetLastHitter InstigatedBy)
  (bind _output_get (Variables|Default|SetHealth (Math|Integer|Max(Integer) (- (Variables|Default|GetHealth) (Math|Float|Truncate Damage)))))
  (Networking|ForceNetUpdate)
  (Variables|Default|SetHit (Utilities|Struct|MakeST_EnvironmentHittableHit (Math|Vector|MakeVectorNetQuantize10 _x _y _z) (+ (.Counter (Utilities|Struct|BreakST_EnvironmentHittableHit (Variables|Default|GetHit))) 1)))
  (if (Math|Boolean|ANDBoolean (== _output_get 0) (Variables|Default|GetCanBeSevered) (not (Variables|Default|GetSevered)))
    (CallFunction|Sever)))

(fn ConstructionScript)

(fn OnRepHit
  (bind _returnvalue (Transformation|GetActorTransform))
  (bind _audio (Variables|Default|GetAudio))
  (bind _volumedamagescale (Variables|Default|GetVolumeDamageScale))
  (bind _pitchdamagescale (Variables|Default|GetPitchDamageScale))
  (bind _hit (Variables|Default|GetHit))
  (bind _impulsedamagescale (Variables|Default|GetImpulseDamageScale))
  (bind _axisxtargetclamp (Variables|Default|GetAxisXTargetClamp))
  (bind _axisytargetclamp (Variables|Default|GetAxisYTargetClamp))
  (bind _axisztargetclamp (Variables|Default|GetAxisZTargetClamp))
  (bind _force (Utilities|Struct|BreakST_EnvironmentHittableHit _hit))
  (bind (_x _y) (Math|Vector2D|BreakVector2D _axisxtargetclamp))
  (bind (_x_2 _y_2) (Math|Vector2D|BreakVector2D _axisytargetclamp))
  (bind (_x_3 _y_3) (Math|Vector2D|BreakVector2D _impulsedamagescale))
  (bind (_x_4 _y_4) (Math|Vector2D|BreakVector2D _pitchdamagescale))
  (bind (_x_5 _y_5) (Math|Vector2D|BreakVector2D _volumedamagescale))
  (bind (_x_6 _y_6) (Math|Vector2D|BreakVector2D _axisztargetclamp))
  (bind _returnvalue_2 (Math|Vector|VectorLength _force))
  (bind _returnvalue_3 (Math|Vector|VectorLength _force))
  (bind _returnvalue_4 (Math|Transform|InverseTransformDirection _returnvalue _force))
  (bind _returnvalue_5 (Math|Float|MapRangeClamped _returnvalue_3 0.0 1e+02 _x_3 _y_3))
  (bind _returnvalue_6 (Math|Conversions|ToVector2D(Vector) _returnvalue_4))
  (bind _returnvalue_7 (Math|Vector2D|Normalize2D _returnvalue_6))
  (bind _returnvalue_8 (* _returnvalue_7 _returnvalue_5))
  (bind _returnvalue_9 (Math|Conversions|ToVector(Vector2D) _returnvalue_8))
  (bind (_x_7 _y_7 _z) (Math|Vector|BreakVector _returnvalue_9))
  (if (not (< (Utilities|Time|GetTimeSeconds) 3.0))
    (Utilities|FlowControl|Sequence
      (:then_0
        (Networking|CanExecuteCosmeticEvents
          (:True
            (Utilities|IsValid (Variables|/Script/Engine.AudioComponent|GetSound _audio)
              (:Is%20Valid
                (Variables|/Script/Engine.AudioComponent|SetVolumeMultiplier _audio (Math|Float|MapRangeClamped _returnvalue_2 0.0 1e+02 _x_5 _y_5))
                (Variables|/Script/Engine.AudioComponent|SetPitchMultiplier _audio (Math|Float|MapRangeClamped _returnvalue_2 0.0 1e+02 _x_4 _y_4))
                (Audio|Components|Audio|Play _audio 0.0))))))
      (:then_1
        (Variables|Default|SetCurrentAnimationTime (Variables|Default|GetAnimationDuration))
        (Variables|Default|SetSpringTime (Variables|Default|GetSpringTimeOnHit))
        (Variables|Default|SetTargetTipLocationOffset (Math|Vector|MakeVector (Math|Float|Clamp(Float) _x_7 _x _y) (Math|Float|Clamp(Float) _y_7 _x_2 _y_2) (Math|Float|Clamp(Float) _z _x_6 _y_6))))
      (:then_2
        (Actor|Tick|SetActorTickEnabled true))
      (:then_3
        (CallFunction|OnHit)))))

(fn OnRepSevered
  (for _array_element (Components|GetChildrenComponents (Variables|Default|GetSeverable) false)
    (if (== (Components|GetOwner _array_element) self)
      (Components|DestroyComponent _array_element))))

(fn Sever
  (bind _projectiletospawnonsever (Variables|Default|GetProjectileToSpawnOnSever))
  (Utilities|FlowControl|Sequence
    (:then_0
      (LocalVariables|SetSpawnTransform (Transformation|GetWorldTransform (Variables|Default|GetProjectileSpawn))))
    (:then_1
      (Variables|Default|SetSevered true))
    (:then_2
      (if (Utilities|IsValidClass _projectiletospawnonsever)
        (bind _returnvalue (Game|SpawnActorfromClass _projectiletospawnonsever (LocalVariables|GetSpawnTransform) "Undefined" 0 0))
        (Utilities|IsValid _returnvalue
          (:Is%20Valid
            (Class|MordhauProjectile|InitializeProjectile _returnvalue (Variables|Default|GetLastHitter) false)
            (Class|MordhauProjectile|Fire _returnvalue)))))))

(fn OnHit)