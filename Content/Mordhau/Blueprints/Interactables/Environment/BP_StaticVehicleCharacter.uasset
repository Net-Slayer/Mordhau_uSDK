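; BP_StaticVehicleCharacter is a short-lived drivable proxy that links a driver to a static vehicle actor.
; The replicated StaticVehicleActor adds it to its VehicleCharacters list through OnRep and drops it on destruction, and supplies the exit transform.
; Animation updates pass its Animation to the Mordhau character anim blueprint as StaticVehicleAnim.
; When driving stops, the server sets a brief lifespan so the proxy cleans itself up.
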(event EventBeginPlay
  (|CallParentFunction) ; This node is disabled and will not be called.\nDrag off pins to build functionality.
)

(event Collision|EventActorBeginOverlap
  (params (OtherActor :type Actor%20Object%20Reference))
  (|CallParentFunction OtherActor) ; This node is disabled and will not be called.\nDrag off pins to build functionality.
)

(event EventDestroyed
  (Utilities|FlowControl|Sequence
    (:then_0
      (Utilities|IsValid (Variables|Default|GetStaticVehicleActor)
        (:Is%20Valid
          (Utilities|Array|RemoveItem (Variables|/Game/Mordhau/Blueprints/Interactables/Environment/BP_StaticVehicleActor.BP_StaticVehicleActor_C|GetVehicleCharacters (Variables|Default|GetStaticVehicleActor)) self))))
    (:then_1
      (|CallParentFunction))))

(event EventTick
  (params (DeltaSeconds :type Float%20%28single-precision%29))
  (|CallParentFunction DeltaSeconds) ; This node is disabled and will not be called.\nDrag off pins to build functionality.
)

(event EventOnStoppedDriving
  (params (Character :type Mordhau%20Character%20Object%20Reference))
  (Networking|SwitchHasAuthority
    (:Authority
      (Actor|SetLifeSpan 0.5))))

(event EventUpdateAnimationfor
  (params (Character :type Mordhau%20Character%20Object%20Reference) (AnimInst :type Mordhau%20Anim%20Instance%20Object%20Reference) (DeltaTime :type Float%20%28single-precision%29))
  (|CallParentFunction Character AnimInst DeltaTime)
  (bind _asab_mordhau_character_animation (Utilities|Casting|CastToAB_MordhauCharacterAnimation AnimInst))
  (Variables|/Game/Mordhau/Animations/Blueprints/AB_MordhauCharacterAnimation.AB_MordhauCharacterAnimation_C|SetStaticVehicleAnim _asab_mordhau_character_animation (Variables|Default|GetAnimation)))

(event Input|ActionEvents|InputActionCycleCamera
  (params (Key :type Key%20Structure)))

(fn ConstructionScript
  (|CallParentFunction))

(fn OnRepStaticVehicleActor
  (bind _staticvehicleactor (Variables|Default|GetStaticVehicleActor))
  (Utilities|IsValid _staticvehicleactor
    (:Is%20Valid
      (Utilities|Array|AddUnique (Variables|/Game/Mordhau/Blueprints/Interactables/Environment/BP_StaticVehicleActor.BP_StaticVehicleActor_C|GetVehicleCharacters _staticvehicleactor) self))))

(fn GetExitTransform
  (bind _staticvehicleactor (Variables|Default|GetStaticVehicleActor))
  (Utilities|IsValid _staticvehicleactor
    (:Is%20Valid
      (return (Transformation|GetWorldTransform (Variables|/Game/Mordhau/Blueprints/Interactables/Environment/BP_StaticVehicleActor.BP_StaticVehicleActor_C|GetVehicleExit _staticvehicleactor))))
    (:Is%20Not%20Valid
      (bind _returnvalue (|CallParentFunction))
      (return _returnvalue))))