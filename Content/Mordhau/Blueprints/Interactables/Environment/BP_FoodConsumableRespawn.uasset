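; Food pickup interactable that restores health and stamina to the character, then respawns after a delay.
; Each use increments a replicated counter whose RepNotify, ignored in the first seconds of world time, plays the sound and particle burst.
; It then hides the food and widget until a retriggerable delay ends.
; CanInteract refuses use while replenishing and can restrict the food to the Frontline kill-objective character.
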(event Custom|HandleConsumptionEffects
  (Variables|/Script/Mordhau.MordhauWidgetComponent|SetOverrideVisible (Variables|Default|GetMordhauWidget) 0)
  (Audio|PlaySoundatLocation 0 (Transformation|GetActorLocation) "0, 0, 0" 5.0 1.0 0.0 0 0 0)
  (Development|SetHiddeninGame (Variables|Default|GetFood) true true)
  (Components|Activation|Activate (Variables|Default|GetP_FoodExplosion) false)
  (Variables|Default|SetReplenishing true)
  (Utilities|FlowControl|RetriggerableDelay (Variables|Default|GetRespawnTimer))
  (Variables|/Script/Mordhau.MordhauWidgetComponent|SetOverrideVisible (Variables|Default|GetMordhauWidget) 1)
  (Variables|Default|SetReplenishing false)
  (Development|SetHiddeninGame (Variables|Default|GetFood) false true))

(event EventBeginPlay
  (|CallParentFunction) ; This node is disabled and will not be called.\nDrag off pins to build functionality.
)

(event Collision|EventActorBeginOverlap
  (params (OtherActor :type Actor%20Object%20Reference))
  (|CallParentFunction OtherActor) ; This node is disabled and will not be called.\nDrag off pins to build functionality.
)

(event EventOnInteractionStart
  (params (Character :type Mordhau%20Character%20Object%20Reference))
  (Class|AdvancedCharacter|OffsetHealth Character (Variables|Default|GetHealthRegen) false)
  (Class|MordhauCharacter|OffsetStamina Character (Variables|Default|GetStamRegen) false)
  (Variables|Default|SetReplicatedConsumptionCounter (+ (Variables|Default|GetReplicatedConsumptionCounter) 1)))

(fn ConstructionScript
  (|CallParentFunction))

(fn OnRepReplicatedConsumptionCounter
  (if (> (Utilities|Time|GetTimeSeconds) 3.0)
    (CallFunction|HandleConsumptionEffects)))

(fn CanInteract
  (params (Character :type Mordhau%20Character%20Object%20Reference))
  (if (Variables|Default|GetReplenishing)
    _
    (elif (Variables|Default|GetKingExclusive)
      (Utilities|Casting|CastToBP_FrontlineKillObjective Character
        (:then
          (return (|CallParentFunction Character)))
        (:CastFailed
          _))
      (else
        (return (|CallParentFunction Character)))))
  (return false))