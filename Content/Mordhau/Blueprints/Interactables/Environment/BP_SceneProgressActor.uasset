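; BP_SceneProgressActor is an environment interactable that moves its Holder component in step with a progress value.
; It records Holder's relative transform at BeginPlay as the start pose.
; Each ProgressUpdated event interpolates from that start to TargetTransform using the progress as alpha, without sweeping.
; The construction script attaches the Audio component to Holder so it follows the movement.
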(event EventBeginPlay
  (Variables|Default|SetStartTransform (Transformation|GetRelativeTransform (Variables|Default|GetHolder))))

(event Collision|EventActorBeginOverlap
  (params (OtherActor :type Actor%20Object%20Reference)))

(event EventProgressUpdated
  (params (Progress :type Float%20%28single-precision%29))
  (Transformation|SetRelativeTransform (Variables|Default|GetHolder) (Math|Transform|Lerp(Transform) (Variables|Default|GetStartTransform) (Variables|Default|GetTargetTransform) Progress) false false))

(event EventTick
  (params (DeltaSeconds :type Float%20%28single-precision%29)))

(fn ConstructionScript
  (Transformation|AttachComponentToComponent (Variables|Default|GetAudio) (Variables|Default|GetHolder) "None" "KeepRelative" "KeepRelative" "KeepRelative" true))