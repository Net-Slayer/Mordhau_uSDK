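; Drivable mortar siege engine that the operator aims, fires and reloads, and that ragdolls when destroyed.
; FireBallista spawns the projectile and cycles State through ready, fired and reloading, with OnRep_State driving ball visibility, effects, sounds and recoil pitch.
; BPLODTick derives smoothed turn velocities for sound and, while ready, draws the local player's predicted arc as distance-scaled instanced meshes.
; Mesh sockets position the ball, third-person camera and operator's hand targets.
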(event Custom|FireBallista
  (params (Location :type Vector) (Rotation :type Rotator))
  (Variables|Default|SetFireLocation Location)
  (Variables|Default|SetFireRotation Rotation)
  (if (== (Variables|Default|GetState) 0)
    (bind _returnvalue (Game|SpawnActorfromClass (Variables|Default|GetProjectileClass) (Math|Transform|MakeTransform Location Rotation) "AlwaysSpawn" self 0))
    (Class|MordhauProjectile|InitializeProjectile _returnvalue (Pawn|GetController) false)
    (Class|MordhauProjectile|Fire _returnvalue)
    (Variables|Default|SetState 1)
    (Utilities|FlowControl|Delay (Variables|Default|GetFireRecoveryTime))
    (Variables|Default|SetState 2)
    (Utilities|FlowControl|Delay (Variables|Default|GetReloadTime))
    (Variables|Default|SetState 0)))

(event EventBPLODTick
  (params (DeltaTime :type Float%20%28single-precision%29))
  (bind _lookupvalue (Variables|Default|GetLookUpValue))
  (bind _mesh (Variables|Character|GetMesh))
  (bind _mesh_2 (Variables|Character|GetMesh))
  (bind _instancedstaticmesh (Variables|Default|GetInstancedStaticMesh))
  (bind _returnvalue (Transformation|GetWorldRotation _mesh_2))
  (bind _yaw (Math|Rotator|BreakRotator _returnvalue))
  (|CallParentFunction DeltaTime)
  (Networking|CanExecuteCosmeticEvents
    (:True
      (Utilities|FlowControl|Sequence
        (:then_0
          (if (or (> (Math|Float|Absolute(Float) (Variables|Default|GetRotationVelocitySmoothed)) 3e+01) (> (Math|Float|Absolute(Float) (Variables|Default|GetPitchVelocitySmoothed)) 15.0))
            (Utilities|IsValid (Variables|Default|GetLastTurnSound)
              (:Is%20Not%20Valid
                (bind _returnvalue_2 (Audio|SpawnSoundAttached "/Game/Mordhau/Audio/Cues/Siege/SC_Ballista_Turn.SC_Ballista_Turn" (Variables|Character|GetMesh) "Yaw" "0, 0, 0" "0, 0, 0" "SnapToTarget" true 1.0 1.0 0.0 0 0))
                (Variables|Default|SetLastTurnSound _returnvalue_2)))
            (elif (and (< (Math|Float|Absolute(Float) (Variables|Default|GetRotationVelocitySmoothed)) 1.0) (< (Math|Float|Absolute(Float) (Variables|Default|GetPitchVelocitySmoothed)) 1.0))
              (Utilities|IsValid (Variables|Default|GetLastTurnSound)
                (:Is%20Valid
                  (Audio|Components|Audio|FadeOut (Variables|Default|GetLastTurnSound) 0.2 0.0 :!class /Script/Engine.AudioComponent)
                  (Variables|Default|SetLastTurnSound 0))))))
        (:then_1
          (bind _output_get (Variables|Default|SetRotationVelocity (/ (- (Variables|Default|GetPreviousActorYaw) _yaw) DeltaTime)))
          (Variables|Default|SetPreviousActorYaw _yaw)
          (Variables|Default|SetRotationVelocitySmoothed (Math|Interpolation|FInterpTo (Variables|Default|GetRotationVelocitySmoothed) _output_get DeltaTime 2e+01))
          (Variables|Default|SetPitchVelocitySmoothed (Math|Interpolation|FInterpTo (Variables|Default|GetPitchVelocitySmoothed) (/ (- (Variables|Default|GetPreviousPitch) _lookupvalue) DeltaTime) DeltaTime 2e+01))
          (Variables|Default|SetPreviousPitch _lookupvalue))
        (:then_2
          (if (Class|AdvancedCharacter|IsLocallyPlayerControlled)
            (if (== (Variables|Default|GetState) 0)
              (bind _predictresult (Class|GameplayStatics|BlueprintPredictProjectilePathAdvanced (Utilities|Struct|MakePredictProjectilePathParams (Transformation|GetSocketLocation _mesh "BallSocket") (Math|Vector|RotateVector (Math|Vector|MakeVector (Variables|Default|GetPredictionLaunchVelocity) 0.0 0.0) (Transformation|GetSocketRotation _mesh "BallSocket")) true 3e+01 (Variables|Default|GetMaxSimTime) true "ECC_WorldStatic" (Utilities|Array|MakeArray "ObjectTypeQuery1") (Utilities|Array|MakeArray self) 2e+01 (* -9.8e+02 (Variables|Default|GetPredictionGravity)) "None" 1.0 true)))
              (Components|InstancedStaticMesh|ClearInstances _instancedstaticmesh)
              (for _array_element (.PathData (Utilities|Struct|BreakPredictProjectilePathResult _predictresult))
                (Class|InstancedStaticMeshComponent|AddInstanceWorldSpace _instancedstaticmesh (Math|Transform|MakeTransform (.Location (Utilities|Struct|BreakPredictProjectilePathPointData _array_element)) "0, 0, 0" (* (Math|Conversions|ToVector(Float) (Variables|Default|GetPredictionSphereScale)) (Math|Conversions|ToVector(Float) (Math|Float|Clamp(Float) (* (Math|Vector|VectorLength (- (Transformation|GetWorldLocation (Variables|Default|GetBall)) (.Location (Utilities|Struct|BreakPredictProjectilePathPointData _array_element)))) 0.0003) 1.0 1e+03))))))
              (Variables|Default|SetAddedInstances true)
              (else
                (if (Variables|Default|GetAddedInstances) :!label _label
                  (Variables|Default|SetAddedInstances false)
                  (Components|InstancedStaticMesh|ClearInstances _instancedstaticmesh))))
            (else
              (goto _label))))))))

(event EventBeginPlay
  (bind _mesh (Variables|Character|GetMesh))
  (Utilities|FlowControl|Sequence
    (:then_0
      (bind _returnvalue (Rendering|Material|CreateDynamicMaterialInstance _mesh 0 (Rendering|Material|GetMaterial _mesh 0) "None" :!class /Script/Engine.PrimitiveComponent))
      (Class|AdvancedCharacter|RegisterMaterialtoDissolve _returnvalue))
    (:then_1
      (Class|MordhauUtilityLibrary|SetCanEverAffectNavigation (Variables|Default|GetCapsuleComponent) false))))

(event EventOnCosmeticHit
  (params (DamageType :type EMordhauDamageType%20Enum :default "Generic") (SubType :type Byte :default 0) (Hit :type Hit%20Result%20Structure%20%28by%20ref%29) (Agent :type Actor%20Object%20Reference))
  (bind (_bblockinghit _binitialoverlap _time _distance _location _impactpoint _normal _impactnormal _physmat _hitactor _hitcomponent _hitbonename) (Collision|BreakHitResult Hit))
  (|CallParentFunction DamageType SubType Hit Agent)
  (bind _force (CallFunction|ComputeRagdollForce Agent DamageType SubType 0 self))
  (Class|PrimitiveComponent|AddForceatLocation (Variables|Character|GetMesh) (* _force 1e+02) _impactpoint _hitbonename))

(event EventUpdateAnimationfor
  (params (Character :type Mordhau%20Character%20Object%20Reference) (AnimInst :type Mordhau%20Anim%20Instance%20Object%20Reference) (DeltaTime :type Float%20%28single-precision%29))
  (bind _mesh (Variables|/Script/Engine.Character|GetMesh Character))
  (bind _mesh_2 (Variables|Character|GetMesh))
  (|CallParentFunction Character AnimInst DeltaTime)
  (bind _asab_mordhau_character_animation (Utilities|Casting|CastToAB_MordhauCharacterAnimation AnimInst))
  (Variables|/Game/Mordhau/Animations/Blueprints/AB_MordhauCharacterAnimation.AB_MordhauCharacterAnimation_C|SetVehicleRightHandTarget _asab_mordhau_character_animation (- (Transformation|GetSocketLocation _mesh_2 "RightHandTarget") (Math|Transform|TransformDirection (Transformation|GetSocketTransform _mesh "RightHand" "RTS_World") "-1.250000,-9.500000,0.500000")))
  (Variables|/Game/Mordhau/Animations/Blueprints/AB_MordhauCharacterAnimation.AB_MordhauCharacterAnimation_C|SetVehicleLeftHandTarget _asab_mordhau_character_animation (- (Transformation|GetSocketLocation _mesh_2 "LeftHandTarget") (Math|Transform|TransformDirection (Transformation|GetSocketTransform _mesh "LeftHand" "RTS_World") "1.250000,-9.500000,0.500000")))
  (Variables|/Game/Mordhau/Animations/Blueprints/AB_MordhauCharacterAnimation.AB_MordhauCharacterAnimation_C|SetVehicleLookUp _asab_mordhau_character_animation (.Pitch (Math|Rotator|BreakRotator (.Rotation (Math|Transform|BreakTransform (Transformation|GetSocketTransform _mesh_2 "Barrel" "RTS_Component"))))))
  (Variables|/Script/Mordhau.MordhauAnimInstance|SetbBallistaReloading _asab_mordhau_character_animation false)
  (Variables|/Game/Mordhau/Animations/Blueprints/AB_MordhauCharacterAnimation.AB_MordhauCharacterAnimation_C|SetVehicleDirection _asab_mordhau_character_animation (Math|Float|MapRangeClamped (Variables|Default|GetRotationVelocity) -45.0 45.0 -1e+02 1e+02)))

(event EventOnDied
  (params (Angle :type Float%20%28single-precision%29) (Type :type EMordhauDamageType%20Enum :default "Generic") (SubType :type Byte :default 0) (bone :type Name%20%28by%20ref%29 :default "None") (Point :type Vector%20%28by%20ref%29 :default "0, 0, 0") (Source :type Actor%20Object%20Reference) (Agent :type Actor%20Object%20Reference))
  (bind _loadingsound (Variables|Default|GetLoadingSound))
  (bind _lastturnsound (Variables|Default|GetLastTurnSound))
  (|CallParentFunction Angle Type SubType bone Point Source Agent)
  (Networking|CanExecuteCosmeticEvents
    (:True
      (Class|AdvancedCharacter|StartRagdoll)
      (bind _force (CallFunction|ComputeRagdollForce Agent Type SubType 0 self))
      (Class|PrimitiveComponent|AddForceatLocation (Variables|Character|GetMesh) (* _force 1e+02) Point bone)
      (Utilities|FlowControl|Sequence
        (:then_0
          (Utilities|IsValid _loadingsound
            (:Is%20Valid
              (Audio|Components|Audio|FadeOut _loadingsound 0.3 0.0 :!class /Script/Engine.AudioComponent))))
        (:then_1
          (Utilities|IsValid _lastturnsound
            (:Is%20Valid
              (Audio|Components|Audio|FadeOut _lastturnsound 0.3 0.0 :!class /Script/Engine.AudioComponent))))
        (:then_2
          (Development|SetHiddeninGame (Variables|Default|GetBall) true false))))))

(event EventUpdateFPCamerafor
  (params (Character :type Mordhau%20Character%20Object%20Reference) (DeltaSeconds :type Float%20%28single-precision%29) (bRotationOnly :type Boolean))
  (|CallParentFunction Character DeltaSeconds bRotationOnly)
  (Class|MordhauCharacter|UpdateFPCamera Character DeltaSeconds 0.0 bRotationOnly (Math|Rotator|MakeRotator 0.0 0.0 0.0)))

(event Input|ActionEvents|InputActionFire
  (params (Key :type Key%20Structure))
  (bind _mesh (Variables|Character|GetMesh))
  (:Pressed
    (if (== (Variables|Default|GetState) 0)
      (CallFunction|FireBallista (Transformation|GetSocketLocation _mesh "BallSocket") (Transformation|GetSocketRotation _mesh "BallSocket")))))

(event Input|ActionEvents|InputActionCycleCamera
  (params (Key :type Key%20Structure)))

(event Input|AxisEvents|InputAxisLookUp
  (params (AxisValue :type Float%20%28single-precision%29))
  (Class|AdvancedCharacter|LookUp AxisValue false))

(event Input|AxisEvents|InputAxisTurnRight
  (params (AxisValue :type Float%20%28single-precision%29))
  (Class|AdvancedCharacter|Turn AxisValue false))

(fn ConstructionScript
  (Transformation|AttachComponentToComponent (Variables|Default|GetBall) (Variables|Character|GetMesh) "BallSocket" "SnapToTarget" "SnapToTarget" "SnapToTarget" false))

(fn OnRepState
  (bind _state (Variables|Default|GetState))
  (if (not (Class|AdvancedCharacter|GetIsDead))
    (Utilities|FlowControl|Sequence
      (:then_0
        (if (== (Variables|Default|GetState) 1)
          (if (Class|AdvancedCharacter|IsLocallyPlayerControlled)
            (Class|AdvancedCharacter|LookUp 2.0 true))))
      (:then_1
        (Networking|CanExecuteCosmeticEvents
          (:True
            (Utilities|FlowControl|Sequence
              (:then_0
                (Rendering|SetVisibility (Variables|Default|GetBall) (== _state 0) false))
              (:then_1
                (switch int (Math|Conversions|ToInteger(Byte) _state)
                  (:0
                    (Utilities|IsValid (Variables|Default|GetLoadingSound)
                      (:Is%20Valid
                        (Audio|Components|Audio|FadeOut (Variables|Default|GetLoadingSound) 0.1 0.0 :!class /Script/Engine.AudioComponent)
                        (Variables|Default|SetLoadingSound 0))))
                  (:1
                    (Audio|PlaySoundatLocation 0 (Transformation|GetWorldLocation (Variables|Default|GetBall)) "0, 0, 0" 1.0 1.0 0.0 0 0 0)
                    (Components|Activation|Activate (Variables|Default|GetP_MortarFire) false)
                    (Camera|PlayWorldCameraShake "/Game/Mordhau/Blueprints/CameraShakes/ImpactShake.ImpactShake_C" (Variables|Default|GetFireLocation) 5e+02 5e+03 1e+01))
                  (:2
                    (bind _returnvalue (Audio|SpawnSoundAttached "/Game/Mordhau/Audio/Cues/Siege/SC_Ballista_Reloading.SC_Ballista_Reloading" (Variables|Character|GetMesh) "Windup" "0, 0, 0" "0, 0, 0" "SnapToTarget" true 1.0 1.0 0.0 0 0))
                    (Variables|Default|SetLoadingSound _returnvalue)))))))))))

(fn PostProcessCameraPOV
  (params (InPOV :type POV%20Structure%20%28by%20ref%29))
  (bind _mesh (Variables|Character|GetMesh))
  (bind _driver (Variables|Default|GetDriver))
  (bind _returnvalue (Transformation|GetSocketTransform _mesh "Camera3P" "RTS_World"))
  (bind (_location _rotation) (Math|Transform|BreakTransform _returnvalue))
  (Utilities|IsValid _driver
    (:Is%20Valid
      (if (Variables|/Script/Mordhau.MordhauCharacter|GetbIsFirstPerson _driver)
        _
        (else
          (return (Utilities|Struct|MakePOV _location _rotation (- (.FOV (Utilities|Struct|BreakPOV InPOV)) 3e+01))))))
    (:Is%20Not%20Valid
      _))
  (return InPOV))

(fn OnRepReplicatedLookUpCap
  (Variables|Default|SetLookUpLimit (Variables|Default|GetReplicatedLookUpCap)))

(fn OnRepReplicatedTurnCap
  (Variables|Default|SetTurnLimit (Variables|Default|GetReplicatedTurnCap)))