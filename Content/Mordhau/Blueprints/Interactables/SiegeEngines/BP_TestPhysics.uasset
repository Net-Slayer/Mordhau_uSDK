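; BP_TestPhysics is a siege engine physics test actor that pushes a skeletal mesh toward a target velocity using forces.
; Each tick with nonzero TargetVelocity, it yaw-rotates that velocity and subtracts the mesh's velocity at a scene component's location.
; The error is clamped per world axis by ForceLimits, scaled by fixed gains and mass, then applied there as force.
; The vertical gain is zero, so only horizontal motion is driven.
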(event EventBeginPlay)

(event Collision|EventActorBeginOverlap
  (params (OtherActor :type Actor%20Object%20Reference)))

(event EventTick
  (params (DeltaSeconds :type Float%20%28single-precision%29))
  (bind _forcelimits (Variables|Default|GetForceLimits))
  (bind _scene (Variables|Default|GetScene))
  (bind _skeletalmesh (Variables|Default|GetSkeletalMesh))
  (bind _returnvalue (Transformation|GetWorldLocation _scene))
  (bind (_x _y _z) (Math|Vector|BreakVector _forcelimits))
  (if (Math|Vector|NotEqual(Vector) (Variables|Default|GetTargetVelocity) "0, 0, 0" 0.0001)
    (bind _returnvalue_2 (Class|PrimitiveComponent|GetPhysicsLinearVelocityatPoint _skeletalmesh _returnvalue "None"))
    (Class|PrimitiveComponent|AddForceatLocation _skeletalmesh (* (* (+ (Math|Vector|ClampVectorSize (Math|Vector|MakeVector (.X (Math|Vector|BreakVector (- (Math|Vector|RotateVector (Variables|Default|GetTargetVelocity) (Math|Rotator|MakeRotator 0.0 0.0 (.Yaw (Math|Rotator|BreakRotator (Transformation|GetActorRotation))))) _returnvalue_2))) 0.0 0.0) 0.0 _x) (Math|Vector|ClampVectorSize (Math|Vector|MakeVector 0.0 (.Y (Math|Vector|BreakVector (- (Math|Vector|RotateVector (Variables|Default|GetTargetVelocity) (Math|Rotator|MakeRotator 0.0 0.0 (.Yaw (Math|Rotator|BreakRotator (Transformation|GetActorRotation))))) _returnvalue_2))) 0.0) 0.0 _y) (Math|Vector|ClampVectorSize (Math|Vector|MakeVector 0.0 0.0 (.Z (Math|Vector|BreakVector (- (Math|Vector|RotateVector (Variables|Default|GetTargetVelocity) (Math|Rotator|MakeRotator 0.0 0.0 (.Yaw (Math|Rotator|BreakRotator (Transformation|GetActorRotation))))) _returnvalue_2)))) 0.0 _z)) "10.000000,20.000000, 0") (Physics|GetMass _skeletalmesh)) _returnvalue "None")))

(fn ConstructionScript)