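; Climbable siege ladder that players mount by interacting and, with a held interaction while unoccupied, drop or raise.
; Climbing spawns a BP_LadderMover at the closest point on the ladder to drive the character.
; LadderState's RepNotify starts a curve-driven Tick animation toward upright or the DroppedMesh placeholder's transform, snapping silently during the first five seconds.
; While dropping, the server damages and trips characters underneath once each; kick-to-drop is disabled.
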(event Custom|BeginAnimatingLadder
  (params (DoEffects :type Boolean))
  (bind _laddermesh (Variables|Default|GetLadderMesh))
  (bind _ladderend (Variables|Default|GetLadderEnd))
  (bind _ladderstart (Variables|Default|GetLadderStart))
  (bind _dropduration (Variables|Default|GetDropDuration))
  (bind _raiseduration (Variables|Default|GetRaiseDuration))
  (bind _returnvalue (Transformation|GetWorldTransform _laddermesh))
  (bind _relativelocation (Variables|/Script/Engine.SceneComponent|GetRelativeLocation _ladderend))
  (bind _relativelocation_2 (Variables|/Script/Engine.SceneComponent|GetRelativeLocation _ladderstart))
  (bind _returnvalue_2 (+ _relativelocation_2 _relativelocation))
  (bind _returnvalue_3 (* _returnvalue_2 0.5))
  (bind _z (Math|Vector|BreakVector _returnvalue_3))
  (bind _returnvalue_4 (Math|Transform|TransformLocation _returnvalue (Math|Vector|MakeVector 0.0 0.0 _z)))
  (Class|PrimitiveComponent|SetWalkableSlopeOverride (Variables|Default|GetLadderMesh) (Utilities|Struct|MakeWalkableSlopeOverride "WalkableSlope_Unwalkable" 0.0))
  (Actor|Tick|SetActorTickEnabled true)
  (Variables|Default|SetbIsInteractable false)
  (Variables|Default|SetbPreventClimbing true)
  (if DoEffects
    (Audio|SpawnSoundAttached (Utilities|Select :Index (Variables|Default|GetLadderState) :Option%200 0 :Option%201 0) (Variables|Default|GetLadderMesh) "None" _returnvalue_4 "0, 0, 0" "KeepWorldPosition" false 1.0 1.0 0.0 0 0)
    (if (== (Variables|Default|GetLadderState) 1)
      ;[1 1 1] dropping
      (Utilities|FlowControl|RetriggerableDelay (* _dropduration 0.562069))
      (Audio|PlaySoundatLocation 0 _returnvalue_4 "0, 0, 0" 1.0 0.9 0.0 0 0 0)
      (Effects|SpawnEmitteratLocation 0 _returnvalue_4 "90.000000,0.000000,0.000000" "0.700000,0.700000,0.700000")
      (Utilities|FlowControl|RetriggerableDelay (* _dropduration 0.279203))
      (Audio|PlaySoundatLocation 0 _returnvalue_4 "0, 0, 0" 0.5 1.2 0.0 0 0 0)
      (Utilities|FlowControl|RetriggerableDelay (* _dropduration 0.159))
      (Audio|PlaySoundatLocation 0 _returnvalue_4 "0, 0, 0" 0.25 1.5 0.0 0 0 0)
      (else
        (Utilities|FlowControl|RetriggerableDelay (* _raiseduration 0.875))
        (Audio|PlaySoundatLocation 0 _returnvalue_4 "0, 0, 0" 0.5 1.2 0.0 0 0 0)
        (Utilities|FlowControl|RetriggerableDelay (* _raiseduration 0.125))
        (Audio|PlaySoundatLocation 0 _returnvalue_4 "0, 0, 0" 0.25 1.5 0.0 0 0 0)))))

(event Custom|ToggleLadderState
  (params (Instigator :type Controller%20Object%20Reference))
  (Variables|Default|SetInteractInstigator Instigator)
  (Variables|Default|SetLadderState (Utilities|Select :Index (Variables|Default|GetLadderState) :Option%200 1 :Option%201 0)))

(event EventOnHeldInteractionStart
  (params (Character :type Mordhau%20Character%20Object%20Reference))
  (Utilities|IsValid Character
    (:Is%20Valid
      (CallFunction|ToggleLadderState (Pawn|GetController Character)))
    (:Is%20Not%20Valid
      (CallFunction|ToggleLadderState))))

(event EventBeginPlay
  (bind _droppedmesh (Variables|Default|GetDroppedMesh))
  (|CallParentFunction)
  (Variables|Default|SetDroppedMeshTransform (Transformation|GetRelativeTransform _droppedmesh))
  (Components|DestroyComponent _droppedmesh)
  (Utilities|FlowControl|Sequence
    (:then_0
      (CallFunction|UpdateInteractionText)
      (if (not (Variables|Default|GetCanDropAndRaise))
        (Variables|Default|SetMaxInteractionHoldTime 0.0)))
    (:then_1
      (Networking|SwitchHasAuthority
        (:Authority
          (if (not (Variables|Default|GetStartAsRaised))
            (Variables|Default|SetLadderState 1)))))))

(event EventOnHighlightMaintained
  (params (Character :type Mordhau%20Character%20Object%20Reference))
  (bind _interactionwidgetcomponent (Variables|Default|GetInteractionWidgetComponent))
  (bind _laddermesh (Variables|Default|GetLadderMesh))
  (bind _relativelocation (Variables|/Script/Engine.SceneComponent|GetRelativeLocation _laddermesh))
  (bind _relativerotation (Variables|/Script/Engine.SceneComponent|GetRelativeRotation _laddermesh))
  (bind _returnvalue (Math|Vector|GetUpVector _relativerotation))
  (Utilities|IsValid _interactionwidgetcomponent
    (:Is%20Valid
      (Transformation|SetRelativeTransform _interactionwidgetcomponent (Math|Transform|MakeTransform (Math|Vector|FindClosestPointonSegment (Math|Transform|InverseTransformLocation (Transformation|GetActorTransform) (+ (Variables|/Script/Mordhau.MordhauCharacter|GetCameraLocation1P Character) (Math|Vector|RotateVector "25.000000, 0, 0" (Variables|/Script/Mordhau.MordhauCharacter|GetCameraRotation1P Character)))) (+ _relativelocation (* _returnvalue (.Z (Math|Vector|BreakVector (Variables|/Script/Engine.SceneComponent|GetRelativeLocation (Variables|Default|GetLadderStart)))))) (+ _relativelocation (* _returnvalue (.Z (Math|Vector|BreakVector (Variables|/Script/Engine.SceneComponent|GetRelativeLocation (Variables|Default|GetLadderEnd)))))))) false false))))

(event Game|Damage|EventAnyDamage
  (params (Damage :type Float%20%28single-precision%29) (DamageType :type Damage%20Type%20Object%20Reference) (InstigatedBy :type Controller%20Object%20Reference) (DamageCauser :type Actor%20Object%20Reference))
  ;[1 1 1] disabled kicking for now
  (Utilities|FlowControl|Sequence
    (:then_1
      (|CallParentFunction Damage DamageType InstigatedBy DamageCauser))))

(event EventTick
  (params (DeltaSeconds :type Float%20%28single-precision%29))
  (bind _returnvalue (Math|Transform|MakeTransform "0, 0, 0" "0,-90.000000, 0"))
  (bind _ladderstatechangetime (Variables|Default|GetLadderStateChangeTime))
  (bind _laddermesh (Variables|Default|GetLadderMesh))
  (bind _droppedmeshtransform (Variables|Default|GetDroppedMeshTransform))
  (|CallParentFunction DeltaSeconds)
  (bind _returnvalue_2 (Class|MordhauUtilityLibrary|GetNormalizedTime _ladderstatechangetime (+ _ladderstatechangetime (Utilities|Select :Index (Variables|Default|GetLadderState) :Option%200 (Variables|Default|GetRaiseDuration) :Option%201 (Variables|Default|GetDropDuration))) (Utilities|Time|GetTimeSeconds)))
  (Utilities|FlowControl|Sequence
    (:then_0
      (if (== (Variables|Default|GetLadderState) 0)
        (Transformation|SetRelativeTransform _laddermesh (Math|Transform|Lerp(Transform) _droppedmeshtransform _returnvalue (Math|Curves|GetFloatValue (Variables|Default|GetRaiseCurve) _returnvalue_2)) false false)
        (else
          (Transformation|SetRelativeTransform _laddermesh (Math|Transform|Lerp(Transform) _returnvalue _droppedmeshtransform (Math|Curves|GetFloatValue (Variables|Default|GetDropCurve) _returnvalue_2)) false false)
          (Networking|SwitchHasAuthority
            (:Authority
              (if (> _returnvalue_2 0.333)
                (bind _outactors (Collision|ComponentOverlapActors _laddermesh (Transformation|GetWorldTransform _laddermesh) (Utilities|Array|MakeArray "ObjectTypeQuery3") "/Script/Mordhau.MordhauCharacter" (Variables|Default|GetFallIgnoreActors)))
                (for _array_element _outactors
                  (bind _asmordhau_character (Utilities|Casting|CastToMordhauCharacter _array_element)
                    (:then
                      (if (or (Variables|/Script/Mordhau.AdvancedCharacter|GetbIsDead _asmordhau_character) (Variables|/Script/Mordhau.AdvancedCharacter|GetbIsRagdollFalling _asmordhau_character))
                        (Utilities|Array|Add (Variables|Default|GetFallIgnoreActors) _array_element :!label _label)
                        (elif (and (< (.X (Math|Vector|BreakVector (Math|Transform|InverseTransformLocation (Transformation|GetActorTransform) (Transformation|GetActorLocation _asmordhau_character)))) -1e+01) (< (Math|Float|Absolute(Float) (.Y (Math|Vector|BreakVector (Math|Transform|InverseTransformLocation (Transformation|GetActorTransform) (Transformation|GetActorLocation _asmordhau_character))))) 5e+01))
                          (Class|AdvancedCharacter|MordhauTakeDamage _asmordhau_character (Variables|Default|GetDropDamage) (Collision|MakeHitResult false false 0.0 0.0 "0, 0, 0" "0, 0, 0" "0,0,1" "0,0,1" 0 0) "Generic" 0 _asmordhau_character self (Variables|Default|GetInteractInstigator))
                          (Class|AdvancedCharacter|Trip _asmordhau_character)
                          (goto _label))))
                    (:CastFailed
                      (goto _label))))))))))
    (:then_1
      (if (== _returnvalue_2 1.0)
        (Utilities|Array|Clear (Variables|Default|GetFallIgnoreActors))
        (Actor|Tick|SetActorTickEnabled false)
        (Variables|Default|SetbIsInteractable true)
        (Class|PrimitiveComponent|SetWalkableSlopeOverride (Variables|Default|GetLadderMesh) (Utilities|Struct|MakeWalkableSlopeOverride "WalkableSlope_Default" 0.0))
        (Variables|Default|SetbPreventClimbing false)))))

(event EventOnInteractionStart
  (params (Character :type Mordhau%20Character%20Object%20Reference))
  (bind _returnvalue (Game|SpawnActorfromClass "/Game/Mordhau/Blueprints/Interactables/SiegeEngines/BP_LadderMover.BP_LadderMover_C" (Math|Transform|MakeTransform (Class|MordhauUtilityLibrary|ClosestPointonLine (Transformation|GetWorldLocation (Variables|Default|GetLadderStart)) (Transformation|GetWorldLocation (Variables|Default|GetLadderEnd)) (Transformation|GetActorLocation Character)) (Transformation|GetActorRotation)) "AlwaysSpawn" 0 0))
  (Variables|/Game/Mordhau/Blueprints/Interactables/SiegeEngines/BP_LadderMover.BP_LadderMover_C|SetLadder _returnvalue self)
  (Class|MordhauVehicle|StartDriving _returnvalue Character))

(fn ConstructionScript
  (bind _droppedmesh (Variables|Default|GetDroppedMesh))
  (|CallParentFunction)
  (if (Variables|Default|GetCanDropAndRaise)
    (Components|StaticMesh|SetStaticMesh _droppedmesh (Variables|/Script/Engine.StaticMeshComponent|GetStaticMesh (Variables|Default|GetLadderMesh)))
    (else
      (Components|StaticMesh|SetStaticMesh _droppedmesh 0))))

(fn CanInteract
  (params (Character :type Mordhau%20Character%20Object%20Reference))
  (bind _returnvalue (Transformation|GetActorLocation Character))
  (bind _returnvalue_2 (|CallParentFunction Character))
  (Utilities|IsValid Character
    (:Is%20Valid
      (if (== (Variables|Default|GetLadderState) 0)
        (if (Variables|/Script/Mordhau.MordhauCharacter|GetbAllowVehicles Character)
          (if _returnvalue_2
            (if (Class|MordhauCharacter|IsLocallyControlledIncludingVehicle Character)
              (if (> (.Z (Math|Vector|BreakVector _returnvalue)) (- (.Z (Math|Vector|BreakVector (Transformation|GetWorldLocation (Variables|Default|GetLadderEnd)))) 75.0))
                _
                (else
                  (return (< (.X (Math|Vector|BreakVector (Math|Transform|InverseTransformLocation (Transformation|GetActorTransform) _returnvalue))) 1e+01)))))
            (return true)
            (else
              _))))
      (return false))
    (:Is%20Not%20Valid
      (return _returnvalue_2))))

(fn CanHeldInteract
  (params (Character :type Mordhau%20Character%20Object%20Reference))
  (if (> (Utilities|Array|Length (Variables|Default|GetMovers)) 0)
    (return false)
    (else
      (return (|CallParentFunction Character)))))

(fn OnRepLadderState
  (bind _returnvalue (Utilities|Time|GetTimeSeconds))
  (bind _returnvalue_2 (< _returnvalue 5.0))
  (Utilities|FlowControl|Sequence
    (:then_0
      (CallFunction|UpdateInteractionText))
    (:then_1
      (Utilities|FlowControl|Sequence
        (:then_0
          (if _returnvalue_2
            (Variables|Default|SetLadderStateChangeTime -1e+03)
            (else
              (Variables|Default|SetLadderStateChangeTime _returnvalue))))
        (:then_1
          (CallFunction|BeginAnimatingLadder (not _returnvalue_2)))))))

(fn UpdateInteractionText
  (if (== (Variables|Default|GetLadderState) 0)
    (Variables|Default|SetHeldInteractionText "Drop")
    (else
      (Variables|Default|SetHeldInteractionText "Raise"))))