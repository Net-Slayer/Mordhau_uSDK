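; BP_ProgressFire is a siege engine fire spot that stays dormant until its ActivateSpot event is triggered.
; Activation starts the fire, flare, smoke and extra particle components, spawns a BP_EnvFireField at the fire's transform and plays a fire sound there.
; A SpotActive flag makes activation one-shot, and this graph has no logic to turn it off.
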(event Custom|ActivateSpot
  (bind _fire (Variables|Default|GetFire))
  (bind _returnvalue (Transformation|GetWorldTransform _fire))
  (if (not (Variables|Default|GetSpotActive))
    (Components|Activation|Activate _fire false)
    (Game|SpawnActorfromClass "/Game/Mordhau/Blueprints/Fields/BP_EnvFireField.BP_EnvFireField_C" _returnvalue "Undefined" 0 0)
    (Audio|PlaySoundatLocation "/Game/StarterContent/Audio/Fire01_Cue.Fire01_Cue" (.Location (Math|Transform|BreakTransform _returnvalue)) "0, 0, 0" 0.5 1.0 0.0 0 0 0)
    (Variables|Default|SetSpotActive true)))

(event EventBeginPlay)

(event Collision|EventActorBeginOverlap
  (params (OtherActor :type Actor%20Object%20Reference)))

(event EventTick
  (params (DeltaSeconds :type Float%20%28single-precision%29)))

(fn ConstructionScript)