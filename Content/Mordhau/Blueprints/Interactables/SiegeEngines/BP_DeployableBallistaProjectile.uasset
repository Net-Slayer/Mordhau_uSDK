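; Projectile fired by the deployable ballista that can grant assist score to the ballista's builder when it kills a character.
; On kill, the server traces the projectile's creator to the ballista and its Builder.
; As wired, the builder receives assist score, scaled by the game mode, only if friendly checks pass for both builder-to-shooter and shooter-to-victim.
; Parent kill handling runs afterward.
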(event EventOnUsedtoKillOther
  (params (Character :type Advanced%20Character%20Object%20Reference) (Type :type EMordhauDamageType%20Enum :default "Generic") (SubType :type Byte :default 0) (bone :type Name%20%28by%20ref%29 :default "None") (Point :type Vector%20%28by%20ref%29 :default "0, 0, 0") (Source :type Actor%20Object%20Reference))
  (Utilities|FlowControl|Sequence
    (:then_0
      (Networking|SwitchHasAuthority
        (:Authority
          (bind _asmordhau_character (Utilities|Casting|CastToMordhauCharacter Character))
          (bind _returnvalue (Class|MordhauProjectile|GetProjectileOwningController))
          (Utilities|IsValid _returnvalue
            (:Is%20Valid
              (bind _returnvalue_2 (Class|MordhauProjectile|GetProjectileCreator))
              (bind _asbp_deployable_ballista (Utilities|Casting|CastToBP_DeployableBallista _returnvalue_2))
              (Utilities|IsValid (Variables|/Game/Mordhau/Blueprints/Interactables/SiegeEngines/BP_DeployableBallista.BP_DeployableBallista_C|GetBuilder _asbp_deployable_ballista)
                (:Is%20Valid
                  (bind _asmordhau_game_state (Utilities|Casting|CastToMordhauGameState (Game|GetGameState)))
                  (bind _returnvalue_3 (Class|MordhauGameState|IsFriendly _asmordhau_game_state (Variables|/Game/Mordhau/Blueprints/Interactables/SiegeEngines/BP_DeployableBallista.BP_DeployableBallista_C|GetBuilder _asbp_deployable_ballista) _returnvalue))
                  (if _returnvalue_3
                    (bind _returnvalue_4 (Class|MordhauGameState|IsFriendly _asmordhau_game_state _returnvalue _asmordhau_character))
                    (if _returnvalue_4
                      (bind _asmordhau_game_mode (Utilities|Casting|CastToMordhauGameMode (Game|GetGameMode)))
                      (Class|MordhauPlayerController|ClientReceiveScoreBP (Variables|/Game/Mordhau/Blueprints/Interactables/SiegeEngines/BP_DeployableBallista.BP_DeployableBallista_C|GetBuilder _asbp_deployable_ballista) "Assist" 0 (* (Variables|/Script/Mordhau.MordhauGameMode|GetAssistScoreFactor _asmordhau_game_mode) 5e+01)))))))))))
    (:then_1
      (|CallParentFunction Character Type SubType bone Point Source))))

(fn ConstructionScript
  (|CallParentFunction))