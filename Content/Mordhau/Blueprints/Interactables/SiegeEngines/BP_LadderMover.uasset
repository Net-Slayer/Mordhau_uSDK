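; Driveable mover that carries a character along a siege ladder, moving on a line between the ladder's start and end via OneDimensionalMovementComponent.
; It feeds look, turn and climb distance into character animation and first-person camera, and forwards equipment, melee and ranged input to the driver.
; Exiting near the top uses LadderExit; jumping off launches the driver along the turned heading, and the server expires the mover once driving stops.
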(event Custom|RequestJumpOff
  (CallFunction|PerformJumpoff))

(event EventOnStepChanged
  (bind _driver (Variables|Default|GetDriver))
  (|CallParentFunction)
  (Utilities|IsValid _driver
    (:Is%20Valid
      (Class|AdvancedCharacter|PlayCharacterSound _driver "/Game/Mordhau/Audio/Cues/Footsteps/SC_LadderStep.SC_LadderStep" "Hips" (Math|Vector|MakeVector 0.0 0.0 0.0) "SnapToTarget" true 0 1.0 1.0))))

(event EventKnockOffDriver
  (params (Character :type Mordhau%20Character%20Object%20Reference))
  (Class|AdvancedCharacter|Trip Character)
  (Class|AdvancedCharacter|Knockback Character (* (Math|Conversions|ToVector(Vector2D) (Math|Vector2D|Normalize2D (Math|Conversions|ToVector2D(Vector) (Transformation|GetActorForwardVector)))) -1.75e+03)))

(event EventDestroyed
  (bind _ladder (Variables|Default|GetLadder))
  (Utilities|FlowControl|Sequence
    (:then_0
      (Utilities|IsValid _ladder
        (:Is%20Valid
          (Utilities|Array|RemoveItem (Variables|/Game/Mordhau/Blueprints/Interactables/SiegeEngines/BP_Ladder.BP_Ladder_C|GetMovers _ladder) self))))
    (:then_1
      (|CallParentFunction))))

(event EventBeginPlay)

(event EventActorBeginOverlap
  (params (OtherActor :type Actor%20Object%20Reference)))

(event EventOnStoppedDriving
  (params (Character :type Mordhau%20Character%20Object%20Reference))
  (Networking|SwitchHasAuthority
    (:Authority
      (Actor|SetLifeSpan 0.5))))

(event EventOnDriverChanged
  (bind _driver (Variables|Default|GetDriver))
  (|CallParentFunction)
  (Utilities|IsValid _driver
    (:Is%20Valid
      (Variables|Default|SetLastDriver _driver))))

(event EventUpdateAnimationfor
  (params (Character :type Mordhau%20Character%20Object%20Reference) (AnimInst :type Mordhau%20Anim%20Instance%20Object%20Reference) (DeltaTime :type Float%20%28single-precision%29))
  (|CallParentFunction Character AnimInst DeltaTime)
  (bind _asab_mordhau_character_animation (Utilities|Casting|CastToAB_MordhauCharacterAnimation AnimInst))
  (Variables|/Script/Mordhau.MordhauAnimInstance|SetVehicleTurn _asab_mordhau_character_animation (Variables|Default|GetSecondaryTurnValue))
  (Variables|/Script/Mordhau.MordhauAnimInstance|SetVehicleLookUp _asab_mordhau_character_animation (Variables|Default|GetLookUpValue))
  (Variables|/Script/Mordhau.MordhauAnimInstance|SetVehicleVelocity _asab_mordhau_character_animation (Math|Vector|VectorLength (- (Transformation|GetWorldLocation (Variables|Character|GetMesh)) (Transformation|GetWorldLocation (Variables|/Game/Mordhau/Blueprints/Interactables/SiegeEngines/BP_Ladder.BP_Ladder_C|GetLadderStart (Variables|Default|GetLadder)))))))

(event EventUpdateFPCamerafor
  (params (Character :type Mordhau%20Character%20Object%20Reference) (DeltaSeconds :type Float%20%28single-precision%29) (bRotationOnly :type Boolean))
  (|CallParentFunction Character DeltaSeconds bRotationOnly)
  (Class|MordhauCharacter|UpdateFPCamera Character DeltaSeconds (Variables|Default|GetLookUpValue) bRotationOnly (Math|Rotator|MakeRotator 0.0 0.0 (Variables|Default|GetSecondaryTurnValue))))

(event Input|ActionEvents|InputActionJump
  (params (Key :type Key%20Structure))
  (:Pressed
    (if (not (Variables|Default|GetRequestedJump))
      (Variables|Default|SetRequestedJump true)
      (Utilities|FlowControl|Sequence
        (:then_1
          (CallFunction|RequestJumpOff))))))

(event Input|ActionEvents|InputActionCycleCamera
  (params (Key :type Key%20Structure)))

(event Input|AxisEvents|InputAxisLookUp
  (params (AxisValue :type Float%20%28single-precision%29))
  (Class|AdvancedCharacter|LookUp AxisValue false))

(event Input|AxisEvents|InputAxisTurnRight
  (params (AxisValue :type Float%20%28single-precision%29))
  (Class|MordhauVehicle|SecondaryTurn AxisValue false))

(fn ConstructionScript
  (|CallParentFunction))

(fn OnRepLadder
  (bind _ladder (Variables|Default|GetLadder))
  (bind _ladder_2 (Variables|Default|GetLadder))
  (Utilities|IsValid _ladder
    (:Is%20Valid
      (Utilities|Array|AddUnique (Variables|/Game/Mordhau/Blueprints/Interactables/SiegeEngines/BP_Ladder.BP_Ladder_C|GetMovers _ladder) self)
      (bind _asone_dimensional_movement_component (Utilities|Casting|CastToOneDimensionalMovementComponent (Variables|Character|GetCharacterMovement)))
      (Utilities|IsValid _ladder_2
        (:Is%20Valid
          (Class|OneDimensionalMovementComponent|SetMovementLine _asone_dimensional_movement_component (Transformation|GetWorldLocation (Variables|/Game/Mordhau/Blueprints/Interactables/SiegeEngines/BP_Ladder.BP_Ladder_C|GetLadderStart _ladder_2)) (Transformation|GetWorldLocation (Variables|/Game/Mordhau/Blueprints/Interactables/SiegeEngines/BP_Ladder.BP_Ladder_C|GetLadderEnd _ladder_2)))
          (Collision|IgnoreActorwhenMoving (Variables|Default|GetCapsuleComponent) _ladder_2 true))))))

(fn GetExitTransform
  (bind _ladder (Variables|Default|GetLadder))
  (bind _returnvalue (|CallParentFunction))
  (Utilities|IsValid _ladder
    (:Is%20Valid
      (if (< (Math|Vector|VectorLength (- (Transformation|GetWorldLocation (Variables|/Game/Mordhau/Blueprints/Interactables/SiegeEngines/BP_Ladder.BP_Ladder_C|GetLadderEnd _ladder)) (Transformation|GetActorLocation))) 5e+01)
        (return (Math|Transform|MakeTransform (Transformation|GetWorldLocation (Variables|/Game/Mordhau/Blueprints/Interactables/SiegeEngines/BP_Ladder.BP_Ladder_C|GetLadderExit _ladder)) (.Rotation (Math|Transform|BreakTransform _returnvalue)) (.Scale (Math|Transform|BreakTransform _returnvalue))))
        (else
          _)))
    (:Is%20Not%20Valid
      _))
  (return (Math|Transform|MakeTransform (+ (* (Math|Vector|GetForwardVector (Transformation|GetActorRotation (Variables|Default|GetLadder))) -5e+01) (.Location (Math|Transform|BreakTransform _returnvalue))) (.Rotation (Math|Transform|BreakTransform _returnvalue)) (.Scale (Math|Transform|BreakTransform _returnvalue)))))

(fn OverrideAttackAngle
  (params (Motion :type Attack%20Motion%20Object%20Reference))
  (return -1.0))

(fn PerformJumpoff
  (bind _driver (Variables|Default|GetDriver))
  (bind _asone_dimensional_movement_component (Utilities|Casting|CastToOneDimensionalMovementComponent (Variables|Character|GetCharacterMovement)))
  (Utilities|IsValid _driver
    (:Is%20Valid
      (bind _output_get (LocalVariables|SetToBounce _driver))
      (bind _asmordhau_movement_component (Utilities|Casting|CastToMordhauMovementComponent (Pawn|GetMovementComponent _output_get)))
      (LocalVariables|SetDirection (Math|Rotator|MakeRotator 0.0 0.0 (+ (Variables|Default|GetSecondaryTurnValue) (.Yaw (Math|Rotator|BreakRotator (Transformation|GetActorRotation))))))
      (Class|MordhauVehicle|StopDriving)
      (Utilities|IsValid _output_get
        (:Is%20Valid
          (if (not (Class|AdvancedCharacter|GetIsDead _output_get))
            (Character|LaunchCharacter _output_get (Math|Vector|RotateVector (* (Math|Vector|MakeVector (* (Math|Float|MapRangeClamped (Variables|/Script/Mordhau.MordhauMovementComponent|GetMaxSpeedFalling _asmordhau_movement_component) 3e+02 999.0 1.0 0.333) 7.5e+02) 0.0 5e+02) (- 1.0 (* (Math|Conversions|ToFloat(Boolean) (<= (- (Variables|/Script/Mordhau.OneDimensionalMovementComponent|GetTotalSteps _asone_dimensional_movement_component) (Variables|/Script/Mordhau.OneDimensionalMovementComponent|GetCurrentStep _asone_dimensional_movement_component)) 0)) 0.66))) (LocalVariables|GetDirection)) false false)
            (Variables|Default|SetReplicatedLadderJump true)))))))

(fn OnRepReplicatedLadderJump
  (bind _lastdriver (Variables|Default|GetLastDriver))
  (Utilities|IsValid _lastdriver
    (:Is%20Valid
      (if (not (Class|AdvancedCharacter|GetIsDead _lastdriver))
        (bind _asab_mordhau_character_animation (Utilities|Casting|CastToAB_MordhauCharacterAnimation (Components|SkeletalMesh|GetAnimInstance (Variables|/Script/Engine.Character|GetMesh _lastdriver))))
        (Default|AnimNotifyGroundtoJumped _asab_mordhau_character_animation)))))

(event Input|ActionEvents|InputActionHolster
  (params (Key :type Key%20Structure))
  (bind _driver (Variables|Default|GetDriver))
  ;[1 1 1] Equipment
  (:Pressed
    (Utilities|IsValid _driver
      (:Is%20Valid
        (Class|MordhauCharacter|EmptyHands _driver)))))

(event Input|ActionEvents|InputActionDrop
  (params (Key :type Key%20Structure))
  (bind _driver (Variables|Default|GetDriver))
  ;[1 1 1] Equipment
  (:Pressed
    (Utilities|IsValid _driver
      (:Is%20Valid
        (Class|MordhauCharacter|RequestDrop _driver)))))

(event Input|ActionEvents|InputActionEquipSlot8
  (params (Key :type Key%20Structure))
  (bind _driver (Variables|Default|GetDriver))
  ;[1 1 1] Equipment
  (:Pressed
    (Utilities|IsValid _driver
      (:Is%20Valid
        (Class|MordhauCharacter|EquipSlot8 _driver)))))

(event Input|ActionEvents|InputActionEquipSlot9
  (params (Key :type Key%20Structure))
  (bind _driver (Variables|Default|GetDriver))
  ;[1 1 1] Equipment
  (:Pressed
    (Utilities|IsValid _driver
      (:Is%20Valid
        (Class|MordhauCharacter|EquipSlot9 _driver)))))

(event Input|ActionEvents|InputActionPreviousEquipment
  (params (Key :type Key%20Structure))
  (bind _driver (Variables|Default|GetDriver))
  ;[1 1 1] Equipment
  (:Pressed
    (Utilities|IsValid _driver
      (:Is%20Valid
        (Class|MordhauCharacter|PreviousEquipmentPressed _driver))))
  (:Released
    (Utilities|IsValid _driver
      (:Is%20Valid
        (Class|MordhauCharacter|PreviousEquipmentReleased _driver)))))

(event Input|ActionEvents|InputActionEquipSlot1
  (params (Key :type Key%20Structure))
  (bind _driver (Variables|Default|GetDriver))
  ;[1 1 1] Equipment
  (:Pressed
    (Utilities|IsValid _driver
      (:Is%20Valid
        (Class|MordhauCharacter|EquipSlot1 _driver)))))

(event Input|ActionEvents|InputActionWeaponMode/Reload
  (params (Key :type Key%20Structure))
  (bind _driver (Variables|Default|GetDriver))
  ;[1 1 1] Equipment
  (:Pressed
    (Utilities|IsValid _driver
      (:Is%20Valid
        (Class|MordhauCharacter|RequestToggleWeaponMode _driver)))))

(event Input|ActionEvents|InputActionEquipSlot2
  (params (Key :type Key%20Structure))
  (bind _driver (Variables|Default|GetDriver))
  ;[1 1 1] Equipment
  (:Pressed
    (Utilities|IsValid _driver
      (:Is%20Valid
        (Class|MordhauCharacter|EquipSlot2 _driver)))))

(event Input|ActionEvents|InputActionEquipSlot3
  (params (Key :type Key%20Structure))
  (bind _driver (Variables|Default|GetDriver))
  ;[1 1 1] Equipment
  (:Pressed
    (Utilities|IsValid _driver
      (:Is%20Valid
        (Class|MordhauCharacter|EquipSlot3 _driver)))))

(event Input|ActionEvents|InputActionNextEquipment
  (params (Key :type Key%20Structure))
  (bind _driver (Variables|Default|GetDriver))
  ;[1 1 1] Equipment
  (:Pressed
    (Utilities|IsValid _driver
      (:Is%20Valid
        (Class|MordhauCharacter|NextEquipmentPressed _driver))))
  (:Released
    (Utilities|IsValid _driver
      (:Is%20Valid
        (Class|MordhauCharacter|NextEquipmentReleased _driver)))))

(event Input|ActionEvents|InputActionEquipSlot4
  (params (Key :type Key%20Structure))
  (bind _driver (Variables|Default|GetDriver))
  ;[1 1 1] Equipment
  (:Pressed
    (Utilities|IsValid _driver
      (:Is%20Valid
        (Class|MordhauCharacter|EquipSlot4 _driver)))))

(event Input|ActionEvents|InputActionEquipSlot5
  (params (Key :type Key%20Structure))
  (bind _driver (Variables|Default|GetDriver))
  ;[1 1 1] Equipment
  (:Pressed
    (Utilities|IsValid _driver
      (:Is%20Valid
        (Class|MordhauCharacter|EquipSlot5 _driver)))))

(event Input|ActionEvents|InputActionEquipSlot6
  (params (Key :type Key%20Structure))
  (bind _driver (Variables|Default|GetDriver))
  ;[1 1 1] Equipment
  (:Pressed
    (Utilities|IsValid _driver
      (:Is%20Valid
        (Class|MordhauCharacter|EquipSlot6 _driver)))))

(event Input|ActionEvents|InputActionEquipSlot7
  (params (Key :type Key%20Structure))
  (bind _driver (Variables|Default|GetDriver))
  ;[1 1 1] Equipment
  (:Pressed
    (Utilities|IsValid _driver
      (:Is%20Valid
        (Class|MordhauCharacter|EquipSlot7 _driver)))))

(event Input|ActionEvents|InputActionLeftStab
  (params (Key :type Key%20Structure))
  (bind _driver (Variables|Default|GetDriver))
  ;[1 1 1] Melee combat
  (:Pressed
    (Utilities|IsValid _driver
      (:Is%20Valid
        (Class|MordhauCharacter|RequestLeftStab _driver)))))

(event Input|ActionEvents|InputActionFlipAttackSide
  (params (Key :type Key%20Structure))
  (bind _driver (Variables|Default|GetDriver))
  (bind _driver_2 (Variables|Default|GetDriver))
  ;[1 1 1] Melee combat
  (:Pressed
    (Utilities|IsValid _driver
      (:Is%20Valid
        (Class|MordhauCharacter|FlipAttackSidePressed _driver))))
  (:Released
    (Utilities|IsValid _driver_2
      (:Is%20Valid
        (Class|MordhauCharacter|FlipAttackSideReleased _driver_2)))))

(event Input|ActionEvents|InputActionFeint
  (params (Key :type Key%20Structure))
  (bind _driver (Variables|Default|GetDriver))
  ;[1 1 1] Melee combat
  (:Pressed
    (Utilities|IsValid _driver
      (:Is%20Valid
        (Class|MordhauCharacter|RequestFeint _driver)))))

(event Input|ActionEvents|InputActionStab
  (params (Key :type Key%20Structure))
  (bind _driver (Variables|Default|GetDriver))
  (bind _driver_2 (Variables|Default|GetDriver))
  ;[1 1 1] Melee combat
  (:Pressed
    (Utilities|IsValid _driver_2
      (:Is%20Valid
        (Class|MordhauCharacter|ListenforStab360 _driver_2))))
  (:Released
    (Utilities|IsValid _driver
      (:Is%20Valid
        (Class|MordhauCharacter|StopListenforStab360 _driver)))))

(event Input|ActionEvents|InputActionLeftUpperStrike
  (params (Key :type Key%20Structure))
  (bind _driver (Variables|Default|GetDriver))
  ;[1 1 1] Melee combat
  (:Pressed
    (Utilities|IsValid _driver
      (:Is%20Valid
        (Class|MordhauCharacter|RequestLeftUpperStrike _driver)))))

(event Input|ActionEvents|InputActionParry
  (params (Key :type Key%20Structure))
  (bind _driver (Variables|Default|GetDriver))
  ;[1 1 1] Melee combat
  (:Pressed
    (Utilities|IsValid _driver
      (:Is%20Valid
        (Class|MordhauCharacter|BlockPressed _driver))))
  (:Released
    (Utilities|IsValid _driver
      (:Is%20Valid
        (Class|MordhauCharacter|BlockReleased _driver)))))

(event Input|ActionEvents|InputActionFeintOrParry
  (params (Key :type Key%20Structure))
  (bind _driver (Variables|Default|GetDriver))
  ;[1 1 1] Melee combat
  (:Pressed
    (Utilities|IsValid _driver
      (:Is%20Valid
        (Class|MordhauCharacter|FeintorBlockPressed _driver))))
  (:Released
    (Utilities|IsValid _driver
      (:Is%20Valid
        (Class|MordhauCharacter|FeintorBlockReleased _driver)))))

(event Input|ActionEvents|InputActionRightUpperStrike
  (params (Key :type Key%20Structure))
  (bind _driver (Variables|Default|GetDriver))
  ;[1 1 1] Melee combat
  (:Pressed
    (Utilities|IsValid _driver
      (:Is%20Valid
        (Class|MordhauCharacter|RequestRightUpperStrike _driver)))))

(event Input|ActionEvents|InputActionRightLowerStrike
  (params (Key :type Key%20Structure))
  (bind _driver (Variables|Default|GetDriver))
  ;[1 1 1] Melee combat
  (:Pressed
    (Utilities|IsValid _driver
      (:Is%20Valid
        (Class|MordhauCharacter|RequestRightLowerStrike _driver)))))

(event Input|ActionEvents|InputActionRightStrike
  (params (Key :type Key%20Structure))
  (bind _driver (Variables|Default|GetDriver))
  ;[1 1 1] Melee combat
  (:Pressed
    (Utilities|IsValid _driver
      (:Is%20Valid
        (Class|MordhauCharacter|RequestRightStrike _driver)))))

(event Input|ActionEvents|InputActionStrike
  (params (Key :type Key%20Structure))
  (bind _driver (Variables|Default|GetDriver))
  (bind _driver_2 (Variables|Default|GetDriver))
  ;[1 1 1] Melee combat
  (:Pressed
    (Utilities|IsValid _driver_2
      (:Is%20Valid
        (Class|MordhauCharacter|ListenforStrike360 _driver_2))))
  (:Released
    (Utilities|IsValid _driver
      (:Is%20Valid
        (Class|MordhauCharacter|StopListenforStrike360 _driver)))))

(event Input|ActionEvents|InputActionRightStab
  (params (Key :type Key%20Structure))
  (bind _driver (Variables|Default|GetDriver))
  ;[1 1 1] Melee combat
  (:Pressed
    (Utilities|IsValid _driver
      (:Is%20Valid
        (Class|MordhauCharacter|RequestRightStab _driver)))))

(event Input|ActionEvents|InputActionLeftLowerStrike
  (params (Key :type Key%20Structure))
  (bind _driver (Variables|Default|GetDriver))
  ;[1 1 1] Melee combat
  (:Pressed
    (Utilities|IsValid _driver
      (:Is%20Valid
        (Class|MordhauCharacter|RequestLeftLowerStrike _driver)))))

(event Input|ActionEvents|InputActionLeftStrike
  (params (Key :type Key%20Structure))
  (bind _driver (Variables|Default|GetDriver))
  ;[1 1 1] Melee combat
  (:Pressed
    (Utilities|IsValid _driver
      (:Is%20Valid
        (Class|MordhauCharacter|RequestLeftStrike _driver)))))

(event Input|ActionEvents|InputActionRangedCancel
  (params (Key :type Key%20Structure))
  (bind _driver (Variables|Default|GetDriver))
  ;[1 1 1] Ranged
  (:Pressed
    (Utilities|IsValid _driver
      (:Is%20Valid
        (Class|MordhauCharacter|RequestRangedCancel _driver)))))

(event Input|ActionEvents|InputActionFire
  (params (Key :type Key%20Structure))
  (bind _driver (Variables|Default|GetDriver))
  (bind _driver_2 (Variables|Default|GetDriver))
  ;[1 1 1] Ranged
  (:Pressed
    (Utilities|IsValid _driver
      (:Is%20Valid
        (Class|MordhauCharacter|FirePressed _driver))))
  (:Released
    (Utilities|IsValid _driver_2
      (:Is%20Valid
        (Class|MordhauCharacter|FireReleased _driver_2)))))