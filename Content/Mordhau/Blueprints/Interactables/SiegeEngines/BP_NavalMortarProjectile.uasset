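; Explosive shell projectile for the naval mortar siege engine, with its behavior defined in the hit handler.
; Hits after a half-second arming time shake nearby cameras and apply server-side radial damage with knockback, ragdoll and flat structure damage.
; Earlier hits act as duds, stripping impact sound, decals and all but the wet-surface particle, and keeping the shell from being destroyed on termination.
; Both paths hide the spark and call the parent hit logic.
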(event EventOnProjectileHit
  (params (HitLocation :type Vector%20%28by%20ref%29 :default "0, 0, 0") (HitNormal :type Vector%20%28by%20ref%29 :default "0, 0, 0") (BounceForce :type Float%20%28single-precision%29) (Surface :type Byte :default 0) (bHasHitWorld :type Boolean) (bHasStopped :type Boolean))
  (bind _surfaceimpactparticles (Variables|Default|GetSurfaceImpactParticles))
  (Development|SetHiddeninGame (Variables|Default|GetP_ExplosiveSpark) true false)
  (if (> (Actor|GetGameTimeSinceCreation) 0.5)
    (Utilities|FlowControl|Sequence
      (:then_0
        (Camera|PlayWorldCameraShake "/Game/Mordhau/Blueprints/CameraShakes/ImpactShake.ImpactShake_C" HitLocation 5e+02 5e+03 1e+01))
      (:then_1
        (Networking|SwitchHasAuthority
          (:Authority
            (bind _returnvalue (Class|MordhauProjectile|GetProjectileOwningController))
            (Class|MordhauUtilityLibrary|MordhauApplyRadialDamagewithFalloff 0 2e+03 1.0 7.2e+02 7.2e+02 HitLocation 2e+02 9e+02 5.0 0 1e+03 5e+02 8e+02 self _returnvalue "ECC_WorldStatic" false))))
      (:then_2
        (|CallParentFunction HitLocation HitNormal BounceForce Surface bHasHitWorld bHasStopped :!label _label)))
    (else
      (Variables|Default|SetImpactSound 0)
      (Utilities|Map|Clear (Variables|Default|GetSurfaceImpactDecals))
      (bind _output_get (Variables|Default|SetWetParticleTemp (.Value (Utilities|Map|Find _surfaceimpactparticles "SurfaceType8"))))
      (Utilities|Map|Clear _surfaceimpactparticles)
      (Utilities|Map|Add _surfaceimpactparticles "SurfaceType8" _output_get)
      (Variables|Default|SetbDestroyWhenTerminated false)
      (goto _label))))

(fn ConstructionScript
  (|CallParentFunction))