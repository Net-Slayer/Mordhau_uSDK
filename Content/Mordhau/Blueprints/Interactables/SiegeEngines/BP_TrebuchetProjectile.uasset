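; Projectile fired by the trebuchet siege engine, extending its parent projectile's hit handling with an area impact and fire.
; On hit it plays a distance-scaled camera shake and, on authority only, deals falloff radial damage to targets and structures with knockback, credited to the owning controller.
; It then spawns a BP_FireField at the hit location, outside the authority check, before calling the parent hit logic.
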(event EventTick
  (params (DeltaSeconds :type Float%20%28single-precision%29)))

(event EventOnProjectileHit
  (params (HitLocation :type Vector%20%28by%20ref%29 :default "0, 0, 0") (HitNormal :type Vector%20%28by%20ref%29 :default "0, 0, 0") (BounceForce :type Float%20%28single-precision%29) (Surface :type Byte :default 0) (bHasHitWorld :type Boolean) (bHasStopped :type Boolean))
  (Utilities|FlowControl|Sequence
    (:then_0
      (Camera|PlayWorldCameraShake "/Game/Mordhau/Blueprints/CameraShakes/ImpactShake.ImpactShake_C" HitLocation 5e+02 1.5e+04 1e+01))
    (:then_1
      (Networking|SwitchHasAuthority
        (:Authority
          (bind _returnvalue (Class|MordhauProjectile|GetProjectileOwningController))
          (Class|MordhauUtilityLibrary|MordhauApplyRadialDamagewithFalloff 0 2.5e+03 1.0 4e+02 2e+01 HitLocation 8e+01 3.4e+02 5.0 0 1e+03 5e+02 3e+02 self _returnvalue "ECC_WorldStatic" false))))
    (:then_2
      (Game|SpawnActorfromClass "/Game/Mordhau/Blueprints/Fields/BP_FireField.BP_FireField_C" (Math|Transform|MakeTransform HitLocation) "AlwaysSpawn" 0 0))
    (:then_3
      (|CallParentFunction HitLocation HitNormal BounceForce Surface bHasHitWorld bHasStopped))))

(fn ConstructionScript
  (|CallParentFunction))