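; BP_DetailedTrebuchet is a trebuchet siege engine child Blueprint that adds a trail effect and launches characters standing on it when fired.
; Construction snaps the trail component to the skeletal mesh's Rope6 socket, and Fire activates it for one second.
; On the authority, Fire also knocks living characters overlapping its Box along the mesh's forward vector, ragdolling those not in a vehicle.
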(event EventBeginPlay
  (|CallParentFunction))

(event Collision|EventActorBeginOverlap
  (params (OtherActor :type Actor%20Object%20Reference)))

(event EventTick
  (params (DeltaSeconds :type Float%20%28single-precision%29)))

(event EventFire
  (bind _p_trebuchettrail (Variables|Default|GetP_TrebuchetTrail))
  (|CallParentFunction)
  (Utilities|FlowControl|Sequence
    (:then_0
      (Networking|SwitchHasAuthority
        (:Authority
          (CallFunction|RagdollThoseStanding))))
    (:then_1
      (Components|Activation|Activate _p_trebuchettrail false)
      (Utilities|FlowControl|Delay 1.0)
      (Components|Activation|Deactivate _p_trebuchettrail))))

(fn ConstructionScript
  (|CallParentFunction)
  (Transformation|AttachComponentToComponent (Variables|Default|GetP_TrebuchetTrail) (Variables|Default|GetSkeletalMesh) "Rope6" "SnapToTarget" "SnapToTarget" "KeepRelative" true))

(fn RagdollThoseStanding
  (bind _output_get (LocalVariables|SetStanders (Collision|GetOverlappingActors (Variables|Default|GetBox) "/Script/Mordhau.AdvancedCharacter" :!class /Script/Engine.PrimitiveComponent)))
  (for _array_element _output_get
    (Utilities|IsValid _array_element
      (:Is%20Valid
        (bind _asadvanced_character (Utilities|Casting|CastToAdvancedCharacter _array_element))
        (if (not (Class|AdvancedCharacter|GetIsDead _asadvanced_character))
          (Class|AdvancedCharacter|Knockback _asadvanced_character (* (Math|Vector|GetForwardVector (Variables|Default|GetSkeletalMesh)) 2.5e+03))
          (bind _asmordhau_character (Utilities|Casting|CastToMordhauCharacter _asadvanced_character))
          (Utilities|IsValid (Variables|/Script/Mordhau.MordhauCharacter|GetCurrentVehicle _asmordhau_character)
            (:Is%20Not%20Valid
              (if (not (Variables|/Script/Mordhau.AdvancedCharacter|GetbIsRagdollFalling _asmordhau_character))
                (Class|AdvancedCharacter|SetIsRagdollFalling _asmordhau_character true)))))))))