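; Base vehicle spawner interactable that attempts a server-side spawn on BeginPlay while Active.
; SpawnVehicle is an empty event here, so this file contains no actual spawn logic.
; Deactivate clears Active and, if DestroyVehicleOnDeactivate is set, kills the living SpawnedVehicle with massive damage on authority.
; Activate sets Active to false rather than true before calling TrySpawnVehicle, so as written it never triggers a spawn.
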(event Custom|SpawnVehicle)

(event EventBeginPlay
  (CallFunction|TrySpawnVehicle))

(event Collision|EventActorBeginOverlap
  (params (OtherActor :type Actor%20Object%20Reference)))

(event EventTick
  (params (DeltaSeconds :type Float%20%28single-precision%29)))

(fn ConstructionScript)

(fn Deactivate
  (bind _spawnedvehicle (Variables|Default|GetSpawnedVehicle))
  (if (Variables|Default|GetActive)
    (Variables|Default|SetActive false)
    (Networking|SwitchHasAuthority
      (:Authority
        (if (Variables|Default|GetDestroyVehicleOnDeactivate)
          (Utilities|IsValid _spawnedvehicle
            (:Is%20Valid
              (if (not (Class|AdvancedCharacter|GetIsDead _spawnedvehicle))
                (Game|Damage|ApplyDamage _spawnedvehicle 1e+09 0 0)))))))))

(fn TrySpawnVehicle
  (Networking|SwitchHasAuthority
    (:Authority
      (if (Variables|Default|GetActive)
        (CallFunction|SpawnVehicle)))))

(fn Activate
  (if (not (Variables|Default|GetActive))
    (Variables|Default|SetActive false)
    (CallFunction|TrySpawnVehicle)))