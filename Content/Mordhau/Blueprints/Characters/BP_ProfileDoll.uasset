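; BP_ProfileDoll is a display character that shows one of the player's saved or default profiles, chosen by ProfileID, in a preview pose.
; Once the HUD reports the singleton loaded, Tick triggers a one-time, authority-only Reroll that applies the profile with equipment and a random pose.
; Reroll hides the mesh, and Tick reveals it two frames later.
; An optional looping curve drives the mesh's spin.
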(event Custom|Reroll
  (bind _returnvalue (Class|MordhauUtilityLibrary|GetMordhauSingleton))
  (bind _profileid (Variables|Default|GetProfileID))
  (bind _characterprofiles (Variables|/Script/Mordhau.MordhauSingleton|GetCharacterProfiles _returnvalue))
  (Networking|SwitchHasAuthority
    (:Authority
      (bind _asbp_mordhau_singleton (Utilities|Casting|CastToBP_MordhauSingleton _returnvalue))
      (if (and (== (Utilities|Array|Length _characterprofiles) 1) (Utilities|Enum|Equal(Enum) (Utilities|String|ToString(Text) (.Name (Utilities|Struct|BreakCharacterProfile (Utilities|Array|Get(acopy) _characterprofiles)))) "Unnamed"))
        (bind _output_get (Variables|Default|SetCurrentProfileStored (Utilities|Array|Get(acopy) (Variables|/Script/Mordhau.MordhauSingleton|GetDefaultProfiles _returnvalue) _profileid)))
        (else
          (Variables|Default|SetCurrentProfileStored (Utilities|Array|Get(acopy) _characterprofiles _profileid))))
      (Class|MordhauSingleton|ApplyProfileto _asbp_mordhau_singleton _output_get self 0 true)
      (Variables|Default|SetRerolledFrame (Class|MordhauUtilityLibrary|GetCurrentFrameBP))
      (Rendering|SetVisibility (Variables|Character|GetMesh) false true)
      (CallFunction|AssumePreviewPose (Math|Random|RandomInteger 1000)))))

(event EventTick
  (params (DeltaSeconds :type Float%20%28single-precision%29))
  (bind _spincurve (Variables|Default|GetSpinCurve))
  (|CallParentFunction DeltaSeconds)
  (Utilities|FlowControl|Sequence
    (:then_0
      (bind _asbp_mordhau_hud (Utilities|Casting|CastToBP_MordhauHUD (Class|MordhauUtilityLibrary|GetMordhauHUD)))
      (if (Variables|/Game/Mordhau/Blueprints/BP_MordhauHUD.BP_MordhauHUD_C|GetLoadedSingleton _asbp_mordhau_hud)
        (Utilities|FlowControl|Sequence
          (:then_0
            (Utilities|FlowControl|DoOnce false
              (:Completed
                (CallFunction|Reroll))))
          (:then_1
            (if (== (+ (Variables|Default|GetRerolledFrame) 2) (Class|MordhauUtilityLibrary|GetCurrentFrameBP))
              (Class|MordhauCharacter|ForceUpdateMeshVisibility)
              (Rendering|SetVisibility (Variables|Character|GetMesh) true true))))))
    (:then_1
      (Utilities|IsValid _spincurve
        (:Is%20Valid
          (Transformation|SetRelativeRotation (Variables|Character|GetMesh) (Math|Rotator|MakeRotator 0.0 0.0 (Math|Curves|GetFloatValue _spincurve (Math|Float|%(Float) (Utilities|Time|GetTimeSeconds) (Variables|Default|GetSpinDuration)))) false false))))))

(fn ConstructionScript
  (|CallParentFunction))