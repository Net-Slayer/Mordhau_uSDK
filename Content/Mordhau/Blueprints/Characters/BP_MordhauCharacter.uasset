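; Mordhau character Blueprint handling climbing, death physics and built-in combat equipment (kick, perk-dependent fists).
; Climbing finds ledges with staged capsule traces, or checks the AI's target, and sends the spot to a server range check.
; Death chooses ragdoll or animation using hit context and a synced random, applying mass-scaled impulses adjusted for prior velocity.
; It also adds dismemberment impulses, death sounds, blood pools and out-of-bounds warning text.
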(event OnThud(Thudder)
  (bind _thudder (Variables|Default|GetThudder))
  (Audio|SpawnSoundAttached "/Game/Mordhau/Audio/Cues/Foley/SC_BodyFall.SC_BodyFall" (Variables|Character|GetMesh) "Hips" "0, 0, 0" "0, 0, 0" "SnapToTarget" true (Math|Float|MapRangeClamped (- (Variables|/Script/Mordhau.ThudderComponent|GetPreviousVelocity _thudder) (Variables|/Script/Mordhau.ThudderComponent|GetCurrentVelocity _thudder)) 75.0 3e+02 0.75 1.0) 1.0 0.0 0 0)
  (if (Variables|Default|GetbIsDead)
    (CallFunction|SpawnBloodPoolUnderneath)))

(event Custom|ReplicatedTripWithKnockback
  (bind _returnvalue (Class|AdvancedCharacter|Trip))
  (if _returnvalue
    (Class|AdvancedCharacter|Knockback (* (Math|Conversions|ToVector(Vector2D) (Math|Vector2D|Normalize2D (Math|Conversions|ToVector2D(Vector) (Transformation|GetVelocity)))) 1.75e+03))))

(event Custom|ServerSetClimbLocation
  (params (NewParam :type Vector%20Net%20Quantize%20Structure))
  (bind _returnvalue (Transformation|GetActorLocation))
  (bind _output_get (Variables|Default|SetClimbTargetLocation NewParam))
  (Utilities|Casting|CastToMordhauAIController (Pawn|GetController)
    (:CastFailed
      (if (Math|Boolean|ORBoolean (> (Math|Float|Absolute(Float) (.X (Math|Vector|BreakVector (- _returnvalue _output_get)))) 2e+02) (> (Math|Float|Absolute(Float) (.Y (Math|Vector|BreakVector (- _returnvalue _output_get)))) 2e+02) (> (Math|Float|Absolute(Float) (.Z (Math|Vector|BreakVector (- _returnvalue _output_get)))) 5e+02))
        (Variables|Default|SetClimbTargetLocation _returnvalue)))))

(event Custom|DebugPossess
  (bind _asmordhau_player_controller (Utilities|Casting|CastToMordhauPlayerController (Game|GetPlayerController 0)))
  (Pawn|Possess _asmordhau_player_controller self))

(event EventOnPostProfileAssigned
  (|CallParentFunction)
  (CallFunction|GiveFists))

(event EventApplyRagdollForce
  (params (Angle :type Float%20%28single-precision%29) (Type :type EMordhauDamageType%20Enum :default "Generic") (SubType :type Byte :default 0) (bone :type Name%20%28by%20ref%29 :default "None") (Point :type Vector%20%28by%20ref%29 :default "0, 0, 0") (Source :type Actor%20Object%20Reference) (Agent :type Actor%20Object%20Reference))
  (bind _mesh (Variables|Character|GetMesh))
  (bind _movecompvelocitybeforedeath (Variables|Default|GetMoveCompVelocityBeforeDeath))
  (bind (_x _y _z) (Math|Vector|BreakVector _movecompvelocitybeforedeath))
  (bind _returnvalue (Class|SkinnedMeshComponent|GetParentBone _mesh bone))
  (bind _returnvalue_2 (Math|Float|Clamp(Float) _z -5e+02 0.0))
  (bind _returnvalue_3 (Math|Vector|MakeVector _x _y _returnvalue_2))
  (if (Class|SceneComponent|IsAnySimulatingPhysics _mesh)
    (bind _returnvalue_4 (Class|MordhauCharacter|IsBoneDismembered bone))
    (bind _force (CallFunction|ComputeRagdollForce Agent Type SubType (Variables|Default|GetDeathSyncedRandom) self))
    (Utilities|FlowControl|Sequence
      (:then_0
        (Class|SkeletalMeshComponent|AddImpulsetoAllBodiesBelow (Variables|Character|GetMesh) _returnvalue_3 "Hips" true true))
      (:then_1
        (if (or _returnvalue_4 (not (Physics|IsSimulatingPhysics _mesh bone)))
          (if (not (Physics|IsSimulatingPhysics _mesh _returnvalue))
            (CallFunction|AddRagdollImpulse (Math|Vector|ClampVectorSize (- _force (Math|Vector|ClampVectorSize (* (Math|Vector|ProjectVectorontoVector (* _returnvalue_3 15.0) _force) (Math|Conversions|ToFloat(Boolean) (< (Class|KismetMathLibrary|DegAcos (Math|Vector|DotProduct _returnvalue_3 _force)) 9e+01))) 0.0 (Math|Vector|VectorLength _force))) 0.0 1.5e+04) Point "Spine1")
            (else
              (CallFunction|AddRagdollImpulse (Math|Vector|ClampVectorSize (- _force (Math|Vector|ClampVectorSize (* (Math|Vector|ProjectVectorontoVector (* _returnvalue_3 15.0) _force) (Math|Conversions|ToFloat(Boolean) (< (Class|KismetMathLibrary|DegAcos (Math|Vector|DotProduct _returnvalue_3 _force)) 9e+01))) 0.0 (Math|Vector|VectorLength _force))) 0.0 1.5e+04) Point _returnvalue)))
          (else
            (CallFunction|AddRagdollImpulse (- _force (Math|Vector|ClampVectorSize (* (Math|Vector|ProjectVectorontoVector (* _returnvalue_3 15.0) _force) (Math|Conversions|ToFloat(Boolean) (< (Class|KismetMathLibrary|DegAcos (Math|Vector|DotProduct _returnvalue_3 _force)) 9e+01))) 0.0 (Math|Vector|VectorLength _force))) Point bone)))))))

(event EventOnPostDismember
  (params (bone :type Name%20%28by%20ref%29 :default "None") (SeparatedPart :type Separated%20Body%20Part%20Object%20Reference) (Agent :type Actor%20Object%20Reference))
  (bind _returnvalue (Transformation|GetActorRightVector SeparatedPart))
  (bind _mesh (Variables|Character|GetMesh))
  (bind _mesh_2 (Variables|/Script/Mordhau.SeparatedBodyPart|GetMesh SeparatedPart))
  (bind _queueddismemberforcedir (Variables|Default|GetQueuedDismemberForceDir))
  (bind _returnvalue_2 (* _returnvalue -1.0))
  (bind _returnvalue_3 (Math|Rotator|MakeRotfromXZ _queueddismemberforcedir _returnvalue_2))
  (bind _returnvalue_4 (Math|Rotator|CombineRotators "-90.000000, 0,0.000000" _returnvalue_3))
  (bind _returnvalue_5 (Class|KismetMathLibrary|NegateRotator _returnvalue_3))
  (bind _returnvalue_6 (Math|Rotator|CombineRotators _returnvalue_5 _returnvalue_4))
  (bind (_roll _pitch _yaw) (Math|Rotator|BreakRotator _returnvalue_6))
  (|CallParentFunction bone SeparatedPart Agent)
  (Utilities|FlowControl|Sequence
    (:then_0
      (if (Math|Boolean|ANDBoolean (Variables|Default|GetbQueuedDismemberIsPartial) (Utilities|Name|Equal(Name) bone "head") (not (Class|SceneComponent|IsAnySimulatingPhysics _mesh)))
        (Audio|SpawnSoundAttached "/Game/Mordhau/Audio/Cues/Foley/SC_DeathGurgle.SC_DeathGurgle" _mesh "Neck" "0, 0, 0" "0, 0, 0" "SnapToTarget" true 1.0 1.0 0.0 0 0)))
    (:then_1
      (if (not (or (Variables|Default|GetbQueuedDismemberIsPartial) (not (Class|SceneComponent|IsAnySimulatingPhysics _mesh_2))))
        (Physics|AddImpulse _mesh_2 (* _queueddismemberforcedir -1.5e+02) bone true)
        (Class|PrimitiveComponent|AddAngularImpulseinDegrees _mesh_2 (* (Math|Vector|MakeVector _roll _pitch _yaw) 1e+01) bone true)))))

(event EventBeginPlay
  (Variables|Default|SetBodyThudder (Variables|Default|GetThudder))
  (Components|Tick|SetComponentTickEnabled (Variables|Default|GetThudder) false)
  (bind _returnvalue (Game|SpawnActorfromClass (Variables|Default|GetKickClass) (Math|Transform|MakeTransform "0, 0, 0") "AlwaysSpawn" 0 0))
  (bind _output_get (Variables|Default|SetKickWeapon _returnvalue))
  (Transformation|AttachActorToActor _output_get self "None" "KeepWorld" "KeepWorld" "KeepWorld" false))

(event EventOnCosmeticHit
  (params (DamageType :type EMordhauDamageType%20Enum :default "Generic") (SubType :type Byte :default 0) (Hit :type Hit%20Result%20Structure%20%28by%20ref%29) (Agent :type Actor%20Object%20Reference))
  (bind (_bblockinghit _binitialoverlap _time _distance _location _impactpoint _normal _impactnormal _physmat _hitactor _hitcomponent _hitbonename) (Collision|BreakHitResult Hit))
  (|CallParentFunction DamageType SubType Hit Agent)
  (if (Class|SceneComponent|IsAnySimulatingPhysics (Variables|Character|GetMesh))
    (bind _returnvalue (Class|MordhauCharacter|IsBoneDismembered _hitbonename))
    (bind _force (CallFunction|ComputeRagdollForce Agent DamageType SubType 255 self))
    (if _returnvalue
      (CallFunction|AddRagdollImpulse (* _force 0.5) _impactpoint "Spine1")
      (else
        (CallFunction|AddRagdollImpulse _force _impactpoint _hitbonename)))))

(event EventSprintingMoveBlockedby
  (params (BlockedBy :type Actor%20Object%20Reference)))

(event EventOnDied
  (params (Angle :type Float%20%28single-precision%29) (Type :type EMordhauDamageType%20Enum :default "Generic") (SubType :type Byte :default 0) (bone :type Name%20%28by%20ref%29 :default "None") (Point :type Vector%20%28by%20ref%29 :default "0, 0, 0") (Source :type Actor%20Object%20Reference) (Agent :type Actor%20Object%20Reference))
  (bind _returnvalue (Class|MordhauCharacter|GetLastUsedVehicle 0.5))
  (|CallParentFunction Angle Type SubType bone Point Source Agent)
  (Utilities|FlowControl|Sequence
    (:then_0
      (bind _asab_mordhau_character_animation (Utilities|Casting|CastToAB_MordhauCharacterAnimation (Components|SkeletalMesh|GetAnimInstance (Variables|Character|GetMesh))))
      (if (Utilities|IsValid _returnvalue)
        (Class|AdvancedCharacter|RequestMeshEnablePhysics _returnvalue 5.0)
        (Class|AdvancedCharacter|StartRagdollwithBlend 0.0 :!label _label)
        (Class|MordhauCharacter|PlayDeathYell (Variables|Default|GetbForceLongDeathYell))
        (elif (Math|Boolean|ORBoolean (Variables|/Script/Mordhau.AdvancedCharacterAnimInstance|GetbIsAirborne _asab_mordhau_character_animation) (not (Class|MordhauUtilityLibrary|HasBeenReallyRecentlyRendered (Variables|Character|GetMesh))) (< (Class|KismetMathLibrary|PercentByteByte (Variables|Default|GetDeathSyncedRandom) 10) 5) (Class|MordhauCharacter|IsLeg bone) (and (== Type (Utilities|Enum|LiteralenumEMordhauDamageType "Melee")) (== SubType (Utilities|Enum|LiteralenumEAttackMove "Couch"))) (== Type (Utilities|Enum|LiteralenumEMordhauDamageType "Fall")) (>= (Math|Vector|VectorLength (Variables|Default|GetMoveCompVelocityBeforeDeath)) 1e+02) (Variables|Default|GetbIsRagdollFalling))
          (goto _label)
          (else
            (bind _asmordhau_actor (Utilities|Casting|CastToMordhauActor Agent)
              (:then
                (if (Variables|/Script/Mordhau.MordhauActor|GetbForceRagdollOnDeath _asmordhau_actor)
                  (goto _label)))
              (:CastFailed
                (bind _asadvanced_character (Utilities|Casting|CastToAdvancedCharacter Agent))
                (if (Variables|/Script/Mordhau.AdvancedCharacter|GetbForceRagdollIfDmgAgent _asadvanced_character)
                  (goto _label))))))))
    (:then_1
      (bind _asab_mordhau_character_animation_2 (Utilities|Casting|CastToAB_MordhauCharacterAnimation (Components|SkeletalMesh|GetAnimInstance (Variables|Character|GetMesh))))
      (Default|PickDeathAnim _asab_mordhau_character_animation_2 Angle Agent bone Point Type SubType)
      (Class|MordhauCharacter|PlayDeathYell true) ; Won't do anything if we're already playing one from the node above us
    )))

(event Input|ActionEvents|InputActionCycleCamera
  (params (Key :type Key%20Structure)))

(fn ConstructionScript
  (|CallParentFunction)
  (Variables|Default|SetMordhauCamera (Variables|Default|GetCamera))
  (Variables|Default|SetBlockCollider (Variables|Default|GetBlockColliderBP))
  (Variables|/Script/Mordhau.ThudderComponent|SetMonitoredComponent (Variables|Default|GetThudder) (Variables|Character|GetMesh)))

(fn FindClimbSpot
  (params (UpwardsCast :type Float%20%28single-precision%29))
  (bind _returnvalue (Math|Vector|MakeVector 0.0 0.0 UpwardsCast))
  (bind _returnvalue_2 (Transformation|GetActorLocation))
  (bind _returnvalue_3 (Transformation|GetActorForwardVector))
  (bind _capsulecomponent (Variables|Default|GetCapsuleComponent))
  (bind _capsulecomponent_2 (Variables|Default|GetCapsuleComponent))
  (bind _capsulecomponent_3 (Variables|Default|GetCapsuleComponent))
  (bind _capsulecomponent_4 (Variables|Default|GetCapsuleComponent))
  (bind _charactermovement (Variables|Character|GetCharacterMovement))
  (bind _charactermovement_2 (Variables|Character|GetCharacterMovement))
  (bind _capsulecomponent_5 (Variables|Default|GetCapsuleComponent))
  (bind _returnvalue_4 (Class|CharacterMovementComponent|GetWalkableFloorZ _charactermovement_2))
  (bind _returnvalue_5 (+ _returnvalue_2 _returnvalue))
  (bind _capsuleradius (Variables|/Script/Engine.CapsuleComponent|GetCapsuleRadius _capsulecomponent_2))
  (bind _capsuleradius_2 (Variables|/Script/Engine.CapsuleComponent|GetCapsuleRadius _capsulecomponent_5))
  (bind _returnvalue_6 (* _capsuleradius_2 0.5))
  (bind _returnvalue_7 (* _returnvalue_6 -1.0))
  (bind _returnvalue_8 (* _returnvalue_3 _returnvalue_7))
  ;[1 1 1] Basic approach for climbing: 1) cast upwards high, 2) cast forward, 3) cast downwards
  (LocalVariables|SetMinHeightToClimb (Math|Float|Max(Float) (- (Class|CharacterMovementComponent|GetMaxJumpHeight _charactermovement) 12.0) (Variables|/Script/Engine.CharacterMovementComponent|GetMaxStepHeight _charactermovement)))
  (bind _asmordhau_aicontroller (Utilities|Casting|CastToMordhauAIController (Pawn|GetController))
    (:then
      ;[0 1 0.07465] Different path for AI, just check end spot
      (bind (_outhit _returnvalue_9) (Class|KismetSystemLibrary|CapsuleTraceSinglebyProfile (+ (Variables|/Script/Mordhau.MordhauAIController|GetDesiredClimbTarget _asmordhau_aicontroller) "0, 0,25.000000") (+ (Variables|/Script/Mordhau.MordhauAIController|GetDesiredClimbTarget _asmordhau_aicontroller) "0, 0,20.000000") (Variables|/Script/Engine.CapsuleComponent|GetCapsuleRadius _capsulecomponent) (Variables|/Script/Engine.CapsuleComponent|GetCapsuleHalfHeight _capsulecomponent) "Pawn" false 0 "None" true))
      (if _returnvalue_9
        (bind _asmordhau_character (Utilities|Casting|CastToMordhauCharacter (.HitActor (Collision|BreakHitResult _outhit)))
          (:then
            (if (Pawn|IsPlayerControlled _asmordhau_character)
              (return true (Variables|/Script/Mordhau.MordhauAIController|GetDesiredClimbTarget _asmordhau_aicontroller))
              (else
                _)))
          (:CastFailed
            _)))
      (return (not _returnvalue_9) (Variables|/Script/Mordhau.MordhauAIController|GetDesiredClimbTarget _asmordhau_aicontroller)))
    (:CastFailed
      (Utilities|FlowControl|Sequence
        (:then_0
          ;[1 1 1] Step1: Cast upwards first
          (bind (_outhit_2 _returnvalue_10) (Class|KismetSystemLibrary|CapsuleTraceSinglebyProfile _returnvalue_2 _returnvalue_5 (Variables|/Script/Engine.CapsuleComponent|GetCapsuleRadius _capsulecomponent_4) (Variables|/Script/Engine.CapsuleComponent|GetCapsuleHalfHeight _capsulecomponent_4) "Pawn" false 0 "None" true))
          (if _returnvalue_10
            (bind _output_get (LocalVariables|SetStage1 (.Location (Collision|BreakHitResult _outhit_2))))
            ;[1 0 0] Failed: Ceiling too low
            (if (< (Math|Vector|VectorLength (- _returnvalue_5 _output_get)) (LocalVariables|GetMinHeightToClimb))
              (return false "0, 0, 0"))
            (else
              (LocalVariables|SetStage1 _returnvalue_5))))
        (:then_1
          ;[1 1 1] Step2: Cast forward
          (bind (_outhit_3 _returnvalue_11) (Class|KismetSystemLibrary|CapsuleTraceSinglebyProfile (LocalVariables|GetStage1) (+ (LocalVariables|GetStage1) (* (Transformation|GetActorForwardVector) (* _capsuleradius 2.0))) _capsuleradius (Variables|/Script/Engine.CapsuleComponent|GetCapsuleHalfHeight _capsulecomponent_2) "Pawn" false 0 "None" true))
          (if _returnvalue_11
            (bind _output_get_2 (LocalVariables|SetStage2 (.Location (Collision|BreakHitResult _outhit_3))))
            ;[1 0 0] Failed: not enough room forward
            (if (< (Math|Vector|VectorLength (- (LocalVariables|GetStage1) _output_get_2)) (* (Variables|/Script/Engine.CapsuleComponent|GetCapsuleRadius (Variables|Default|GetCapsuleComponent)) 0.5))
              (return false "0, 0, 0"))
            (else
              (LocalVariables|SetStage2 (+ (LocalVariables|GetStage1) (* (Transformation|GetActorForwardVector) (* _capsuleradius 2.0)))))))
        (:then_2
          ;[1 1 1] Step3: cast back down
          (bind (_outhit_4 _returnvalue_12) (Class|KismetSystemLibrary|CapsuleTraceSinglebyProfile (LocalVariables|GetStage2) (+ (LocalVariables|GetStage2) (Math|Vector|MakeVector 0.0 0.0 (* UpwardsCast -1.0))) (Variables|/Script/Engine.CapsuleComponent|GetCapsuleRadius _capsulecomponent_3) (Variables|/Script/Engine.CapsuleComponent|GetCapsuleHalfHeight _capsulecomponent_3) "Pawn" false 0 "None" true))
          (if (not _returnvalue_12)
            ;[1 0 0] Failed: can't find ground
            (return false "0, 0,0.000000")))
        (:then_3
          ;[1 1 1] Step4: are we firmly grounded with our capsule or just on the edge?
          (bind (_outhit_5 _returnvalue_13) (Class|KismetSystemLibrary|CapsuleTraceSinglebyProfile (+ (LocalVariables|GetStage2) _returnvalue_8) (+ (+ (LocalVariables|GetStage2) (Math|Vector|MakeVector 0.0 0.0 (* UpwardsCast -1.0))) _returnvalue_8) _returnvalue_6 (Variables|/Script/Engine.CapsuleComponent|GetCapsuleHalfHeight _capsulecomponent_5) "Pawn" false 0 "None" true))
          (if _returnvalue_13
            (bind _output_get_3 (LocalVariables|SetStage3 (.Location (Collision|BreakHitResult _outhit_4))))
            (else
              ;[1 0 0] Failed: landed on edge of capsule. TODO: try to perform a vault in this case?
              (return false "0, 0,0.000000"))))
        (:then_4
          ;[1 1 1] Step5: Does the actor allow us to climb onto and walk on?
          (LocalVariables|SetFinalActorToCheck (.HitActor (Collision|BreakHitResult _outhit_4)))
          (Utilities|IsValid (Transformation|GetAttachParent (.HitComponent (Collision|BreakHitResult _outhit_4)))
            (:Is%20Valid
              (LocalVariables|SetFinalActorToCheck (Components|GetOwner (Transformation|GetAttachParent (.HitComponent (Collision|BreakHitResult _outhit_4))))))
            (:Is%20Not%20Valid
              _))
          (Utilities|Casting|CastToEnvironmentMovable (LocalVariables|GetFinalActorToCheck)
            (:then
              ;[1 0 0] Failed: actor doesn't allow us to climb or stand on it or walk on its slope
              (return false "0, 0,0.000000"))
            (:CastFailed
              (Utilities|Casting|CastToBP_BaseProgressActor (LocalVariables|GetFinalActorToCheck)
                (:then
                  (return false "0, 0,0.000000"))
                (:CastFailed
                  (bind _asmordhau_actor (Utilities|Casting|CastToMordhauActor (LocalVariables|GetFinalActorToCheck))
                    (:then
                      (if (Variables|/Script/Mordhau.MordhauActor|GetbPreventClimbing _asmordhau_actor)
                        (return false "0, 0,0.000000")
                        (else
                          (if (Math|Boolean|ORBoolean (< (- (.Z (Math|Vector|BreakVector _output_get_3)) (.Z (Math|Vector|BreakVector (Transformation|GetActorLocation)))) (LocalVariables|GetMinHeightToClimb)) (not (Class|PrimitiveComponent|CanCharacterStepUp (.HitComponent (Collision|BreakHitResult _outhit_4)) self)) (Math|Boolean|ORBoolean (> (- (.Z (Math|Vector|BreakVector (.Location (Collision|BreakHitResult _outhit_4)))) (.Z (Math|Vector|BreakVector (.Location (Collision|BreakHitResult _outhit_5))))) 25.0) (< (.Z (Math|Vector|BreakVector (.ImpactNormal (Collision|BreakHitResult _outhit_4)))) _returnvalue_4) (< (.Z (Math|Vector|BreakVector (.ImpactNormal (Collision|BreakHitResult _outhit_5)))) _returnvalue_4))) :!label _label
                            (return false "0, 0,0.000000")))))
                    (:CastFailed
                      (goto _label))))))))
        (:then_5
          (return true (LocalVariables|GetStage3)))))))

(fn AttemptClimb
  (bind _returnvalue (Class|AdvancedCharacter|GetMotion))
  (bind _returnvalue_2 (Transformation|GetActorLocation))
  (bind _righthandequipment (Variables|Default|GetRightHandEquipment))
  (bind _capsulecomponent (Variables|Default|GetCapsuleComponent))
  (if (or (Variables|Default|GetbIsRagdollFalling) (not (Variables|Default|GetbAllowClimbing)))
    (return false)
    (else
      (Utilities|IsValid _righthandequipment
        (:Is%20Valid
          (if (Variables|/Script/Mordhau.MordhauEquipment|GetbPreventsClimbing _righthandequipment)
            (return false)
            (else
              (Utilities|Casting|CastToClimbingMotion _returnvalue :!label _label
                (:then
                  (return false))
                (:CastFailed
                  (Utilities|Casting|CastToParryMotion _returnvalue
                    (:then
                      (return false))
                    (:CastFailed
                      (bind _asattack_motion (Utilities|Casting|CastToAttackMotion _returnvalue)
                        (:then
                          (if (Utilities|Enum|Equal(Enum) (Variables|/Script/Mordhau.AttackMotion|GetStage _asattack_motion) "Recovery")
                            (bind (_succeeded _targetspot) (CallFunction|FindClimbSpot 2e+02 :!label _label_2)) ; max height, might not clear headroom so we'll try a shorter one if it fails
                            (if _succeeded
                              (Variables|Default|SetClimbTargetLocation _targetspot)
                              (else
                                (bind (_succeeded_2 _targetspot_2) (CallFunction|FindClimbSpot 1e+02)) ; if higher cast didn't have headroom, try lower height
                                (if _succeeded_2
                                  (Variables|Default|SetClimbTargetLocation _targetspot_2)
                                  (else
                                    (return false)))))
                            (else
                              (return false))))
                        (:CastFailed
                          (goto _label_2))))))))))
        (:Is%20Not%20Valid
          (goto _label)))
      (CallFunction|ServerSetClimbLocation (Math|Vector|MakeVectorNetQuantize (.X (Math|Vector|BreakVector (Variables|Default|GetClimbTargetLocation))) (.Y (Math|Vector|BreakVector (Variables|Default|GetClimbTargetLocation))) (.Z (Math|Vector|BreakVector (Variables|Default|GetClimbTargetLocation)))))
      (Utilities|FlowControl|Sequence
        (:then_0
          (if (< (.Z (Math|Vector|BreakVector (Transformation|GetVelocity))) -5e+02)
            (LocalVariables|SetIsSlowClimb true)
            (else
              (bind (_outhit _returnvalue_3) (Class|KismetSystemLibrary|CapsuleTraceSinglebyProfile _returnvalue_2 (+ _returnvalue_2 (Math|Vector|MakeVector 0.0 0.0 -2e+02)) (* (Variables|/Script/Engine.CapsuleComponent|GetCapsuleRadius _capsulecomponent) 0.75) (Variables|/Script/Engine.CapsuleComponent|GetCapsuleHalfHeight _capsulecomponent) "Pawn" false 0 "None" true)) ; check if there's no ground below us, in this case we should slow/pullup
              (if _returnvalue_3
                (if (> (.Z (Math|Vector|BreakVector (- (Variables|Default|GetClimbTargetLocation) (.Location (Collision|BreakHitResult _outhit))))) 125.0)
                  (LocalVariables|SetIsSlowClimb true :!label _label_3))
                (else
                  (goto _label_3))))))
        (:then_1
          (Class|MordhauCharacter|RequestClimb (Variables|Default|GetClimbTargetLocation) (LocalVariables|GetIsSlowClimb))
          (return true))))))

(fn CalculateLedgeOffsetandNormal
  (params (ClimbingMotion :type Climbing%20Motion%20Object%20Reference))
  (bind _returnvalue (Transformation|GetActorLocation))
  (bind _capsulecomponent (Variables|Default|GetCapsuleComponent))
  (bind _returnvalue_2 (+ _returnvalue "0, 0,50.000000"))
  (bind (_outhit _returnvalue_3) (Class|KismetSystemLibrary|CapsuleTraceSinglebyProfile _returnvalue_2 (+ _returnvalue_2 (* (Transformation|GetActorForwardVector) 105.0)) (Variables|/Script/Engine.CapsuleComponent|GetCapsuleRadius _capsulecomponent) (Variables|/Script/Engine.CapsuleComponent|GetCapsuleHalfHeight _capsulecomponent) "Pawn" false 0 "None" true))
  (if _returnvalue_3
    (return (Math|Vector|MakeVector (.X (Math|Vector|BreakVector (- (.Location (Collision|BreakHitResult _outhit)) _returnvalue_2))) (.Y (Math|Vector|BreakVector (- (.Location (Collision|BreakHitResult _outhit)) _returnvalue_2))) 0.0) (Math|Vector|Normalize (Math|Vector|MakeVector (.X (Math|Vector|BreakVector (* (.ImpactNormal (Collision|BreakHitResult _outhit)) -1.0))) (.Y (Math|Vector|BreakVector (* (.ImpactNormal (Collision|BreakHitResult _outhit)) -1.0))) 0.0)))
    (else
      (return "0, 0, 0" "0, 0, 0"))))

(fn TryClimbing
  (if (or (Character|CanJump) (and (Class|AdvancedCharacter|IsAirborne) (> (.Z (Math|Vector|BreakVector (Transformation|GetVelocity))) -9e+02)))
    (bind _succeeded (CallFunction|AttemptClimb))
    (if _succeeded
      (return true)
      (else
        _)))
  (return false))

(fn AddRagdollImpulse
  (params (Impulse :type Vector) (Location :type Vector) (Bone :type Name))
  (bind _mesh (Variables|Character|GetMesh))
  (Physics|AddImpulseatLocation _mesh (* Impulse (Math|Float|Max(Float) (/ (Class|SkeletalMeshComponent|GetBoneMass _mesh Bone true) 15.0) 0.5)) Location Bone))

(fn GetOutOfBoundsText
  (if (Class|MordhauCharacter|IsinEnemyTeamArea)
    (return "Too close to enemy spawn! Fall back!")
    (else
      (return "Get back to the fight, coward!"))))

(fn GetOutOfBoundsSubtext
  (return (Utilities|Text|FormatText "Death in {a} seconds" (Math|Float|Ceil (Class|AdvancedCharacter|GetOutOfBoundsTimeUntilDeath)))))

(fn SpawnBloodPoolUnderneath
  (bind _mesh (Variables|Character|GetMesh))
  (bind _returnvalue (Transformation|GetSocketLocation _mesh "Neck"))
  (if (stale _returnvalue)
    (bind (_outhit _returnvalue_2) (Collision|LineTraceForObjects _returnvalue (+ _returnvalue "0, 0,-200.000000") (Utilities|Array|MakeArray "ObjectTypeQuery1") false 0 "None"))
    (if _returnvalue_2
      (bind _returnvalue_3 (Class|MordhauUtilityLibrary|SpawnBloodDecalatLocation 0 "/Game/Mordhau/Assets/Environment/DecalMaterials/INST_DM_Bloodpuddle.INST_DM_Bloodpuddle" "50.000000,150.000000,150.000000" (.ImpactPoint (Collision|BreakHitResult _outhit)) (Math|Rotator|MakeRotfromX (* (.ImpactNormal (Collision|BreakHitResult _outhit)) -1.0)) 9e+01))
      (Utilities|IsValid _returnvalue_3
        (:Is%20Valid
          (Rendering|Components|Decal|SetFadeOut _returnvalue_3 9e+01 0.25 false)
          (Class|MordhauUtilityLibrary|SetDecalFadeScreenSize _returnvalue_3 0.05)
          (Class|DecalComponent|SetSortOrder _returnvalue_3 1)
          (bind _returnvalue_4 (Rendering|Material|CreateDynamicMaterialInstance _returnvalue_3 :!class /Script/Engine.DecalComponent))
          (Rendering|Material|SetScalarParameterValue _returnvalue_4 "Row" (Math|Conversions|ToFloat(Integer) (Math|Random|RandomIntegerinRange 0 3)) :!class /Script/Engine.MaterialInstanceDynamic)
          (Rendering|Material|SetScalarParameterValue _returnvalue_4 "Column" (Math|Conversions|ToFloat(Integer) (Math|Random|RandomIntegerinRange 0 3)) :!class /Script/Engine.MaterialInstanceDynamic)
          (Rendering|Material|SetScalarParameterValue _returnvalue_4 "StartTime" (Utilities|Time|GetGameTimeinSeconds) :!class /Script/Engine.MaterialInstanceDynamic)
          (Rendering|Material|SetScalarParameterValue _returnvalue_4 "FillDuration" 15.0 :!class /Script/Engine.MaterialInstanceDynamic))))))

(fn IsAnUpgrade
  (params (Wearable :type BP%20Wearable%20Pickup%20Object%20Reference))
  (return true))

(fn OnBeforeReceiveWearablePickup
  (params (WearablePickup :type BP%20Wearable%20Pickup%20Object%20Reference)))

(fn GiveFists
  (bind _equipment (Variables|Default|GetEquipment))
  (bind _returnvalue (Utilities|Array|Length _equipment))
  (bind _returnvalue_2 (- _returnvalue 1))
  (bind _output (Utilities|Array|Get(acopy) _equipment _returnvalue_2))
  (Utilities|FlowControl|Sequence
    (:then_0
      (if (Class|MordhauCharacter|HasPerk (Utilities|Enum|LiteralenumEPerk "Pugilist"))
        (LocalVariables|SetDesiredFists "/Game/Mordhau/Blueprints/Equipment/Weapons/BP_PugilistFistsWeapon.BP_PugilistFistsWeapon_C")
        (else
          (LocalVariables|SetDesiredFists "/Game/Mordhau/Blueprints/Equipment/Weapons/BP_FistsWeapon.BP_FistsWeapon_C"))))
    (:then_1
      (Utilities|IsValid _output
        (:Is%20Valid
          (if (not (== (Utilities|GetClass _output) (LocalVariables|GetDesiredFists)))
            (bind _returnvalue_3 (Class|MordhauCharacter|DropEquipment _output true))
            (Actor|DestroyActor _returnvalue_3)
            (bind _returnvalue_4 (Game|SpawnActorfromClass (LocalVariables|GetDesiredFists) (Math|Transform|MakeTransform "0, 0, 0") "AlwaysSpawn" 0 0 :!label _label))
            (Class|MordhauCharacter|PickUptoSlot _returnvalue_4 (Math|Conversions|ToByte(Integer) (- (Utilities|Array|Length (Variables|Default|GetEquipment)) 1)))))
        (:Is%20Not%20Valid
          (goto _label))))))