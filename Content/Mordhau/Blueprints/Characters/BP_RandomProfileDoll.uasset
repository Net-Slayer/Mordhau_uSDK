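; BP_RandomProfileDoll is a character doll that shows a random player profile in a preview pose.
; Once the HUD reports the singleton loaded, it rerolls on authority, picking a saved profile, or a default one if the only saved profile is "Unnamed".
; It applies that profile with equipment and hides the mesh, then forces a visibility update and shows it two frames later.
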(event Custom|Reroll
  (bind _returnvalue (Class|MordhauUtilityLibrary|GetMordhauSingleton))
  (bind _characterprofiles (Variables|/Script/Mordhau.MordhauSingleton|GetCharacterProfiles _returnvalue))
  (bind _defaultprofiles (Variables|/Script/Mordhau.MordhauSingleton|GetDefaultProfiles _returnvalue))
  (bind _returnvalue_2 (Utilities|Array|Length _characterprofiles))
  (Networking|SwitchHasAuthority
    (:Authority
      (bind _asbp_mordhau_singleton (Utilities|Casting|CastToBP_MordhauSingleton _returnvalue))
      (if (and (== _returnvalue_2 1) (Utilities|Enum|Equal(Enum) (Utilities|String|ToString(Text) (.Name (Utilities|Struct|BreakCharacterProfile (Utilities|Array|Get(acopy) _characterprofiles)))) "Unnamed"))
        (Variables|Default|SetCurrentProfileStored (Utilities|Array|Get(acopy) _defaultprofiles (Math|Random|RandomInteger (Utilities|Array|Length _defaultprofiles))))
        (else
          (Variables|Default|SetCurrentProfileStored (Utilities|Array|Get(acopy) _characterprofiles (Math|Random|RandomInteger _returnvalue_2)))))
      (Class|MordhauSingleton|ApplyProfileto _asbp_mordhau_singleton (Variables|Default|GetCurrentProfileStored) self 0 true)
      (Variables|Default|SetRerolledFrame (Class|MordhauUtilityLibrary|GetCurrentFrameBP))
      (Rendering|SetVisibility (Variables|Character|GetMesh) false true)
      (CallFunction|AssumePreviewPose (Math|Random|RandomInteger 1000)))))

(event EventTick
  (params (DeltaSeconds :type Float%20%28single-precision%29))
  (|CallParentFunction DeltaSeconds)
  (bind _asbp_mordhau_hud (Utilities|Casting|CastToBP_MordhauHUD (Class|MordhauUtilityLibrary|GetMordhauHUD)))
  (if (Variables|/Game/Mordhau/Blueprints/BP_MordhauHUD.BP_MordhauHUD_C|GetLoadedSingleton _asbp_mordhau_hud)
    (Utilities|FlowControl|Sequence
      (:then_0
        (Utilities|FlowControl|DoOnce false
          (:Completed
            (CallFunction|Reroll))))
      (:then_1
        (if (== (+ (Variables|Default|GetRerolledFrame) 2) (Class|MordhauUtilityLibrary|GetCurrentFrameBP))
          (Class|MordhauCharacter|ForceUpdateMeshVisibility)
          (Rendering|SetVisibility (Variables|Character|GetMesh) true true))))))

(fn ConstructionScript
  (|CallParentFunction))