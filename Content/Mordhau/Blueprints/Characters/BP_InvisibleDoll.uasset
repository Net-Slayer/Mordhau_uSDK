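; Invisible doll character that can be given a full character profile or a single wearable in a chosen slot.
; GiveProfileToDoll applies a profile to the doll through the BP_MordhauSingleton.
; GiveWearableObjectToDoll sets the HumanMeshComponent's single-slot mode and wearable, then passes an empty, force-validated profile, without inventory validation, to GiveProfileToDoll.
; The event graph and construction script add no logic of their own.
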(event EventBeginPlay
  (|CallParentFunction))

(event EventActorBeginOverlap
  (params (OtherActor :type Actor%20Object%20Reference)))

(event EventTick
  (params (DeltaSeconds :type Float%20%28single-precision%29))
  (|CallParentFunction 0.0))

(fn ConstructionScript
  (|CallParentFunction))

(fn GiveProfiletoDoll
  (params (Profile :type Character%20Profile%20Structure))
  (bind _asbp_mordhau_singleton (Utilities|Casting|CastToBP_MordhauSingleton (Class|MordhauUtilityLibrary|GetMordhauSingleton)))
  (Class|MordhauSingleton|ApplyProfileto _asbp_mordhau_singleton Profile self 0 false))

(fn GiveWearableObjecttoDoll
  (params (Wearable :type Mordhau%20Wearable%20Class%20Reference) (Slot :type EWearableSlot%20Enum :default "Head"))
  (bind _ashuman_mesh_component (Utilities|Casting|CastToHumanMeshComponent (Variables|Character|GetMesh)))
  (Variables|/Script/Mordhau.HumanMeshComponent|SetSingleSlotMode _ashuman_mesh_component Slot)
  (Variables|/Script/Mordhau.HumanMeshComponent|SetSingleSlotModeWearableToUse _ashuman_mesh_component Wearable)
  (bind _returnvalue (Class|MordhauUtilityLibrary|MakeEmptyProfile "/Game/Mordhau/Blueprints/Characters/BP_MordhauCharacter.BP_MordhauCharacter_C" false))
  (bind _forcevalidatedprofile (Class|MordhauUtilityLibrary|ForceValidCharacterProfile (Utilities|Struct|MakeCharacterProfile "" (.GearCustomization (Utilities|Struct|BreakCharacterProfile _returnvalue)) (.AppearanceCustomization (Utilities|Struct|BreakCharacterProfile _returnvalue)) (.FaceCustomization (Utilities|Struct|BreakCharacterProfile _returnvalue)) (.SkillsCustomization (Utilities|Struct|BreakCharacterProfile _returnvalue))) false))
  (CallFunction|GiveProfiletoDoll _forcevalidatedprofile))