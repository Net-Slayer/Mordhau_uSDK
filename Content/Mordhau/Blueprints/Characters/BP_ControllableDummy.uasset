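; BP_ControllableDummy is a Mordhau character dummy that spawns dressed and equipped as a chosen character profile.
; On BeginPlay the server applies the profile indexed by ProfileID from the MordhauSingleton, including equipment, then runs parent setup.
; Each tick a non-zero MovementInput vector, taken in actor-local space, drives movement, with sprinting triggered when ShouldSprint is set.
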(event EventBeginPlay
  (Utilities|FlowControl|Sequence
    (:then_0
      (Networking|SwitchHasAuthority
        (:Authority
          (bind _asbp_mordhau_singleton (Utilities|Casting|CastToBP_MordhauSingleton (Class|MordhauUtilityLibrary|GetMordhauSingleton)))
          (Class|MordhauSingleton|ApplyProfileto _asbp_mordhau_singleton (Utilities|Array|Get(acopy) (Variables|/Script/Mordhau.MordhauSingleton|GetCharacterProfiles _asbp_mordhau_singleton) (Math|Conversions|ToInteger(Byte) (Variables|Default|GetProfileID))) self 0 true))))
    (:then_1
      (|CallParentFunction))))

(event EventActorBeginOverlap
  (params (OtherActor :type Actor%20Object%20Reference)))

(event EventTick
  (params (DeltaSeconds :type Float%20%28single-precision%29))
  (bind _movementinput (Variables|Default|GetMovementInput))
  (|CallParentFunction DeltaSeconds)
  (if (not (== (Math|Vector|VectorLength _movementinput) 0.0))
    (Pawn|Input|AddMovementInput (Math|Transform|TransformDirection (Transformation|GetActorTransform) _movementinput) 1.0 false)
    (if (Variables|Default|GetShouldSprint)
      (Class|MordhauCharacter|StartSprinting))))

(fn ConstructionScript
  (|CallParentFunction))