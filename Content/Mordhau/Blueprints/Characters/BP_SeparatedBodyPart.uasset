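; Severed body part spawned by dismemberment, which reacts to hits and impacts and leaves a blood puddle.
; The parent class handles dismemberment setup, while cosmetic hits add a scaled-down ragdoll impulse to the mesh.
; A Thudder component monitors the fake root bone, triggering a fall sound scaled by velocity loss.
; With blood enabled, it polls until the part nearly stops, then traces down for a randomized, gradually filling puddle decal.
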(event OnThud(Thudder)
  (bind _fakerootbone (Variables|Default|GetFakeRootBone))
  (bind _thudder (Variables|Default|GetThudder))
  (bind _mesh (Variables|Character|GetMesh))
  (bind _returnvalue (Transformation|GetSocketLocation _mesh _fakerootbone))
  (bind _currentvelocity (Variables|/Script/Mordhau.ThudderComponent|GetCurrentVelocity _thudder))
  (Audio|SpawnSoundAttached "/Game/Mordhau/Audio/Cues/Foley/SC_BodyPartFall.SC_BodyPartFall" (Variables|Character|GetMesh) _fakerootbone "0, 0, 0" "0, 0, 0" "SnapToTarget" true (Math|Float|MapRangeClamped (- (Variables|/Script/Mordhau.ThudderComponent|GetPreviousVelocity _thudder) _currentvelocity) 3e+02 5e+02 0.5 0.75) 1.0 0.0 0 0)
  (if (stale _returnvalue)
    (Utilities|FlowControl|RetriggerableDelay 0.5 :!label _label)
    (if (< _currentvelocity 1e+01)
      (bind (_outhit _returnvalue_2) (Collision|LineTraceForObjects _returnvalue (+ _returnvalue "0, 0,-200.000000") (Utilities|Array|MakeArray "ObjectTypeQuery1") false 0 "None"))
      (if _returnvalue_2
        (bind _returnvalue_3 (Class|MordhauUtilityLibrary|SpawnBloodDecalatLocation 0 "/Game/Mordhau/Assets/Environment/DecalMaterials/INST_DM_Bloodpuddle.INST_DM_Bloodpuddle" "50.000000,100.000000,100.000000" (.ImpactPoint (Collision|BreakHitResult _outhit)) (Math|Rotator|MakeRotfromX (* (.ImpactNormal (Collision|BreakHitResult _outhit)) -1.0)) 9e+01))
        (Utilities|IsValid _returnvalue_3
          (:Is%20Valid
            (Rendering|Components|Decal|SetFadeOut _returnvalue_3 9e+01 0.25 false)
            (Class|MordhauUtilityLibrary|SetDecalFadeScreenSize _returnvalue_3 0.075)
            (Class|DecalComponent|SetSortOrder _returnvalue_3 1)
            (bind _returnvalue_4 (Rendering|Material|CreateDynamicMaterialInstance _returnvalue_3 :!class /Script/Engine.DecalComponent))
            (Rendering|Material|SetScalarParameterValue _returnvalue_4 "Row" (Math|Conversions|ToFloat(Integer) (Math|Random|RandomIntegerinRange 0 3)) :!class /Script/Engine.MaterialInstanceDynamic)
            (Rendering|Material|SetScalarParameterValue _returnvalue_4 "Column" (Math|Conversions|ToFloat(Integer) (Math|Random|RandomIntegerinRange 0 3)) :!class /Script/Engine.MaterialInstanceDynamic)
            (Rendering|Material|SetScalarParameterValue _returnvalue_4 "StartTime" (Utilities|Time|GetRealTimeSeconds) :!class /Script/Engine.MaterialInstanceDynamic)
            (Rendering|Material|SetScalarParameterValue _returnvalue_4 "FillDuration" 15.0 :!class /Script/Engine.MaterialInstanceDynamic))))
      (else
        (goto _label)))))

(event EventOnCosmeticHit
  (params (DamageType :type EMordhauDamageType%20Enum :default "Generic") (SubType :type Byte :default 0) (Hit :type Hit%20Result%20Structure%20%28by%20ref%29) (Agent :type Actor%20Object%20Reference))
  (|CallParentFunction DamageType SubType Hit Agent)
  (bind _force (CallFunction|ComputeRagdollForce Agent DamageType SubType 255 self))
  (Physics|AddImpulseatLocation (Variables|Character|GetMesh) (* _force 0.1) (.ImpactPoint (Collision|BreakHitResult Hit)) "None"))

(event EventInitializeDismemberment
  (params (Source :type Mordhau%20Character%20Object%20Reference) (bone :type Name%20%28by%20ref%29 :default "None") (SourceBoneTransform :type Transform%20%28by%20ref%29) (bIsPartial :type Boolean) (bIsBluntForce :type Boolean))
  (Utilities|FlowControl|Sequence
    (:then_0
      (|CallParentFunction Source bone SourceBoneTransform bIsPartial bIsBluntForce))
    (:then_1
      (Variables|/Script/Mordhau.ThudderComponent|SetMonitoredBone (Variables|Default|GetThudder) (Variables|Default|GetFakeRootBone)))))

(fn ConstructionScript
  (|CallParentFunction)
  (Variables|/Script/Mordhau.ThudderComponent|SetMonitoredComponent (Variables|Default|GetThudder) (Variables|Character|GetMesh)))