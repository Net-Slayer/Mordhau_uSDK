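; Purchase effect actor that plays a burst of audiovisual feedback, presumably when the player buys something.
; On BeginPlay it activates the purchase sound and ember particle components and resets a timer.
; Each tick advances the timer and samples an intensity curve to drive both the post-process blend weight and a scaled point light intensity.
; The construction script initializes both from the timer variable, and the actor has no cleanup logic of its own.
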(event EventBeginPlay
  (Components|Activation|Activate (Variables|Default|GetSC_Purchase) false)
  (Components|Activation|Activate (Variables|Default|GetP_PurchaseEmberEffect) false)
  (Variables|Default|SetIntensityTime 0.0))

(event Collision|EventActorBeginOverlap
  (params (OtherActor :type Actor%20Object%20Reference)))

(event EventTick
  (params (DeltaSeconds :type Float%20%28single-precision%29))
  (Variables|Default|SetIntensityTime (+ DeltaSeconds (Variables|Default|GetIntensityTime)))
  (Variables|/Script/Engine.PostProcessComponent|SetBlendWeight (Variables|Default|GetPPPurchase) (Math|Curves|GetFloatValue (Variables|Default|GetIntensity%20Curve) (Variables|Default|GetIntensityTime)))
  (Rendering|Components|Light|SetIntensity (Variables|Default|GetPointLight) (* (Math|Curves|GetFloatValue (Variables|Default|GetIntensity%20Curve) (Variables|Default|GetIntensityTime)) 1e+04)))

(fn ConstructionScript
  (bind _intensitytime (Variables|Default|GetIntensityTime))
  (Variables|/Script/Engine.PostProcessComponent|SetBlendWeight (Variables|Default|GetPPPurchase) _intensitytime)
  (Rendering|Components|Light|SetIntensity (Variables|Default|GetPointLight) _intensitytime))