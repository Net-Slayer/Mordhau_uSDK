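; Mordhau's AI controller, which runs a behavior tree (deathmatch by default) and restarts or stops its logic as pawns are possessed or released.
; It resets the blackboard only for a new character or once the last is dead or invalid, so vehicle changes keep state; returning to the same character forces a perception update.
; Perception events update the perceives-ally key.
; In team modes, the navigation query filter follows the character's team.
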(event EventOnStartedPerceivingCharacter
  (params (PerceivedCharacter :type Advanced%20Character%20Object%20Reference) (PerceptionInfo :type Perception%20Info%20Structure%20%28by%20ref%29))
  (bind _returnvalue (Class|MordhauAIController|PerceivesAlly))
  (AI|Components|Blackboard|SetValueasBool (AI|GetBlackboard (Pawn|GetControlledPawn)) (Variables|Default|GetPerceivesAllyKey) _returnvalue))

(event EventOnStoppedPerceivingCharacter
  (params (PerceivedCharacter :type Advanced%20Character%20Object%20Reference) (PerceptionInfo :type Perception%20Info%20Structure%20%28by%20ref%29))
  (bind _returnvalue (Class|MordhauAIController|PerceivesAlly))
  (AI|Components|Blackboard|SetValueasBool (AI|GetBlackboard (Pawn|GetControlledPawn)) (Variables|Default|GetPerceivesAllyKey) _returnvalue))

(event EventOnAfterUnPossess
  (|CallParentFunction)
  (AI|Logic|StopLogic (Variables|Default|GetBrainComponent) ""))

(event EventOnPossess
  (params (PossessedPawn :type Pawn%20Object%20Reference))
  (bind _braincomponent (Variables|Default|GetBrainComponent))
  (|CallParentFunction PossessedPawn)
  (Utilities|FlowControl|Sequence
    (:then_0
      (Utilities|IsValid _braincomponent
        (:Is%20Valid
          (Class|BrainComponent|RestartLogic _braincomponent))))
    (:then_1
      ;[1 1 1] Don't reset blackboard unless we're possessing a new character, avoids vehicle changes from affecting this
      ; Also force a perception update if we're returning to the same char, useful for vehicles like ladders that can forget why they're there
      (bind _asmordhau_character (Utilities|Casting|CastToMordhauCharacter PossessedPawn)
        (:then
          (if (!= (Variables|Default|GetLastPossessedCharacter) _asmordhau_character)
            (Variables|Default|SetLastPossessedCharacter _asmordhau_character)
            (Utilities|IsValid (Variables|Default|GetBrainComponent) :!label _label
              (:Is%20Valid
                (Utilities|ResetBlackboard)))
            (else
              (Utilities|FlowControl|Delay 0.2)
              (Class|AIPerceptionComponent|RequestStimuliListenerUpdate (Class|AIController|GetAIPerceptionComponent)))))
        (:CastFailed
          (Utilities|IsValid (Variables|Default|GetLastPossessedCharacter)
            (:Is%20Valid
              (if (Class|AdvancedCharacter|GetIsDead (Variables|Default|GetLastPossessedCharacter))
                (goto _label)))
            (:Is%20Not%20Valid
              (goto _label))))))))

(event EventBeginPlay
  (Utilities|FlowControl|Sequence
    (:then_0
      (Utilities|IsValid (Variables|Default|GetBehaviorTree)
        (:Is%20Not%20Valid
          (Variables|Default|SetBehaviorTree "/Game/Mordhau/AI/BehaviorTrees/BT_Deathmatch.BT_Deathmatch"))))
    (:then_1
      (AI|RunBehaviorTree (Variables|Default|GetBehaviorTree)))))

(fn ConstructionScript)

(fn GetTeamFilterClass
  (bind _asadvanced_character (Utilities|Casting|CastToAdvancedCharacter (Pawn|GetControlledPawn))
    (:then
      (bind _asbp_mordhau_game_state (Utilities|Casting|CastToBP_MordhauGameState (Game|GetGameState))
        (:then
          (if (Variables|/Script/Mordhau.MordhauGameState|GetbIsTeamMode _asbp_mordhau_game_state)
            (return (Utilities|Select :Index (Variables|/Script/Mordhau.AdvancedCharacter|GetTeam _asadvanced_character) :Option%200 (Variables|Default|GetTeam1NavQueryFilter) :Option%201 (Variables|Default|GetTeam2NavQueryFilter)))
            (else
              _)))
        (:CastFailed
          _)))
    (:CastFailed
      _))
  (return "/Game/Mordhau/AI/Navigation/BP_NavFilter_Default.BP_NavFilter_Default_C"))