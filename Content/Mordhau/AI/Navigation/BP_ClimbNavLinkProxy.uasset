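; Smart nav link proxy that makes AI-controlled Mordhau characters climb when they reach the link.
; For a living bot, it sets the controller's climb target above the link's End point and calls TryClimbing, ignoring the result.
; A timestamp on the game state throttles climb attempts across all bots to one per short interval.
; Throttled bots skip the climb, and path following resumes whether or not a climb was attempted.
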(event EventBeginPlay)

(event Collision|EventActorBeginOverlap
  (params (OtherActor :type Actor%20Object%20Reference)))

(event EventTick
  (params (DeltaSeconds :type Float%20%28single-precision%29)))

(event EventSmartLinkReached
  (params (Agent :type Actor%20Object%20Reference) (Destination :type Vector%20%28by%20ref%29 :default "0, 0, 0"))
  (bind _returnvalue (Utilities|Time|GetTimeSeconds))
  (bind _asmordhau_character (Utilities|Casting|CastToMordhauCharacter Agent)
    (:then
      (bind _asmordhau_aicontroller (Utilities|Casting|CastToMordhauAIController (Pawn|GetController _asmordhau_character))
        (:then
          (bind _asmordhau_game_state (Utilities|Casting|CastToMordhauGameState (Game|GetGameState)))
          (if (not (Class|AdvancedCharacter|GetIsDead _asmordhau_character))
            (if (< (+ (Variables|/Script/Mordhau.MordhauGameState|GetLastBotClimbTime _asmordhau_game_state) 0.1) _returnvalue)
              (Variables|/Script/Mordhau.MordhauGameState|SetLastBotClimbTime _asmordhau_game_state _returnvalue)
              (Variables|/Script/Mordhau.MordhauAIController|SetDesiredClimbTarget _asmordhau_aicontroller (+ (Variables|Default|GetEnd) "0, 0,100.000000"))
              (bind _returnvalue_2 (Class|MordhauCharacter|TryClimbing _asmordhau_character))
              (if _returnvalue_2
                _
                (else
                  _)))
            (Class|NavLinkProxy|ResumePathFollowing _asmordhau_character :!label _label)))
        (:CastFailed
          (goto _label))))
    (:CastFailed
      (goto _label))))

(fn ConstructionScript
  (|CallParentFunction))