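; AI nav link proxy that lets Mordhau AI characters use a BP_Ladder to ascend or descend.
; On BeginPlay it finds an unset ladder by runtime sphere overlap, supporting sublevels, or destroys itself.
; Descending links enable tick to check ladder state, intended to disable the link when the ladder isn't up.
; Reaching the link starts climbing or toggles the ladder's state; vehicle users and non-interactable ladders resume path following.
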(event EventBeginPlay
  (Utilities|FlowControl|Sequence
    (:then_0
      ;[1 1 1] We need to disable if descending and ladder isnt up, because we can't bring it up from the top..
      (if (not (Variables|Default|GetAscending))
        (Actor|Tick|SetActorTickEnabled true)))
    (:then_1
      ;[1 1 1] Sometimes, ladders are on a sublevel, so we need to do a sphere check at runtime, not ideal, but better than forcing navlinks on only one level for now.
      (Utilities|IsValid (Variables|Default|GetLadder)
        (:Is%20Not%20Valid
          (bind _outactors (Collision|SphereOverlapActors (select (Variables|Default|GetAscending) (Variables|Default|GetStart) (Variables|Default|GetEnd)) 3e+02 (Utilities|Array|MakeArray "ObjectTypeQuery1") "/Game/Mordhau/Blueprints/Interactables/SiegeEngines/BP_Ladder.BP_Ladder_C"))
          (if (> (Utilities|Array|Length _outactors) 0)
            (bind _asbp_ladder (Utilities|Casting|CastToBP_Ladder (Utilities|Array|Get(acopy) _outactors)))
            (Variables|Default|SetLadder _asbp_ladder)
            (else
              (Development|PrintString "Could not find ladder, destroying navlink")
              (Actor|DestroyActor))))))))

(event EventTick
  (params (DeltaSeconds :type Float%20%28single-precision%29))
  (bind _ladder (Variables|Default|GetLadder))
  (bind _ladderstate (Variables|/Game/Mordhau/Blueprints/Interactables/SiegeEngines/BP_Ladder.BP_Ladder_C|GetLadderState _ladder))
  (bind _returnvalue (== _ladderstate 0))
  (Utilities|IsValid _ladder
    (:Is%20Valid
      (if (Math|Boolean|NotEqual(Boolean) _returnvalue (Class|NavLinkProxy|IsSmartLinkEnabled))
        (Class|NavLinkProxy|SetSmartLinkEnabled (not _returnvalue))))))

(event EventSmartLinkReached
  (params (Agent :type Actor%20Object%20Reference) (Destination :type Vector%20%28by%20ref%29 :default "0, 0, 0"))
  (bind _ladder (Variables|Default|GetLadder))
  (bind _asmordhau_character (Utilities|Casting|CastToMordhauCharacter Agent)
    (:then
      (Utilities|IsValid (Variables|/Script/Mordhau.MordhauCharacter|GetCurrentVehicle _asmordhau_character)
        (:Is%20Valid
          (Class|NavLinkProxy|ResumePathFollowing _asmordhau_character :!label _label))
        (:Is%20Not%20Valid
          (if (not (Class|AdvancedCharacter|GetIsDead _asmordhau_character))
            (bind _asmordhau_aicontroller (Utilities|Casting|CastToMordhauAIController (Pawn|GetController _asmordhau_character))
              (:then
                (if (Variables|/Script/Mordhau.MordhauActor|GetbIsInteractable _ladder)
                  (if (== (Variables|/Game/Mordhau/Blueprints/Interactables/SiegeEngines/BP_Ladder.BP_Ladder_C|GetLadderState _ladder) 0)
                    (Variables|/Script/Mordhau.MordhauAIController|SetbWants1DMovementBackwards _asmordhau_aicontroller (not (Variables|Default|GetAscending)))
                    (Class|MordhauActor|InteractionStart _ladder _asmordhau_character)
                    (else
                      (Default|ToggleLadderState _ladder)
                      (goto _label)))
                  (else
                    (goto _label))))
              (:CastFailed
                (goto _label)))))))
    (:CastFailed
      (goto _label))))

(fn ConstructionScript
  (|CallParentFunction))