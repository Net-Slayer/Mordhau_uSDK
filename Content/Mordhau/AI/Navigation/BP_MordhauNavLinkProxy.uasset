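; Mordhau's AI nav link proxy, which fits a smart link between Start and End points.
; The construction script works around SmartLinkComp endpoints not being editable in Blueprints by transforming the root component instead.
; It places the root at Start, yaws it toward End, and scales X and Z by the horizontal and vertical offsets over 100.
; The event graph holds only disabled default events.
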(event EventBeginPlay)

(event Collision|EventActorBeginOverlap
  (params (OtherActor :type Actor%20Object%20Reference)))

(event EventTick
  (params (DeltaSeconds :type Float%20%28single-precision%29)))

(fn ConstructionScript
  (bind _returnvalue (Math|Vector|MakeVector 0.0 0.0 1.0))
  (bind _start (Variables|Default|GetStart))
  (bind _end (Variables|Default|GetEnd))
  (bind _returnvalue_2 (- _end _start))
  (bind _returnvalue_3 (Math|Conversions|ToVector2D(Vector) _returnvalue_2))
  (bind _returnvalue_4 (Math|Vector2D|Normalize2D _returnvalue_3))
  (bind _returnvalue_5 (Math|Conversions|ToVector(Vector2D) _returnvalue_4))
  (bind _returnvalue_6 (Math|Rotator|MakeRotfromXZ _returnvalue_5 _returnvalue))
  (bind _returnvalue_7 (Math|Vector|UnrotateVector _returnvalue_2 _returnvalue_6))
  (bind (_x _y _z) (Math|Vector|BreakVector _returnvalue_7))
  ;[1 1 1] SmartLinkComp endpoints are not editable for blueprints, this is a bizarre engine choice and probably a bug, but we work around this using scale instead and some rotations
  (Transformation|SetRelativeTransform (Variables|Transformation|GetRootComponent) (Math|Transform|MakeTransform _start _returnvalue_6 (Math|Vector|MakeVector (/ _x 1e+02) 1.0 (/ _z 1e+02))) false false))