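; BP_FoodConsumable is a food pickup in the Feitoria map resources that restores some health and stamina to the character who interacts with it.
; When interaction starts, the server applies both offsets with their replicate flag off.
; It then randomly makes one of two mouth sound calls, only one of which names a sound and both at zero volume multiplier, before destroying itself.
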(event EventBeginPlay
  (|CallParentFunction) ; This node is disabled and will not be called.\nDrag off pins to build functionality.
)

(event Collision|EventActorBeginOverlap
  (params (OtherActor :type Actor%20Object%20Reference))
  (|CallParentFunction OtherActor) ; This node is disabled and will not be called.\nDrag off pins to build functionality.
)

(event EventTick
  (params (DeltaSeconds :type Float%20%28single-precision%29))
  (|CallParentFunction DeltaSeconds) ; This node is disabled and will not be called.\nDrag off pins to build functionality.
)

(event EventOnInteractionStart
  (params (Character :type Mordhau%20Character%20Object%20Reference))
  (Networking|SwitchHasAuthority
    (:Authority
      (Class|AdvancedCharacter|OffsetHealth Character 20 false)
      (Class|MordhauCharacter|OffsetStamina Character 10 false)
      (switch int (Math|Random|RandomIntegerinRange 0 1)
        (:0
          (Class|MordhauCharacter|PlayMouthSound Character 0 0.0))
        (:1
          (Class|MordhauCharacter|PlayMouthSound Character "/Game/Mordhau/Audio/Raw/Weapons/Hits/Sweetener/bone_2.bone_2" 0.0)))
      (Actor|DestroyActor self))))

(fn ConstructionScript
  (|CallParentFunction))