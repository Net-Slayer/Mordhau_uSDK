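; Interactable equipment bag that gives the interacting character a new item of its configured SpawnClass.
; The server spawns the equipment and attempts a pickup; on failure it messages the player to free a slot and destroys the item.
; Each interaction briefly disables the bag as a cooldown.
; A text label from the class defaults is set at construction, refreshed shortly after BeginPlay, and rotated every tick from the first player controller's rotation.
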(event Custom|SpawnEquipment
  (params (Char :type Mordhau%20Character%20Object%20Reference))
  (Networking|SwitchHasAuthority
    (:Authority
      (bind _returnvalue (Game|SpawnActorfromClass (Variables|Default|GetSpawnClass) (Transformation|GetActorTransform) "AlwaysSpawn" 0 0))
      (bind _asmordhau_equipment (Utilities|Casting|CastToMordhauEquipment _returnvalue))
      (bind _returnvalue_2 (Class|MordhauCharacter|PickUp Char _asmordhau_equipment))
      (if (not _returnvalue_2)
        (bind _asmordhau_player_controller (Utilities|Casting|CastToMordhauPlayerController (Pawn|GetController Char)))
        (bind _asmordhau_player_state (Utilities|Casting|CastToMordhauPlayerState (Variables|/Script/Engine.Pawn|GetPlayerState Char)))
        (Class|MordhauPlayerController|ClientReceiveMessage _asmordhau_player_controller (Utilities|String|Append "(to: " (PlayerState|GetPlayerName _asmordhau_player_state) ") Can't grab equipment, make sure a slot is free!"))
        (Actor|DestroyActor _returnvalue)))))

(event EventBeginPlay
  ;[0.7054 0 0.1173] Redundancy in case editor equipment name differs from in game equipment name
  (|CallParentFunction)
  (bind _asmordhau_equipment (Utilities|Casting|CastToMordhauEquipmentClass (Variables|Default|GetSpawnClass)))
  (Utilities|FlowControl|Delay 3.0)
  (Rendering|Components|TextRender|SetText (Variables|Default|GetTextRender) (Utilities|GetClassDefaults _asmordhau_equipment)))

(event EventTick
  (params (DeltaSeconds :type Float%20%28single-precision%29))
  (bind _textrender (Variables|Default|GetTextRender))
  (Transformation|SetWorldRotation _textrender (.rotation (Transformation|GetActorTransform (Game|GetPlayerController 0))) false false)
  (Transformation|AddLocalRotation _textrender "0,180.000000, 0" false false))

(event EventOnInteractionStart
  (params (Character :type Mordhau%20Character%20Object%20Reference))
  (|CallParentFunction Character)
  (CallFunction|SpawnEquipment Character)
  (Variables|Default|SetbIsInteractable false)
  (Utilities|FlowControl|Delay 1.0)
  (Variables|Default|SetbIsInteractable true))

(fn ConstructionScript
  (bind _textrender (Variables|Default|GetTextRender))
  (Utilities|FlowControl|Sequence
    (:then_0
      (|CallParentFunction)
      (bind _asmordhau_equipment (Utilities|Casting|CastToMordhauEquipmentClass (Variables|Default|GetSpawnClass)))
      (Rendering|Components|TextRender|SetText (Variables|Default|GetTextRender) (Utilities|GetClassDefaults _asmordhau_equipment)))
    (:then_1
      (Transformation|SetAbsolute _textrender false true false)
      (Transformation|SetWorldRotation _textrender "0, 0, 0" false false))))

(fn CanInteract
  (params (Character :type Mordhau%20Character%20Object%20Reference))
  (|CallParentFunction Character)
  (return true))