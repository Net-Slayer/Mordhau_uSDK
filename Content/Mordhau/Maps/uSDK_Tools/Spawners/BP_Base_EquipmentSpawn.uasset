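; Base map spawner that places a piece of Mordhau equipment at its own transform, showing a selectable preview mesh through its construction script.
; On BeginPlay the server spawns the chosen equipment class with cleanup disabled, then assigns a random skin, parts, colors, pattern and emblem.
; Destroying the spawner on the server also destroys the equipment it spawned, if still valid.
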(event EventBeginPlay
  (bind _returnvalue (Class|MordhauUtilityLibrary|GetMordhauSingleton))
  (bind _returnvalue_2 (Transformation|GetActorTransform))
  (bind (_location _rotation) (Math|Transform|BreakTransform _returnvalue_2))
  (bind _emblemcolortable (Variables|/Script/Mordhau.MordhauSingleton|GetEmblemColorTable _returnvalue))
  (bind _returnvalue_3 (Utilities|Array|Length (.entries _emblemcolortable)))
  (bind _returnvalue_4 (Math|Random|RandomInteger _returnvalue_3))
  (bind _returnvalue_5 (Math|Conversions|ToByte(Integer) _returnvalue_4))
  (Networking|SwitchHasAuthority
    (:Authority
      (bind _returnvalue_6 (Game|SpawnActorfromClass (Variables|Default|GetSELECTEquipmentClass) (Math|Transform|MakeTransform _location _rotation) "AlwaysSpawn" 0 0))
      (Utilities|IsValid _returnvalue_6
        (:Is%20Valid
          (Variables|Default|SetEquipment _returnvalue_6)
          (Variables|/Script/Mordhau.MordhauEquipment|SetbAllowCleanup _returnvalue_6 false)
          ;[0.5701 0 0.2542] skin
          (bind (_id _skin) (Class|MordhauUtilityLibrary|GetRandomSkin _returnvalue_6 "Legendary"))
          (Variables|Default|SetSkinId _id)
          ;[0 0.2416 0.5797] parts
          (for _array_element (.PartTypes (Utilities|Struct|BreakEquipmentSkinEntry _skin))
            (Utilities|Array|Add (Variables|Default|GetPartsIds) (Math|Conversions|ToByte(Integer) (Math|Random|RandomInteger (Utilities|Array|Length (.parts _array_element))))))
          ;;[0.5604 0 0.264] colors
          (for _array_element_2 (.ColorTables (Utilities|Struct|BreakEquipmentSkinEntry _skin))
            (Utilities|Array|Add (Variables|Default|GetColorIds) (Math|Conversions|ToByte(Integer) (Math|Random|RandomInteger (Utilities|Array|Length (.entries (Utilities|Array|Get(acopy) (Variables|/Script/Mordhau.MordhauSingleton|GetColorTables (Class|MordhauUtilityLibrary|GetMordhauSingleton)))))))))
          ;;;[0.5797 0.2416 0] pattern
          (Variables|Default|SetPatternId (Math|Conversions|ToByte(Integer) (Math|Random|RandomInteger (Utilities|Array|Length (.Patterns (Utilities|Struct|BreakEquipmentSkinEntry _skin))))))
          ;;[0.5797 0 0.2444] emblem
          (Variables|Default|SetEmblemId (Math|Conversions|ToByte(Integer) (Math|Random|RandomInteger (Utilities|Array|Length (Variables|/Script/Mordhau.MordhauSingleton|GetEmblems _returnvalue)))))
          ;[0.0773 0 0.7529] emblem colors
          (Variables|Default|SetEmblemColor1 _returnvalue_5)
          (Variables|Default|SetEmblemColor2 _returnvalue_5)
          (Class|MordhauEquipment|AssignCustomization (Variables|Default|GetEquipment) (Utilities|Struct|MakeEquipmentCustomization 0 (Variables|Default|GetColorIds) (Variables|Default|GetPartsIds) (Variables|Default|GetPatternId) (Math|Conversions|ToByte(Integer) (Variables|Default|GetSkinId))) (Variables|Default|GetEmblemId) (Variables|Default|GetEmblemColor1) (Variables|Default|GetEmblemColor2)))))))

(event EventDestroyed
  (bind _equipment (Variables|Default|GetEquipment))
  (Networking|SwitchHasAuthority
    (:Authority
      (Utilities|IsValid _equipment ; if still valid, destruction was initiated by external code so spawned equipment must be destroyed as well
        (:Is%20Valid
          (Actor|DestroyActor _equipment))))))

(fn ConstructionScript
  (Class|SkinnedMeshComponent|SetSkeletalMesh (Variables|Default|GetPreview) (Variables|Default|GetPreviewMesh) true))