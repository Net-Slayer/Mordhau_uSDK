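; Map tool volume that deletes level content inside its box whose name contains any of the configured substrings.
; Three seconds after BeginPlay or Reloaded, it box-traces on Visibility and checks hits through LookForMatch.
; Separate toggles match actor, component or static mesh asset names, with mesh matches optionally destroying the parent actor.
; Targets are set to replicate before destruction, and instanced mesh matches remove whole components.
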(event Custom|Reloaded
  (bind _box (Variables|Default|GetBox))
  (bind _returnvalue (Transformation|GetWorldLocation _box))
  (Utilities|FlowControl|Delay 3.0)
  (bind _outhits (Class|KismetSystemLibrary|BoxTraceMulti (Math|Vector|MakeVector (.x _returnvalue) (.y _returnvalue) (- (.z _returnvalue) 1.0)) (Math|Vector|MakeVector (.x _returnvalue) (.y _returnvalue) (.z _returnvalue)) (Components|Box|GetScaledBoxExtent _box) (Transformation|GetWorldRotation _box) "TraceTypeQuery1" false 0 "None" true))
  (Variables|Default|SetHits _outhits)
  (Utilities|FlowControl|Sequence
    (:then_0
      (if (Variables|Default|GetKillNamedActors)
        (for _array_element (Variables|Default|GetHits)
          (bind _match (CallFunction|LookforMatch (Utilities|GetDisplayName (.HitActor (Collision|BreakHitResult _array_element)))))
          (if _match
            (Networking|SetReplicates (.HitActor (Collision|BreakHitResult _array_element)) true)
            (Actor|DestroyActor (.HitActor (Collision|BreakHitResult _array_element)))))))
    (:then_1
      (if (Variables|Default|GetKillNamedComponents)
        (for _array_element_2 (Variables|Default|GetHits)
          (bind _match_2 (CallFunction|LookforMatch (Utilities|GetDisplayName (.HitComponent (Collision|BreakHitResult _array_element_2)))))
          (if _match_2
            (Class|ActorComponent|SetIsReplicated (.HitComponent (Collision|BreakHitResult _array_element_2)) true)
            (Components|DestroyComponent (.HitComponent (Collision|BreakHitResult _array_element_2)))))))
    (:then_2
      (if (Variables|Default|GetKillNamedMeshComponents)
        (for _array_element_3 (Variables|Default|GetHits)
          (bind _asstatic_mesh_component (Utilities|Casting|CastToStaticMeshComponent (.HitComponent (Collision|BreakHitResult _array_element_3)))
            (:then
              (bind _match_3 (CallFunction|LookforMatch (Utilities|GetDisplayName (Variables|/Script/Engine.StaticMeshComponent|GetStaticMesh _asstatic_mesh_component))))
              (if _match_3
                (if (Variables|Default|GetDestroyParent%20ActorOfComponent) :!label _label
                  (Networking|SetReplicates (.HitActor (Collision|BreakHitResult _array_element_3)) true)
                  (Actor|DestroyActor (.HitActor (Collision|BreakHitResult _array_element_3)))
                  (else
                    (Class|ActorComponent|SetIsReplicated (.HitComponent (Collision|BreakHitResult _array_element_3)) true)
                    (Components|DestroyComponent (.HitComponent (Collision|BreakHitResult _array_element_3)))))))
            (:CastFailed
              (bind _aslodstatic_mesh_component (Utilities|Casting|CastToLODStaticMeshComponent (.HitComponent (Collision|BreakHitResult _array_element_3)))
                (:then
                  (bind _match_4 (CallFunction|LookforMatch (Utilities|GetDisplayName (Variables|/Script/Engine.StaticMeshComponent|GetStaticMesh _aslodstatic_mesh_component))))
                  (if _match_4
                    (goto _label)))
                (:CastFailed
                  (bind _asinstanced_static_mesh_component (Utilities|Casting|CastToInstancedStaticMeshComponent (.HitComponent (Collision|BreakHitResult _array_element_3)))
                    (:then
                      (bind _match_5 (CallFunction|LookforMatch (Utilities|GetDisplayName (Variables|/Script/Engine.StaticMeshComponent|GetStaticMesh _asinstanced_static_mesh_component))))
                      (if _match_5
                        (goto _label)))
                    (:CastFailed
                      (bind _ashierarchical_instanced_static_mesh_component (Utilities|Casting|CastToHierarchicalInstancedStaticMeshComponent (.HitComponent (Collision|BreakHitResult _array_element_3))))
                      (bind _match_6 (CallFunction|LookforMatch (Utilities|GetDisplayName (Variables|/Script/Engine.StaticMeshComponent|GetStaticMesh _ashierarchical_instanced_static_mesh_component))))
                      (if _match_6
                        (goto _label)))))))))))))

(event EventBeginPlay
  (bind _box (Variables|Default|GetBox))
  (bind _returnvalue (Transformation|GetWorldLocation _box))
  (Utilities|FlowControl|Delay 3.0)
  (bind _outhits (Class|KismetSystemLibrary|BoxTraceMulti (Math|Vector|MakeVector (.x _returnvalue) (.y _returnvalue) (- (.z _returnvalue) 1.0)) (Math|Vector|MakeVector (.x _returnvalue) (.y _returnvalue) (.z _returnvalue)) (Components|Box|GetScaledBoxExtent _box) (Transformation|GetWorldRotation _box) "TraceTypeQuery1" false 0 "None" true))
  (Variables|Default|SetHits _outhits)
  (Utilities|FlowControl|Sequence
    (:then_0
      (if (Variables|Default|GetKillNamedActors)
        (for _array_element (Variables|Default|GetHits)
          (bind _match (CallFunction|LookforMatch (Utilities|GetDisplayName (.HitActor (Collision|BreakHitResult _array_element)))))
          (if _match
            (Networking|SetReplicates (.HitActor (Collision|BreakHitResult _array_element)) true)
            (Actor|DestroyActor (.HitActor (Collision|BreakHitResult _array_element)))))))
    (:then_1
      (if (Variables|Default|GetKillNamedComponents)
        (for _array_element_2 (Variables|Default|GetHits)
          (bind _match_2 (CallFunction|LookforMatch (Utilities|GetDisplayName (.HitComponent (Collision|BreakHitResult _array_element_2)))))
          (if _match_2
            (Class|ActorComponent|SetIsReplicated (.HitComponent (Collision|BreakHitResult _array_element_2)) true)
            (Components|DestroyComponent (.HitComponent (Collision|BreakHitResult _array_element_2)))))))
    (:then_2
      (if (Variables|Default|GetKillNamedMeshComponents)
        (for _array_element_3 (Variables|Default|GetHits)
          (bind _asstatic_mesh_component (Utilities|Casting|CastToStaticMeshComponent (.HitComponent (Collision|BreakHitResult _array_element_3)))
            (:then
              (bind _match_3 (CallFunction|LookforMatch (Utilities|GetDisplayName (Variables|/Script/Engine.StaticMeshComponent|GetStaticMesh _asstatic_mesh_component))))
              (if _match_3
                (if (Variables|Default|GetDestroyParent%20ActorOfComponent) :!label _label
                  (Networking|SetReplicates (.HitActor (Collision|BreakHitResult _array_element_3)) true)
                  (Actor|DestroyActor (.HitActor (Collision|BreakHitResult _array_element_3)))
                  (else
                    (Class|ActorComponent|SetIsReplicated (.HitComponent (Collision|BreakHitResult _array_element_3)) true)
                    (Components|DestroyComponent (.HitComponent (Collision|BreakHitResult _array_element_3)))))))
            (:CastFailed
              (bind _aslodstatic_mesh_component (Utilities|Casting|CastToLODStaticMeshComponent (.HitComponent (Collision|BreakHitResult _array_element_3)))
                (:then
                  (bind _match_4 (CallFunction|LookforMatch (Utilities|GetDisplayName (Variables|/Script/Engine.StaticMeshComponent|GetStaticMesh _aslodstatic_mesh_component))))
                  (if _match_4
                    (goto _label)))
                (:CastFailed
                  (bind _asinstanced_static_mesh_component (Utilities|Casting|CastToInstancedStaticMeshComponent (.HitComponent (Collision|BreakHitResult _array_element_3)))
                    (:then
                      (bind _match_5 (CallFunction|LookforMatch (Utilities|GetDisplayName (Variables|/Script/Engine.StaticMeshComponent|GetStaticMesh _asinstanced_static_mesh_component))))
                      (if _match_5
                        (goto _label)))
                    (:CastFailed
                      (bind _ashierarchical_instanced_static_mesh_component (Utilities|Casting|CastToHierarchicalInstancedStaticMeshComponent (.HitComponent (Collision|BreakHitResult _array_element_3))))
                      (bind _match_6 (CallFunction|LookforMatch (Utilities|GetDisplayName (Variables|/Script/Engine.StaticMeshComponent|GetStaticMesh _ashierarchical_instanced_static_mesh_component))))
                      (if _match_6
                        (goto _label)))))))))))))

(fn ConstructionScript)

(fn LookforMatch
  (params (Name :type String))
  (bind _array_element (Utilities|Array|ForEachLoopwithBreak (Variables|SubStrings|GetSubStrings) :!label _label)
    (:LoopBody
      (if (Utilities|String|Contains Name _array_element)
        (LocalVariables|SetFound true)
        (goto _label Break)))
    (:Completed
      (return (LocalVariables|GetFound)))))