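; Thrown projectile for Mordhau equipment whose visible model comes from components attached under its skeletal mesh.
; On firing, it hides the creator equipment's mesh hierarchy and shows the projectile's attachments; stopping the trail reverses this.
; SwitchVisibility reveals a whole hierarchy, then after a zero-length delay hides only the parent skeletal mesh, leaving its children visible.
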(event Custom|SwitchVisibility
  (params (Equipment/Weapon :type Boolean) (Projectile :type Boolean))
  (bind _skeletalmeshcomponent (Variables|Default|GetSkeletalMeshComponent))
  (Utilities|FlowControl|Sequence
    (:then_0
      (bind _returnvalue (Class|MordhauProjectile|GetProjectileCreator))
      (bind _asmordhau_equipment (Utilities|Casting|CastToMordhauEquipment _returnvalue))
      (if Equipment/Weapon
        (Rendering|SetVisibility (Variables|/Script/Mordhau.MordhauEquipment|GetSkeletalMeshComponent _asmordhau_equipment) true true)
        (Utilities|FlowControl|Delay 0.0)
        (Rendering|SetVisibility (Variables|/Script/Mordhau.MordhauEquipment|GetSkeletalMeshComponent _asmordhau_equipment) false false)
        (else
          (Rendering|SetVisibility (Variables|/Script/Mordhau.MordhauEquipment|GetSkeletalMeshComponent _asmordhau_equipment) false true))))
    (:then_1
      (if Projectile
        (Rendering|SetVisibility _skeletalmeshcomponent true true)
        (Utilities|FlowControl|Delay 0.0)
        (Rendering|SetVisibility _skeletalmeshcomponent false false)
        (else
          (Rendering|SetVisibility (Variables|Default|GetSkeletalMeshComponent) false true))))))

(event EventStopTrail
  (|CallParentFunction)
  (CallFunction|SwitchVisibility true false)
  (Rendering|SetVisibility (Variables|Default|GetSkeletalMeshComponent) false true))

(event EventOnProjectileFired
  (|CallParentFunction)
  (CallFunction|SwitchVisibility false true))

(fn ConstructionScript
  (|CallParentFunction))